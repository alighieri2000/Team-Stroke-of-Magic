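; Paint actor that draws a brush trail while within paint bounds, with points that a frog overlap event can hide.
; Construction pools hidden static meshes, reused as a ring buffer.
; While inside, FollowCube tracks the brush and a self-restarting timeline places the next mesh after enough movement, facing the previous one.
; Wrapped indices taper the newest ten points, and placed locations are recorded, the first after entry becoming ChaseLocation.
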(event Custom|Frog%20Overlap%20Paint
  (params (Dimension%201 :type Integer))
  (Rendering|SetVisibility (Utilities|Array|Get(acopy) (Variables|References|GetPaintObjects) Dimension%201) false false))

(event Custom|Painting
  (bind _followcube (Variables|Default|GetFollowCube))
  (bind _followcube_2 (Variables|Default|GetFollowCube))
  (bind _paintlocs (Variables|Default|GetPaintLocs))
  (bind _iswithinpaintbounds (Variables|SurfaceParentCommunication|GetisWithinPaintBounds))
  (bind _relativelocation (Variables|/Script/Engine.SceneComponent|GetRelativeLocation _followcube))
  (bind _relativelocation_2 (Variables|/Script/Engine.SceneComponent|GetRelativeLocation _followcube_2))
  ;[1 1 1] Paint trail loop: Spawns a particle on a timer
  (if _iswithinpaintbounds
    (Timeline|Timeline_0 PlayFromStart
      (:Finished
        (Utilities|FlowControl|Sequence
          (:then_0
            (if (> (Math|Vector|VectorLength (- (Math|Vector|MakeVector (.x _relativelocation) (.y _relativelocation) 0.0) (Math|Vector|MakeVector (.x (Variables|/Script/Engine.SceneComponent|GetRelativeLocation (Utilities|Array|Get(acopy) (Variables|References|GetPaintObjects) (Math|Integer|SelectInt (Variables|Trailendvariables|GetMinus1) (- (Variables|Default|GetInkSeq) 1) (== (Variables|Default|GetInkSeq) 0))))) (.y (Variables|/Script/Engine.SceneComponent|GetRelativeLocation (Utilities|Array|Get(acopy) (Variables|References|GetPaintObjects) (Math|Integer|SelectInt (Variables|Trailendvariables|GetMinus1) (- (Variables|Default|GetInkSeq) 1) (== (Variables|Default|GetInkSeq) 0))))) 0.0))) 0.8)
              (Transformation|SetRelativeLocation (Utilities|Array|Get(acopy) (Variables|References|GetPaintObjects) (Variables|Default|GetInkSeq)) (Math|Vector|MakeVector (.x _relativelocation_2) (.y _relativelocation_2) (+ 0.0 (Math|Float|SelectFloat 0.03 0.0 false))) false false)
              (bind _returnvalue (Utilities|Array|Add _paintlocs (Transformation|GetWorldLocation (Utilities|Array|Get(acopy) (Variables|References|GetPaintObjects) (Variables|Default|GetInkSeq)))))
              (Utilities|FlowControl|Sequence
                (:then_0
                  (Transformation|SetRelativeRotation (Utilities|Array|Get(acopy) (Variables|References|GetPaintObjects) (Variables|Default|GetInkSeq)) (Math|Rotator|FindLookatRotation (Math|Vector|MakeVector (.x (Variables|/Script/Engine.SceneComponent|GetRelativeLocation (Utilities|Array|Get(acopy) (Variables|References|GetPaintObjects) (Variables|Default|GetInkSeq)))) (.y (Variables|/Script/Engine.SceneComponent|GetRelativeLocation (Utilities|Array|Get(acopy) (Variables|References|GetPaintObjects) (Variables|Default|GetInkSeq)))) 0.0) (Math|Vector|MakeVector (.x (Variables|/Script/Engine.SceneComponent|GetRelativeLocation (Utilities|Array|Get(acopy) (Variables|References|GetPaintObjects) (Math|Integer|SelectInt (Variables|Trailendvariables|GetMinus1) (- (Variables|Default|GetInkSeq) 1) (== (Variables|Default|GetInkSeq) 0))))) (.y (Variables|/Script/Engine.SceneComponent|GetRelativeLocation (Utilities|Array|Get(acopy) (Variables|References|GetPaintObjects) (Math|Integer|SelectInt (Variables|Trailendvariables|GetMinus1) (- (Variables|Default|GetInkSeq) 1) (== (Variables|Default|GetInkSeq) 0))))) 0.0)) false false)
                  (Utilities|FlowControl|Sequence
                    (:then_0
                      (Utilities|SetPaintTrail-minus5)
                      (Utilities|SizeTrail)
                      (if _iswithinpaintbounds
                        (Rendering|SetVisibility (Utilities|Array|Get(acopy) (Variables|References|GetPaintObjects) (Variables|Default|GetInkSeq)) true false)
                        (else
                          (Rendering|SetVisibility (Utilities|Array|Get(acopy) (Variables|References|GetPaintObjects) (Variables|Default|GetInkSeq)) false false)))
                      (Variables|Default|SetInkSeq (+ (Variables|Default|GetInkSeq) 1))
                      (if (== (Variables|Default|GetInkSeq) (Variables|Default|GetNumberOfPaintPoints))
                        (Variables|Default|SetInkSeq 0))
                      (CallFunction|Painting))))
                (:then_1
                  (Utilities|FlowControl|DoOnce false
                    (:Completed
                      (Variables|Default|SetChaseLocation (Utilities|Array|Get(acopy) _paintlocs _returnvalue))))))
              (else
                (CallFunction|Painting)))))))))

(event Custom|Entered
  (params (Paints%20Enum :type Enum_Paints%20Enum :default "NewEnumerator3"))
  ;[1 1 1] Starts tracking the location of the brush, triggered when first point is entered
  (if (not (Variables|SurfaceParentCommunication|GetLineCompleted))
    (Variables|SurfaceParentCommunication|SetisWithinPaintBounds true)
    (CallFunction|Painting)
    (Timeline|Timeline_1 Play
      (:Update
        (Transformation|SetWorldLocation (Variables|Default|GetFollowCube) (Transformation|GetWorldLocation (Variables|/Game/Blueprints/Paintbrush/Paintrbsuh.Paintrbsuh_C|GetCollisionSphere (Variables|References|GetBrushRefVar))) false false)))))

(event Custom|Exited
  ;[1 1 1] Failed to stay in bounds, removes trail
  (Variables|SurfaceParentCommunication|SetisWithinPaintBounds false)
  (Utilities|FlowControl|Sequence
    (:then_0
      ;[1 1 1] Starts tracking the location of the brush, triggered when first point is entered
      (Timeline|Timeline_1 Stop
        (:Update
          (Transformation|SetWorldLocation (Variables|Default|GetFollowCube) (Transformation|GetWorldLocation (Variables|/Game/Blueprints/Paintbrush/Paintrbsuh.Paintrbsuh_C|GetCollisionSphere (Variables|References|GetBrushRefVar))) false false))))
    (:then_1
      ;[1 1 1] Paint trail loop: Spawns a particle on a timer
      (Utilities|FlowControl|DoOnce false) ; enters at Reset
    )))

(event EventBeginPlay
  (bind _paintpointarray (Variables|References|GetPaintPointArray))
  ;[1 1 1] BeginPlay
  (Variables|References|SetPaintObjects _paintpointarray)
  (bind _returnvalue (Actor|GetActorOfClass "/Game/Blueprints/Paintbrush/Paintrbsuh.Paintrbsuh_C"))
  (Variables|References|SetBrushRefVar _returnvalue)
  (Rendering|SetVisibility (Utilities|Array|Get(acopy) _paintpointarray) false false))

(fn ConstructionScript
  (for _index (range 0 (Variables|Default|GetNumberOfPaintPoints))
    (bind _returnvalue (AddComponent|AddStaticMeshComponent false))
    (Rendering|SetVisibility _returnvalue false false)
    (Utilities|Array|Add (Variables|References|GetPaintPointArray) _returnvalue)))