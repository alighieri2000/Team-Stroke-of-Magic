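; BP_LibraryKey is a grabbable key prop for the library puzzle that can appear with a poof-in animation and be destroyed through Kill.
; PoofIn runs a timeline that scales the static mesh up from near zero while spinning it around its roll axis.
; When GrabComponent reports a drop, a fixed delay returns the mesh to its BeginPlay location, with no check for being grabbed again.
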(event OnDropped(GrabComponent)
  (Utilities|FlowControl|Delay 4e+01)
  (Transformation|SetWorldLocation (Variables|Default|GetStaticMesh) (Variables|Default|GetStartLoc) false false))

(event Custom|Kill
  (Actor|DestroyActor))

(event Custom|Poof%20In
  (bind _staticmesh (Variables|Default|GetStaticMesh))
  (bind _newtrack_0 (Timeline|Timeline_0 PlayFromStart)
    (:Update
      (Transformation|SetRelativeScale3D _staticmesh (Math|Vector|Lerp(Vector) "0.001000,0.001000,0.001000" "0.200000,0.200000,0.200000" _newtrack_0))
      (Transformation|SetRelativeRotation _staticmesh (Math|Rotator|MakeRotator (Math|Float|Lerp 4.2e+02 9e+01 _newtrack_0) 9e+01 9e+01) false false))))

(event EventBeginPlay
  (Variables|Default|SetStartLoc (Transformation|GetWorldLocation (Variables|Default|GetStaticMesh))))

(fn ConstructionScript)