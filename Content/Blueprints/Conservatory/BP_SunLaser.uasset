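; BP_SunLaser is the Conservatory puzzle payoff that fires a sun laser once three cosmos pieces are correctly set.
; Three Dropped events track ready flags and, when all are true, flag the planets aligned on the paintbrush and trigger the laser.
; One timeline stretches the beam with audio, then a second rotates a scene component while lowering the jewel and flagging the gem obtained.
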(event Custom|Laser
  (bind _cube (Variables|Default|GetCube))
  (Audio|Components|Audio|Play (Variables|Default|GetLaserBeam_Cast_Cue) 0.0)
  (bind _newtrack_0 (Timeline|Timeline_0 PlayFromStart)
    (:Update
      (Utilities|FlowControl|Sequence
        (:then_0
          (Transformation|SetRelativeScale3D _cube (Math|Vector|Lerp(Vector) "0.040000,0.000000,0.040000" "0.040000,22.917974,0.040000" _newtrack_0))
          (Transformation|SetRelativeLocation _cube (Math|Vector|Lerp(Vector) "0, 0, 0" "1122.903564,0.000000, 0" _newtrack_0) false false))
        (:then_1
          (Transformation|SetRelativeLocation (Variables|Default|GetLaserBeam_End_Cue) (Math|Vector|Lerp(Vector) "0, 0, 0" "1972.324097,-20.533016,21.659151" _newtrack_0) false false))))
    (:Finished
      (Audio|Components|Audio|Play (Variables|Default|GetCageRattle_Cue) 0.0)
      (bind _newtrack_0_2 (Timeline|Timeline_1 PlayFromStart)
        (:Update
          (Transformation|SetRelativeRotation (Variables|Default|GetScene1) (Math|Rotator|MakeRotator (Math|Float|Lerp 0.0 9e+01 _newtrack_0_2) 0.0 0.0) false false)
          (Default|Lower (Variables|Default|GetJewelRef))
          (Variables|/Game/Blueprints/Paintbrush/Paintrbsuh.Paintrbsuh_C|SetRestrictedAreaGemObtained? (Variables|Default|GetpaintbrushRef) true))))))

(event Custom|3Dropped
  (params (3Ready :type Boolean))
  (if 3Ready
    (bind _output_get (Variables|Default|Set3Ready true))
    (if (Math|Boolean|ANDBoolean (stale Custom|1Dropped _output_get) (stale Custom|2Dropped _output_get) _output_get)
      (Variables|/Game/Blueprints/Paintbrush/Paintrbsuh.Paintrbsuh_C|SetRestrictedAreaPlanetsAlligned? (Variables|Default|GetpaintbrushRef) true)
      (CallFunction|Laser))
    (else
      (Variables|Default|Set3Ready false))))

(event Custom|1Dropped
  (params (Condition :type Boolean))
  (if Condition
    (bind _output_get (Variables|Default|Set1Ready true))
    (if (Math|Boolean|ANDBoolean _output_get (stale Custom|2Dropped _output_get) (stale Custom|3Dropped _output_get))
      (Variables|/Game/Blueprints/Paintbrush/Paintrbsuh.Paintrbsuh_C|SetRestrictedAreaPlanetsAlligned? (Variables|Default|GetpaintbrushRef) true)
      (CallFunction|Laser))
    (else
      (Variables|Default|Set1Ready false))))

(event Custom|2Dropped
  (params (Condition :type Boolean))
  (if Condition
    (bind _output_get (Variables|Default|Set2Ready true))
    (if (Math|Boolean|ANDBoolean (stale Custom|1Dropped _output_get) _output_get (stale Custom|3Dropped _output_get))
      (Variables|/Game/Blueprints/Paintbrush/Paintrbsuh.Paintrbsuh_C|SetRestrictedAreaPlanetsAlligned? (Variables|Default|GetpaintbrushRef) true)
      (CallFunction|Laser))
    (else
      (Variables|Default|Set2Ready false))))

(event EventBeginPlay
  (bind _returnvalue (Actor|GetActorOfClass "/Game/Blueprints/Conservatory/BP_CosmosPuzzle.BP_CosmosPuzzle_C"))
  (Variables|Default|Setcosmos1%20%20ref _returnvalue)
  (bind _returnvalue_2 (Actor|GetActorOfClass "/Game/Blueprints/Conservatory/BP_CosmosPuzzle2.BP_CosmosPuzzle2_C"))
  (Variables|Default|Setcosmos2%20%20ref _returnvalue_2)
  (bind _returnvalue_3 (Actor|GetActorOfClass "/Game/Blueprints/Conservatory/BP_CosmosPuzzle3.BP_CosmosPuzzle3_C"))
  (Variables|Default|SetCosmos3%20ref _returnvalue_3)
  (bind _returnvalue_4 (Actor|GetActorOfClass "/Game/Blueprints/BP/BP_Jewel.BP_Jewel_C"))
  (Variables|Default|SetJewelRef _returnvalue_4)
  (bind _returnvalue_5 (Actor|GetActorOfClass "/Game/Blueprints/Paintbrush/Paintrbsuh.Paintrbsuh_C"))
  (Variables|Default|SetpaintbrushRef _returnvalue_5))

(fn ConstructionScript)