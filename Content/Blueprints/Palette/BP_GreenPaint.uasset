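; Paint trail actor that lays a line of paint points behind the brush and records them in a sequence for the frog.
; A construction-script pool of static meshes is recycled as a ring buffer by a self-restarting timeline, while a second timeline tracks the brush.
; Helper functions compute wrapped indices to scale recent points into a taper.
; Exiting hides unfinished lines, finishing applies glow, and resetting restores red paint.
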(event Custom|Finished
  ;[1 1 1] Line completed
  (Variables|SurfaceParentCommunication|SetLineCompleted true)
  (Transformation|SetRelativeScale3D (Variables|Default|GetTrail) "0, 0, 0")
  (for (_array_element _array_index) (Variables|References|GetPaintObjects)
    (Utilities|IsValid _array_element
      (:Is%20Valid
        (Rendering|Material|SetMaterial _array_element 0 "/Game/Materials/Alphas/GlowTrail.GlowTrail")
        (Transformation|SetRelativeScale3D _array_element "0.800000,0.800000,0.800000")
        (if (== _array_index 0)
          (Transformation|SetRelativeScale3D _array_element "0, 0, 0"))))))

(event Custom|Frog%20Overlap%20Paint
  (params (Dimension%201 :type Integer))
  (Rendering|SetVisibility (Utilities|Array|Get(acopy) (Variables|References|GetPaintObjects) Dimension%201) false false))

(event Custom|Painting
  (params (Paints%20Enum :type Enum_Paints%20Enum :default "NewEnumerator0"))
  (bind _followcube (Variables|Default|GetFollowCube))
  (bind _relativelocation (Variables|/Script/Engine.SceneComponent|GetRelativeLocation _followcube))
  ;[1 1 1] Paint trail loop: Spawns a particle on a timer
  (if (Variables|SurfaceParentCommunication|GetisWithinPaintBounds)
    (Utilities|FlowControl|Sequence
      (:then_0
        (Timeline|Timeline_0 PlayFromStart
          (:Finished
            (Transformation|SetRelativeLocation (Utilities|Array|Get(acopy) (Variables|References|GetPaintObjects) (Variables|Default|GetInkSeq)) (Math|Vector|MakeVector (.x _relativelocation) (.y _relativelocation) (+ (.z (Variables|Default|GetSpawnLoc)) 5.0)) false false)
            (Utilities|SetPaintTrail-minus5)
            (Utilities|SizeTrail)
            (Rendering|SetVisibility (Utilities|Array|Get(acopy) (Variables|References|GetPaintObjects) (Variables|Default|GetInkSeq)) true false)
            (Utilities|Array|Add (Variables|References|GetFrogLickSequence) (Utilities|Array|Get(acopy) (Variables|References|GetPaintObjects) (Variables|Default|GetInkSeq)))
            (Variables|Default|SetInkSeq (+ (Variables|Default|GetInkSeq) 1))
            (if (== (Variables|Default|GetInkSeq) (- (Variables|Default|GetNumberOfPaintPoints) 1))
              (Variables|Default|SetInkSeq 0))
            (CallFunction|Painting "NewEnumerator3"))))
      (:then_1))))

(event Custom|ResetLine
  ;[1 1 1] Reset Path
  (Variables|SurfaceParentCommunication|SetLineCompleted false)
  (CallFunction|Exited)
  (Utilities|FlowControl|Sequence
    (:then_0
      (for _array_element (Variables|References|GetPaintObjects)
        (Utilities|IsValid _array_element
          (:Is%20Valid
            (Rendering|Material|SetMaterial _array_element 0 "/Game/Materials/RedPaint.RedPaint")))))))

(event Custom|Entered
  (params (Paints%20Enum :type Enum_Paints%20Enum :default "NewEnumerator3"))
  (bind _followcube (Variables|Default|GetFollowCube))
  (bind _relativelocation (Variables|/Script/Engine.SceneComponent|GetRelativeLocation _followcube))
  ;[1 1 1] Starts tracking the location of the brush, triggered when first point is entered
  (if (not (Variables|SurfaceParentCommunication|GetLineCompleted))
    (Variables|SurfaceParentCommunication|SetisWithinPaintBounds true)
    (CallFunction|Painting Paints%20Enum)
    (Timeline|Timeline_1 Play
      (:Update
        (Transformation|SetWorldLocation _followcube (Transformation|GetWorldLocation (Variables|/Game/Blueprints/Paintbrush/Paintrbsuh.Paintrbsuh_C|GetCollisionSphere (Variables|References|GetBrushRefVar))) false false)
        (Transformation|SetRelativeLocation (Variables|Default|GetTrail) (Math|Vector|MakeVector (.x _relativelocation) (.y _relativelocation) 5.0) false false)))))

(event Custom|Exited
  (bind _followcube (Variables|Default|GetFollowCube))
  (bind _relativelocation (Variables|/Script/Engine.SceneComponent|GetRelativeLocation _followcube))
  ;[1 1 1] Failed to stay in bounds, removes trail
  (Utilities|FlowControl|Sequence
    (:then_0
      ;[1 1 1] Starts tracking the location of the brush, triggered when first point is entered
      (Timeline|Timeline_1 Stop
        (:Update
          (Transformation|SetWorldLocation _followcube (Transformation|GetWorldLocation (Variables|/Game/Blueprints/Paintbrush/Paintrbsuh.Paintrbsuh_C|GetCollisionSphere (Variables|References|GetBrushRefVar))) false false)
          (Transformation|SetRelativeLocation (Variables|Default|GetTrail) (Math|Vector|MakeVector (.x _relativelocation) (.y _relativelocation) 5.0) false false))))
    (:then_1
      (if (not (Variables|SurfaceParentCommunication|GetLineCompleted))
        (for _array_element (Variables|References|GetPaintObjects)
          (Utilities|IsValid _array_element
            (:Is%20Valid
              _)
            (:Is%20Not%20Valid
              (Utilities|FlowControl|Delay 0.1)))
          (Transformation|SetRelativeLocation _array_element "37.000000,-57.000000,0.000000" false false)
          (Rendering|SetVisibility _array_element false false)
          (Variables|Default|SetInkSeq 0))))))

(event EventBeginPlay
  (bind _paintpointarray (Variables|References|GetPaintPointArray))
  ;[1 1 1] BeginPlay
  (Variables|References|SetPaintObjects _paintpointarray)
  (bind _returnvalue (Actor|GetActorOfClass "/Game/Blueprints/Paintbrush/Paintrbsuh.Paintrbsuh_C"))
  (Variables|References|SetBrushRefVar _returnvalue)
  (Niagara|SetNiagaraVariable(Float) (Variables|Default|GetTrail) "ParticleScale" 0.0)
  (Rendering|SetVisibility (Utilities|Array|Get(acopy) _paintpointarray) false false)
  (Variables|References|SetFrogLickSequence (Utilities|Array|MakeArray 0)))

(fn ConstructionScript
  (for _index (range 0 (Variables|Default|GetNumberOfPaintPoints))
    (bind _returnvalue (AddComponent|AddStaticMeshComponent false))
    (Rendering|SetVisibility _returnvalue false false)
    (Utilities|Array|Add (Variables|References|GetPaintPointArray) _returnvalue)))