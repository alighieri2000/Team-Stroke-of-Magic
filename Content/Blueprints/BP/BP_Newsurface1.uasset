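; Paintable puzzle surface where a brush carrying paint draws a line between two points, with spinning magic effects and red point markers.
; Painting re-triggers itself through a timeline while drawing, cycling a pool of pre-placed paint objects onto FollowCube's position as the stroke.
; Completion logic reddens Point2, raises PathVis and calls OnTTT on MiniWater.
; Stop logic hides and parks the paint objects.
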(event Custom|PoweredUp)

(event Custom|Painting
  (bind _followcube (Variables|Default|GetFollowCube))
  (bind _paintobjects (Variables|Default|GetPaintObjects))
  (bind _relativelocation (Variables|/Script/Engine.SceneComponent|GetRelativeLocation _followcube))
  (if (Variables|Default|GetLineStarted)
    (if (Variables|/Game/Blueprints/Paintbrush/Paintrbsuh.Paintrbsuh_C|GetPaint1_OnBrush (Variables|Default|GetBrushRefVar))
      (if (Variables|Default|GetisDrawing)
        (Timeline|Timeline_0 PlayFromStart
          (:Finished
            (if (== (Variables|Default|GetInkSeq) 0)
              (Transformation|SetRelativeLocation (Utilities|Array|Get(acopy) _paintobjects (Variables|Default|GetInkSeq)) (Math|Vector|MakeVector (.x _relativelocation) (.y _relativelocation) 3.0) false false)
              (CallFunction|Painting)
              (Variables|Default|SetInkSeq (+ (Variables|Default|GetInkSeq) 1))
              (elif (> (Math|Vector|VectorLength (- (Variables|/Script/Engine.SceneComponent|GetRelativeLocation (Utilities|Array|Get(acopy) _paintobjects (Utilities|Select :Index (Variables|Default|GetSwitchIndex) :Option%200 (- (Variables|Default|GetInkSeq) 1) :Option%201 (Utilities|Array|LastIndex _paintobjects)))) "0, 0, 0")) 2.0)
                (if true
                  (Transformation|SetRelativeLocation (Utilities|Array|Get(acopy) _paintobjects (Variables|Default|GetInkSeq)) (Math|Vector|MakeVector (.x _relativelocation) (.y _relativelocation) 3.0) false false)
                  (Rendering|SetVisibility (Utilities|Array|Get(acopy) _paintobjects (Variables|Default|GetInkSeq)) true false)
                  (Variables|Default|SetInkSeq (+ (Variables|Default|GetInkSeq) 1))
                  (if (== (Variables|Default|GetInkSeq) 29)
                    (Variables|Default|SetInkSeq 0)
                    (Variables|Default|SetSwitchIndex 1)
                    (else
                      (Variables|Default|SetSwitchIndex 0)))
                  (CallFunction|Painting))
                (else
                  (CallFunction|Painting)))))))
      (else
        (CallFunction|Exited)))))

(event Custom|Entered)

(event Custom|Exited)

(fn ConstructionScript)