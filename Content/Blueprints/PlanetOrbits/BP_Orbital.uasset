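; BP_Orbital is a Blueprint for an orbiting body, such as a planet, that circles a center point while spinning on its own axis.
; On BeginPlay it caches the starting roll and pitch of the mesh and orbit center, then plays two timelines at OrbitSpeed and SpinSpeed rates.
; Each timeline drives a yaw scaled to 360 degrees on its component, preserving the cached tilt.
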(event Custom|Orbitting
  (bind _rotation (Timeline|OrbitTimeline Play)
    (:Update
      (Transformation|SetRelativeRotation (Variables|Default|GetOrbitCenter) (Math|Rotator|MakeRotator (Variables|Default|GetOrbitCenterX) (Variables|Default|GetOrbitCenterY) (* 360 _rotation)) false false))))

(event Custom|Spinning
  (bind _spinning (Timeline|SpinTimeline Play)
    (:Update
      (Transformation|SetRelativeRotation (Variables|Default|GetStaticMesh) (Math|Rotator|MakeRotator (Variables|Default|GetPlanetX) (Variables|Default|GetPlanetY) (* 360 _spinning)) false false))))

(event EventBeginPlay
  (bind _staticmesh (Variables|Default|GetStaticMesh))
  (bind _orbitcenter (Variables|Default|GetOrbitCenter))
  (bind _relativerotation (Variables|/Script/Engine.SceneComponent|GetRelativeRotation _staticmesh))
  (bind _relativerotation_2 (Variables|/Script/Engine.SceneComponent|GetRelativeRotation _orbitcenter))
  (Variables|Default|SetPlanetX (.roll _relativerotation))
  (Variables|Default|SetPlanetY (.pitch _relativerotation))
  (Variables|Default|SetOrbitCenterY (.pitch _relativerotation_2))
  (Variables|Default|SetOrbitCenterX (.roll _relativerotation_2))
  (Components|Timeline|SetPlayRate (Variables|Default|GetOrbitTimeline) (Variables|Default|GetOrbitSpeed))
  (Components|Timeline|SetPlayRate (Variables|Default|GetSpinTimeline) (Variables|Default|GetSpinSpeed))
  (CallFunction|Orbitting)
  (CallFunction|Spinning))

(fn ConstructionScript)