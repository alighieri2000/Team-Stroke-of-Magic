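; Puzzle cauldron that reacts when the Paintrbsuh actor's collision sphere dips into its water surface.
; BeginPlay caches the brush, parks FollowCube below WaterLevel and, if CauldronActive, positions the boil bubbles.
; On overlap it starts brush loading and bubble audio, raises FollowCube and uses a timeline to track the brush in XY.
; End overlap reverses this, with paired DoOnce gates preventing repeat triggers.
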(event OnComponentBeginOverlap(WaterSurfaceCollision)
  (params (OverlappedComponent :type Primitive%20Component%20Object%20Reference) (OtherActor :type Actor%20Object%20Reference) (OtherComp :type Primitive%20Component%20Object%20Reference) (OtherBodyIndex :type Integer) (bFromSweep :type Boolean) (SweepResult :type Hit%20Result%20Structure%20%28by%20ref%29))
  (bind _followcube (Variables|Default|GetFollowCube))
  (bind _brushrefvar (Variables|Default|GetBrushRefVar))
  (bind _location0 (Variables|Default|GetLocation0))
  (bind _location0_2 (Variables|Default|GetLocation0))
  (bind _brushrefvar_2 (Variables|Default|GetBrushRefVar))
  (bind _collisionsphere (Variables|/Game/Blueprints/Paintbrush/Paintrbsuh.Paintrbsuh_C|GetCollisionSphere _brushrefvar_2))
  (bind _returnvalue (Transformation|GetWorldLocation _collisionsphere))
  (if (== (Variables|/Game/Blueprints/Paintbrush/Paintrbsuh.Paintrbsuh_C|GetCollisionSphere (Variables|Default|GetBrushRefVar)) OtherComp)
    (Utilities|FlowControl|Sequence
      (:then_0
        (Utilities|FlowControl|DoOnce false
          (:Completed
            (Default|Loading _brushrefvar "NewEnumerator0")
            (Utilities|FlowControl|Sequence
              (:then_0
                (Audio|Components|Audio|Play (Variables|Default|GetAC_CauldronBubbles) 0.0)
                (Variables|Default|SetIsInWater true))
              (:then_1
                (Transformation|SetRelativeLocation (Variables|Default|GetFollowCube) (Math|Vector|MakeVector _location0 _location0 (Variables|Default|GetWaterLevel)) false false))
              (:then_2
                (Timeline|Timeline_1 Play
                  (:Update
                    (Transformation|SetWorldLocation _followcube (Math|Vector|MakeVector (.x _returnvalue) (.y _returnvalue) (.z (Transformation|GetWorldLocation _followcube))) false false))))))))
      (:then_1
        (Utilities|FlowControl|DoOnce false) ; enters at Reset
      ))))

(event OnComponentEndOverlap(WaterSurfaceCollision)
  (params (OverlappedComponent :type Primitive%20Component%20Object%20Reference) (OtherActor :type Actor%20Object%20Reference) (OtherComp :type Primitive%20Component%20Object%20Reference) (OtherBodyIndex :type Integer))
  (bind _followcube (Variables|Default|GetFollowCube))
  (bind _brushrefvar (Variables|Default|GetBrushRefVar))
  (bind _location0 (Variables|Default|GetLocation0))
  (bind _location0_2 (Variables|Default|GetLocation0))
  (bind _brushrefvar_2 (Variables|Default|GetBrushRefVar))
  (bind _collisionsphere (Variables|/Game/Blueprints/Paintbrush/Paintrbsuh.Paintrbsuh_C|GetCollisionSphere _brushrefvar_2))
  (bind _returnvalue (Transformation|GetWorldLocation _collisionsphere))
  (if (== (Variables|/Game/Blueprints/Paintbrush/Paintrbsuh.Paintrbsuh_C|GetCollisionSphere (Variables|Default|GetBrushRefVar)) OtherComp)
    (Utilities|FlowControl|Sequence
      (:then_0
        (Utilities|FlowControl|DoOnce false
          (:Completed
            (Default|StopLoading _brushrefvar)
            (Utilities|FlowControl|Sequence
              (:then_0
                (Audio|Components|Audio|Stop (Variables|Default|GetAC_CauldronBubbles))
                (Variables|Default|SetIsInWater false)
                (Transformation|SetRelativeLocation (Variables|Default|GetFollowCube) (Math|Vector|MakeVector _location0_2 _location0_2 (- (Variables|Default|GetWaterLevel) 5.0)) false false))
              (:then_1
                (Timeline|Timeline_1 Stop
                  (:Update
                    (Transformation|SetWorldLocation _followcube (Math|Vector|MakeVector (.x _returnvalue) (.y _returnvalue) (.z (Transformation|GetWorldLocation _followcube))) false false))))))))
      (:then_1
        (Utilities|FlowControl|DoOnce false) ; enters at Reset
      ))))

(event EventBeginPlay
  (bind _location0 (Variables|Default|GetLocation0))
  (bind _location0_2 (Variables|Default|GetLocation0))
  (bind _location0_3 (Variables|Default|GetLocation0))
  (Utilities|FlowControl|Sequence
    (:then_0
      (Audio|Components|Audio|StopDelayed (Variables|Default|GetAC_CauldronBubbles) 0.0)
      (Transformation|SetRelativeLocation (Variables|Default|GetFollowCube) (Math|Vector|MakeVector _location0 _location0 (Variables|Default|GetWaterLevel)) false false)
      (bind _returnvalue (Actor|GetActorOfClass "/Game/Blueprints/Paintbrush/Paintrbsuh.Paintrbsuh_C"))
      (Variables|Default|SetBrushRefVar _returnvalue)
      (if (Variables|Default|GetRises)
        _))
    (:then_1
      (Transformation|SetRelativeLocation (Variables|Default|GetFollowCube) (Math|Vector|MakeVector _location0_2 _location0_2 (- (Variables|Default|GetWaterLevel) 5.0)) false false))
    (:then_2
      (if (Variables|Default|GetCauldronActive)
        (Transformation|SetRelativeTransform (Variables|Default|GetBoilBubbles) (Math|Transform|MakeTransform (Math|Vector|MakeVector _location0_3 _location0_3 (- (Variables|Default|GetWaterLevel) 6.0)) "0, 0, 0" "1,1,1") false false)))))

(fn ConstructionScript)