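; Puzzle actor for a spice transport line with a missing pipe segment, which feeds the grinder puzzle tied to the cauldron.
; SpiceFlow animates a mesh press-in via timeline and exposes the leak effect if no pipe is set.
; Overlapping a BP_SoloPipe consumes it, reveals the fitted pipe and stops the leak.
; Once pipe and flow are both set, in either order, it notifies BP_Cauldron and Paintrbsuh, both found at BeginPlay.
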(event OnComponentBeginOverlap(Box)
  (params (OverlappedComponent :type Primitive%20Component%20Object%20Reference) (OtherActor :type Actor%20Object%20Reference) (OtherComp :type Primitive%20Component%20Object%20Reference) (OtherBodyIndex :type Integer) (bFromSweep :type Boolean) (SweepResult :type Hit%20Result%20Structure%20%28by%20ref%29))
  (bind _cauldref (Variables|Default|GetCauldRef))
  (bind _asbp_solo_pipe (Utilities|Casting|CastToBP_SoloPipe OtherActor))
  (Default|KillMe _asbp_solo_pipe)
  (Audio|Components|Audio|Stop (Variables|Default|GetA_Water))
  (Rendering|SetVisibility (Variables|Default|GetStaticMesh6) true false)
  (Variables|Default|SetpipeSet true)
  (Variables|/Game/Blueprints/Paintbrush/Paintrbsuh.Paintrbsuh_C|SetGrindPz_Pipe? (Variables|Default|GetRefBrush) true)
  (Audio|Components|Audio|Play (Variables|Default|GetPipePlace_Cue) 0.0)
  (CallFunction|StopFlow)
  (if (and (Variables|Default|GetpipeSet) (Variables|Default|GetSpiceFlowing))
    (Variables|/Game/Blueprints/PuzzleElements/BP_Cauldron.BP_Cauldron_C|SetSpicePuzzleDone _cauldref true)
    (Default|GrindButtonActivate _cauldref)
    (Default|CompleteGrinder (Variables|Default|GetRefBrush))))

(event Custom|Spice%20Flow
  (bind _cauldref (Variables|Default|GetCauldRef))
  (Variables|Default|SetSpiceFlowing true)
  (Utilities|FlowControl|Sequence
    (:then_0
      (bind _newtrack_0 (Timeline|Timeline_0 Play)
        (:Update
          (Transformation|SetRelativeScale3D (Variables|Default|GetCube) (Math|Vector|Lerp(Vector) "0.293613,0.070688,0.293613" "0.293613,0.021207,0.293613" _newtrack_0))
          (Transformation|SetRelativeLocation (Variables|Default|GetStaticMesh13) (Math|Vector|Lerp(Vector) "115.868080,-36.215256,104.605774" "115.868080,-29.653219,86.577126" _newtrack_0) false false))))
    (:then_1
      (if (and (Variables|Default|GetpipeSet) (Variables|Default|GetSpiceFlowing)) :!label _label
        (Variables|/Game/Blueprints/PuzzleElements/BP_Cauldron.BP_Cauldron_C|SetSpicePuzzleDone _cauldref true)
        (Default|GrindButtonActivate _cauldref)
        (Default|CompleteGrinder (Variables|Default|GetRefBrush))))
    (:then_2
      (if (not (Variables|Default|GetpipeSet))
        (Transformation|SetRelativeLocation (Variables|Default|GetNiagara) "283.615967,0.000000,4.997959" false false)
        (Rendering|SetVisibility (Variables|Default|GetStaticMesh15) true false)
        (Variables|Default|SetSpiceFlowing true)
        (goto _label)))))

(event Custom|Stop%20Flow
  (Transformation|SetRelativeLocation (Variables|Default|GetNiagara) "283.615967,0.000000,-200.000000" false false)
  (Rendering|SetVisibility (Variables|Default|GetStaticMesh15) false false))

(event Custom|Actually%20flowing)

(event EventBeginPlay
  (bind _returnvalue (Actor|GetActorOfClass "/Game/Blueprints/PuzzleElements/BP_Cauldron.BP_Cauldron_C"))
  (Variables|Default|SetCauldRef _returnvalue)
  (bind _returnvalue_2 (Actor|GetActorOfClass "/Game/Blueprints/Paintbrush/Paintrbsuh.Paintrbsuh_C"))
  (Variables|Default|SetRefBrush _returnvalue_2)
  (Rendering|SetVisibility (Variables|Default|GetStaticMesh6) false false)
  (Transformation|SetRelativeLocation (Variables|Default|GetNiagara) "283.615967,-200.000000,4.997959" false false))

(fn ConstructionScript)