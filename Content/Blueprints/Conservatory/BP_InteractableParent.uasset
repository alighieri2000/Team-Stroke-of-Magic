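; Parent Blueprint for grabbable interactables that slide or rotate along chosen axes, with optional limits.
; While grabbed, a timeline copies the free Hitbox to FollowCube, whose relative transform drives RecieveTransform, using pivot look-at angles or hitbox rotation when rotating.
; On drop, the hitbox stops simulating physics and resets, and RecieveTransform can lerp back to its initial transform.
; Empty grab, drop and return events serve as hooks.
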(event OnGrabbed(GrabComponent)
  (bind _initialtransform (Variables|Default|GetInitialTransform))
  (bind _hitbox_ (Variables|Default|GetHitbox_))
  (bind _pivot_point (Variables|Default|GetPivot%20Point))
  (bind _maximum_limit (Variables|Default|GetMaximum%20Limit))
  (bind _minimum_limit (Variables|Default|GetMinimum%20Limit))
  (bind _limit_value (Variables|Default|GetLimit%20Value))
  (bind _pivot_point_2 (Variables|Default|GetPivot%20Point))
  (bind _maximum_limit_2 (Variables|Default|GetMaximum%20Limit))
  (bind _minimum_limit_2 (Variables|Default|GetMinimum%20Limit))
  (bind _limit_value_2 (Variables|Default|GetLimit%20Value))
  (bind _maximum_limit_3 (Variables|Default|GetMaximum%20Limit))
  (bind _minimum_limit_3 (Variables|Default|GetMinimum%20Limit))
  (bind _limit_value_3 (Variables|Default|GetLimit%20Value))
  (bind _recievetransform (Variables|Default|GetRecieveTransform))
  (bind _recievetransform_2 (Variables|Default|GetRecieveTransform))
  (bind _follow_cube (Variables|Default|GetFollow%20Cube))
  (bind _follow_cube_2 (Variables|Default|GetFollow%20Cube))
  (bind _follow_cube_3 (Variables|Default|GetFollow%20Cube))
  (bind _follow_cube_4 (Variables|Default|GetFollow%20Cube))
  (bind _follow_cube_5 (Variables|Default|GetFollow%20Cube))
  (bind _recievetransform_3 (Variables|Default|GetRecieveTransform))
  (bind _follow_cube_6 (Variables|Default|GetFollow%20Cube))
  (bind _returnvalue (Transformation|GetWorldLocation _hitbox_))
  (bind _returnvalue_2 (Transformation|GetRelativeTransform _initialtransform))
  (bind _returnvalue_3 (Transformation|GetRelativeTransform _recievetransform_3))
  (bind _relativelocation (Variables|/Script/Engine.SceneComponent|GetRelativeLocation _follow_cube_5))
  (bind _relativelocation_2 (Variables|/Script/Engine.SceneComponent|GetRelativeLocation _pivot_point))
  (bind _relativelocation_3 (Variables|/Script/Engine.SceneComponent|GetRelativeLocation _follow_cube_6))
  (bind _relativerotation (Variables|/Script/Engine.SceneComponent|GetRelativeRotation _follow_cube_2))
  (bind _relativelocation_4 (Variables|/Script/Engine.SceneComponent|GetRelativeLocation _pivot_point_2))
  (bind _relativerotation_2 (Variables|/Script/Engine.SceneComponent|GetRelativeRotation _follow_cube_4))
  (bind _relativerotation_3 (Variables|/Script/Engine.SceneComponent|GetRelativeRotation _follow_cube_3))
  (bind (_x _y _z) (Math|Vector|BreakVector _relativelocation_2))
  (bind (_x_2 _y_2 _z_2) (Math|Vector|BreakVector _relativelocation_4))
  (bind _returnvalue_4 (- _z_2 _minimum_limit))
  (bind _returnvalue_5 (- _x_2 _minimum_limit_2))
  (bind _returnvalue_6 (- _y_2 _minimum_limit_3))
  (bind _returnvalue_7 (Math|Vector|MakeVector (.x _relativelocation) (.y _relativelocation) _z))
  (bind _returnvalue_8 (Math|Vector|MakeVector _x (.y _relativelocation) (.z _relativelocation)))
  (bind _returnvalue_9 (Math|Vector|MakeVector (.x _relativelocation) _y (.z _relativelocation)))
  (bind _returnvalue_10 (+ _x_2 _maximum_limit_2))
  (bind _returnvalue_11 (+ _y_2 _maximum_limit_3))
  (bind _returnvalue_12 (+ _z_2 _maximum_limit))
  (bind _returnvalue_13 (Math|Rotator|FindLookatRotation _relativelocation_2 _returnvalue_9))
  (bind _returnvalue_14 (Math|Rotator|FindLookatRotation _relativelocation_2 _returnvalue_7))
  (bind _returnvalue_15 (Math|Rotator|FindLookatRotation _relativelocation_2 _returnvalue_8))
  (bind _returnvalue_16 (Math|Float|Clamp(Float) (.z _relativelocation_3) _returnvalue_4 _returnvalue_12))
  (bind _returnvalue_17 (Math|Float|Clamp(Float) (.x _relativelocation_3) _returnvalue_5 _returnvalue_10))
  (bind _returnvalue_18 (Math|Float|Clamp(Float) (.y _relativelocation_3) _returnvalue_6 _returnvalue_11))
  (bind _returnvalue_19 (Math|Float|SelectFloat _returnvalue_16 (.z _relativelocation_3) _limit_value))
  (bind _returnvalue_20 (Math|Float|SelectFloat _returnvalue_17 (.x _relativelocation_3) _limit_value_2))
  (bind _returnvalue_21 (Math|Float|SelectFloat _returnvalue_18 (.y _relativelocation_3) _limit_value_3))
  (bind _returnvalue_22 (> (.yaw _returnvalue_15) -8e+01))
  (bind _returnvalue_23 (> (.yaw _returnvalue_13) 1.7e+02))
  (bind _returnvalue_24 (+ (.pitch _returnvalue_13) 9e+01))
  (bind _returnvalue_25 (+ (.pitch _returnvalue_15) 9e+01))
  (bind _returnvalue_26 (Math|Float|SelectFloat -1.0 1.0 _returnvalue_22))
  (bind _returnvalue_27 (Math|Float|SelectFloat -1.0 1.0 _returnvalue_23))
  (bind _returnvalue_28 (* _returnvalue_27 _returnvalue_24))
  (bind _returnvalue_29 (* _returnvalue_26 _returnvalue_25))
  ;[1 1 1] On component grabbed
  (if (not (Variables|Default|GetGrabLocked))
    (Utilities|FlowControl|Sequence
      (:then_0
        (CallFunction|OnGrabbed)
        (Timeline|Timeline_0 PlayFromStart
          (:Update
            (switch Utilities|FlowControl|Switch|SwitchonFollowHandleEnum (Variables|Default|GetInteract%20Type)
              (:NewEnumerator0
                (Transformation|SetWorldLocation _follow_cube _returnvalue false false)
                (bind _output_get (Variables|Default|SetOut%20Vector (Math|Vector|SelectVector (Utilities|SecondaryDirectionSolve _returnvalue_20 _returnvalue_21 _returnvalue_19) (Utilities|Select :Index (Variables|Default|GetXYZ%20Direction) :NewEnumerator0 (Math|Vector|MakeVector _returnvalue_20 _y_2 _z_2) :NewEnumerator1 (Math|Vector|MakeVector _x_2 _returnvalue_21 _z_2) :NewEnumerator2 (Math|Vector|MakeVector _x_2 _y_2 _returnvalue_19)) (Variables|Default|GetSecondaryMovementAxis))))
                (Transformation|SetRelativeLocation _recievetransform_2 _output_get false false))
              (:NewEnumerator1
                (if (Variables|Default|GetRotation%20Relative%20To%20Hitbox)
                  (Transformation|SetWorldRotation _follow_cube (Transformation|GetWorldRotation _hitbox_) false false)
                  (else
                    (Transformation|SetWorldLocation _follow_cube _returnvalue false false)))
                (bind _output_get_2 (Variables|Default|SetOut%20Rotation (Utilities|Select :Index (Variables|Default|GetXYZ%20Direction) :NewEnumerator0 (select (Variables|Default|GetRotation%20relative%20to%20hitbox) (Math|Rotator|MakeRotator (Math|Float|SelectFloat (Math|Float|Clamp(Float) (.roll _relativerotation_2) (Variables|Default|GetMinimum%20Limit) (Variables|Default|GetMaximum%20Limit)) (.roll _relativerotation_2) (Variables|Default|GetLimit%20Value)) 0.0 0.0) (Math|Rotator|MakeRotator (+ (Math|Float|SelectFloat (Math|Float|Clamp(Float) _returnvalue_29 (Variables|Default|GetMinimum%20Limit) (Variables|Default|GetMaximum%20Limit)) _returnvalue_29 (Variables|Default|GetLimit%20Value)) (+ 9e+01 (Variables|Default|GetXRotSolve))) 0.0 0.0)) :NewEnumerator1 (select (Variables|Default|GetRotation%20relative%20to%20hitbox) (Math|Rotator|MakeRotator 0.0 (Math|Float|SelectFloat (Math|Float|Clamp(Float) (.pitch _relativerotation_3) (Variables|Default|GetMinimum%20Limit) (Variables|Default|GetMaximum%20Limit)) (.pitch _relativerotation_3) (Variables|Default|GetLimit%20Value)) 0.0) (Math|Rotator|MakeRotator 0.0 (+ (Math|Float|SelectFloat (Math|Float|Clamp(Float) _returnvalue_28 (Variables|Default|GetMinimum%20Limit) (Variables|Default|GetMaximum%20Limit)) _returnvalue_28 (Variables|Default|GetLimit%20Value)) -1.8e+02) 0.0)) :NewEnumerator2 (select (Variables|Default|GetRotation%20relative%20to%20hitbox) (Math|Rotator|MakeRotator 0.0 0.0 (Math|Float|SelectFloat (Math|Float|Clamp(Float) (.yaw _relativerotation) (Variables|Default|GetMinimum%20Limit) (Variables|Default|GetMaximum%20Limit)) (.yaw _relativerotation) (Variables|Default|GetLimit%20Value))) (Math|Rotator|MakeRotator 0.0 0.0 (Math|Float|SelectFloat (Math|Float|Clamp(Float) (.yaw _returnvalue_14) (Variables|Default|GetMinimum%20Limit) (Variables|Default|GetMaximum%20Limit)) (.yaw _returnvalue_14) (Variables|Default|GetLimit%20Value)))))))
                (Transformation|SetRelativeRotation _recievetransform_2 _output_get_2 false false))))))
      (:then_1
        ;[1 1 1] On component dropped
        (bind _newtrack_0 (Timeline|Timeline_1 Stop)
          (:Update
            (switch Utilities|FlowControl|Switch|SwitchonFollowHandleEnum (Variables|Default|GetInteract%20Type)
              (:NewEnumerator0
                (bind _output_get_3 (Variables|Default|SetOut%20Vector (Math|Vector|Lerp(Vector) (.location _returnvalue_3) (.location _returnvalue_2) _newtrack_0)))
                (Transformation|SetRelativeLocation _recievetransform _output_get_3 false false)
                (Transformation|SetWorldLocation (Variables|Default|GetHitbox_) (Transformation|GetWorldLocation (Variables|Default|GetHitboxLoc)) false false))
              (:NewEnumerator1
                (bind _output_get_4 (Variables|Default|SetOut%20Rotation (Math|Rotator|Lerp(Rotator) (.rotation _returnvalue_3) (.rotation _returnvalue_2) _newtrack_0)))
                (Transformation|SetRelativeRotation _recievetransform _output_get_4 false false))))
          (:Finished
            (CallFunction|BacktoOriginal)))))))

(event OnDropped(GrabComponent)
  (bind _initialtransform (Variables|Default|GetInitialTransform))
  (bind _hitbox_ (Variables|Default|GetHitbox_))
  (bind _pivot_point (Variables|Default|GetPivot%20Point))
  (bind _maximum_limit (Variables|Default|GetMaximum%20Limit))
  (bind _minimum_limit (Variables|Default|GetMinimum%20Limit))
  (bind _limit_value (Variables|Default|GetLimit%20Value))
  (bind _pivot_point_2 (Variables|Default|GetPivot%20Point))
  (bind _maximum_limit_2 (Variables|Default|GetMaximum%20Limit))
  (bind _minimum_limit_2 (Variables|Default|GetMinimum%20Limit))
  (bind _limit_value_2 (Variables|Default|GetLimit%20Value))
  (bind _maximum_limit_3 (Variables|Default|GetMaximum%20Limit))
  (bind _minimum_limit_3 (Variables|Default|GetMinimum%20Limit))
  (bind _limit_value_3 (Variables|Default|GetLimit%20Value))
  (bind _hitboxloc (Variables|Default|GetHitboxLoc))
  (bind _recievetransform (Variables|Default|GetRecieveTransform))
  (bind _recievetransform_2 (Variables|Default|GetRecieveTransform))
  (bind _hitbox__2 (Variables|Default|GetHitbox_))
  (bind _follow_cube (Variables|Default|GetFollow%20Cube))
  (bind _follow_cube_2 (Variables|Default|GetFollow%20Cube))
  (bind _follow_cube_3 (Variables|Default|GetFollow%20Cube))
  (bind _follow_cube_4 (Variables|Default|GetFollow%20Cube))
  (bind _follow_cube_5 (Variables|Default|GetFollow%20Cube))
  (bind _recievetransform_3 (Variables|Default|GetRecieveTransform))
  (bind _follow_cube_6 (Variables|Default|GetFollow%20Cube))
  (bind _returnvalue (Transformation|GetWorldLocation _hitbox_))
  (bind _returnvalue_2 (Transformation|GetRelativeTransform _initialtransform))
  (bind _returnvalue_3 (Transformation|GetRelativeTransform _recievetransform_3))
  (bind _returnvalue_4 (Transformation|GetWorldLocation _hitboxloc))
  (bind _relativelocation (Variables|/Script/Engine.SceneComponent|GetRelativeLocation _follow_cube_5))
  (bind _relativelocation_2 (Variables|/Script/Engine.SceneComponent|GetRelativeLocation _pivot_point))
  (bind _relativelocation_3 (Variables|/Script/Engine.SceneComponent|GetRelativeLocation _follow_cube_6))
  (bind _relativerotation (Variables|/Script/Engine.SceneComponent|GetRelativeRotation _follow_cube_2))
  (bind _relativelocation_4 (Variables|/Script/Engine.SceneComponent|GetRelativeLocation _pivot_point_2))
  (bind _relativerotation_2 (Variables|/Script/Engine.SceneComponent|GetRelativeRotation _follow_cube_4))
  (bind _relativerotation_3 (Variables|/Script/Engine.SceneComponent|GetRelativeRotation _follow_cube_3))
  (bind (_x _y _z) (Math|Vector|BreakVector _relativelocation_2))
  (bind (_x_2 _y_2 _z_2) (Math|Vector|BreakVector _relativelocation_4))
  (bind _returnvalue_5 (- _z_2 _minimum_limit))
  (bind _returnvalue_6 (- _x_2 _minimum_limit_2))
  (bind _returnvalue_7 (- _y_2 _minimum_limit_3))
  (bind _returnvalue_8 (Math|Vector|MakeVector (.x _relativelocation) (.y _relativelocation) _z))
  (bind _returnvalue_9 (Math|Vector|MakeVector _x (.y _relativelocation) (.z _relativelocation)))
  (bind _returnvalue_10 (Math|Vector|MakeVector (.x _relativelocation) _y (.z _relativelocation)))
  (bind _returnvalue_11 (+ _x_2 _maximum_limit_2))
  (bind _returnvalue_12 (+ _y_2 _maximum_limit_3))
  (bind _returnvalue_13 (+ _z_2 _maximum_limit))
  (bind _returnvalue_14 (Math|Rotator|FindLookatRotation _relativelocation_2 _returnvalue_10))
  (bind _returnvalue_15 (Math|Rotator|FindLookatRotation _relativelocation_2 _returnvalue_8))
  (bind _returnvalue_16 (Math|Rotator|FindLookatRotation _relativelocation_2 _returnvalue_9))
  (bind _returnvalue_17 (Math|Float|Clamp(Float) (.z _relativelocation_3) _returnvalue_5 _returnvalue_13))
  (bind _returnvalue_18 (Math|Float|Clamp(Float) (.x _relativelocation_3) _returnvalue_6 _returnvalue_11))
  (bind _returnvalue_19 (Math|Float|Clamp(Float) (.y _relativelocation_3) _returnvalue_7 _returnvalue_12))
  (bind _returnvalue_20 (Math|Float|SelectFloat _returnvalue_17 (.z _relativelocation_3) _limit_value))
  (bind _returnvalue_21 (Math|Float|SelectFloat _returnvalue_18 (.x _relativelocation_3) _limit_value_2))
  (bind _returnvalue_22 (Math|Float|SelectFloat _returnvalue_19 (.y _relativelocation_3) _limit_value_3))
  (bind _returnvalue_23 (> (.yaw _returnvalue_16) -8e+01))
  (bind _returnvalue_24 (> (.yaw _returnvalue_14) 1.7e+02))
  (bind _returnvalue_25 (+ (.pitch _returnvalue_14) 9e+01))
  (bind _returnvalue_26 (+ (.pitch _returnvalue_16) 9e+01))
  (bind _returnvalue_27 (Math|Float|SelectFloat -1.0 1.0 _returnvalue_23))
  (bind _returnvalue_28 (Math|Float|SelectFloat -1.0 1.0 _returnvalue_24))
  (bind _returnvalue_29 (* _returnvalue_28 _returnvalue_25))
  (bind _returnvalue_30 (* _returnvalue_27 _returnvalue_26))
  ;[1 1 1] On component dropped
  (CallFunction|OnDropped)
  (Physics|SetSimulatePhysics _hitbox__2 false)
  (Utilities|FlowControl|Sequence
    (:then_0
      (Transformation|SetRelativeRotation _hitbox__2 (.rotation (Variables|Default|GetHitbox%20Relative%20Transform)) false false)
      (if (Variables|Default|GetSnap%20To%20Original%20Transform)
        (bind _newtrack_0 (Timeline|Timeline_1 PlayFromStart)
          (:Update
            (switch Utilities|FlowControl|Switch|SwitchonFollowHandleEnum (Variables|Default|GetInteract%20Type)
              (:NewEnumerator0
                (bind _output_get (Variables|Default|SetOut%20Vector (Math|Vector|Lerp(Vector) (.location _returnvalue_3) (.location _returnvalue_2) _newtrack_0)))
                (Transformation|SetRelativeLocation _recievetransform _output_get false false)
                (Transformation|SetWorldLocation (Variables|Default|GetHitbox_) _returnvalue_4 false false))
              (:NewEnumerator1
                (bind _output_get_2 (Variables|Default|SetOut%20Rotation (Math|Rotator|Lerp(Rotator) (.rotation _returnvalue_3) (.rotation _returnvalue_2) _newtrack_0)))
                (Transformation|SetRelativeRotation _recievetransform _output_get_2 false false))))
          (:Finished
            (CallFunction|BacktoOriginal)))
        (else
          (Transformation|SetWorldLocation _hitbox__2 _returnvalue_4 false false))))
    (:then_1
      ;[1 1 1] On component grabbed
      (Timeline|Timeline_0 Stop
        (:Update
          (switch Utilities|FlowControl|Switch|SwitchonFollowHandleEnum (Variables|Default|GetInteract%20Type)
            (:NewEnumerator0
              (Transformation|SetWorldLocation _follow_cube _returnvalue false false)
              (bind _output_get_3 (Variables|Default|SetOut%20Vector (Math|Vector|SelectVector (Utilities|SecondaryDirectionSolve _returnvalue_21 _returnvalue_22 _returnvalue_20) (Utilities|Select :Index (Variables|Default|GetXYZ%20Direction) :NewEnumerator0 (Math|Vector|MakeVector _returnvalue_21 _y_2 _z_2) :NewEnumerator1 (Math|Vector|MakeVector _x_2 _returnvalue_22 _z_2) :NewEnumerator2 (Math|Vector|MakeVector _x_2 _y_2 _returnvalue_20)) (Variables|Default|GetSecondaryMovementAxis))))
              (Transformation|SetRelativeLocation _recievetransform_2 _output_get_3 false false))
            (:NewEnumerator1
              (if (Variables|Default|GetRotation%20Relative%20To%20Hitbox)
                (Transformation|SetWorldRotation _follow_cube (Transformation|GetWorldRotation _hitbox_) false false)
                (else
                  (Transformation|SetWorldLocation _follow_cube _returnvalue false false)))
              (bind _output_get_4 (Variables|Default|SetOut%20Rotation (Utilities|Select :Index (Variables|Default|GetXYZ%20Direction) :NewEnumerator0 (select (Variables|Default|GetRotation%20relative%20to%20hitbox) (Math|Rotator|MakeRotator (Math|Float|SelectFloat (Math|Float|Clamp(Float) (.roll _relativerotation_2) (Variables|Default|GetMinimum%20Limit) (Variables|Default|GetMaximum%20Limit)) (.roll _relativerotation_2) (Variables|Default|GetLimit%20Value)) 0.0 0.0) (Math|Rotator|MakeRotator (+ (Math|Float|SelectFloat (Math|Float|Clamp(Float) _returnvalue_30 (Variables|Default|GetMinimum%20Limit) (Variables|Default|GetMaximum%20Limit)) _returnvalue_30 (Variables|Default|GetLimit%20Value)) (+ 9e+01 (Variables|Default|GetXRotSolve))) 0.0 0.0)) :NewEnumerator1 (select (Variables|Default|GetRotation%20relative%20to%20hitbox) (Math|Rotator|MakeRotator 0.0 (Math|Float|SelectFloat (Math|Float|Clamp(Float) (.pitch _relativerotation_3) (Variables|Default|GetMinimum%20Limit) (Variables|Default|GetMaximum%20Limit)) (.pitch _relativerotation_3) (Variables|Default|GetLimit%20Value)) 0.0) (Math|Rotator|MakeRotator 0.0 (+ (Math|Float|SelectFloat (Math|Float|Clamp(Float) _returnvalue_29 (Variables|Default|GetMinimum%20Limit) (Variables|Default|GetMaximum%20Limit)) _returnvalue_29 (Variables|Default|GetLimit%20Value)) -1.8e+02) 0.0)) :NewEnumerator2 (select (Variables|Default|GetRotation%20relative%20to%20hitbox) (Math|Rotator|MakeRotator 0.0 0.0 (Math|Float|SelectFloat (Math|Float|Clamp(Float) (.yaw _relativerotation) (Variables|Default|GetMinimum%20Limit) (Variables|Default|GetMaximum%20Limit)) (.yaw _relativerotation) (Variables|Default|GetLimit%20Value))) (Math|Rotator|MakeRotator 0.0 0.0 (Math|Float|SelectFloat (Math|Float|Clamp(Float) (.yaw _returnvalue_15) (Variables|Default|GetMinimum%20Limit) (Variables|Default|GetMaximum%20Limit)) (.yaw _returnvalue_15) (Variables|Default|GetLimit%20Value)))))))
              (Transformation|SetRelativeRotation _recievetransform_2 _output_get_4 false false))))))))

(event Custom|On%20Grabbed
  ;[1 1 1] On component grabbed
)

(event Custom|On%20Dropped
  ;[1 1 1] On component dropped
)

(event Custom|Break%20Grip
  (bind _initialtransform (Variables|Default|GetInitialTransform))
  (bind _hitbox_ (Variables|Default|GetHitbox_))
  (bind _pivot_point (Variables|Default|GetPivot%20Point))
  (bind _maximum_limit (Variables|Default|GetMaximum%20Limit))
  (bind _minimum_limit (Variables|Default|GetMinimum%20Limit))
  (bind _limit_value (Variables|Default|GetLimit%20Value))
  (bind _pivot_point_2 (Variables|Default|GetPivot%20Point))
  (bind _maximum_limit_2 (Variables|Default|GetMaximum%20Limit))
  (bind _minimum_limit_2 (Variables|Default|GetMinimum%20Limit))
  (bind _limit_value_2 (Variables|Default|GetLimit%20Value))
  (bind _maximum_limit_3 (Variables|Default|GetMaximum%20Limit))
  (bind _minimum_limit_3 (Variables|Default|GetMinimum%20Limit))
  (bind _limit_value_3 (Variables|Default|GetLimit%20Value))
  (bind _hitboxloc (Variables|Default|GetHitboxLoc))
  (bind _recievetransform (Variables|Default|GetRecieveTransform))
  (bind _recievetransform_2 (Variables|Default|GetRecieveTransform))
  (bind _hitbox__2 (Variables|Default|GetHitbox_))
  (bind _follow_cube (Variables|Default|GetFollow%20Cube))
  (bind _follow_cube_2 (Variables|Default|GetFollow%20Cube))
  (bind _follow_cube_3 (Variables|Default|GetFollow%20Cube))
  (bind _follow_cube_4 (Variables|Default|GetFollow%20Cube))
  (bind _follow_cube_5 (Variables|Default|GetFollow%20Cube))
  (bind _recievetransform_3 (Variables|Default|GetRecieveTransform))
  (bind _follow_cube_6 (Variables|Default|GetFollow%20Cube))
  (bind _returnvalue (Transformation|GetWorldLocation _hitbox_))
  (bind _returnvalue_2 (Transformation|GetRelativeTransform _initialtransform))
  (bind _returnvalue_3 (Transformation|GetRelativeTransform _recievetransform_3))
  (bind _returnvalue_4 (Transformation|GetWorldLocation _hitboxloc))
  (bind _relativelocation (Variables|/Script/Engine.SceneComponent|GetRelativeLocation _follow_cube_5))
  (bind _relativelocation_2 (Variables|/Script/Engine.SceneComponent|GetRelativeLocation _pivot_point))
  (bind _relativelocation_3 (Variables|/Script/Engine.SceneComponent|GetRelativeLocation _follow_cube_6))
  (bind _relativerotation (Variables|/Script/Engine.SceneComponent|GetRelativeRotation _follow_cube_2))
  (bind _relativelocation_4 (Variables|/Script/Engine.SceneComponent|GetRelativeLocation _pivot_point_2))
  (bind _relativerotation_2 (Variables|/Script/Engine.SceneComponent|GetRelativeRotation _follow_cube_4))
  (bind _relativerotation_3 (Variables|/Script/Engine.SceneComponent|GetRelativeRotation _follow_cube_3))
  (bind (_x _y _z) (Math|Vector|BreakVector _relativelocation_2))
  (bind (_x_2 _y_2 _z_2) (Math|Vector|BreakVector _relativelocation_4))
  (bind _returnvalue_5 (- _z_2 _minimum_limit))
  (bind _returnvalue_6 (- _x_2 _minimum_limit_2))
  (bind _returnvalue_7 (- _y_2 _minimum_limit_3))
  (bind _returnvalue_8 (Math|Vector|MakeVector (.x _relativelocation) (.y _relativelocation) _z))
  (bind _returnvalue_9 (Math|Vector|MakeVector _x (.y _relativelocation) (.z _relativelocation)))
  (bind _returnvalue_10 (Math|Vector|MakeVector (.x _relativelocation) _y (.z _relativelocation)))
  (bind _returnvalue_11 (+ _x_2 _maximum_limit_2))
  (bind _returnvalue_12 (+ _y_2 _maximum_limit_3))
  (bind _returnvalue_13 (+ _z_2 _maximum_limit))
  (bind _returnvalue_14 (Math|Rotator|FindLookatRotation _relativelocation_2 _returnvalue_10))
  (bind _returnvalue_15 (Math|Rotator|FindLookatRotation _relativelocation_2 _returnvalue_8))
  (bind _returnvalue_16 (Math|Rotator|FindLookatRotation _relativelocation_2 _returnvalue_9))
  (bind _returnvalue_17 (Math|Float|Clamp(Float) (.z _relativelocation_3) _returnvalue_5 _returnvalue_13))
  (bind _returnvalue_18 (Math|Float|Clamp(Float) (.x _relativelocation_3) _returnvalue_6 _returnvalue_11))
  (bind _returnvalue_19 (Math|Float|Clamp(Float) (.y _relativelocation_3) _returnvalue_7 _returnvalue_12))
  (bind _returnvalue_20 (Math|Float|SelectFloat _returnvalue_17 (.z _relativelocation_3) _limit_value))
  (bind _returnvalue_21 (Math|Float|SelectFloat _returnvalue_18 (.x _relativelocation_3) _limit_value_2))
  (bind _returnvalue_22 (Math|Float|SelectFloat _returnvalue_19 (.y _relativelocation_3) _limit_value_3))
  (bind _returnvalue_23 (> (.yaw _returnvalue_16) -8e+01))
  (bind _returnvalue_24 (> (.yaw _returnvalue_14) 1.7e+02))
  (bind _returnvalue_25 (+ (.pitch _returnvalue_14) 9e+01))
  (bind _returnvalue_26 (+ (.pitch _returnvalue_16) 9e+01))
  (bind _returnvalue_27 (Math|Float|SelectFloat -1.0 1.0 _returnvalue_23))
  (bind _returnvalue_28 (Math|Float|SelectFloat -1.0 1.0 _returnvalue_24))
  (bind _returnvalue_29 (* _returnvalue_28 _returnvalue_25))
  (bind _returnvalue_30 (* _returnvalue_27 _returnvalue_26))
  ;[1 1 1] On component dropped
  (Physics|SetSimulatePhysics _hitbox__2 false)
  (Utilities|FlowControl|Sequence
    (:then_0
      (Transformation|SetRelativeRotation _hitbox__2 (.rotation (Variables|Default|GetHitbox%20Relative%20Transform)) false false)
      (if (Variables|Default|GetSnap%20To%20Original%20Transform)
        (bind _newtrack_0 (Timeline|Timeline_1 PlayFromStart)
          (:Update
            (switch Utilities|FlowControl|Switch|SwitchonFollowHandleEnum (Variables|Default|GetInteract%20Type)
              (:NewEnumerator0
                (bind _output_get (Variables|Default|SetOut%20Vector (Math|Vector|Lerp(Vector) (.location _returnvalue_3) (.location _returnvalue_2) _newtrack_0)))
                (Transformation|SetRelativeLocation _recievetransform _output_get false false)
                (Transformation|SetWorldLocation (Variables|Default|GetHitbox_) _returnvalue_4 false false))
              (:NewEnumerator1
                (bind _output_get_2 (Variables|Default|SetOut%20Rotation (Math|Rotator|Lerp(Rotator) (.rotation _returnvalue_3) (.rotation _returnvalue_2) _newtrack_0)))
                (Transformation|SetRelativeRotation _recievetransform _output_get_2 false false))))
          (:Finished
            (CallFunction|BacktoOriginal)))
        (else
          (Transformation|SetWorldLocation _hitbox__2 _returnvalue_4 false false))))
    (:then_1
      ;[1 1 1] On component grabbed
      (Timeline|Timeline_0 Stop
        (:Update
          (switch Utilities|FlowControl|Switch|SwitchonFollowHandleEnum (Variables|Default|GetInteract%20Type)
            (:NewEnumerator0
              (Transformation|SetWorldLocation _follow_cube _returnvalue false false)
              (bind _output_get_3 (Variables|Default|SetOut%20Vector (Math|Vector|SelectVector (Utilities|SecondaryDirectionSolve _returnvalue_21 _returnvalue_22 _returnvalue_20) (Utilities|Select :Index (Variables|Default|GetXYZ%20Direction) :NewEnumerator0 (Math|Vector|MakeVector _returnvalue_21 _y_2 _z_2) :NewEnumerator1 (Math|Vector|MakeVector _x_2 _returnvalue_22 _z_2) :NewEnumerator2 (Math|Vector|MakeVector _x_2 _y_2 _returnvalue_20)) (Variables|Default|GetSecondaryMovementAxis))))
              (Transformation|SetRelativeLocation _recievetransform_2 _output_get_3 false false))
            (:NewEnumerator1
              (if (Variables|Default|GetRotation%20Relative%20To%20Hitbox)
                (Transformation|SetWorldRotation _follow_cube (Transformation|GetWorldRotation _hitbox_) false false)
                (else
                  (Transformation|SetWorldLocation _follow_cube _returnvalue false false)))
              (bind _output_get_4 (Variables|Default|SetOut%20Rotation (Utilities|Select :Index (Variables|Default|GetXYZ%20Direction) :NewEnumerator0 (select (Variables|Default|GetRotation%20relative%20to%20hitbox) (Math|Rotator|MakeRotator (Math|Float|SelectFloat (Math|Float|Clamp(Float) (.roll _relativerotation_2) (Variables|Default|GetMinimum%20Limit) (Variables|Default|GetMaximum%20Limit)) (.roll _relativerotation_2) (Variables|Default|GetLimit%20Value)) 0.0 0.0) (Math|Rotator|MakeRotator (+ (Math|Float|SelectFloat (Math|Float|Clamp(Float) _returnvalue_30 (Variables|Default|GetMinimum%20Limit) (Variables|Default|GetMaximum%20Limit)) _returnvalue_30 (Variables|Default|GetLimit%20Value)) (+ 9e+01 (Variables|Default|GetXRotSolve))) 0.0 0.0)) :NewEnumerator1 (select (Variables|Default|GetRotation%20relative%20to%20hitbox) (Math|Rotator|MakeRotator 0.0 (Math|Float|SelectFloat (Math|Float|Clamp(Float) (.pitch _relativerotation_3) (Variables|Default|GetMinimum%20Limit) (Variables|Default|GetMaximum%20Limit)) (.pitch _relativerotation_3) (Variables|Default|GetLimit%20Value)) 0.0) (Math|Rotator|MakeRotator 0.0 (+ (Math|Float|SelectFloat (Math|Float|Clamp(Float) _returnvalue_29 (Variables|Default|GetMinimum%20Limit) (Variables|Default|GetMaximum%20Limit)) _returnvalue_29 (Variables|Default|GetLimit%20Value)) -1.8e+02) 0.0)) :NewEnumerator2 (select (Variables|Default|GetRotation%20relative%20to%20hitbox) (Math|Rotator|MakeRotator 0.0 0.0 (Math|Float|SelectFloat (Math|Float|Clamp(Float) (.yaw _relativerotation) (Variables|Default|GetMinimum%20Limit) (Variables|Default|GetMaximum%20Limit)) (.yaw _relativerotation) (Variables|Default|GetLimit%20Value))) (Math|Rotator|MakeRotator 0.0 0.0 (Math|Float|SelectFloat (Math|Float|Clamp(Float) (.yaw _returnvalue_15) (Variables|Default|GetMinimum%20Limit) (Variables|Default|GetMaximum%20Limit)) (.yaw _returnvalue_15) (Variables|Default|GetLimit%20Value)))))))
              (Transformation|SetRelativeRotation _recievetransform_2 _output_get_4 false false))))))))

(event Custom|Back%20to%20original
  ;[1 1 1] On component dropped
)

(event EventBeginPlay
  ;[1 1 1] BeginPlay
  (Variables|Default|SetInitial%20Recieve%20Transform (Transformation|GetRelativeTransform (Variables|Default|GetInitialTransform)))
  (Variables|Default|SetHitbox%20Relative%20Transform (Transformation|GetRelativeTransform (Variables|Default|GetHitbox_)))
  (Variables|Default|SetHBLoc (Transformation|GetWorldLocation (Variables|Default|GetHitboxLoc)))
  (CallFunction|BreakGrip))

(fn ConstructionScript)