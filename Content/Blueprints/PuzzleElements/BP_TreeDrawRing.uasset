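; BP_TreeDrawRing is a draw-ring puzzle element for the Library Tree, a child Blueprint that reports brush sphere overlaps on its mesh to parent logic.
; UpdatePrimedList checks whether every Library Tree Dot is primed, then calls Finished and grows the BP_Vine.
; It also plays a timeline moving three Niagara effects along their splines.
; The level-transfer reference is cached, but its unlock is unconnected.
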(event OnComponentBeginOverlap(StaticMesh4)
  (params (OverlappedComponent :type Primitive%20Component%20Object%20Reference) (OtherActor :type Actor%20Object%20Reference) (OtherComp :type Primitive%20Component%20Object%20Reference) (OtherBodyIndex :type Integer) (bFromSweep :type Boolean) (SweepResult :type Hit%20Result%20Structure%20%28by%20ref%29))
  (if (== (Variables|/Game/Blueprints/Paintbrush/Paintrbsuh.Paintrbsuh_C|GetCollisionSphere (Variables|Default|GetBrushRefVar)) OtherComp)
    (CallFunction|ParentBegin)))

(event OnComponentEndOverlap(StaticMesh4)
  (params (OverlappedComponent :type Primitive%20Component%20Object%20Reference) (OtherActor :type Actor%20Object%20Reference) (OtherComp :type Primitive%20Component%20Object%20Reference) (OtherBodyIndex :type Integer))
  (if (== (Variables|/Game/Blueprints/Paintbrush/Paintrbsuh.Paintrbsuh_C|GetCollisionSphere (Variables|Default|GetBrushRefVar)) OtherComp)
    (CallFunction|ExitedParent)))

(event Custom|UpdatePrimedList
  (Variables|Default|SetAllPrimed_0 true)
  (for _array_element (stale EventBeginPlay _output_get)
    (switch Utilities|FlowControl|Switch|SwitchonRoomEnum (Variables|/Game/Blueprints/Spline_BP/Dot.Dot_C|Getenum _array_element)
      (:NewEnumerator7
        (if (not (Variables|/Game/Blueprints/Spline_BP/Dot.Dot_C|GetPrimed? _array_element))
          (Variables|Default|SetAllPrimed_0 false)))))
  (if (Variables|Default|GetAllPrimed_0)
    (CallFunction|Finished)
    (Default|VineGrow (Variables|Default|GetVine))
    (CallFunction|D01 false)))

(event Custom|D01
  (params (Condition :type Boolean))
  (bind _spline1 (Variables|Default|GetSpline1))
  (bind _spline (Variables|Default|GetSpline))
  (bind _spline2 (Variables|Default|GetSpline2))
  (bind _newtrack_0 (Timeline|Timeline_0 PlayFromStart)
    (:Update
      (Transformation|SetWorldLocation (Variables|Default|GetNiagara) (Spline|GetLocationatDistanceAlongSpline _spline (Math|Float|Lerp 0.0 (Spline|GetSplineLength _spline) _newtrack_0) "World") false false)
      (Transformation|SetWorldLocation (Variables|Default|GetNiagara1) (Spline|GetLocationatDistanceAlongSpline _spline1 (Math|Float|Lerp 0.0 (Spline|GetSplineLength _spline1) _newtrack_0) "World") false false)
      (Transformation|SetWorldLocation (Variables|Default|GetNiagara2) (Spline|GetLocationatDistanceAlongSpline _spline2 (Math|Float|Lerp 0.0 (Spline|GetSplineLength _spline2) _newtrack_0) "World") false false))))

(event EventBeginPlay
  (|CallParentFunction)
  (bind _returnvalue (Actor|GetActorOfClass "/Game/Blueprints/BP/BP_LevelTransfer.BP_LevelTransfer_C"))
  (Variables|Default|SetTransfer _returnvalue)
  (bind _returnvalue_2 (Actor|GetActorOfClass "/Game/Blueprints/Conservatory/BP_Vine.BP_Vine_C"))
  (Variables|Default|SetVine _returnvalue_2)
  (bind _outactors (Actor|GetAllActorsOfClass "/Game/Blueprints/Spline_BP/Dot.Dot_C"))
  (bind _output_get (Variables|Default|SetOut%20Actors _outactors)))

(event EventFinished)

(fn ConstructionScript
  (|CallParentFunction))