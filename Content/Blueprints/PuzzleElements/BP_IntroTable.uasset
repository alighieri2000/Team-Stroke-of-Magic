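; BP_IntroTable is a puzzle element for an intro table that extends a parent paint Blueprint and sets its paint type on BeginPlay.
; DripDip chains two timelines into a self-repeating cycle, switching MainGreen's static paint on with an Entered call, then off with Exited.
; BrushBounds2 overlaps forward to the parent's begin and exit logic, only for the referenced brush's collision sphere.
; Nothing in this file starts DripDip.
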(event OnComponentBeginOverlap(BrushBounds2)
  (params (OverlappedComponent :type Primitive%20Component%20Object%20Reference) (OtherActor :type Actor%20Object%20Reference) (OtherComp :type Primitive%20Component%20Object%20Reference) (OtherBodyIndex :type Integer) (bFromSweep :type Boolean) (SweepResult :type Hit%20Result%20Structure%20%28by%20ref%29))
  (if (== OtherComp (Variables|/Game/Blueprints/Paintbrush/Paintrbsuh.Paintrbsuh_C|GetCollisionSphere (Variables|Default|GetBrushRefVar)))
    (CallFunction|ParentBegin)))

(event OnComponentEndOverlap(BrushBounds2)
  (params (OverlappedComponent :type Primitive%20Component%20Object%20Reference) (OtherActor :type Actor%20Object%20Reference) (OtherComp :type Primitive%20Component%20Object%20Reference) (OtherBodyIndex :type Integer))
  (if (== OtherComp (Variables|/Game/Blueprints/Paintbrush/Paintrbsuh.Paintrbsuh_C|GetCollisionSphere (Variables|Default|GetBrushRefVar)))
    (CallFunction|ExitedParent)))

(event Custom|Drip%20Dip
  (bind _maingreen (Variables|Default|GetMainGreen))
  (Timeline|Timeline_0 PlayFromStart
    (:Finished
      (Variables|Default|SetIs%20Within%20Paint%20Bounds true)
      (Variables|/Game/Blueprints/Palette/BP_MainGreenPaint.BP_MainGreenPaint_C|SetStaticPaint _maingreen true)
      (Default|Entered _maingreen "NewEnumerator3")
      (Timeline|Timeline_1 PlayFromStart
        (:Finished
          (Variables|/Game/Blueprints/Palette/BP_MainGreenPaint.BP_MainGreenPaint_C|SetStaticPaint _maingreen false)
          (Default|Exited _maingreen)
          (CallFunction|DripDip))))))

(event EventBeginPlay
  (|CallParentFunction)
  (Variables|Default|SetEnum%20paints "NewEnumerator1"))

(fn ConstructionScript
  (|CallParentFunction))