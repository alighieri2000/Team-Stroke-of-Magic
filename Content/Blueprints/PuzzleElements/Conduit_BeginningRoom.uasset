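; Beginning-room variant of the conduit puzzle element, which starts powered and opens the way when its puzzle is finished.
; BeginPlay runs the parent logic, then calls PoweredUp.
; Finished plays the clockwork gear audio while two timelines spin the conduit and chain holders and sink the conduit.
; After a short delay it lowers the gate, found through GetActorOfClass on BP_Gate rather than a set reference.
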(event EventBeginPlay
  (|CallParentFunction)
  (CallFunction|PoweredUp))

(event EventFinished
  (bind _conduit (Variables|Default|GetConduit))
  ;[1 1 1] Finished puzzle
  (Utilities|FlowControl|Sequence
    (:then_0
      (Audio|Components|Audio|Play (Variables|Default|GetA_ClockworkGears) 0.0)
      (bind _newtrack_0 (Timeline|Timeline_2 Play)
        (:Update
          (Transformation|SetRelativeRotation _conduit (Math|Rotator|Lerp(Rotator) "0, 0, 0" "0.000000,720.000000, 0" _newtrack_0) false false)
          (Transformation|SetRelativeRotation (Variables|Default|Getsm_ChainHolder4) (Math|Rotator|MakeRotator 9e+01 0.0 (.Yaw (Math|Rotator|BreakRotator (Math|Rotator|Lerp(Rotator) "0, 0, 0" "0.000000,720.000000, 0" _newtrack_0)))) false false)
          (Transformation|SetRelativeRotation (Variables|Default|Getsm_ChainHolder5) (Math|Rotator|Lerp(Rotator) "0, 0, 0" "720.000000,0.000000, 0" _newtrack_0) false false)
          (Transformation|SetRelativeRotation (Variables|Default|Getsm_ChainHolder7) (Math|Rotator|Lerp(Rotator) "0, 0, 0" "-720.000000,0.000000, 0" _newtrack_0) false false))))
    (:then_1
      (bind _newtrack_0_2 (Timeline|Timeline_3 Play)
        (:Update
          (Transformation|SetRelativeLocation _conduit (Math|Vector|MakeVector 0.0 0.0 (Math|Float|Lerp 0.0 -31.0 _newtrack_0_2)) false false))))
    (:then_2
      ;;[1 1 1] Lowers Gate
      (Utilities|FlowControl|Delay 0.5)
      (bind _returnvalue (Actor|GetActorOfClass "/Game/Blueprints/BP/BP_Gate.BP_Gate_C"))
      (Default|LowerGate _returnvalue))))

(fn ConstructionScript
  (|CallParentFunction))