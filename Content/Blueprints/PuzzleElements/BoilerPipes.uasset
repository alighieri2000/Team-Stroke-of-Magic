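; VR boiler-pipe puzzle element with a grabbable handle that redirects water between pipe outlets.
; While held, look-at math rotates the handle with clicks; on release, a Boing timeline snaps it toward the last direction set by trigger overlaps.
; Timeline-scaled meshes animate the water, and left flow pumps BP_Boiler, whose completion blocks further grabs.
; Other triggers handle paintbrush exit and clear its paint while a hazard mesh is active.
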(event OnComponentBeginOverlap(TopDir)
  (params (OverlappedComponent :type Primitive%20Component%20Object%20Reference) (OtherActor :type Actor%20Object%20Reference) (OtherComp :type Primitive%20Component%20Object%20Reference) (OtherBodyIndex :type Integer) (bFromSweep :type Boolean) (SweepResult :type Hit%20Result%20Structure%20%28by%20ref%29))
  (if (== OtherComp (Variables|Default|Getp4))
    (CallFunction|WaterUp)
    (Variables|Default|SetRotDir 1.8e+02)
    (Audio|PlaySoundatLocation "/Game/Audio/Click__1__Cue1.Click__1__Cue1" (Variables|/Script/Engine.SceneComponent|GetRelativeLocation (Variables|Default|GetCube1)) "0, 0, 0" 1.0 1.0 0.0 "/Game/Audio-Revised/Master-Mixer/ATT/ATT_ObjectSmall.ATT_ObjectSmall" 0 0)))

(event OnComponentBeginOverlap(BottomDir)
  (params (OverlappedComponent :type Primitive%20Component%20Object%20Reference) (OtherActor :type Actor%20Object%20Reference) (OtherComp :type Primitive%20Component%20Object%20Reference) (OtherBodyIndex :type Integer) (bFromSweep :type Boolean) (SweepResult :type Hit%20Result%20Structure%20%28by%20ref%29))
  (if (== OtherComp (Variables|Default|Getp4))
    (CallFunction|WaterDown)
    (Variables|Default|SetRotDir 0.0)
    (Audio|PlaySoundatLocation "/Game/Audio/Click__1__Cue1.Click__1__Cue1" (Variables|/Script/Engine.SceneComponent|GetRelativeLocation (Variables|Default|GetCube1)) "0, 0, 0" 1.0 1.0 0.0 "/Game/Audio-Revised/Master-Mixer/ATT/ATT_ObjectSmall.ATT_ObjectSmall" 0 0)))

(event OnGrabbed(GrabComponent)
  (bind _p3 (Variables|Default|Getp3))
  (bind _cube (Variables|Default|GetCube))
  (bind _cube1 (Variables|Default|GetCube1))
  (bind _cube1_2 (Variables|Default|GetCube1))
  (bind _relativelocation (Variables|/Script/Engine.SceneComponent|GetRelativeLocation _cube))
  (bind _returnvalue (Math|Rotator|FindLookatRotation (Math|Vector|MakeVector 147.195343 17.221565 187.974838) (Math|Vector|MakeVector (.x _relativelocation) 17.221565 (.z _relativelocation))))
  (bind (_roll _pitch _yaw) (Math|Rotator|BreakRotator _returnvalue))
  (if (not (Variables|/Game/Blueprints/BP/BP_Boiler.BP_Boiler_C|GetBoilDone (Variables|Default|GetBoilerRef)))
    (Utilities|FlowControl|Sequence
      (:then_0
        (Timeline|Timeline_9 PlayFromStart
          (:Update
            (Transformation|SetWorldLocation (Variables|Default|GetCube) (Transformation|GetWorldLocation (Variables|Default|Getp3)) false false))))
      (:then_1
        (Timeline|Timeline_8 PlayFromStart
          (:Update
            (bind _output_get (Variables|Default|SetRotVal (* (Math|Float|SelectFloat -1.0 1.0 (> _yaw 179.0)) (+ _pitch 9e+01))))
            (Transformation|SetRelativeRotation _cube1 (Math|Rotator|MakeRotator 0.0 _output_get 0.0) false false))))
      (:then_2
        (bind _newtrack_0 (Timeline|Boing Stop)
          (:Update
            (Transformation|SetRelativeRotation _cube1 (Math|Rotator|MakeRotator 0.0 (Math|Float|Lerp (Variables|Default|GetRot%20Val2) (Variables|Default|GetRot%20Dir2) _newtrack_0) 0.0) false false))
          (:Finished
            (Transformation|SetWorldLocation _p3 (Transformation|GetWorldLocation (Variables|Default|Getp5)) false false)
            (Transformation|SetRelativeRotation (Variables|Default|Getp3) (Variables|/Script/Engine.SceneComponent|GetRelativeRotation _cube1_2) false false)
            (Physics|SetSimulatePhysics _p3 false)
            (Timeline|Timeline_8 Stop))))
      (:then_3
        (bind _output_get_2 (Variables|Default|SetClickDist (Math|Float|MapRangeClamped (Variables|Default|GetRotVal) -1.8e+02 1.8e+02 0.0 1.0)))
        (Timeline|ClickTime PlayFromStart
          (:Update
            (if (or (> (- (Math|Float|MapRangeClamped (Variables|Default|GetRotVal) -1.8e+02 1.8e+02 0.0 1.0) _output_get_2) 0.05) (< (- (Math|Float|MapRangeClamped (Variables|Default|GetRotVal) -1.8e+02 1.8e+02 0.0 1.0) _output_get_2) -0.05))
              (Audio|PlaySoundatLocation "/Game/Audio/Click__1__Cue.Click__1__Cue" (Variables|/Script/Engine.SceneComponent|GetRelativeLocation _cube1_2) "0, 0, 0" 1.0 1.0 0.0 "/Game/Audio-Revised/Master-Mixer/ATT/ATT_ObjectSmall.ATT_ObjectSmall" 0 0)
              (Variables|Default|SetClickDist (Math|Float|MapRangeClamped (Variables|Default|GetRotVal) -1.8e+02 1.8e+02 0.0 1.0)))))))))

(event OnComponentBeginOverlap(P1_L2)
  (params (OverlappedComponent :type Primitive%20Component%20Object%20Reference) (OtherActor :type Actor%20Object%20Reference) (OtherComp :type Primitive%20Component%20Object%20Reference) (OtherBodyIndex :type Integer) (bFromSweep :type Boolean) (SweepResult :type Hit%20Result%20Structure%20%28by%20ref%29))
  (if (== OtherComp (Variables|Default|GetBox2))
    (Variables|Default|Set2 true)))

(event OnComponentBeginOverlap(P1_R2)
  (params (OverlappedComponent :type Primitive%20Component%20Object%20Reference) (OtherActor :type Actor%20Object%20Reference) (OtherComp :type Primitive%20Component%20Object%20Reference) (OtherBodyIndex :type Integer) (bFromSweep :type Boolean) (SweepResult :type Hit%20Result%20Structure%20%28by%20ref%29))
  (if (== OtherComp (Variables|Default|GetBox2))
    (Variables|Default|Set2 false)))

(event OnDropped(GrabComponent)
  (bind _p3 (Variables|Default|Getp3))
  (bind _cube (Variables|Default|GetCube))
  (bind _cube1 (Variables|Default|GetCube1))
  (bind _cube1_2 (Variables|Default|GetCube1))
  (bind _rotdir (Variables|Default|GetRotDir))
  (bind _relativelocation (Variables|/Script/Engine.SceneComponent|GetRelativeLocation _cube))
  (bind _returnvalue (Math|Rotator|FindLookatRotation (Math|Vector|MakeVector 147.195343 17.221565 187.974838) (Math|Vector|MakeVector (.x _relativelocation) 17.221565 (.z _relativelocation))))
  (bind (_roll _pitch _yaw) (Math|Rotator|BreakRotator _returnvalue))
  (Variables|Default|SetRot%20Val2 (Variables|Default|GetRotVal))
  (if (> (Variables|Default|GetRotVal) 0.0)
    (Variables|Default|SetRot%20Dir2 _rotdir)
    (else
      (Variables|Default|SetRot%20Dir2 (* _rotdir -1.0))))
  (Utilities|FlowControl|Sequence
    (:then_0
      (Timeline|Timeline_8 Stop
        (:Update
          (bind _output_get (Variables|Default|SetRotVal (* (Math|Float|SelectFloat -1.0 1.0 (> _yaw 179.0)) (+ _pitch 9e+01))))
          (Transformation|SetRelativeRotation _cube1 (Math|Rotator|MakeRotator 0.0 _output_get 0.0) false false))))
    (:then_1
      (Timeline|Timeline_9 Stop
        (:Update
          (Transformation|SetWorldLocation (Variables|Default|GetCube) (Transformation|GetWorldLocation (Variables|Default|Getp3)) false false))))
    (:then_2
      (bind _newtrack_0 (Timeline|Boing PlayFromStart)
        (:Update
          (Transformation|SetRelativeRotation _cube1 (Math|Rotator|MakeRotator 0.0 (Math|Float|Lerp (Variables|Default|GetRot%20Val2) (Variables|Default|GetRot%20Dir2) _newtrack_0) 0.0) false false))
        (:Finished
          (Transformation|SetWorldLocation _p3 (Transformation|GetWorldLocation (Variables|Default|Getp5)) false false)
          (Transformation|SetRelativeRotation (Variables|Default|Getp3) (Variables|/Script/Engine.SceneComponent|GetRelativeRotation _cube1_2) false false)
          (Physics|SetSimulatePhysics _p3 false)
          (Timeline|Timeline_8 Stop))))
    (:then_3
      (Timeline|ClickTime Stop
        (:Update
          (if (or (> (- (Math|Float|MapRangeClamped (Variables|Default|GetRotVal) -1.8e+02 1.8e+02 0.0 1.0) (stale OnGrabbed(GrabComponent) _output_get_2)) 0.05) (< (- (Math|Float|MapRangeClamped (Variables|Default|GetRotVal) -1.8e+02 1.8e+02 0.0 1.0) (stale OnGrabbed(GrabComponent) _output_get_2)) -0.05))
            (Audio|PlaySoundatLocation "/Game/Audio/Click__1__Cue.Click__1__Cue" (Variables|/Script/Engine.SceneComponent|GetRelativeLocation _cube1_2) "0, 0, 0" 1.0 1.0 0.0 "/Game/Audio-Revised/Master-Mixer/ATT/ATT_ObjectSmall.ATT_ObjectSmall" 0 0)
            (Variables|Default|SetClickDist (Math|Float|MapRangeClamped (Variables|Default|GetRotVal) -1.8e+02 1.8e+02 0.0 1.0))))))))

(event OnComponentBeginOverlap(StaticMesh8)
  (params (OverlappedComponent :type Primitive%20Component%20Object%20Reference) (OtherActor :type Actor%20Object%20Reference) (OtherComp :type Primitive%20Component%20Object%20Reference) (OtherBodyIndex :type Integer) (bFromSweep :type Boolean) (SweepResult :type Hit%20Result%20Structure%20%28by%20ref%29))
  (bind _brushref (Variables|Default|GetbrushRef))
  (if (== OtherActor (Variables|/Game/Blueprints/Paintbrush/Paintrbsuh.Paintrbsuh_C|GetCollisionSphere _brushref))
    (if (Variables|Default|GetBadOn)
      (Default|Paint1Cleared _brushref))))

(event OnComponentBeginOverlap(Box)
  (params (OverlappedComponent :type Primitive%20Component%20Object%20Reference) (OtherActor :type Actor%20Object%20Reference) (OtherComp :type Primitive%20Component%20Object%20Reference) (OtherBodyIndex :type Integer) (bFromSweep :type Boolean) (SweepResult :type Hit%20Result%20Structure%20%28by%20ref%29))
  (bind _brushref (Variables|Default|GetbrushRef))
  (if (== (Variables|/Game/Blueprints/Paintbrush/Paintrbsuh.Paintrbsuh_C|GetCollisionSphere _brushref) OtherComp)
    (Default|ExitedParent (Variables|Default|GetBoilerCondRef))
    (Default|Exited _brushref)))

(event OnComponentBeginOverlap(P1_L)
  (params (OverlappedComponent :type Primitive%20Component%20Object%20Reference) (OtherActor :type Actor%20Object%20Reference) (OtherComp :type Primitive%20Component%20Object%20Reference) (OtherBodyIndex :type Integer) (bFromSweep :type Boolean) (SweepResult :type Hit%20Result%20Structure%20%28by%20ref%29))
  (if (== OtherComp 0)
    (Variables|Default|Set1 true)
    (Rendering|SetVisibility (Variables|Default|GetWaterfallRight) false false)))

(event OnComponentEndOverlap(Box2)
  (params (OverlappedComponent :type Primitive%20Component%20Object%20Reference) (OtherActor :type Actor%20Object%20Reference) (OtherComp :type Primitive%20Component%20Object%20Reference) (OtherBodyIndex :type Integer))
  (bind _cube12 (Variables|Default|GetCube12))
  (bind _cube14 (Variables|Default|GetCube14))
  (bind _relativerotation (Variables|/Script/Engine.SceneComponent|GetRelativeRotation _cube12))
  (Utilities|FlowControl|Sequence
    (:then_0
      (Utilities|FlowControl|DoOnce false
        (:Completed
          (Utilities|FlowControl|Delay 5.0)
          (Timeline|Timeline_1 Stop
            (:Update
              (if (< (.roll _relativerotation) 0.0)
                (Transformation|SetRelativeRotation _cube14 (Math|Rotator|MakeRotator 0.0 (+ (* (.pitch _relativerotation) -1.0) -9e+01) 0.0) false false)
                (else
                  (Transformation|SetRelativeRotation _cube14 (Math|Rotator|MakeRotator 0.0 (+ (.pitch _relativerotation) 9e+01) 0.0) false false))))))))
    (:then_1
      (Utilities|FlowControl|DoOnce false) ; enters at Reset
    )))

(event OnComponentBeginOverlap(Box2)
  (params (OverlappedComponent :type Primitive%20Component%20Object%20Reference) (OtherActor :type Actor%20Object%20Reference) (OtherComp :type Primitive%20Component%20Object%20Reference) (OtherBodyIndex :type Integer) (bFromSweep :type Boolean) (SweepResult :type Hit%20Result%20Structure%20%28by%20ref%29))
  (bind _cube12 (Variables|Default|GetCube12))
  (bind _cube14 (Variables|Default|GetCube14))
  (bind _relativerotation (Variables|/Script/Engine.SceneComponent|GetRelativeRotation _cube12))
  (Utilities|FlowControl|Sequence
    (:then_0
      (Utilities|FlowControl|DoOnce false
        (:Completed
          (Timeline|Timeline_1 PlayFromStart
            (:Update
              (if (< (.roll _relativerotation) 0.0)
                (Transformation|SetRelativeRotation _cube14 (Math|Rotator|MakeRotator 0.0 (+ (* (.pitch _relativerotation) -1.0) -9e+01) 0.0) false false)
                (else
                  (Transformation|SetRelativeRotation _cube14 (Math|Rotator|MakeRotator 0.0 (+ (.pitch _relativerotation) 9e+01) 0.0) false false))))))))
    (:then_1
      (Utilities|FlowControl|DoOnce false) ; enters at Reset
    )))

(event OnComponentBeginOverlap(RightDir)
  (params (OverlappedComponent :type Primitive%20Component%20Object%20Reference) (OtherActor :type Actor%20Object%20Reference) (OtherComp :type Primitive%20Component%20Object%20Reference) (OtherBodyIndex :type Integer) (bFromSweep :type Boolean) (SweepResult :type Hit%20Result%20Structure%20%28by%20ref%29))
  (if (== OtherComp (Variables|Default|Getp4))
    (CallFunction|WaterRight)
    (Variables|Default|SetRotDir 9e+01)
    (Audio|PlaySoundatLocation "/Game/Audio/Click__1__Cue1.Click__1__Cue1" (Variables|/Script/Engine.SceneComponent|GetRelativeLocation (Variables|Default|GetCube1)) "0, 0, 0" 1.0 1.0 0.0 "/Game/Audio-Revised/Master-Mixer/ATT/ATT_ObjectSmall.ATT_ObjectSmall" 0 0)))

(event OnComponentBeginOverlap(LeftDir)
  (params (OverlappedComponent :type Primitive%20Component%20Object%20Reference) (OtherActor :type Actor%20Object%20Reference) (OtherComp :type Primitive%20Component%20Object%20Reference) (OtherBodyIndex :type Integer) (bFromSweep :type Boolean) (SweepResult :type Hit%20Result%20Structure%20%28by%20ref%29))
  (if (== OtherComp (Variables|Default|Getp4))
    (CallFunction|WaterLeft)
    (Variables|Default|SetRotDir 9e+01)
    (Audio|PlaySoundatLocation "/Game/Audio/Click__1__Cue1.Click__1__Cue1" (Variables|/Script/Engine.SceneComponent|GetRelativeLocation (Variables|Default|GetCube1)) "0, 0, 0" 1.0 1.0 0.0 "/Game/Audio-Revised/Master-Mixer/ATT/ATT_ObjectSmall.ATT_ObjectSmall" 0 0)))

(event Custom|BoilerOn
  (Rendering|SetVisibility (Variables|Default|GetStaticMesh8) true false)
  (Variables|Default|SetBadOn true))

(event Custom|BoilerOff
  (Rendering|SetVisibility (Variables|Default|GetStaticMesh8) false false)
  (Variables|Default|SetBadOn false))

(event Custom|WaterRight
  (Variables|Default|SetRight true)
  (CallFunction|ResetLeft)
  (CallFunction|DownReset)
  (Transformation|SetRelativeScale3D (Variables|Default|GetWaterFlatRight) (Math|Vector|MakeVector 0.301191 0.360641 0.0))
  (Transformation|SetRelativeScale3D (Variables|Default|GetWaterfallRight) (Math|Vector|MakeVector 1.0 1.0 0.0))
  (Transformation|SetRelativeScale3D (Variables|Default|GetWaterScaler) (Math|Vector|MakeVector 0.301191 0.360641 0.162823))
  (Variables|Default|SetWaterfalSeq false)
  (bind _newtrack_0 (Timeline|Waterflow PlayFromStart)
    (:Update
      (if (Variables|Default|GetWaterfalSeq)
        (Transformation|SetRelativeScale3D (Variables|Default|GetWaterfallRight) (Math|Vector|MakeVector 1.0 1.0 (Math|Float|Lerp 0.0 1.0 _newtrack_0)))
        (else
          (Transformation|SetRelativeScale3D (Variables|Default|GetWaterFlatRight) (Math|Vector|MakeVector 0.301191 0.360641 (Math|Float|Lerp 0.0 0.070759 _newtrack_0))))))
    (:Finished
      (if (not (Variables|Default|GetWaterfalSeq))
        (Variables|Default|SetWaterfalSeq true)
        (Timeline|Waterflow PlayFromStart)))))

(event Custom|WaterLeft
  (bind _waterflatleft (Variables|Default|GetWaterFlatLeft))
  (Variables|Default|SetLeft true)
  (CallFunction|DownReset)
  (CallFunction|ResetRight)
  (Default|Pumpin (Variables|Default|GetBoilerRef))
  (Transformation|SetRelativeScale3D _waterflatleft (Math|Vector|MakeVector 0.475917 0.453531 0.0))
  (Rendering|SetVisibility _waterflatleft true false)
  (Transformation|SetRelativeScale3D (Variables|Default|GetWaterfallLeft) (Math|Vector|MakeVector 1.459603 0.989117 0.0))
  (Transformation|SetRelativeScale3D (Variables|Default|GetWaterScaler1) (Math|Vector|MakeVector 0.342805 0.361086 0.162823))
  (Variables|Default|SetWaterfalSeq false)
  (bind _newtrack_0 (Timeline|Timeline_4 PlayFromStart)
    (:Update
      (if (Variables|Default|GetWaterfalSeq)
        (Transformation|SetRelativeScale3D (Variables|Default|GetWaterfallLeft) (Math|Vector|MakeVector 1.459603 0.989117 (Math|Float|Lerp 0.0 2.518253 _newtrack_0)))
        (else
          (Transformation|SetRelativeScale3D (Variables|Default|GetWaterFlatLeft) (Math|Vector|MakeVector 0.475917 0.453531 (Math|Float|Lerp 0.0 0.079829 _newtrack_0))))))
    (:Finished
      (if (not (Variables|Default|GetWaterfalSeq))
        (Variables|Default|SetWaterfalSeq true)
        (Timeline|Timeline_4 PlayFromStart)))))

(event Custom|WaterUp
  (CallFunction|ResetLeft)
  (CallFunction|ResetRight)
  (CallFunction|DownReset))

(event Custom|WaterDown
  (Variables|Default|SetDown true)
  (CallFunction|ResetRight)
  (CallFunction|ResetLeft)
  (Transformation|SetRelativeScale3D (Variables|Default|GetWaterScaler2) (Math|Vector|MakeVector 0.342805 0.361086 0.162823))
  (Transformation|SetRelativeScale3D (Variables|Default|GetWaterfallRBott) (Math|Vector|MakeVector 1.437515 1.193711 0.0))
  (bind _newtrack_0 (Timeline|Timeline_6 PlayFromStart)
    (:Update
      (Transformation|SetRelativeScale3D (Variables|Default|GetWaterfallRBott) (Math|Vector|MakeVector 1.437515 1.193711 (Math|Float|Lerp 0.0 1.0 _newtrack_0))))))

(event Custom|ResetRight
  (if (Variables|Default|GetRight)
    (Variables|Default|SetRight false)
    (bind _newtrack_0 (Timeline|WaterReverse PlayFromStart)
      (:Update
        (Transformation|SetRelativeScale3D (Variables|Default|GetWaterFlatRight) (Math|Vector|MakeVector (Math|Float|Lerp 0.301191 0.0 _newtrack_0) 0.360641 0.070759))
        (Transformation|SetRelativeScale3D (Variables|Default|GetWaterScaler) (Math|Vector|MakeVector 0.342805 0.361086 (Math|Float|Lerp 0.162823 0.0 _newtrack_0)))))))

(event Custom|ResetLeft
  (bind _waterflatleft (Variables|Default|GetWaterFlatLeft))
  (if (Variables|Default|GetLeft)
    (Default|StopPump (Variables|Default|GetBoilerRef))
    (Variables|Default|SetLeft false)
    (bind _newtrack_0 (Timeline|Timeline_5 PlayFromStart)
      (:Update
        (Transformation|SetRelativeScale3D _waterflatleft (Math|Vector|MakeVector (Math|Float|Lerp 0.475917 0.01 _newtrack_0) 0.453531 0.079829))
        (Transformation|SetRelativeScale3D (Variables|Default|GetWaterScaler1) (Math|Vector|MakeVector 0.342805 0.361086 (Math|Float|Lerp 0.162823 0.0 _newtrack_0))))
      (:Finished
        (Rendering|SetVisibility _waterflatleft false false)))))

(event Custom|DownReset
  (if (Variables|Default|GetDown)
    (Variables|Default|SetDown false)
    (bind _newtrack_0 (Timeline|Timeline_7 PlayFromStart)
      (:Update
        (Transformation|SetRelativeScale3D (Variables|Default|GetWaterScaler2) (Math|Vector|MakeVector 0.342805 0.361086 (Math|Float|Lerp 0.162823 0.0 _newtrack_0)))))))

(event EventBeginPlay
  (bind _p3 (Variables|Default|Getp3))
  (bind _cube (Variables|Default|GetCube))
  (bind _cube1 (Variables|Default|GetCube1))
  (bind _cube1_2 (Variables|Default|GetCube1))
  (bind _relativelocation (Variables|/Script/Engine.SceneComponent|GetRelativeLocation _cube))
  (bind _returnvalue (Math|Rotator|FindLookatRotation (Math|Vector|MakeVector 147.195343 17.221565 187.974838) (Math|Vector|MakeVector (.x _relativelocation) 17.221565 (.z _relativelocation))))
  (bind (_roll _pitch _yaw) (Math|Rotator|BreakRotator _returnvalue))
  (bind _returnvalue_2 (Actor|GetActorOfClass "/Game/Blueprints/Paintbrush/Paintrbsuh.Paintrbsuh_C"))
  (Variables|Default|SetbrushRef _returnvalue_2)
  (bind _returnvalue_3 (Actor|GetActorOfClass "/Game/Blueprints/VR_Character/BP_VrPlayerCharacter_FINAL.BP_VrPlayerCharacter_FINAL_C"))
  (Variables|Default|SetCharRef _returnvalue_3)
  (bind _returnvalue_4 (Actor|GetActorOfClass "/Game/Blueprints/BP/BP_Boiler.BP_Boiler_C"))
  (Variables|Default|SetBoilerRef _returnvalue_4)
  (bind _returnvalue_5 (Actor|GetActorOfClass "/Game/Blueprints/PuzzleElements/Conduit_Boiler.Conduit_Boiler_C"))
  (Variables|Default|SetBoilerCondRef _returnvalue_5)
  (Variables|Default|SetPuzzleSuccSeq 0)
  (CallFunction|DownReset)
  (CallFunction|ResetRight)
  (Variables|Default|SetRotDir 9e+01)
  (Variables|Default|SetRotVal -1.0)
  (Variables|Default|SetRot%20Val2 (Variables|Default|GetRotVal))
  (if (> (Variables|Default|GetRotVal) 0.0)
    (Variables|Default|SetRot%20Dir2 (Variables|Default|GetRotDir))
    (else
      (Variables|Default|SetRot%20Dir2 (* (Variables|Default|GetRotDir) -1.0))))
  (Utilities|FlowControl|Sequence
    (:then_0
      (Timeline|Timeline_8 Stop
        (:Update
          (bind _output_get (Variables|Default|SetRotVal (* (Math|Float|SelectFloat -1.0 1.0 (> _yaw 179.0)) (+ _pitch 9e+01))))
          (Transformation|SetRelativeRotation _cube1 (Math|Rotator|MakeRotator 0.0 _output_get 0.0) false false))))
    (:then_1
      (Timeline|Timeline_9 Stop
        (:Update
          (Transformation|SetWorldLocation (Variables|Default|GetCube) (Transformation|GetWorldLocation (Variables|Default|Getp3)) false false))))
    (:then_2
      (bind _newtrack_0 (Timeline|Boing PlayFromStart)
        (:Update
          (Transformation|SetRelativeRotation _cube1 (Math|Rotator|MakeRotator 0.0 (Math|Float|Lerp (Variables|Default|GetRot%20Val2) (Variables|Default|GetRot%20Dir2) _newtrack_0) 0.0) false false))
        (:Finished
          (Transformation|SetWorldLocation _p3 (Transformation|GetWorldLocation (Variables|Default|Getp5)) false false)
          (Transformation|SetRelativeRotation (Variables|Default|Getp3) (Variables|/Script/Engine.SceneComponent|GetRelativeRotation _cube1_2) false false)
          (Physics|SetSimulatePhysics _p3 false)
          (Timeline|Timeline_8 Stop))))
    (:then_3
      (Timeline|ClickTime Stop
        (:Update
          (if (or (> (- (Math|Float|MapRangeClamped (Variables|Default|GetRotVal) -1.8e+02 1.8e+02 0.0 1.0) (stale OnGrabbed(GrabComponent) _output_get_2)) 0.05) (< (- (Math|Float|MapRangeClamped (Variables|Default|GetRotVal) -1.8e+02 1.8e+02 0.0 1.0) (stale OnGrabbed(GrabComponent) _output_get_2)) -0.05))
            (Audio|PlaySoundatLocation "/Game/Audio/Click__1__Cue.Click__1__Cue" (Variables|/Script/Engine.SceneComponent|GetRelativeLocation _cube1_2) "0, 0, 0" 1.0 1.0 0.0 "/Game/Audio-Revised/Master-Mixer/ATT/ATT_ObjectSmall.ATT_ObjectSmall" 0 0)
            (Variables|Default|SetClickDist (Math|Float|MapRangeClamped (Variables|Default|GetRotVal) -1.8e+02 1.8e+02 0.0 1.0))))))))

(event EventTick
  (params (DeltaSeconds :type Float%20%28single-precision%29))
  (Utilities|FlowControl|Sequence
    (:then_0
      (if (Variables|Default|Get1)
        (Utilities|FlowControl|Sequence
          (:then_0
            (if (Variables|Default|Get2)
              (Utilities|FlowControl|Sequence)))
          (:then_1
            (if (Variables|Default|Get4)
              (CallFunction|Boileron)
              (else
                (CallFunction|BoilerOff)))))))))

(fn ConstructionScript)