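; Conservatory cosmos puzzle piece where a grabbable control slides a planet mesh along its local Y axis.
; While grabbed and unfinished, a timeline acts as an update loop, stepping the mesh by the control's roll direction outside a small dead zone, within clamped limits.
; On release, it stops and tells the level's BP_SunLaser whether the mesh sits near center.
; Chain sound calls are unwired.
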(event EventBeginPlay
  (|CallParentFunction)
  (bind _returnvalue (Actor|GetActorOfClass "/Game/Blueprints/Conservatory/BP_SunLaser.BP_SunLaser_C"))
  (Variables|Default|SetSunlaser_ref _returnvalue))

(event EventOnGrabbed
  (bind _out_rotation (Variables|Default|GetOut%20Rotation))
  (bind _returnvalue (> (.roll _out_rotation) 2e+02))
  ;[1 1 1] Tracking Planet controls
  (if (not (Variables|Default|GetFinished))
    (Timeline|Timeline_2 Play
      (:Update
        (if (or (and (> (.roll _out_rotation) 3.0) (< (.roll _out_rotation) 2e+02)) (and _returnvalue (< (.roll _out_rotation) 357.0)))
          (Variables|Default|SetNew%20Location%20Y (Math|Float|Clamp(Float) (+ (Variables|Default|GetNew%20Location%20Y) (Math|Float|SelectFloat -1.0 1.0 _returnvalue)) -215.0 215.0))
          (Transformation|SetRelativeLocation (Variables|Default|GetStaticMesh5) (Math|Vector|MakeVector 0.0 (Variables|Default|GetNew%20Location%20Y) 0.0) false false))))))

(event EventOnDropped
  (bind _out_rotation (Variables|Default|GetOut%20Rotation))
  (bind _returnvalue (> (.roll _out_rotation) 2e+02))
  ;[1 1 1] Tracking Planet controls
  (Default|1Dropped (Variables|Default|GetSunlaser_ref) (and (< (Variables|Default|GetNew%20Location%20Y) 2e+01) (> (Variables|Default|GetNew%20Location%20Y) -2e+01)))
  (Timeline|Timeline_2 Stop
    (:Update
      (if (or (and (> (.roll _out_rotation) 3.0) (< (.roll _out_rotation) 2e+02)) (and _returnvalue (< (.roll _out_rotation) 357.0)))
        (Variables|Default|SetNew%20Location%20Y (Math|Float|Clamp(Float) (+ (Variables|Default|GetNew%20Location%20Y) (Math|Float|SelectFloat -1.0 1.0 _returnvalue)) -215.0 215.0))
        (Transformation|SetRelativeLocation (Variables|Default|GetStaticMesh5) (Math|Vector|MakeVector 0.0 (Variables|Default|GetNew%20Location%20Y) 0.0) false false)))))

(fn ConstructionScript
  (|CallParentFunction))