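; BP_Boiler is a puzzle actor that completes once its shovels run and water is pumped in, then notifies the brush and cauldron.
; ShovelsPlay and Pumpin/StopPump drive timeline animations, indicators and audio, each start checking the other's state.
; Box overlaps toggle shovel-load meshes, while a grabbable door follows the grab cube via look-at rotation and eases shut on release.
; Steam and other Niagara effects are moved into place rather than spawned, with SetSteams staggering the steam.
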(event OnComponentBeginOverlap(Box1)
  (params (OverlappedComponent :type Primitive%20Component%20Object%20Reference) (OtherActor :type Actor%20Object%20Reference) (OtherComp :type Primitive%20Component%20Object%20Reference) (OtherBodyIndex :type Integer) (bFromSweep :type Boolean) (SweepResult :type Hit%20Result%20Structure%20%28by%20ref%29))
  (if (== OtherComp (Variables|Default|GetBox))
    (Utilities|FlowControl|DoOnce false
      (:Completed
        (Audio|Components|Audio|Play (Variables|Default|GetShovel%20Dig) 0.0)
        (Rendering|SetVisibility (Variables|Default|GetStaticMesh) true false)))
    (elif (== OtherComp (Variables|Default|GetBox3))
      (Utilities|FlowControl|DoOnce false
        (:Completed
          (Audio|Components|Audio|Play (Variables|Default|GetShovel%20Dig1) 0.0)
          (Rendering|SetVisibility (Variables|Default|GetStaticMesh1) true false))))))

(event OnComponentEndOverlap(Box1)
  (params (OverlappedComponent :type Primitive%20Component%20Object%20Reference) (OtherActor :type Actor%20Object%20Reference) (OtherComp :type Primitive%20Component%20Object%20Reference) (OtherBodyIndex :type Integer))
  (if (== OtherComp (Variables|Default|GetBox))
    (Utilities|FlowControl|DoOnce false) ; enters at Reset
    (elif (== OtherComp (Variables|Default|GetBox3))
      (Utilities|FlowControl|DoOnce false) ; enters at Reset
      (elif (== OtherActor 0)
        _))))

(event OnComponentBeginOverlap(Box2)
  (params (OverlappedComponent :type Primitive%20Component%20Object%20Reference) (OtherActor :type Actor%20Object%20Reference) (OtherComp :type Primitive%20Component%20Object%20Reference) (OtherBodyIndex :type Integer) (bFromSweep :type Boolean) (SweepResult :type Hit%20Result%20Structure%20%28by%20ref%29))
  (bind _a_thud (Variables|Default|GetA_Thud))
  (bind _niagara (Variables|Default|GetNiagara))
  (if (== OtherComp (Variables|Default|GetBox))
    (Utilities|FlowControl|DoOnce false
      (:Completed
        (Rendering|SetVisibility (Variables|Default|GetStaticMesh) false false)
        (Transformation|SetRelativeLocation _niagara "-0.631691, 0,20.000000" false false)
        (Audio|Components|Audio|Play _a_thud 0.0)
        (Utilities|FlowControl|Delay 1.0)
        (Transformation|SetRelativeLocation _niagara "-0.631691, 0,10.000000" false false)))
    (elif (== OtherComp (Variables|Default|GetBox3))
      (Utilities|FlowControl|DoOnce false
        (:Completed
          (Rendering|SetVisibility (Variables|Default|GetStaticMesh1) false false)
          (Audio|Components|Audio|Play _a_thud 0.0))))))

(event OnComponentEndOverlap(Box2)
  (params (OverlappedComponent :type Primitive%20Component%20Object%20Reference) (OtherActor :type Actor%20Object%20Reference) (OtherComp :type Primitive%20Component%20Object%20Reference) (OtherBodyIndex :type Integer))
  (bind _a_thud (Variables|Default|GetA_Thud))
  (bind _niagara (Variables|Default|GetNiagara))
  (if (== OtherComp (Variables|Default|GetBox))
    (Utilities|FlowControl|DoOnce false) ; enters at Reset
    (elif (== OtherComp (Variables|Default|GetBox3))
      (Utilities|FlowControl|DoOnce false) ; enters at Reset
    )))

(event OnGrabbed(GrabComponent)
  (bind _followcube (Variables|Default|GetFollowCube))
  (bind _relativelocation (Variables|/Script/Engine.SceneComponent|GetRelativeLocation _followcube))
  (Audio|Components|Audio|Play (Variables|Default|GetboilerDoorOpen_Cue) 0.0)
  (Utilities|FlowControl|Sequence
    (:then_0
      (Timeline|Timeline_4 PlayFromStart
        (:Update
          (Transformation|SetWorldTransform (Variables|Default|GetFollowCube) (Transformation|GetWorldTransform (Variables|Default|GetGrabCube)) false false))))
    (:then_1
      (Timeline|Timeline_5 PlayFromStart
        (:Update
          (bind _output_get (Variables|Default|SetDoorRotVal (Math|Float|Clamp(Float) (+ (* -1 (.pitch (Math|Rotator|FindLookatRotation (Math|Vector|MakeVector -1.0 22.499453 42.88472) (Math|Vector|MakeVector -1.0 (.y _relativelocation) (.z _relativelocation))))) -9e+01) -1.3e+02 0.0)))
          (Transformation|SetRelativeRotation (Variables|Default|GetBoilerDoor) (Math|Rotator|MakeRotator _output_get 0.0 0.0) false false))))))

(event OnDropped(GrabComponent)
  (bind _followcube (Variables|Default|GetFollowCube))
  (bind _boilerdoor (Variables|Default|GetBoilerDoor))
  (bind _p5 (Variables|Default|Getp5))
  (bind _grabcube (Variables|Default|GetGrabCube))
  (bind _relativelocation (Variables|/Script/Engine.SceneComponent|GetRelativeLocation _followcube))
  (Audio|Components|Audio|Play (Variables|Default|GetboilerDoorClose_Cue) 0.0)
  (Physics|SetSimulatePhysics _grabcube false)
  (Utilities|FlowControl|Sequence
    (:then_0
      (bind _newtrack_0 (Timeline|Timeline_6 PlayFromStart)
        (:Update
          (bind _output_get (Variables|Default|SetDoorRotVal (Math|Float|Lerp (.roll (Variables|/Script/Engine.SceneComponent|GetRelativeRotation _boilerdoor)) 0.0 _newtrack_0)))
          (Transformation|SetRelativeRotation _boilerdoor (Math|Rotator|MakeRotator _output_get 0.0 0.0) false false)
          (Transformation|SetRelativeLocation (Variables|Default|GetFollowCube) (Variables|/Script/Engine.SceneComponent|GetRelativeLocation _p5) false false)
          (Transformation|SetWorldLocation _grabcube (Transformation|GetWorldLocation _p5) false true)
          (Transformation|SetWorldRotation _grabcube (Transformation|GetWorldRotation _p5) false false))))
    (:then_1
      (Timeline|Timeline_5 Stop
        (:Update
          (bind _output_get_2 (Variables|Default|SetDoorRotVal (Math|Float|Clamp(Float) (+ (* -1 (.pitch (Math|Rotator|FindLookatRotation (Math|Vector|MakeVector -1.0 22.499453 42.88472) (Math|Vector|MakeVector -1.0 (.y _relativelocation) (.z _relativelocation))))) -9e+01) -1.3e+02 0.0)))
          (Transformation|SetRelativeRotation (Variables|Default|GetBoilerDoor) (Math|Rotator|MakeRotator _output_get_2 0.0 0.0) false false))))
    (:then_2
      (Timeline|Timeline_4 Stop
        (:Update
          (Transformation|SetWorldTransform (Variables|Default|GetFollowCube) (Transformation|GetWorldTransform (Variables|Default|GetGrabCube)) false false))))))

(event Custom|ShovelsPlay
  (bind _newcaulref (Variables|Default|GetNewCaulRef))
  (Rendering|SetVisibility (Variables|Default|GetSM_Boiler_INDred2) false false)
  (Rendering|SetVisibility (Variables|Default|GetSM_Boiler_INDgreen2) true false)
  (Utilities|FlowControl|Sequence
    (:then_0
      (Variables|Default|SetShovelOn true)
      (Variables|/Game/Blueprints/Paintbrush/Paintrbsuh.Paintrbsuh_C|SetBoilPz_Conduit? (Variables|Default|GetBrushRef) true)
      (bind _newtrack_0 (Timeline|Timeline_0 Play)
        (:Update
          (Transformation|SetRelativeLocation (Variables|Default|GetSkeletalMesh) (Math|Vector|Lerp(Vector) "-165.450607,-1.280131,5.759066" "-65.000000,3.489098,7.000000" _newtrack_0) false false)
          (Transformation|SetRelativeRotation (Variables|Default|GetBoilerDoor1) (Math|Rotator|Lerp(Rotator) "0,90.000000,10.000000" "0,90.000000,-110.000000" _newtrack_0) false false)
          (Transformation|SetRelativeLocation (Variables|Default|GetSkeletalMesh1) (Math|Vector|Lerp(Vector) "-165.450607,-1.280131,5.759066" "-55.000000,3.489098,9.000000" _newtrack_0) false false))
        (:Finished
          (if (Variables|Default|GetWaterFlowing)
            (Transformation|SetRelativeLocation (Variables|Default|GetNiagara1) "-1.535403,-2.256087,73.982254" false false)
            (Variables|Default|SetBoilDone true)
            (Variables|/Game/Blueprints/Paintbrush/Paintrbsuh.Paintrbsuh_C|SetBoilPz_Complete? (Variables|Default|GetBrushRef) true)
            (Variables|/Game/Blueprints/PuzzleElements/BP_Cauldron.BP_Cauldron_C|SetBoilPuzzleDone _newcaulref true)
            (Default|BoilButtonActivate _newcaulref)
            (Utilities|FlowControl|Sequence
              (:then_0
                (bind _newtrack_0_2 (Timeline|Timeline_8 PlayFromStart)))
              (:then_1
                (bind _newtrack_0_3 (Timeline|Timeline_7 PlayFromStart)
                  (:Update
                    (Transformation|SetRelativeLocation (Variables|Default|GetBoilerBase) (Math|Vector|MakeVector (Math|Float|Lerp -1.639178 -0.938745 _newtrack_0_3) -0.370995 (Math|Float|Lerp 20.262554 2e+01 _newtrack_0_2)) false false))
                  (:Finished
                    (Utilities|SetSteams true))))
              (:then_2
                (Transformation|SetRelativeLocation (Variables|Default|GetNiagara12) "-2.065938,20.288607,55.096134" false false)
                (Default|CompleteBoiler (Variables|Default|GetBrushRef))
                (Audio|Components|Audio|Play (Variables|Default|GetBoilerCreak_Cue) 0.0))
              (:then_3
                (Audio|Components|Audio|Play (Variables|Default|GetA_Steam_Cue4) 0.0)))))))
    (:then_1
      (Utilities|FlowControl|Delay 5.0)
      (Audio|Components|Audio|Play (Variables|Default|GetA_Fire) 0.0))))

(event Custom|Pumpin
  (bind _newcaulref (Variables|Default|GetNewCaulRef))
  (bind _chainmoving_cue (Variables|Default|GetchainMoving_Cue))
  (Rendering|SetVisibility (Variables|Default|GetSM_Boiler_INDgreen) true false)
  (Rendering|SetVisibility (Variables|Default|GetSM_Boiler_INDred) false false)
  (Audio|Components|Audio|Play _chainmoving_cue 0.0)
  (Audio|Components|Audio|AdjustVolume _chainmoving_cue 1.0 1.0 "Linear" :!class /Script/Engine.AudioComponent)
  (Variables|Default|SetWaterFlowing true)
  (Variables|/Game/Blueprints/Paintbrush/Paintrbsuh.Paintrbsuh_C|SetBoilPz_WaterInBoiler? (Variables|Default|GetBrushRef) true)
  (Transformation|SetRelativeScale3D (Variables|Default|GetWaterFill) "0.105894,0.058199,0.001000")
  (Utilities|FlowControl|Sequence
    (:then_0
      (bind _newtrack_0 (Timeline|Timeline_1 Play)
        (:Update
          (Transformation|SetRelativeScale3D (Variables|Default|GetCube2) (Math|Vector|Lerp(Vector) "0.109982,0.080515,0.109982" "0.109982,0.037467,0.109982" _newtrack_0))
          (Transformation|SetRelativeLocation (Variables|Default|GetPump9) (Math|Vector|Lerp(Vector) "-277.578156,9.139264,12.707488" "-352.446442,9.139264,12.709663" _newtrack_0) false false))))
    (:then_1
      (bind _newtrack_0_2 (Timeline|Timeline_2 Play)
        (:Update
          (Transformation|SetRelativeRotation (Variables|Default|GetPump6) (Math|Rotator|Lerp(Rotator) "0, 0,90.000000" "0,360.000000,90.000000" _newtrack_0_2) false false)
          (Transformation|SetRelativeRotation (Variables|Default|GetPump5) (Math|Rotator|Lerp(Rotator) "0,360.000000,90.000000" "0,0.000000,90.000000" _newtrack_0_2) false false))))
    (:then_2
      (bind _newtrack_0_3 (Timeline|Timeline_3 PlayFromStart)
        (:Update
          (Transformation|SetRelativeScale3D (Variables|Default|GetWaterFill) (Math|Vector|Lerp(Vector) "0.105894,0.058199,-0.001000" "0.105894,0.058199,-0.004000" _newtrack_0_3)))
        (:Finished
          (if (not (Variables|Default|GetWaterFlowing))
            (Transformation|SetRelativeScale3D (Variables|Default|GetWaterFill) "0.001000,0.001000,0.001000")))))
    (:then_3
      (if (Variables|Default|GetShovelOn)
        (Transformation|SetRelativeLocation (Variables|Default|GetNiagara1) "-1.535403,-2.256087,73.982254" false false)
        (Variables|Default|SetBoilDone true)
        (Variables|/Game/Blueprints/Paintbrush/Paintrbsuh.Paintrbsuh_C|SetBoilPz_Complete? (Variables|Default|GetBrushRef) true)
        (Variables|/Game/Blueprints/PuzzleElements/BP_Cauldron.BP_Cauldron_C|SetBoilPuzzleDone _newcaulref true)
        (Default|BoilButtonActivate _newcaulref)
        (Utilities|FlowControl|Sequence
          (:then_0
            (bind _newtrack_0_4 (Timeline|Timeline_8 PlayFromStart)))
          (:then_1
            (bind _newtrack_0_5 (Timeline|Timeline_7 PlayFromStart)
              (:Update
                (Transformation|SetRelativeLocation (Variables|Default|GetBoilerBase) (Math|Vector|MakeVector (Math|Float|Lerp -1.639178 -0.938745 _newtrack_0_5) -0.370995 (Math|Float|Lerp 20.262554 2e+01 _newtrack_0_4)) false false))
              (:Finished
                (Utilities|SetSteams true))))
          (:then_2
            (Transformation|SetRelativeLocation (Variables|Default|GetNiagara12) "-2.065938,20.288607,55.096134" false false)
            (Default|CompleteBoiler (Variables|Default|GetBrushRef))
            (Audio|Components|Audio|Play (Variables|Default|GetBoilerCreak_Cue) 0.0))
          (:then_3
            (Audio|Components|Audio|Play (Variables|Default|GetA_Steam_Cue4) 0.0)))))))

(event Custom|StopPump
  (Rendering|SetVisibility (Variables|Default|GetSM_Boiler_INDgreen) false false)
  (Rendering|SetVisibility (Variables|Default|GetSM_Boiler_INDred) true false)
  (Utilities|FlowControl|Sequence
    (:then_0
      (Variables|Default|SetWaterFlowing false)
      (Variables|/Game/Blueprints/Paintbrush/Paintrbsuh.Paintrbsuh_C|SetBoilPz_WaterInBoiler? (Variables|Default|GetBrushRef) false)
      (Transformation|SetRelativeLocation (Variables|Default|GetNiagara1) "-1.533389,-2.256057,184.138062" false false)
      (Utilities|SetSteams false)
      (Utilities|FlowControl|Sequence
        (:then_0
          (bind _newtrack_0 (Timeline|Timeline_1 Stop)
            (:Update
              (Transformation|SetRelativeScale3D (Variables|Default|GetCube2) (Math|Vector|Lerp(Vector) "0.109982,0.080515,0.109982" "0.109982,0.037467,0.109982" _newtrack_0))
              (Transformation|SetRelativeLocation (Variables|Default|GetPump9) (Math|Vector|Lerp(Vector) "-277.578156,9.139264,12.707488" "-352.446442,9.139264,12.709663" _newtrack_0) false false))))
        (:then_1
          (bind _newtrack_0_2 (Timeline|Timeline_2 Stop)
            (:Update
              (Transformation|SetRelativeRotation (Variables|Default|GetPump6) (Math|Rotator|Lerp(Rotator) "0, 0,90.000000" "0,360.000000,90.000000" _newtrack_0_2) false false)
              (Transformation|SetRelativeRotation (Variables|Default|GetPump5) (Math|Rotator|Lerp(Rotator) "0,360.000000,90.000000" "0,0.000000,90.000000" _newtrack_0_2) false false))))
        (:then_2
          (bind _newtrack_0_3 (Timeline|Timeline_3 ReverseFromEnd)
            (:Update
              (Transformation|SetRelativeScale3D (Variables|Default|GetWaterFill) (Math|Vector|Lerp(Vector) "0.105894,0.058199,-0.001000" "0.105894,0.058199,-0.004000" _newtrack_0_3)))
            (:Finished
              (if (not (Variables|Default|GetWaterFlowing))
                (Transformation|SetRelativeScale3D (Variables|Default|GetWaterFill) "0.001000,0.001000,0.001000")))))))
    (:then_1
      (Audio|Components|Audio|AdjustVolume (Variables|Default|GetchainMoving_Cue) 1.0 0.0 "Linear" :!class /Script/Engine.AudioComponent))))

(event Custom|blop
  (Utilities|FlowControl|Delay 4.0)
  (CallFunction|StopPump)
  (Utilities|FlowControl|Delay 4.0)
  (CallFunction|Pumpin)
  (Utilities|FlowControl|Delay 4.0))

(event EventBeginPlay
  (Transformation|SetRelativeLocation (Variables|Default|GetSkeletalMesh) "-165.450607,-1.280131,5.759066" false false)
  (Transformation|SetRelativeLocation (Variables|Default|GetSkeletalMesh1) "-151.783646,-1.280192,5.759066" false false)
  (bind _returnvalue (Actor|GetActorOfClass "/Game/Blueprints/Paintbrush/Paintrbsuh.Paintrbsuh_C"))
  (Variables|Default|SetBrushRef _returnvalue)
  (bind _returnvalue_2 (Actor|GetActorOfClass "/Game/Blueprints/PuzzleElements/BP_Cauldron.BP_Cauldron_C"))
  (Variables|Default|SetNewCaulRef _returnvalue_2)
  (Transformation|SetRelativeScale3D (Variables|Default|GetWaterFill) "0.001000,0.001000,0.001000")
  (Transformation|SetRelativeLocation (Variables|Default|GetNiagara1) "-1.533389,-2.256057,184.138062" false false)
  (Utilities|SetSteams false))

(fn ConstructionScript)