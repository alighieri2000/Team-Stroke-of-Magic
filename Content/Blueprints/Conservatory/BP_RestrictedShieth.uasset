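; Restricted-area gate in the Conservatory, opened by a button that the VR pawn triggers by overlapping its box.
; The overlap plays a timeline that presses the button mesh down, with a delayed gate opening and paintbrush flag chained from its Update pin.
; OpenGates raises the centre mesh on one timeline and the two side meshes on a second, slightly delayed one.
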(event OnComponentBeginOverlap(Box)
  (params (OverlappedComponent :type Primitive%20Component%20Object%20Reference) (OtherActor :type Actor%20Object%20Reference) (OtherComp :type Primitive%20Component%20Object%20Reference) (OtherBodyIndex :type Integer) (bFromSweep :type Boolean) (SweepResult :type Hit%20Result%20Structure%20%28by%20ref%29))
  (if (== OtherActor (Variables|Default|GetVRRef))
    (bind _newtrack_0 (Timeline|Timeline_2 PlayFromStart)
      (:Update
        (Transformation|SetRelativeLocation (Variables|Default|GetStaticMesh43) (Math|Vector|Lerp(Vector) "0, 0,5.934679" "0, 0,3.600000" _newtrack_0) false false)
        (Utilities|FlowControl|Delay 2.0)
        (CallFunction|OpenGates)
        (Variables|/Game/Blueprints/Paintbrush/Paintrbsuh.Paintrbsuh_C|SetRestrictedAreaButtonPushed? (Variables|Default|GetpaintbrushRef) true)))))

(event Custom|OpenGates
  (Utilities|FlowControl|Sequence
    (:then_0
      (bind _newtrack_0 (Timeline|Timeline_0 PlayFromStart)
        (:Update
          (Transformation|SetRelativeLocation (Variables|Default|GetStaticMesh) (Math|Vector|MakeVector 0.0 0.0 (Math|Float|Lerp 0.0 3e+02 _newtrack_0)) false false))))
    (:then_1
      (Utilities|FlowControl|Delay 0.2)
      (bind _newtrack_0_2 (Timeline|Timeline_1 PlayFromStart)
        (:Update
          (Transformation|SetRelativeLocation (Variables|Default|GetStaticMesh1) (Math|Vector|MakeVector 0.0 293.036652 (Math|Float|Lerp 0.0 3e+02 _newtrack_0_2)) false false)
          (Transformation|SetRelativeLocation (Variables|Default|GetStaticMesh2) (Math|Vector|MakeVector 0.0 -277.416412 (Math|Float|Lerp 0.0 3e+02 _newtrack_0_2)) false false))))))

(event EventBeginPlay
  (bind _returnvalue (Actor|GetActorOfClass "/Game/Blueprints/VR_Character/BP_UpdatedVRPawn.BP_UpdatedVRPawn_C"))
  (Variables|Default|SetVRRef _returnvalue)
  (bind _returnvalue_2 (Actor|GetActorOfClass "/Game/Blueprints/Paintbrush/Paintrbsuh.Paintrbsuh_C"))
  (Variables|Default|SetpaintbrushRef _returnvalue_2))

(fn ConstructionScript)