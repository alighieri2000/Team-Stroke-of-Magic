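; Grabbable sliding piece in the Conservatory that connects to the conduit shelves, built on a parent slide Blueprint.
; When dropped past a threshold near the end of its travel, it snaps to the end, locks, breaks the grip and calls 1Connected on BP_Conduit_Shelves, found at BeginPlay.
; UnlockLeft sets the slide's maximum limit, and Finished locks grabbing.
; A roller sound plays while the piece is held.
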(event OnGrabbed(GrabComponent)
  (Audio|Components|Audio|Play (Variables|Default|GetRollers_Small_Cue) 0.0))

(event OnDropped(GrabComponent)
  (Audio|Components|Audio|Stop (Variables|Default|GetRollers_Small_Cue)))

(event Custom|UnlockLeft
  (Variables|Default|SetMaximum%20Limit 175.0))

(event Custom|Finished
  (Variables|Default|SetGrabLocked true))

(event EventBeginPlay
  (|CallParentFunction)
  (bind _returnvalue (Actor|GetActorOfClass "/Game/Blueprints/PuzzleElements/BP_Conduit_Shelves.BP_Conduit_Shelves_C"))
  (Variables|Default|SetConduitRef _returnvalue))

(event Collision|EventActorBeginOverlap
  (params (OtherActor :type Actor%20Object%20Reference)))

(event EventTick
  (params (DeltaSeconds :type Float%20%28single-precision%29)))

(event EventOnDropped
  (if (> (.x (Variables|Default|GetOut%20Vector)) 173.0)
    (Variables|Default|SetGrabLocked true)
    (Transformation|SetRelativeLocation (Variables|Default|GetRecieveTransform) (Math|Vector|MakeVector 175.0 0.0 0.0) false false)
    (CallFunction|BreakGrip)
    (Default|1Connected (Variables|Default|GetConduitRef))))

(fn ConstructionScript
  (|CallParentFunction))