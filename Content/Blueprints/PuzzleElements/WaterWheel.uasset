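; Water wheel puzzle element that animates a wheel and gear train with sound and switches a linked Conduit_Grinder.
; Starts running on BeginPlay; SetOn and SetOff toggle timeline-driven rotation, audio, grinder, mesh visibility and Niagara position.
; A grabbable valve cube drives a follower cube and a look-at-based ValveRotVal, then snaps back when dropped.
; ValveRotVal is unused here, SetOn and SetOff have no internal caller, and several disconnected valve-logic fragments remain.
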(event OnGrabbed(GrabComponent1)
  (bind _followcube (Variables|Default|GetFollowCube))
  (bind _valveturn_cue (Variables|Default|GetvalveTurn_Cue))
  (bind _relativelocation (Variables|/Script/Engine.SceneComponent|GetRelativeLocation _followcube))
  (bind _returnvalue (Math|Rotator|FindLookatRotation (Math|Vector|MakeVector -253.253464 421.898712 -24.533714) (Math|Vector|MakeVector (.x _relativelocation) 421.898712 (.z _relativelocation))))
  (Audio|Components|Audio|AdjustVolume _valveturn_cue 1.5 1.0 "Linear" :!class /Script/Engine.AudioComponent)
  (Audio|Components|Audio|Play _valveturn_cue 0.0)
  (Utilities|FlowControl|Sequence
    (:then_0
      (Timeline|Timeline_3 PlayFromStart
        (:Update
          (Transformation|SetWorldTransform (Variables|Default|GetFollowCube) (Transformation|GetWorldTransform (Variables|Default|GetGrabCube)) false false))))
    (:then_1
      (Timeline|Timeline_4 PlayFromStart
        (:Update
          (Variables|Default|SetValveRotVal (* (Math|Float|SelectFloat -1.0 1.0 (> (.yaw _returnvalue) 1.7e+02)) (+ (.pitch _returnvalue) -9e+01))))))))

(event OnDropped(GrabComponent1)
  (bind _followcube (Variables|Default|GetFollowCube))
  (bind _staticmesh (Variables|Default|GetStaticMesh))
  (bind _grabcube (Variables|Default|GetGrabCube))
  (bind _relativelocation (Variables|/Script/Engine.SceneComponent|GetRelativeLocation _followcube))
  (bind _returnvalue (Math|Rotator|FindLookatRotation (Math|Vector|MakeVector -253.253464 421.898712 -24.533714) (Math|Vector|MakeVector (.x _relativelocation) 421.898712 (.z _relativelocation))))
  (Audio|Components|Audio|AdjustVolume (Variables|Default|GetvalveTurn_Cue) 1.5 0.0 "Linear" :!class /Script/Engine.AudioComponent)
  (Utilities|FlowControl|Sequence
    (:then_0
      (Timeline|Timeline_3 Stop
        (:Update
          (Transformation|SetWorldTransform (Variables|Default|GetFollowCube) (Transformation|GetWorldTransform (Variables|Default|GetGrabCube)) false false))))
    (:then_1
      (Timeline|Timeline_4 Stop
        (:Update
          (Variables|Default|SetValveRotVal (* (Math|Float|SelectFloat -1.0 1.0 (> (.yaw _returnvalue) 1.7e+02)) (+ (.pitch _returnvalue) -9e+01))))))
    (:then_2
      (Transformation|SetRelativeLocation (Variables|Default|GetFollowCube) (Variables|/Script/Engine.SceneComponent|GetRelativeLocation _staticmesh) false false)
      (Physics|SetSimulatePhysics _grabcube false)
      (Transformation|SetWorldLocation _grabcube (Transformation|GetWorldLocation _staticmesh) false false)
      (Transformation|SetRelativeRotation _grabcube "0, 0, 0" false false))))

(event Custom|Start
  (Audio|Components|Audio|Play (Variables|Default|GetwaterWheel_Cue) 0.0)
  (Audio|Components|Audio|Play (Variables|Default|GetAC_Gear_Grinding) 0.0)
  (bind _newtrack_0 (Timeline|Timeline_1 Play)
    (:Update
      (Transformation|SetRelativeRotation (Variables|Default|GetWaterWheel) (Math|Rotator|MakeRotator 0.0 _newtrack_0 0.0) false false)
      (Transformation|SetRelativeRotation (Variables|Default|GetStaticMesh17) (Math|Rotator|MakeRotator 0.0 _newtrack_0 9e+01) false false)
      (Transformation|SetRelativeRotation (Variables|Default|GetStaticMesh16) (Math|Rotator|MakeRotator 0.0 (* -1 _newtrack_0) 0.0) false false)
      (Transformation|SetRelativeRotation (Variables|Default|GetStaticMesh18) (Math|Rotator|MakeRotator 0.0 (* -1 _newtrack_0) 9e+01) false false))))

(event Custom|Stop
  (Audio|Components|Audio|Stop (Variables|Default|GetwaterWheel_Cue))
  (Audio|Components|Audio|Stop (Variables|Default|GetAC_Gear_Grinding))
  (bind _newtrack_0 (Timeline|Timeline_1 Stop)
    (:Update
      (Transformation|SetRelativeRotation (Variables|Default|GetWaterWheel) (Math|Rotator|MakeRotator 0.0 _newtrack_0 0.0) false false)
      (Transformation|SetRelativeRotation (Variables|Default|GetStaticMesh17) (Math|Rotator|MakeRotator 0.0 _newtrack_0 9e+01) false false)
      (Transformation|SetRelativeRotation (Variables|Default|GetStaticMesh16) (Math|Rotator|MakeRotator 0.0 (* -1 _newtrack_0) 0.0) false false)
      (Transformation|SetRelativeRotation (Variables|Default|GetStaticMesh18) (Math|Rotator|MakeRotator 0.0 (* -1 _newtrack_0) 9e+01) false false))))

(event Custom|SetOn
  (Utilities|FlowControl|Sequence
    (:then_0
      (Audio|Components|Audio|Play (Variables|Default|GetAC_Water_Wheel) 0.0))
    (:then_1
      (Default|GrinderStart (Variables|Default|GetGrinderRef))
      (CallFunction|Start)
      (Rendering|SetVisibility (Variables|Default|GetStaticMesh10) true false)
      (Transformation|SetRelativeLocation (Variables|Default|GetNiagara) "-105.620712, 0,-96.219269" false false)
      (bind _newtrack_0 (Timeline|Timeline_0 ReverseFromEnd)))))

(event Custom|SetOff
  (Utilities|FlowControl|Sequence
    (:then_0
      (Audio|Components|Audio|Stop (Variables|Default|GetAC_Water_Wheel)))
    (:then_1
      (Default|GrinderStop (Variables|Default|GetGrinderRef))
      (CallFunction|Stop)
      (Rendering|SetVisibility (Variables|Default|GetStaticMesh10) false false)
      (Transformation|SetRelativeLocation (Variables|Default|GetNiagara) "-105.620712,-268.053864,-96.219269" false false)
      (bind _newtrack_0 (Timeline|Timeline_0 PlayFromStart)))))

(event EventBeginPlay
  (bind _returnvalue (Actor|GetActorOfClass "/Game/Blueprints/Paintbrush/Paintrbsuh.Paintrbsuh_C"))
  (Variables|Default|SetNewVar_1 _returnvalue)
  (bind _returnvalue_2 (Actor|GetActorOfClass "/Game/Blueprints/PuzzleElements/Conduit_Grinder.Conduit_Grinder_C"))
  (Variables|Default|SetGrinderRef _returnvalue_2)
  (Actor|GetActorOfClass "/Game/Blueprints/PuzzleElements/Bp_SpiceTransport.Bp_SpiceTransport_C")
  (CallFunction|Start)
  (Transformation|SetWorldLocation (Variables|Default|GetGrabCube) (Transformation|GetWorldLocation (Variables|Default|GetStaticMesh)) false false)
  (Audio|Components|Audio|Play (Variables|Default|GetAC_Water_Wheel) 0.0))

(fn ConstructionScript)