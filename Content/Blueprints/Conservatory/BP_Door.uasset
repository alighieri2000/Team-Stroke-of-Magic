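; BP_Door is a grabbable door or similar interactable that either slides or rotates, based on its InteractType.
; On BeginPlay it spawns and attaches a BP_FollowHandle configured from the hitbox and axis settings.
; While grabbed, a timeline drives the handle's FollowCube from the Hitbox and applies the handle's resulting move or rotation value to RecieveTransform.
; Release stops the timeline, disables Hitbox physics and snaps it back to its stored relative transform.
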(event OnGrabbed(GrabComponent)
  (bind _recievetransform (Variables|Default|GetRecieveTransform))
  (bind _hitbox_ (Variables|Default|GetHitbox_))
  (bind _rotation_relative_to_hitbox (Variables|Default|GetRotation%20Relative%20To%20Hitbox))
  (bind _follow_handle_ref (Variables|Default|GetFollow%20Handle%20Ref))
  (bind _returnvalue (Transformation|GetWorldRotation _hitbox_))
  (bind _returnvalue_2 (Transformation|GetWorldLocation _hitbox_))
  (bind _followcube (Variables|/Game/Blueprints/Conservatory/BP_FollowHandle.BP_FollowHandle_C|GetFollowCube _follow_handle_ref))
  (Utilities|FlowControl|Sequence
    (:then_0
      (Default|Grabbed _follow_handle_ref))
    (:then_1
      (Timeline|Timeline_0 PlayFromStart
        (:Update
          (switch Utilities|FlowControl|Switch|SwitchonFollowHandleEnum (Variables|Default|GetInteract%20Type)
            (:NewEnumerator0
              (if _rotation_relative_to_hitbox
                (Transformation|SetWorldRotation _followcube _returnvalue false false)
                (else
                  (Transformation|SetWorldLocation _followcube _returnvalue_2 false false)))
              (Transformation|SetRelativeLocation _recievetransform (Variables|/Game/Blueprints/Conservatory/BP_FollowHandle.BP_FollowHandle_C|GetMove%20Val _follow_handle_ref) false false))
            (:NewEnumerator1
              (if _rotation_relative_to_hitbox
                (Transformation|SetWorldRotation _followcube _returnvalue false false)
                (else
                  (Transformation|SetWorldLocation _followcube _returnvalue_2 false false)))
              (Transformation|SetRelativeRotation _recievetransform (Variables|/Game/Blueprints/Conservatory/BP_FollowHandle.BP_FollowHandle_C|GetRotVal _follow_handle_ref) false false))))))))

(event OnDropped(GrabComponent)
  (bind _recievetransform (Variables|Default|GetRecieveTransform))
  (bind _hitbox_ (Variables|Default|GetHitbox_))
  (bind _hitbox__2 (Variables|Default|GetHitbox_))
  (bind _rotation_relative_to_hitbox (Variables|Default|GetRotation%20Relative%20To%20Hitbox))
  (bind _follow_handle_ref (Variables|Default|GetFollow%20Handle%20Ref))
  (bind _returnvalue (Transformation|GetWorldRotation _hitbox_))
  (bind _returnvalue_2 (Transformation|GetWorldLocation _hitbox_))
  (bind _followcube (Variables|/Game/Blueprints/Conservatory/BP_FollowHandle.BP_FollowHandle_C|GetFollowCube _follow_handle_ref))
  (Physics|SetSimulatePhysics _hitbox__2 false)
  (Transformation|SetRelativeTransform _hitbox__2 (Variables|/Game/Blueprints/Conservatory/BP_FollowHandle.BP_FollowHandle_C|GetHitBox%20Relative%20Transform (Variables|Default|GetFollow%20Handle%20Ref)) false false)
  (Utilities|FlowControl|Sequence
    (:then_0
      (Default|Dropped _follow_handle_ref))
    (:then_1
      (Timeline|Timeline_0 Stop
        (:Update
          (switch Utilities|FlowControl|Switch|SwitchonFollowHandleEnum (Variables|Default|GetInteract%20Type)
            (:NewEnumerator0
              (if _rotation_relative_to_hitbox
                (Transformation|SetWorldRotation _followcube _returnvalue false false)
                (else
                  (Transformation|SetWorldLocation _followcube _returnvalue_2 false false)))
              (Transformation|SetRelativeLocation _recievetransform (Variables|/Game/Blueprints/Conservatory/BP_FollowHandle.BP_FollowHandle_C|GetMove%20Val _follow_handle_ref) false false))
            (:NewEnumerator1
              (if _rotation_relative_to_hitbox
                (Transformation|SetWorldRotation _followcube _returnvalue false false)
                (else
                  (Transformation|SetWorldLocation _followcube _returnvalue_2 false false)))
              (Transformation|SetRelativeRotation _recievetransform (Variables|/Game/Blueprints/Conservatory/BP_FollowHandle.BP_FollowHandle_C|GetRotVal _follow_handle_ref) false false))))))))

(event Custom|Break
  (bind _recievetransform (Variables|Default|GetRecieveTransform))
  (bind _hitbox_ (Variables|Default|GetHitbox_))
  (bind _hitbox__2 (Variables|Default|GetHitbox_))
  (bind _rotation_relative_to_hitbox (Variables|Default|GetRotation%20Relative%20To%20Hitbox))
  (bind _follow_handle_ref (Variables|Default|GetFollow%20Handle%20Ref))
  (bind _returnvalue (Transformation|GetWorldRotation _hitbox_))
  (bind _returnvalue_2 (Transformation|GetWorldLocation _hitbox_))
  (bind _followcube (Variables|/Game/Blueprints/Conservatory/BP_FollowHandle.BP_FollowHandle_C|GetFollowCube _follow_handle_ref))
  (Physics|SetSimulatePhysics _hitbox__2 false)
  (Transformation|SetRelativeTransform _hitbox__2 (Variables|/Game/Blueprints/Conservatory/BP_FollowHandle.BP_FollowHandle_C|GetHitBox%20Relative%20Transform (Variables|Default|GetFollow%20Handle%20Ref)) false false)
  (Utilities|FlowControl|Sequence
    (:then_0
      (Default|Dropped _follow_handle_ref))
    (:then_1
      (Timeline|Timeline_0 Stop
        (:Update
          (switch Utilities|FlowControl|Switch|SwitchonFollowHandleEnum (Variables|Default|GetInteract%20Type)
            (:NewEnumerator0
              (if _rotation_relative_to_hitbox
                (Transformation|SetWorldRotation _followcube _returnvalue false false)
                (else
                  (Transformation|SetWorldLocation _followcube _returnvalue_2 false false)))
              (Transformation|SetRelativeLocation _recievetransform (Variables|/Game/Blueprints/Conservatory/BP_FollowHandle.BP_FollowHandle_C|GetMove%20Val _follow_handle_ref) false false))
            (:NewEnumerator1
              (if _rotation_relative_to_hitbox
                (Transformation|SetWorldRotation _followcube _returnvalue false false)
                (else
                  (Transformation|SetWorldLocation _followcube _returnvalue_2 false false)))
              (Transformation|SetRelativeRotation _recievetransform (Variables|/Game/Blueprints/Conservatory/BP_FollowHandle.BP_FollowHandle_C|GetRotVal _follow_handle_ref) false false))))))))

(event EventBeginPlay
  (bind _hitbox_ (Variables|Default|GetHitbox_))
  (bind _returnvalue (Game|SpawnActorfromClass "/Game/Blueprints/Conservatory/BP_FollowHandle.BP_FollowHandle_C" (Transformation|GetRelativeTransform (Variables|Default|GetRotPoint)) "AlwaysSpawn" 0 (Variables|Default|GetInteract%20Type) (Variables|Default|GetXYZ%20Direction) (Transformation|GetRelativeTransform _hitbox_) (Variables|/Script/Engine.StaticMeshComponent|GetStaticMesh _hitbox_) 0.0 3.6e+02 false true (Variables|Default|GetRotation%20Relative%20To%20Hitbox) 0))
  (bind _output_get (Variables|Default|SetFollow%20Handle%20Ref _returnvalue))
  (Transformation|AttachActorToActor _output_get self "None" "KeepRelative" "KeepRelative" "KeepRelative" true)
  (Utilities|FlowControl|Delay 0.2)
  (CallFunction|Break))

(fn ConstructionScript)