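; Restricted gate in the library puzzle that unlocks when the BP_LibraryKey actor enters its trigger box.
; On BeginPlay it caches the first key and Paintrbsuh actors found.
; The overlap kills the key, reveals its own Key mesh, plays a rattle cue and chains timelines to insert and turn it.
; Three further timelines then move the lock, Cube and sliding mesh together, and the slide's completion sets RestrictedGateUnlocked on the paintbrush.
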(event OnComponentBeginOverlap(Box)
  (params (OverlappedComponent :type Primitive%20Component%20Object%20Reference) (OtherActor :type Actor%20Object%20Reference) (OtherComp :type Primitive%20Component%20Object%20Reference) (OtherBodyIndex :type Integer) (bFromSweep :type Boolean) (SweepResult :type Hit%20Result%20Structure%20%28by%20ref%29))
  (bind _keyref (Variables|Default|GetKeyRef))
  (bind _key (Variables|Default|GetKey))
  (if (== OtherActor _keyref)
    (Default|Kill _keyref)
    (Rendering|SetVisibility (Variables|Default|GetKey) true false)
    (Audio|Components|Audio|Play (Variables|Default|GetCageRattle_Cue) 0.0)
    (bind _newtrack_0 (Timeline|Timeline_0 Play)
      (:Update
        (Transformation|SetRelativeLocation _key (Math|Vector|Lerp(Vector) "0, 0,68.000000" "0, 0,22.000000" _newtrack_0) false false))
      (:Finished
        (bind _newtrack_0_2 (Timeline|Timeline_1 PlayFromStart)
          (:Update
            (Transformation|SetRelativeRotation _key (Math|Rotator|Lerp(Rotator) "0,-90.000000,90.000000" "0,-180.000000,90.000000" _newtrack_0_2) false false))
          (:Finished
            (Utilities|FlowControl|Sequence
              (:then_0
                (bind _newtrack_0_3 (Timeline|Timeline_2 PlayFromStart)
                  (:Update
                    (Transformation|SetRelativeLocation (Variables|Default|GetLock1) (Math|Vector|Lerp(Vector) "0,23.031660, 0" "0,33.238327, 0" _newtrack_0_3) false false))))
              (:then_1
                (bind _newtrack_0_4 (Timeline|Timeline_3 PlayFromStart)
                  (:Update
                    (Transformation|SetRelativeRotation (Variables|Default|GetCube) (Math|Rotator|Lerp(Rotator) "0, 0,-30.000000" "-34.000000,23.000000,-34.000000" _newtrack_0_4) false false))))
              (:then_2
                (bind _newtrack_0_5 (Timeline|Timeline_4 PlayFromStart)
                  (:Update
                    (Transformation|SetRelativeLocation (Variables|Default|GetStaticMesh) (Math|Vector|Lerp(Vector) "-2.473274, 0,-10.000000" "122.566895, 0,-10.000000" _newtrack_0_5) false false))
                  (:Finished
                    (Variables|/Game/Blueprints/Paintbrush/Paintrbsuh.Paintrbsuh_C|SetRestrictedGateUnlocked? (Variables|Default|GetpaintbrushRef) true)))))))))))

(event EventBeginPlay
  (bind _returnvalue (Actor|GetActorOfClass "/Game/Blueprints/Library_Puzzle_Elements/BP_LibraryKey.BP_LibraryKey_C"))
  (Variables|Default|SetKeyRef _returnvalue)
  (bind _returnvalue_2 (Actor|GetActorOfClass "/Game/Blueprints/Paintbrush/Paintrbsuh.Paintrbsuh_C"))
  (Variables|Default|SetpaintbrushRef _returnvalue_2))

(event Collision|EventActorBeginOverlap
  (params (OtherActor :type Actor%20Object%20Reference)))

(event EventTick
  (params (DeltaSeconds :type Float%20%28single-precision%29)))

(fn ConstructionScript)