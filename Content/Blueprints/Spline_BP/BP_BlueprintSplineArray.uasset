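; Spline tool actor that fills a spline with child actors of a chosen class at construction time.
; The construction script steps along the spline by Spacing, adding a child actor component at each point with a base transform offset.
; Optional surface projection line-traces for height and sets only location; otherwise rotation (derived from the location vector) and scale also apply.
; Random-stream variation is wired in, but its range is zero.
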(event EventBeginPlay)

(event Collision|EventActorBeginOverlap
  (params (OtherActor :type Actor%20Object%20Reference)))

(event EventTick
  (params (DeltaSeconds :type Float%20%28single-precision%29)))

(fn ConstructionScript
  (bind _spline (Variables|Components|GetSpline))
  (bind _base_instance_transform (Variables|Default|GetBase%20Instance%20Transform))
  (bind _base_instance_transform_2 (Variables|Default|GetBase%20Instance%20Transform))
  (Variables|Default|GetActor%20Class
    (:then
      ;[1 1 1] While Loop
      (while (<= (LocalVariables|GetNextDistance) (Spline|GetSplineLength (Variables|Components|GetSpline)))
        (LocalVariables|SetRandomStreamNumber (Math|Random|RandomFloatinRangefromStream 0.0 0.0 (Variables|Default|GetRandomStream)))
        ;[1 1 1] Branch to Switch
        (if (Variables|Default|GetProject%20to%20Surface)
          ;[1 1 1] Project to surface
          (bind _outhit (Collision|LineTraceByChannel (+ (+ (Spline|GetLocationatDistanceAlongSpline _spline (LocalVariables|GetNextDistance) "World") (.location _base_instance_transform_2) (* (.location _base_instance_transform) (LocalVariables|GetRandomStreamNumber))) "0, 0,250.000000") (+ (+ (Spline|GetLocationatDistanceAlongSpline _spline (LocalVariables|GetNextDistance) "World") (.location _base_instance_transform_2) (* (.location _base_instance_transform) (LocalVariables|GetRandomStreamNumber))) "0, 0,-500.000000") "TraceTypeQuery1" true 0 "None"))
          (bind _returnvalue (AddComponent|AddChildActorComponent false (Math|Transform|MakeTransform (Math|Vector|MakeVector (.X (Math|Vector|BreakVector (+ (Spline|GetLocationatDistanceAlongSpline _spline (LocalVariables|GetNextDistance) "World") (.location _base_instance_transform_2) (* (.location _base_instance_transform) (LocalVariables|GetRandomStreamNumber))))) (.Y (Math|Vector|BreakVector (+ (Spline|GetLocationatDistanceAlongSpline _spline (LocalVariables|GetNextDistance) "World") (.location _base_instance_transform_2) (* (.location _base_instance_transform) (LocalVariables|GetRandomStreamNumber))))) (.Z (Math|Vector|BreakVector (.location _outhit)))) "0, 0, 0" "1,1,1")))
          (ChildActorComponent|SetChildActorClass _returnvalue (Variables|Default|GetActor%20Class))
          (else
            ;[1 1 1] Add Child Blueprint
            (bind _returnvalue_2 (AddComponent|AddChildActorComponent true (Math|Transform|MakeTransform (+ (Spline|GetLocationatDistanceAlongSpline _spline (LocalVariables|GetNextDistance) "World") (.location _base_instance_transform_2) (* (.location _base_instance_transform) (LocalVariables|GetRandomStreamNumber))) (Math|Rotator|CombineRotators (Math|Rotator|CombineRotators (Math|Conversions|RotationFromXVector (Spline|GetLocationatDistanceAlongSpline _spline (LocalVariables|GetNextDistance) "World")) (.rotation _base_instance_transform_2)) (* (.rotation _base_instance_transform) (LocalVariables|GetRandomStreamNumber))) (+ (.scale _base_instance_transform_2) (* (.scale _base_instance_transform) (LocalVariables|GetRandomStreamNumber))))))
            (ChildActorComponent|SetChildActorClass _returnvalue_2 (Variables|Default|GetActor%20Class))))
        (LocalVariables|SetNextDistance (+ (LocalVariables|GetNextDistance) (Variables|Default|GetSpacing)))))
    (:else)))