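; BP_Painting1 is a brush-tracing puzzle painting that reports a win to MagicThing.
; StartPower1 powers it, swapping a mesh to a pink material and rotating Cube1 by timeline.
; With power on, water off and paint 1 on the brush, entering Box1 starts a line, and leaving Box fails it.
; Reaching Box2 with the line intact rotates Cube2 and calls Win.
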(event OnComponentBeginOverlap(Box1)
  (params (OverlappedComponent :type Primitive%20Component%20Object%20Reference) (OtherActor :type Actor%20Object%20Reference) (OtherComp :type Primitive%20Component%20Object%20Reference) (OtherBodyIndex :type Integer) (bFromSweep :type Boolean) (SweepResult :type Hit%20Result%20Structure%20%28by%20ref%29))
  (if (== OtherActor (Variables|Default|GetbrushRef))
    (if (not (Variables|Default|GetWaterOn))
      (if (and (Variables|/Game/Blueprints/Paintbrush/Paintrbsuh.Paintrbsuh_C|GetPaint1_OnBrush (Variables|Default|GetbrushRef)) (Variables|Default|GetPowerOn))
        (Variables|Default|SetLineStarted true)
        (Development|PrintString "STARTED")))))

(event OnComponentEndOverlap(Box)
  (params (OverlappedComponent :type Primitive%20Component%20Object%20Reference) (OtherActor :type Actor%20Object%20Reference) (OtherComp :type Primitive%20Component%20Object%20Reference) (OtherBodyIndex :type Integer))
  (if (== OtherActor (Variables|Default|GetbrushRef))
    (Variables|Default|SetLineStarted false)
    (Development|PrintString "FAILED")))

(event OnComponentBeginOverlap(Box2)
  (params (OverlappedComponent :type Primitive%20Component%20Object%20Reference) (OtherActor :type Actor%20Object%20Reference) (OtherComp :type Primitive%20Component%20Object%20Reference) (OtherBodyIndex :type Integer) (bFromSweep :type Boolean) (SweepResult :type Hit%20Result%20Structure%20%28by%20ref%29))
  (if (== OtherActor (Variables|Default|GetbrushRef))
    (if (Variables|Default|GetLineStarted)
      (Utilities|FlowControl|Sequence
        (:then_0
          (bind _newtrack_0 (Timeline|Timeline_3 Play)
            (:Update
              (Transformation|SetRelativeRotation (Variables|Default|GetCube2) (Math|Rotator|MakeRotator 0.0 0.0 _newtrack_0) false false))))
        (:then_1
          (Default|Win (Variables|Default|GetMagicRef)))))))

(event Custom|StartPower1
  (Variables|Default|SetPowerOn true)
  (Rendering|Material|SetMaterial (Variables|Default|GetStaticMesh3) 0 "/Game/Import/Materials/Pink.Pink")
  (Utilities|FlowControl|Sequence
    (:then_1
      (bind _newtrack_0 (Timeline|Timeline_2 Play)
        (:Update
          (Transformation|SetRelativeRotation (Variables|Default|GetCube1) (Math|Rotator|MakeRotator 0.0 0.0 _newtrack_0) false false))))))

(event Custom|WaterTurnOn
  (Variables|Default|SetWaterOn true))

(event Custom|WaterturnOff
  (Variables|Default|SetWaterOn false))

(event EventBeginPlay
  (bind _returnvalue (Actor|GetActorOfClass "/Game/Blueprints/Paintbrush/Paintrbsuh.Paintrbsuh_C"))
  (Variables|Default|SetbrushRef _returnvalue)
  (bind _returnvalue_2 (Actor|GetActorOfClass "/Game/Blueprints/BP/MagicThing.MagicThing_C"))
  (Variables|Default|SetMagicRef _returnvalue_2))

(fn ConstructionScript)