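; BP_CrystalLight is a configurable floating crystal that bobs vertically while playing a sound.
; The construction script applies the chosen mesh, material and sound to its components.
; On BeginPlay it starts the audio and a timeline, with rate scaled by Duration and a randomized start time to vary the phase.
; The timeline track interpolates the crystal's relative Z between HowFarZ and zero.
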(event EventBeginPlay
  (bind _duration (Variables|Default|GetDuration))
  (bind _timeline_0 (Variables|Default|GetTimeline_0))
  (Audio|Components|Audio|Play (Variables|Default|GetGemstoneFloating_Cue) 0.0)
  (Components|Timeline|SetPlayRate _timeline_0 (Math|Float|SafeDivide 1.0 _duration))
  (Components|Timeline|SetNewTime _timeline_0 (Math|Float|Lerp 0.0 _duration (Math|Random|RandomFloat)))
  (bind _newtrack_0 (Timeline|Timeline_0 Play)
    (:Update
      (Transformation|SetRelativeTransform (Variables|Default|GetSM_Crystal) (Math|Transform|MakeTransform (Math|Vector|MakeVector 0.0 0.0 (Math|Float|Lerp (Variables|Default|GethowFarZ) 0.0 _newtrack_0)) "0, 0, 0" "1,1,1") false false))))

(fn ConstructionScript
  (bind _sm_crystal (Variables|Default|GetSM_Crystal))
  (Components|StaticMesh|SetStaticMesh _sm_crystal (Variables|Default|GetNew%20Mesh))
  (Rendering|Material|SetMaterial _sm_crystal 0 (Variables|Default|GetMaterial))
  (Audio|Components|Audio|SetSound (Variables|Default|GetGemstoneFloating_Cue) (Variables|Default|GetSoundBase)))