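; Grabbable sliding shelf in the Conservatory that plays a roller sound while held and can be shown or hidden.
; ShelfInt selects which slide surface it references at BeginPlay.
; Finished locks grabbing, unlocks that surface's left side and flags the shelf pushed, notifying the paintbrush only if both of this instance's pushed flags are true.
; An unconnected snap-into-place branch targeting the conduit shelves never runs.
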(event OnGrabbed(GrabComponent)
  (Audio|Components|Audio|Play (Variables|Default|GetRollers_Large_Cue) 0.0))

(event OnDropped(GrabComponent)
  (Audio|Components|Audio|Stop (Variables|Default|GetRollers_Large_Cue)))

(event Custom|HideShelves
  (Rendering|SetVisibility (Variables|Default|Getddddd) false true))

(event Custom|ShowShelves
  (Rendering|SetVisibility (Variables|Default|Getddddd) true true))

(event Custom|Finished
  (Variables|Default|SetGrabLocked true)
  (switch int (Variables|Default|GetShelfInt)
    (:1
      (Default|UnlockLeft (Variables|Default|GetSurfaceRef))
      (bind _output_get (Variables|Default|SetShelf1Pushed true)))
    (:2
      (Default|UnlockLeft (Variables|Default|GetSurface2Ref))
      (bind _output_get_2 (Variables|Default|SetShelf2Pushed true))))
  (if (and _output_get _output_get_2)
    (Variables|/Game/Blueprints/Paintbrush/Paintrbsuh.Paintrbsuh_C|SetshelvesPushedInPlace? (Variables|Default|GetpaintbrushRef) true)))

(event EventBeginPlay
  (|CallParentFunction)
  (bind _returnvalue (Actor|GetActorOfClass "/Game/Blueprints/Paintbrush/Paintrbsuh.Paintrbsuh_C"))
  (Variables|Default|SetpaintbrushRef _returnvalue)
  (bind _returnvalue_2 (Actor|GetActorOfClass "/Game/Blueprints/PuzzleElements/BP_Conduit_Shelves.BP_Conduit_Shelves_C"))
  (Variables|Default|SetShelfRef _returnvalue_2)
  (switch int (Variables|Default|GetShelfInt)
    (:1
      (bind _returnvalue_3 (Actor|GetActorOfClass "/Game/Blueprints/Conservatory/Slide_surface1.Slide_surface1_C"))
      (Variables|Default|SetSurfaceRef _returnvalue_3))
    (:2
      (bind _returnvalue_4 (Actor|GetActorOfClass "/Game/Blueprints/Conservatory/Slide_surface2.Slide_surface2_C"))
      (Variables|Default|SetSurface2Ref _returnvalue_4))))

(fn ConstructionScript
  (|CallParentFunction))