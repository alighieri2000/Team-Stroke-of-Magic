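; PuzzleWater is a toggleable water volume that unprimes the paintbrush when its sphere touches the water.
; It finds the Paintrbsuh actor on BeginPlay and calls SetUnprimed on cube overlap while WaterOn is true.
; WaterTurnOn shows the cube at full height instantly.
; WaterOff plays a timeline that lerps its Z scale nearly flat, then hides it and clears WaterOn.
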(event OnComponentBeginOverlap(Cube)
  (params (OverlappedComponent :type Primitive%20Component%20Object%20Reference) (OtherActor :type Actor%20Object%20Reference) (OtherComp :type Primitive%20Component%20Object%20Reference) (OtherBodyIndex :type Integer) (bFromSweep :type Boolean) (SweepResult :type Hit%20Result%20Structure%20%28by%20ref%29))
  (bind _brushref (Variables|Default|GetBrushRef))
  (if (== (Variables|/Game/Blueprints/Paintbrush/Paintrbsuh.Paintrbsuh_C|GetSphere _brushref) OtherComp)
    (if (Variables|Default|GetwaterOn)
      (Default|SetUnprimed _brushref))))

(event Custom|WaterOff
  (bind _newtrack_0 (Timeline|Timeline_0 Play)
    (:Update
      (Transformation|SetRelativeScale3D (Variables|Default|GetCube) (Math|Vector|Lerp(Vector) "0.528348,0.807484,0.167174" "0.528348,0.807484,0.010000" _newtrack_0)))
    (:Finished
      (Rendering|SetVisibility (Variables|Default|GetCube) false false)
      (Variables|Default|SetwaterOn false))))

(event Custom|WaterTurnOn
  (Transformation|SetRelativeScale3D (Variables|Default|GetCube) "0.528348,0.807484,0.167174")
  (Rendering|SetVisibility (Variables|Default|GetCube) true false)
  (Variables|Default|SetwaterOn true))

(event EventBeginPlay
  (bind _returnvalue (Actor|GetActorOfClass "/Game/Blueprints/Paintbrush/Paintrbsuh.Paintrbsuh_C"))
  (Variables|Default|SetBrushRef _returnvalue))

(fn ConstructionScript)