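; Interactables is a configurable physics prop Blueprint whose mesh and material are set through variables.
; The construction script applies WhichMesh and WhichMat to the StaticMesh component.
; BeginPlay enables physics simulation, gravity and query-and-physics collision, then sets WhichMat again by the slot name "None".
; No interaction logic is present in these graphs.
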(event EventBeginPlay
  (bind _staticmesh (Variables|Default|GetStaticMesh))
  (Physics|SetSimulatePhysics _staticmesh true)
  (Physics|SetEnableGravity _staticmesh true)
  (Collision|SetCollisionEnabled _staticmesh "QueryAndPhysics")
  (Rendering|Material|SetMaterialbyName _staticmesh "None" (Variables|Default|GetWhich%20Mat)))

(fn ConstructionScript
  (bind _staticmesh (Variables|Default|GetStaticMesh))
  (bind _output_get (Variables|Default|SetWhich%20Mesh (Variables|Default|GetWhich%20Mesh)))
  (bind _output_get_2 (Variables|Default|SetWhich%20Mat (Variables|Default|GetWhich%20Mat)))
  (Components|StaticMesh|SetStaticMesh _staticmesh _output_get)
  (Rendering|Material|SetMaterial _staticmesh 0 _output_get_2))