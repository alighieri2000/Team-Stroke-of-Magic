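; BP_LevelTransfer is a lockable door trigger that moves the VR player to another level, named by LevelName.
; UnlockDoor and LockDoor toggle IsUnlocked; unlocking also checks for pawns already inside the box.
; When BP_UpdatedVRPawn overlaps while unlocked, it triggers a fade to black, then after a delay opens the level and calls a fade to clear.
; Door and transfer sound logic is present but disconnected.
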(event OnComponentBeginOverlap(Box)
  (params (OverlappedComponent :type Primitive%20Component%20Object%20Reference) (OtherActor :type Actor%20Object%20Reference) (OtherComp :type Primitive%20Component%20Object%20Reference) (OtherBodyIndex :type Integer) (bFromSweep :type Boolean) (SweepResult :type Hit%20Result%20Structure%20%28by%20ref%29))
  (Utilities|Casting|CastToBP_UpdatedVRPawn OtherActor)
  (if (Variables|Default|GetIsUnlocked)
    (Utilities|FlowControl|Sequence
      (:then_0
        (bind _asbp_updated_vrpawn (Utilities|Casting|CastToBP_UpdatedVRPawnClass "/Game/Blueprints/VR_Character/BP_UpdatedVRPawn.BP_UpdatedVRPawn_C"))
        (bind _returnvalue (Actor|GetActorOfClass _asbp_updated_vrpawn))
        (Class|BPIScreenFade|FadetoBlack(Message) _returnvalue))
      (:then_1
        (Utilities|FlowControl|Delay 3.0)
        (Game|OpenLevel(byName) (Variables|Default|GetLevel%20Name)))
      (:then_2
        (Utilities|FlowControl|Delay 3.0)
        (bind _asbp_updated_vrpawn_2 (Utilities|Casting|CastToBP_UpdatedVRPawnClass "/Game/Blueprints/VR_Character/BP_UpdatedVRPawn.BP_UpdatedVRPawn_C"))
        (bind _returnvalue_2 (Actor|GetActorOfClass _asbp_updated_vrpawn_2))
        (Class|BPIScreenFade|FadetoClear(Message) _returnvalue_2)))))

(event EventBeginPlay)

(event Collision|EventActorBeginOverlap
  (params (OtherActor :type Actor%20Object%20Reference)))

(event EventTick
  (params (DeltaSeconds :type Float%20%28single-precision%29)))

(event EventUnlockDoor
  (Variables|Default|SetIsUnlocked true)
  (for _array_element (Collision|GetOverlappingActors (Variables|Default|GetBox) "/Game/Blueprints/VR_Character/BP_UpdatedVRPawn.BP_UpdatedVRPawn_C" :!class /Script/Engine.PrimitiveComponent)
    (Utilities|Casting|CastToBP_UpdatedVRPawn _array_element)
    (if (Variables|Default|GetIsUnlocked)
      (Utilities|FlowControl|Sequence
        (:then_0
          (bind _asbp_updated_vrpawn (Utilities|Casting|CastToBP_UpdatedVRPawnClass "/Game/Blueprints/VR_Character/BP_UpdatedVRPawn.BP_UpdatedVRPawn_C"))
          (bind _returnvalue (Actor|GetActorOfClass _asbp_updated_vrpawn))
          (Class|BPIScreenFade|FadetoBlack(Message) _returnvalue))
        (:then_1
          (Utilities|FlowControl|Delay 3.0)
          (Game|OpenLevel(byName) (Variables|Default|GetLevel%20Name)))
        (:then_2
          (Utilities|FlowControl|Delay 3.0)
          (bind _asbp_updated_vrpawn_2 (Utilities|Casting|CastToBP_UpdatedVRPawnClass "/Game/Blueprints/VR_Character/BP_UpdatedVRPawn.BP_UpdatedVRPawn_C"))
          (bind _returnvalue_2 (Actor|GetActorOfClass _asbp_updated_vrpawn_2))
          (Class|BPIScreenFade|FadetoClear(Message) _returnvalue_2))))))

(event EventLockDoor
  (Variables|Default|SetIsUnlocked false))

(fn ConstructionScript)