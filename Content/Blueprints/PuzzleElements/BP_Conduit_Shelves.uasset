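; Shelves conduit puzzle element that, when finished, opens a glass case and unlocks the fancy book.
; Two surface-connection events gate a Connected flag, though 2Connected sets its own flag false.
; Once connected, brush sphere overlap with SM_WeirdCollision starts the parent conduit logic, and leaving exits it.
; Finishing moves Part1 along a spline, then plays a sound and flattens PZ7 by timeline, unlocking the book after delay.
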(event OnComponentBeginOverlap(BrushBounds2)
  (params (OverlappedComponent :type Primitive%20Component%20Object%20Reference) (OtherActor :type Actor%20Object%20Reference) (OtherComp :type Primitive%20Component%20Object%20Reference) (OtherBodyIndex :type Integer) (bFromSweep :type Boolean) (SweepResult :type Hit%20Result%20Structure%20%28by%20ref%29)))

(event OnComponentEndOverlap(BrushBounds2)
  (params (OverlappedComponent :type Primitive%20Component%20Object%20Reference) (OtherActor :type Actor%20Object%20Reference) (OtherComp :type Primitive%20Component%20Object%20Reference) (OtherBodyIndex :type Integer)))

(event OnComponentBeginOverlap(SM_WeirdCollision)
  (params (OverlappedComponent :type Primitive%20Component%20Object%20Reference) (OtherActor :type Actor%20Object%20Reference) (OtherComp :type Primitive%20Component%20Object%20Reference) (OtherBodyIndex :type Integer) (bFromSweep :type Boolean) (SweepResult :type Hit%20Result%20Structure%20%28by%20ref%29))
  (if (== OtherComp (Variables|/Game/Blueprints/Paintbrush/Paintrbsuh.Paintrbsuh_C|GetCollisionSphere (Variables|Default|GetBrushRefVar)))
    (if (Variables|Default|GetConnected)
      (CallFunction|ParentBegin)
      (Development|PrintString "XXXXXXXXXXXXXXXXXX" true true "(R=1.000000,G=0.000000,B=0.649016,A=1.000000)"))))

(event OnComponentBeginOverlap(Box)
  (params (OverlappedComponent :type Primitive%20Component%20Object%20Reference) (OtherActor :type Actor%20Object%20Reference) (OtherComp :type Primitive%20Component%20Object%20Reference) (OtherBodyIndex :type Integer) (bFromSweep :type Boolean) (SweepResult :type Hit%20Result%20Structure%20%28by%20ref%29)))

(event OnComponentEndOverlap(SM_WeirdCollision)
  (params (OverlappedComponent :type Primitive%20Component%20Object%20Reference) (OtherActor :type Actor%20Object%20Reference) (OtherComp :type Primitive%20Component%20Object%20Reference) (OtherBodyIndex :type Integer))
  (if (== OtherComp (Variables|/Game/Blueprints/Paintbrush/Paintrbsuh.Paintrbsuh_C|GetCollisionSphere (Variables|Default|GetBrushRefVar)))
    (CallFunction|ExitedParent)))

(event Custom|2Connected
  (Variables|Default|SetSurf2Connected false)
  (if (Variables|Default|GetSurf1Connected)
    (bind _output_get (Variables|Default|SetConnected true))
    (Development|PrintString (Utilities|String|ToString(Boolean) _output_get))))

(event Custom|1Connected
  (Variables|Default|SetSurf1Connected true)
  (if (Variables|Default|GetSurf2Connected)
    (bind _output_get (Variables|Default|SetConnected true))
    (Development|PrintString (Utilities|String|ToString(Boolean) _output_get))))

(event Custom|D01
  (params (Condition :type Boolean))
  (bind _spline (Variables|Default|GetSpline))
  (Utilities|FlowControl|Sequence
    (:then_0
      (bind _newtrack_0 (Timeline|Timeline_0 Play)
        (:Update
          (Transformation|SetWorldLocation (Variables|Default|GetPart1) (Spline|GetLocationatDistanceAlongSpline _spline (Math|Float|Lerp 0.0 (Spline|GetSplineLength _spline) _newtrack_0) "World") false false))))
    (:then_1
      (Utilities|FlowControl|Delay 2.0)
      (Audio|Components|Audio|Play (Variables|Default|GetGlassCaseOpening_Cue) 0.0)
      (bind _newtrack_0_2 (Timeline|Timeline_1 PlayFromStart)
        (:Update
          (Transformation|SetRelativeScale3D (Variables|Default|GetPZ7) (Math|Vector|Lerp(Vector) "0.053550,0.053550,0.053550" "0.053550,0.053550,0.001000" _newtrack_0_2)))))))

(event EventBeginPlay
  (|CallParentFunction)
  (CallFunction|PoweredUp)
  (bind _returnvalue (Actor|GetActorOfClass "/Game/Blueprints/Conservatory/Slide_surface1.Slide_surface1_C"))
  (Variables|Default|SetSurfRef1 _returnvalue)
  (bind _returnvalue_2 (Actor|GetActorOfClass "/Game/Blueprints/Conservatory/Slide_surface2.Slide_surface2_C"))
  (Variables|Default|SetSurfRef2 _returnvalue_2)
  (bind _returnvalue_3 (Actor|GetActorOfClass "/Game/Blueprints/BP/BP_FancyBook.BP_FancyBook_C"))
  (Variables|Default|SetFancyBookRef _returnvalue_3))

(event EventFinished
  (CallFunction|D01 false)
  (Utilities|FlowControl|Delay 2.0)
  (Default|Unlcok (Variables|Default|GetFancyBookRef)))

(fn ConstructionScript
  (|CallParentFunction))