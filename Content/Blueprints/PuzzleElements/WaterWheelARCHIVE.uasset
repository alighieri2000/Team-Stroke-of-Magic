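; Water wheel puzzle actor that drives a Conduit_Grinder and can be switched off and on by rotating a grabbable piece.
; It starts running on BeginPlay, with Timeline_1 spinning the wheel and counter-rotating gear meshes.
; Timeline_2 polls Piece2's pitch until the grab is dropped.
; Each 90-degree change from the stored pitch flip-flops the wheel, grinder, audio, mesh visibility and Niagara position.
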(event OnGrabbed(GrabComponent1)
  (bind _ac_pipe_wheel (Variables|Default|GetAC_Pipe_Wheel))
  (bind _grinderref (Variables|Default|GetGrinderRef))
  (Variables|Default|SetRelative%20Rotation%20Y%20%28Pitch%29 (.pitch (Variables|/Script/Engine.SceneComponent|GetRelativeRotation (Variables|Default|GetPiece2))))
  (Timeline|Timeline_2 PlayFromStart
    (:Update
      (if (>= (Math|Float|Absolute(Float) (- (.pitch (Variables|/Script/Engine.SceneComponent|GetRelativeRotation (Variables|Default|GetPiece2))) (Variables|Default|GetRelative%20Rotation%20Y%20%28Pitch%29))) 9e+01)
        (Utilities|FlowControl|DoOnce false :!label _label
          (:Completed
            (Variables|Default|SetRelative%20Rotation%20Y%20%28Pitch%29 (.pitch (Variables|/Script/Engine.SceneComponent|GetRelativeRotation (Variables|Default|GetPiece2))))
            (Utilities|FlowControl|FlipFlop
              (:A
                (Utilities|FlowControl|Sequence
                  (:then_0
                    (Audio|Components|Audio|Stop (Variables|Default|GetAC_Pipe_Wheel))
                    (Audio|Components|Audio|Stop (Variables|Default|GetAC_Water_Wheel)))
                  (:then_1
                    (Default|GrinderStop _grinderref)
                    (CallFunction|Stop)
                    (Rendering|SetVisibility (Variables|Default|GetStaticMesh10) false false)
                    (Transformation|SetRelativeLocation (Variables|Default|GetNiagara) "-105.620712,-268.053864,-96.219269" false false)
                    (bind _newtrack_0 (Timeline|Timeline_0 PlayFromStart)))))
              (:B
                (Utilities|FlowControl|Sequence
                  (:then_0
                    (Audio|Components|Audio|Play _ac_pipe_wheel 0.0)
                    (Audio|Components|Audio|StopDelayed _ac_pipe_wheel 1.3)
                    (Audio|Components|Audio|Play (Variables|Default|GetAC_Water_Wheel) 0.0))
                  (:then_1
                    (Default|GrinderStart _grinderref)
                    (CallFunction|Start)
                    (Rendering|SetVisibility (Variables|Default|GetStaticMesh10) true false)
                    (Transformation|SetRelativeLocation (Variables|Default|GetNiagara) "-105.620712, 0,-96.219269" false false)
                    (Timeline|Timeline_0 ReverseFromEnd)))))))
        (else
          (goto _label Reset))))))

(event OnDropped(GrabComponent1)
  (bind _ac_pipe_wheel (Variables|Default|GetAC_Pipe_Wheel))
  (bind _grinderref (Variables|Default|GetGrinderRef))
  (Timeline|Timeline_2 Stop
    (:Update
      (if (>= (Math|Float|Absolute(Float) (- (.pitch (Variables|/Script/Engine.SceneComponent|GetRelativeRotation (Variables|Default|GetPiece2))) (Variables|Default|GetRelative%20Rotation%20Y%20%28Pitch%29))) 9e+01)
        (Utilities|FlowControl|DoOnce false :!label _label
          (:Completed
            (Variables|Default|SetRelative%20Rotation%20Y%20%28Pitch%29 (.pitch (Variables|/Script/Engine.SceneComponent|GetRelativeRotation (Variables|Default|GetPiece2))))
            (Utilities|FlowControl|FlipFlop
              (:A
                (Utilities|FlowControl|Sequence
                  (:then_0
                    (Audio|Components|Audio|Stop (Variables|Default|GetAC_Pipe_Wheel))
                    (Audio|Components|Audio|Stop (Variables|Default|GetAC_Water_Wheel)))
                  (:then_1
                    (Default|GrinderStop _grinderref)
                    (CallFunction|Stop)
                    (Rendering|SetVisibility (Variables|Default|GetStaticMesh10) false false)
                    (Transformation|SetRelativeLocation (Variables|Default|GetNiagara) "-105.620712,-268.053864,-96.219269" false false)
                    (bind _newtrack_0 (Timeline|Timeline_0 PlayFromStart)))))
              (:B
                (Utilities|FlowControl|Sequence
                  (:then_0
                    (Audio|Components|Audio|Play _ac_pipe_wheel 0.0)
                    (Audio|Components|Audio|StopDelayed _ac_pipe_wheel 1.3)
                    (Audio|Components|Audio|Play (Variables|Default|GetAC_Water_Wheel) 0.0))
                  (:then_1
                    (Default|GrinderStart _grinderref)
                    (CallFunction|Start)
                    (Rendering|SetVisibility (Variables|Default|GetStaticMesh10) true false)
                    (Transformation|SetRelativeLocation (Variables|Default|GetNiagara) "-105.620712, 0,-96.219269" false false)
                    (Timeline|Timeline_0 ReverseFromEnd)))))))
        (else
          (goto _label Reset))))))

(event Custom|Start
  (Audio|Components|Audio|Play (Variables|Default|GetAC_Gear_Grinding) 0.0)
  (bind _newtrack_0 (Timeline|Timeline_1 Play)
    (:Update
      (Transformation|SetRelativeRotation (Variables|Default|GetWaterWheel) (Math|Rotator|MakeRotator 0.0 _newtrack_0 0.0) false false)
      (Transformation|SetRelativeRotation (Variables|Default|GetStaticMesh17) (Math|Rotator|MakeRotator 0.0 _newtrack_0 9e+01) false false)
      (Transformation|SetRelativeRotation (Variables|Default|GetStaticMesh16) (Math|Rotator|MakeRotator 0.0 (* -1 _newtrack_0) 0.0) false false)
      (Transformation|SetRelativeRotation (Variables|Default|GetStaticMesh18) (Math|Rotator|MakeRotator 0.0 (* -1 _newtrack_0) 9e+01) false false))))

(event Custom|Stop
  (Audio|Components|Audio|Stop (Variables|Default|GetAC_Gear_Grinding))
  (bind _newtrack_0 (Timeline|Timeline_1 Stop)
    (:Update
      (Transformation|SetRelativeRotation (Variables|Default|GetWaterWheel) (Math|Rotator|MakeRotator 0.0 _newtrack_0 0.0) false false)
      (Transformation|SetRelativeRotation (Variables|Default|GetStaticMesh17) (Math|Rotator|MakeRotator 0.0 _newtrack_0 9e+01) false false)
      (Transformation|SetRelativeRotation (Variables|Default|GetStaticMesh16) (Math|Rotator|MakeRotator 0.0 (* -1 _newtrack_0) 0.0) false false)
      (Transformation|SetRelativeRotation (Variables|Default|GetStaticMesh18) (Math|Rotator|MakeRotator 0.0 (* -1 _newtrack_0) 9e+01) false false))))

(event Custom|Tearrr
  (bind _ac_pipe_wheel (Variables|Default|GetAC_Pipe_Wheel))
  (bind _grinderref (Variables|Default|GetGrinderRef))
  (Variables|Default|SetRelative%20Rotation%20Y%20%28Pitch%29 (.pitch (Variables|/Script/Engine.SceneComponent|GetRelativeRotation (Variables|Default|GetPiece2))))
  (Timeline|Timeline_2 PlayFromStart
    (:Update
      (if (>= (Math|Float|Absolute(Float) (- (.pitch (Variables|/Script/Engine.SceneComponent|GetRelativeRotation (Variables|Default|GetPiece2))) (Variables|Default|GetRelative%20Rotation%20Y%20%28Pitch%29))) 9e+01)
        (Utilities|FlowControl|DoOnce false :!label _label
          (:Completed
            (Variables|Default|SetRelative%20Rotation%20Y%20%28Pitch%29 (.pitch (Variables|/Script/Engine.SceneComponent|GetRelativeRotation (Variables|Default|GetPiece2))))
            (Utilities|FlowControl|FlipFlop
              (:A
                (Utilities|FlowControl|Sequence
                  (:then_0
                    (Audio|Components|Audio|Stop (Variables|Default|GetAC_Pipe_Wheel))
                    (Audio|Components|Audio|Stop (Variables|Default|GetAC_Water_Wheel)))
                  (:then_1
                    (Default|GrinderStop _grinderref)
                    (CallFunction|Stop)
                    (Rendering|SetVisibility (Variables|Default|GetStaticMesh10) false false)
                    (Transformation|SetRelativeLocation (Variables|Default|GetNiagara) "-105.620712,-268.053864,-96.219269" false false)
                    (bind _newtrack_0 (Timeline|Timeline_0 PlayFromStart)))))
              (:B
                (Utilities|FlowControl|Sequence
                  (:then_0
                    (Audio|Components|Audio|Play _ac_pipe_wheel 0.0)
                    (Audio|Components|Audio|StopDelayed _ac_pipe_wheel 1.3)
                    (Audio|Components|Audio|Play (Variables|Default|GetAC_Water_Wheel) 0.0))
                  (:then_1
                    (Default|GrinderStart _grinderref)
                    (CallFunction|Start)
                    (Rendering|SetVisibility (Variables|Default|GetStaticMesh10) true false)
                    (Transformation|SetRelativeLocation (Variables|Default|GetNiagara) "-105.620712, 0,-96.219269" false false)
                    (Timeline|Timeline_0 ReverseFromEnd)))))))
        (else
          (goto _label Reset))))))

(event EventBeginPlay
  (bind _returnvalue (Actor|GetActorOfClass "/Game/Blueprints/Paintbrush/Paintrbsuh.Paintrbsuh_C"))
  (Variables|Default|SetNewVar_1 _returnvalue)
  (bind _returnvalue_2 (Actor|GetActorOfClass "/Game/Blueprints/PuzzleElements/Conduit_Grinder.Conduit_Grinder_C"))
  (Variables|Default|SetGrinderRef _returnvalue_2)
  (Actor|GetActorOfClass "/Game/Blueprints/PuzzleElements/Bp_SpiceTransport.Bp_SpiceTransport_C")
  (CallFunction|Start)
  (Audio|Components|Audio|Play (Variables|Default|GetAC_Water_Wheel) 0.0)
  (CallFunction|Tearrr))

(fn ConstructionScript)