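; Apple is a grabbable actor that reports to the Paintbrush actor, found on BeginPlay, whether it has been dropped away from the big toad.
; Mesh overlaps with BP_BigToad's Box1 set a NearToads flag.
; Grabbing clears the paintbrush's AppleDropped flag, and dropping sets it unless near a toad.
; Grow resets the mesh position and hides a second mesh, Kill destroys the actor, and a mesh-variant selection is left unwired.
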(event OnGrabbed(GrabComponent)
  (Variables|/Game/Blueprints/Paintbrush/Paintrbsuh.Paintrbsuh_C|SetAppleDropped? (Variables|Default|GetpaintbrushRef) false))

(event OnDropped(GrabComponent)
  (if (not (Variables|Default|GetnearToads?))
    (Variables|/Game/Blueprints/Paintbrush/Paintrbsuh.Paintrbsuh_C|SetAppleDropped? (Variables|Default|GetpaintbrushRef) true)))

(event OnComponentBeginOverlap(StaticMesh)
  (params (OverlappedComponent :type Primitive%20Component%20Object%20Reference) (OtherActor :type Actor%20Object%20Reference) (OtherComp :type Primitive%20Component%20Object%20Reference) (OtherBodyIndex :type Integer) (bFromSweep :type Boolean) (SweepResult :type Hit%20Result%20Structure%20%28by%20ref%29))
  (bind _asbp_big_toad (Utilities|Casting|CastToBP_BigToad OtherActor))
  (if (== (Variables|/Game/Blueprints/Conservatory/BP_BigToad.BP_BigToad_C|GetBox1 _asbp_big_toad) OtherComp)
    (Variables|Default|SetnearToads? true)))

(event OnComponentEndOverlap(StaticMesh)
  (params (OverlappedComponent :type Primitive%20Component%20Object%20Reference) (OtherActor :type Actor%20Object%20Reference) (OtherComp :type Primitive%20Component%20Object%20Reference) (OtherBodyIndex :type Integer))
  (bind _asbp_big_toad (Utilities|Casting|CastToBP_BigToad OtherActor))
  (if (== (Variables|/Game/Blueprints/Conservatory/BP_BigToad.BP_BigToad_C|GetBox1 _asbp_big_toad) OtherComp)
    (Variables|Default|SetnearToads? false)))

(event Custom|Kill
  (Actor|DestroyActor))

(event Custom|Grow
  (Transformation|SetRelativeLocation (Variables|Default|GetStaticMesh) "0, 0, 0" false false)
  (Rendering|SetVisibility (Variables|Default|GetStaticMesh1) false false))

(event EventBeginPlay
  (bind _returnvalue (Actor|GetActorOfClass "/Game/Blueprints/Paintbrush/Paintrbsuh.Paintrbsuh_C"))
  (Variables|Default|SetpaintbrushRef _returnvalue))

(fn ConstructionScript)