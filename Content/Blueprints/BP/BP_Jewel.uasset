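; BP_Jewel is a grabbable gem actor that plays a resonance cue from BeginPlay and tracks its proximity to BP_BigToad.
; Overlaps with the toad's Box1 set NearToad, so dropping the gem elsewhere flags JewelDropped on the paintbrush actor, and grabbing clears it.
; Lower runs a timeline that sinks and spins the mesh, while Kill destroys the actor.
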(event OnDropped(GrabComponent)
  (if (not (Variables|Default|GetnearToad?))
    (Variables|/Game/Blueprints/Paintbrush/Paintrbsuh.Paintrbsuh_C|SetJewelDropped? (Variables|Default|GetpaintbrushRef) true)))

(event OnComponentBeginOverlap(StaticMesh)
  (params (OverlappedComponent :type Primitive%20Component%20Object%20Reference) (OtherActor :type Actor%20Object%20Reference) (OtherComp :type Primitive%20Component%20Object%20Reference) (OtherBodyIndex :type Integer) (bFromSweep :type Boolean) (SweepResult :type Hit%20Result%20Structure%20%28by%20ref%29))
  (bind _asbp_big_toad (Utilities|Casting|CastToBP_BigToad OtherActor))
  (if (== (Variables|/Game/Blueprints/Conservatory/BP_BigToad.BP_BigToad_C|GetBox1 _asbp_big_toad) OtherComp)
    (Variables|Default|SetnearToad? true)))

(event OnComponentEndOverlap(StaticMesh)
  (params (OverlappedComponent :type Primitive%20Component%20Object%20Reference) (OtherActor :type Actor%20Object%20Reference) (OtherComp :type Primitive%20Component%20Object%20Reference) (OtherBodyIndex :type Integer))
  (bind _asbp_big_toad (Utilities|Casting|CastToBP_BigToad OtherActor))
  (if (== (Variables|/Game/Blueprints/Conservatory/BP_BigToad.BP_BigToad_C|GetBox1 _asbp_big_toad) OtherComp)
    (Variables|Default|SetnearToad? false)))

(event OnGrabbed(GrabComponent)
  (Variables|/Game/Blueprints/Paintbrush/Paintrbsuh.Paintrbsuh_C|SetJewelDropped? (Variables|Default|GetpaintbrushRef) false))

(event Custom|Kill
  ;[1 1 1] death
  (Actor|DestroyActor))

(event Custom|Lower
  (bind _staticmesh (Variables|Default|GetStaticMesh))
  (bind _newtrack_0 (Timeline|Timeline_0 PlayFromStart)
    (:Update
      (Transformation|SetRelativeLocation _staticmesh (Math|Vector|Lerp(Vector) "0, 0, 0" "0, 0,-70.000000" _newtrack_0) false false)
      (Transformation|SetRelativeRotation _staticmesh (Math|Rotator|MakeRotator 0.0 0.0 (Math|Float|Lerp 1.2e+02 7.2e+02 _newtrack_0)) false false))))

(event EventBeginPlay
  (Audio|Components|Audio|Play (Variables|Default|GetGemResonance_Cue) 0.0)
  (bind _returnvalue (Actor|GetActorOfClass "/Game/Blueprints/Paintbrush/Paintrbsuh.Paintrbsuh_C"))
  (Variables|Default|SetpaintbrushRef _returnvalue))

(event Collision|EventActorBeginOverlap
  (params (OtherActor :type Actor%20Object%20Reference)))

(event EventTick
  (params (DeltaSeconds :type Float%20%28single-precision%29)))

(fn ConstructionScript)