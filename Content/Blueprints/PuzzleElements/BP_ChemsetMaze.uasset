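; Chemset maze puzzle element that, once solved, enables the cauldron's distill button.
; A ScrewBulp_FRONT bulb entering BulbBox is killed, replaced by an animated screw-in mesh, then powers the puzzle.
; Brush overlaps with the bounds and maze mesh drive inherited enter/exit logic.
; Finishing completes the brush's chemset, fills flask liquids via timeline and restores Niagara effects, which are pooled by offsetting them rather than spawning.
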(event OnComponentBeginOverlap(BrushBounds1)
  (params (OverlappedComponent :type Primitive%20Component%20Object%20Reference) (OtherActor :type Actor%20Object%20Reference) (OtherComp :type Primitive%20Component%20Object%20Reference) (OtherBodyIndex :type Integer) (bFromSweep :type Boolean) (SweepResult :type Hit%20Result%20Structure%20%28by%20ref%29))
  (if (== OtherComp (Variables|/Game/Blueprints/Paintbrush/Paintrbsuh.Paintrbsuh_C|GetCollisionSphere (Variables|Default|GetBrushRefVar)))
    (CallFunction|ParentBegin)))

(event OnComponentBeginOverlap(StaticMesh1)
  (params (OverlappedComponent :type Primitive%20Component%20Object%20Reference) (OtherActor :type Actor%20Object%20Reference) (OtherComp :type Primitive%20Component%20Object%20Reference) (OtherBodyIndex :type Integer) (bFromSweep :type Boolean) (SweepResult :type Hit%20Result%20Structure%20%28by%20ref%29))
  (if (== OtherComp (Variables|/Game/Blueprints/Paintbrush/Paintrbsuh.Paintrbsuh_C|GetCollisionSphere (Variables|Default|GetBrushRefVar)))
    (CallFunction|ExitedParent)))

(event OnComponentBeginOverlap(BulbBox)
  (params (OverlappedComponent :type Primitive%20Component%20Object%20Reference) (OtherActor :type Actor%20Object%20Reference) (OtherComp :type Primitive%20Component%20Object%20Reference) (OtherBodyIndex :type Integer) (bFromSweep :type Boolean) (SweepResult :type Hit%20Result%20Structure%20%28by%20ref%29))
  (bind _magicpos (Variables|Default|GetMagicPos))
  (bind _asscrew_bulp_front (Utilities|Casting|CastToScrewBulp_FRONT OtherActor))
  (Default|Kill _asscrew_bulp_front)
  (Rendering|SetVisibility _magicpos true true)
  (Utilities|FlowControl|Sequence
    (:then_0
      (Audio|SpawnSoundAttached "/Game/Audio-Revised/Assets/Object-AMBX/CoreMechanics/cue/conduitScrewIn_Cue.conduitScrewIn_Cue" _magicpos "None" "0, 0, 0" "0, 0, 0" "KeepRelativeOffset" false 1.0 1.0 0.0 0 0))
    (:then_1
      (bind _newtrack_0 (Timeline|Timeline_2 PlayFromStart)
        (:Update
          (Transformation|SetRelativeLocation _magicpos (Math|Vector|MakeVector 0.0 0.0 _newtrack_0) false false))
        (:Finished
          (Audio|SpawnSoundAttached "/Game/Audio-Revised/Assets/Object-AMBX/CoreMechanics/cue/conduitIdleSpin_Cue.conduitIdleSpin_Cue" _magicpos "None" "0, 0, 0" "0, 0, 0" "KeepRelativeOffset" false 1.0 1.0 0.0 0 0))))
    (:then_2
      (Utilities|FlowControl|Delay 0.7)
      (CallFunction|PoweredUp))))

(event OnComponentEndOverlap(BrushBounds1)
  (params (OverlappedComponent :type Primitive%20Component%20Object%20Reference) (OtherActor :type Actor%20Object%20Reference) (OtherComp :type Primitive%20Component%20Object%20Reference) (OtherBodyIndex :type Integer))
  (if (== OtherComp (Variables|/Game/Blueprints/Paintbrush/Paintrbsuh.Paintrbsuh_C|GetCollisionSphere (Variables|Default|GetBrushRefVar)))
    (CallFunction|ExitedParent)))

(event EventBeginPlay
  (|CallParentFunction)
  (Utilities|FlowControl|Sequence
    (:then_0
      (bind _returnvalue (Actor|GetActorOfClass "/Game/Blueprints/PuzzleElements/BP_Cauldron.BP_Cauldron_C"))
      (Variables|Default|SetCauldRef _returnvalue)
      (Rendering|SetVisibility (Variables|Default|GetMagicPos) false true))
    (:then_1
      (for _array_element (Variables|Default|GetParticleSystems)
        (Variables|Default|SetArray_0 (Utilities|Array|MakeArray "-40.188095,-28.103455,10.971440" "-13.609211,-17.270983,10.971819" "15.919579,-11.702761,10.171737" "10.240402,49.589081,15.638292")))
      (CallFunction|DeacParticles))))

(event Collision|EventActorBeginOverlap
  (params (OtherActor :type Actor%20Object%20Reference)))

(event EventTick
  (params (DeltaSeconds :type Float%20%28single-precision%29)))

(event EventFinished
  (bind _cauldref (Variables|Default|GetCauldRef))
  (Variables|/Game/Blueprints/PuzzleElements/BP_Cauldron.BP_Cauldron_C|SetMazePuzzleDone _cauldref true)
  (Default|DistillButtonActivate _cauldref)
  (Utilities|FlowControl|Sequence
    (:then_0
      (Default|CompleteChemset (Variables|Default|GetBrushRefVar)))
    (:then_1
      (CallFunction|ActiParticles)
      (CallFunction|FillFlask))))

(event Custom|FillFlask
  ;[1 1 1] Liquid filling up anim
  (bind _newtrack_0 (Timeline|Timeline_0 Play)
    (:Update
      (Utilities|FlowControl|Sequence
        (:then_0
          (Transformation|SetWorldScale3D (Variables|Default|GetLiquid1) (Math|Vector|Lerp(Vector) "0.090000,0.090000,0.040000" "0.090000,0.090000,0.200000" _newtrack_0)))
        (:then_1
          (Transformation|SetWorldScale3D (Variables|Default|GetLiquid2) (Math|Vector|Lerp(Vector) "0.060000,0.060000,0.020000" "0.060000,0.060000,0.090000" _newtrack_0)))))))

(event Custom|ActiParticles
  ;[1 1 1] Particle pooling system
  (Utilities|FlowControl|DoOnce false
    (:Completed
      (for _array_element (Variables|Default|GetParticleSystems)
        (Transformation|AddWorldOffset _array_element "-100.000000, 0, 0" false false)))))

(event Custom|DeacParticles
  ;[1 1 1] Particle pooling system
  (Utilities|FlowControl|DoOnce false
    (:Completed
      (bind _output_get (Variables|Default|SetParticleSystems (Utilities|Array|MakeArray (Variables|Default|GetNiagara1) (Variables|Default|GetNiagara2) (Variables|Default|GetNiagara3) (Variables|Default|GetNiagara))))
      (for _array_element _output_get
        (Transformation|AddWorldOffset _array_element "100.000000, 0, 0" false false)))))

(fn ConstructionScript
  (|CallParentFunction))