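; BP_Vine is a Conservatory vine actor that grows along with its fruit when VineGrow is called.
; A timeline lerps both meshes' scales from shrunken to full size; BeginPlay runs it in reverse and caches the paintbrush actor.
; VineGrow plays a fruit-grow cue and the timeline, whose every update also sets FruitGrown on the paintbrush.
; HudeApple hides the second mesh, apparently the apple.
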(event Custom|VineGrow
  (Audio|Components|Audio|Play (Variables|Default|GetFruitGrow_Cue) 0.0)
  (bind _newtrack_0 (Timeline|Timeline_0 PlayFromStart)
    (:Update
      (Transformation|SetRelativeScale3D (Variables|Default|GetStaticMesh) (Math|Vector|Lerp(Vector) "0.500000,0.500000,0.001000" "1.000000,1.000000,1.000000" _newtrack_0))
      (Transformation|SetRelativeScale3D (Variables|Default|GetStaticMesh1) (Math|Vector|Lerp(Vector) "0.001000,0.001000,0.001000" "0.954751,0.954751,0.954751" _newtrack_0))
      (Variables|/Game/Blueprints/Paintbrush/Paintrbsuh.Paintrbsuh_C|SetFruitGrown? (Variables|Default|GetpaintbrushRef) true))))

(event Custom|HudeApple
  ;[1 0.2967 0.9159] Hude? XD Please get some sleep, Dante
  (Rendering|SetVisibility (Variables|Default|GetStaticMesh1) false false))

(event EventBeginPlay
  (Utilities|FlowControl|Sequence
    (:then_0
      (bind _newtrack_0 (Timeline|Timeline_0 Reverse)
        (:Update
          (Transformation|SetRelativeScale3D (Variables|Default|GetStaticMesh) (Math|Vector|Lerp(Vector) "0.500000,0.500000,0.001000" "1.000000,1.000000,1.000000" _newtrack_0))
          (Transformation|SetRelativeScale3D (Variables|Default|GetStaticMesh1) (Math|Vector|Lerp(Vector) "0.001000,0.001000,0.001000" "0.954751,0.954751,0.954751" _newtrack_0))
          (Variables|/Game/Blueprints/Paintbrush/Paintrbsuh.Paintrbsuh_C|SetFruitGrown? (Variables|Default|GetpaintbrushRef) true))))
    (:then_1
      (bind _returnvalue (Actor|GetActorOfClass "/Game/Blueprints/Paintbrush/Paintrbsuh.Paintrbsuh_C"))
      (Variables|Default|SetpaintbrushRef _returnvalue))))

(event Collision|EventActorBeginOverlap
  (params (OtherActor :type Actor%20Object%20Reference)))

(event EventTick
  (params (DeltaSeconds :type Float%20%28single-precision%29)))

(fn ConstructionScript)