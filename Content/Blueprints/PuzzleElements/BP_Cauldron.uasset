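; VR cauldron puzzle hub where boil, grind and distill steps prepare a potion for the paintbrush.
; External activate events mark each puzzle done and reveal its billboard.
; Pawn overlaps press buttons that, once unlocked, run one-shot effects, shrink billboards and flag the brush when all three finish.
; Dipping the brush plays bubbles, moves a surface cube along with it, and starts brush loading if all puzzles are done.
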(event OnComponentBeginOverlap(WaterSurfaceCollision)
  (params (OverlappedComponent :type Primitive%20Component%20Object%20Reference) (OtherActor :type Actor%20Object%20Reference) (OtherComp :type Primitive%20Component%20Object%20Reference) (OtherBodyIndex :type Integer) (bFromSweep :type Boolean) (SweepResult :type Hit%20Result%20Structure%20%28by%20ref%29))
  (bind _followcube (Variables|Default|GetFollowCube))
  (bind _location0 (Variables|Default|GetLocation0))
  (bind _brushrefvar (Variables|References|GetBrushRefVar))
  (bind _collisionsphere (Variables|/Game/Blueprints/Paintbrush/Paintrbsuh.Paintrbsuh_C|GetCollisionSphere _brushrefvar))
  (bind _returnvalue (Transformation|GetWorldLocation _collisionsphere))
  ;[1 1 1 1 30] Dip in water
  (if (== (Variables|/Game/Blueprints/Paintbrush/Paintrbsuh.Paintrbsuh_C|GetCollisionSphere (Variables|References|GetBrushRefVar)) OtherComp)
    (Utilities|FlowControl|Sequence
      (:then_0
        (Audio|Components|Audio|Play (Variables|Default|GetAC_CauldronBubbles) 0.0))
      (:then_1
        (Transformation|SetRelativeLocation (Variables|Default|GetFollowCube) (Math|Vector|MakeVector _location0 _location0 (Variables|Default|GetWaterLevel)) false false))
      (:then_2
        (Timeline|Timeline_1 Play
          (:Update
            (Transformation|SetWorldLocation _followcube (Math|Vector|MakeVector (.x _returnvalue) (.y _returnvalue) (.z (Transformation|GetWorldLocation _followcube))) false false))))
      (:then_3
        (if (Math|Boolean|ANDBoolean (Variables|Puzzles|GetBoilPuzzleDone) (Variables|Puzzles|GetSpicePuzzleDone) (Variables|Puzzles|GetMazePuzzleDone))
          (Default|Loading (Variables|References|GetBrushRefVar) "NewEnumerator4"))))))

(event OnComponentEndOverlap(WaterSurfaceCollision)
  (params (OverlappedComponent :type Primitive%20Component%20Object%20Reference) (OtherActor :type Actor%20Object%20Reference) (OtherComp :type Primitive%20Component%20Object%20Reference) (OtherBodyIndex :type Integer))
  (bind _followcube (Variables|Default|GetFollowCube))
  (bind _location0 (Variables|Default|GetLocation0))
  (bind _brushrefvar (Variables|References|GetBrushRefVar))
  (bind _collisionsphere (Variables|/Game/Blueprints/Paintbrush/Paintrbsuh.Paintrbsuh_C|GetCollisionSphere _brushrefvar))
  (bind _returnvalue (Transformation|GetWorldLocation _collisionsphere))
  ;[1 1 1 1 30] Dip in water
  (if (== (Variables|/Game/Blueprints/Paintbrush/Paintrbsuh.Paintrbsuh_C|GetCollisionSphere (Variables|References|GetBrushRefVar)) OtherComp)
    (Utilities|FlowControl|Sequence
      (:then_0
        (Audio|Components|Audio|Stop (Variables|Default|GetAC_CauldronBubbles))
        (Transformation|SetRelativeLocation (Variables|Default|GetFollowCube) (Math|Vector|MakeVector _location0 _location0 (- (Variables|Default|GetWaterLevel) 5.0)) false false))
      (:then_1
        (Timeline|Timeline_1 Stop
          (:Update
            (Transformation|SetWorldLocation _followcube (Math|Vector|MakeVector (.x _returnvalue) (.y _returnvalue) (.z (Transformation|GetWorldLocation _followcube))) false false))))
      (:then_2
        (Default|StopLoading (Variables|References|GetBrushRefVar))))))

(event OnComponentBeginOverlap(BoilBox)
  (params (OverlappedComponent :type Primitive%20Component%20Object%20Reference) (OtherActor :type Actor%20Object%20Reference) (OtherComp :type Primitive%20Component%20Object%20Reference) (OtherBodyIndex :type Integer) (bFromSweep :type Boolean) (SweepResult :type Hit%20Result%20Structure%20%28by%20ref%29))
  ;[1 1 1 1 30] PressButton
  (if (== OtherActor (Variables|References|GetPawnRef))
    (Utilities|FlowControl|DoOnce false
      (:Completed
        (Utilities|FlowControl|Sequence
          (:then_0
            (bind _newtrack_0 (Timeline|Timeline_5 PlayFromStart)
              (:Update
                (Transformation|SetRelativeLocation (Variables|Default|GetStaticMesh12) (Math|Vector|Lerp(Vector) "0, 0,-11.141861" "0.000000, 0,-3.580315" _newtrack_0) false false))))
          (:then_1
            (if (Variables|Puzzles|GetBoilPuzzleDone)
              (Variables|/Game/Blueprints/Paintbrush/Paintrbsuh.Paintrbsuh_C|SetCauld_FirePressable? (Variables|References|GetBrushRefVar) true)
              (CallFunction|WaterIsBoiling))))))))

(event OnComponentEndOverlap(BoilBox)
  (params (OverlappedComponent :type Primitive%20Component%20Object%20Reference) (OtherActor :type Actor%20Object%20Reference) (OtherComp :type Primitive%20Component%20Object%20Reference) (OtherBodyIndex :type Integer))
  ;[1 1 1 1 30] PressButton
  (if (== OtherActor (Variables|References|GetPawnRef))
    (Utilities|FlowControl|DoOnce false) ; enters at Reset
  ))

(event OnComponentBeginOverlap(GrindBox)
  (params (OverlappedComponent :type Primitive%20Component%20Object%20Reference) (OtherActor :type Actor%20Object%20Reference) (OtherComp :type Primitive%20Component%20Object%20Reference) (OtherBodyIndex :type Integer) (bFromSweep :type Boolean) (SweepResult :type Hit%20Result%20Structure%20%28by%20ref%29))
  ;[1 1 1 1 30] PressButton
  (if (== OtherActor (Variables|References|GetPawnRef))
    (Utilities|FlowControl|DoOnce false
      (:Completed
        (Utilities|FlowControl|Sequence
          (:then_0
            (bind _newtrack_0 (Timeline|Timeline_6 PlayFromStart)
              (:Update
                (Transformation|SetRelativeLocation (Variables|Default|GetStaticMesh36) (Math|Vector|Lerp(Vector) "0, 0,-7.578993" "0, 0, 0" _newtrack_0) false false))))
          (:then_1
            (if (Variables|Puzzles|GetSpicePuzzleDone)
              (Variables|/Game/Blueprints/Paintbrush/Paintrbsuh.Paintrbsuh_C|SetCauld_HerbPressable? (Variables|References|GetBrushRefVar) true)
              (CallFunction|Spiced))))))))

(event OnComponentBeginOverlap(DistillBox)
  (params (OverlappedComponent :type Primitive%20Component%20Object%20Reference) (OtherActor :type Actor%20Object%20Reference) (OtherComp :type Primitive%20Component%20Object%20Reference) (OtherBodyIndex :type Integer) (bFromSweep :type Boolean) (SweepResult :type Hit%20Result%20Structure%20%28by%20ref%29))
  ;[1 1 1 1 30] PressButton
  (if (== OtherActor (Variables|References|GetPawnRef))
    (Utilities|FlowControl|DoOnce false
      (:Completed
        (Utilities|FlowControl|Sequence
          (:then_0
            (bind _newtrack_0 (Timeline|Timeline_7 PlayFromStart)
              (:Update
                (Transformation|SetRelativeLocation (Variables|Default|GetStaticMesh42) (Math|Vector|Lerp(Vector) "0, 0,-6.609025" "0, 0,0.200000" _newtrack_0) false false))))
          (:then_1
            (if (Variables|Puzzles|GetMazePuzzleDone)
              (Variables|/Game/Blueprints/Paintbrush/Paintrbsuh.Paintrbsuh_C|SetCauld_MagicPressble? (Variables|References|GetBrushRefVar) true)
              (CallFunction|DistillMagic))))))))

(event OnComponentEndOverlap(GrindBox)
  (params (OverlappedComponent :type Primitive%20Component%20Object%20Reference) (OtherActor :type Actor%20Object%20Reference) (OtherComp :type Primitive%20Component%20Object%20Reference) (OtherBodyIndex :type Integer))
  ;[1 1 1 1 30] PressButton
  (if (== OtherActor (Variables|References|GetPawnRef))
    (Utilities|FlowControl|DoOnce false) ; enters at Reset
  ))

(event OnComponentEndOverlap(DistillBox)
  (params (OverlappedComponent :type Primitive%20Component%20Object%20Reference) (OtherActor :type Actor%20Object%20Reference) (OtherComp :type Primitive%20Component%20Object%20Reference) (OtherBodyIndex :type Integer))
  ;[1 1 1 1 30] PressButton
  (if (== OtherActor (Variables|References|GetPawnRef))
    (Utilities|FlowControl|DoOnce false) ; enters at Reset
  ))

(event Custom|BoilButtonActivate
  ;[0.05521 0.05521 0.05521] ButtonActivation
  ;;[1 1 1] Puzzle completion activation effect
  ;;;[1 0.6035 0.3941] Boil
  (Utilities|FlowControl|DoOnce false
    (:Completed
      (Variables|Puzzles|SetBoilPuzzleDone true)
      (Rendering|SetVisibility (Variables|Default|GetFireBillboard) true false)
      (Rendering|Material|SetMaterial (Variables|Default|GetFireBack) 0 "/Game/Materials/M_BrushRing.M_BrushRing"))))

(event Custom|BoilPressed
  ;[0.05521 0.05521 0.05521] ButtonActivation
  ;;[1 0.6035 0.3941] Boil
  (Utilities|FlowControl|DoOnce false
    (:Completed
      (bind _newtrack_0 (Timeline|BoilBillboardShrink Play)
        (:Update
          (Transformation|SetRelativeScale3D (Variables|Default|GetFireBillboard) (Math|Conversions|ToVector(Float) (Math|Float|Lerp 6.0 0.0 _newtrack_0))))
        (:Finished
          (Rendering|SetVisibility (Variables|Default|GetFireBillboard) false false)
          (Variables|Default|SetFirePressed? true)
          (if (and (and (Variables|Default|GetHerbPressed?) (Variables|Default|GetMagicPressed?)) (Variables|Default|GetFirePressed?))
            (Variables|/Game/Blueprints/Paintbrush/Paintrbsuh.Paintrbsuh_C|SetButtonsPressed? (Variables|References|GetBrushRefVar) true)))))))

(event Custom|WaterIsBoiling
  ;[1 1 1 1 30] Activating Water
  (Utilities|FlowControl|DoOnce false
    (:Completed
      (Audio|Components|Audio|Play (Variables|Default|GetAC_Boiling) 0.0)
      (Transformation|SetRelativeLocation (Variables|Default|GetBoilBubbles) "0, 0,110.000000" false false)
      (Variables|CauldronEffects|SetPotionBoiling true)
      (CallFunction|BoilPressed))))

(event Custom|DistillMagic
  (bind _drip (Variables|Default|GetDrip))
  ;[1 1 1 1 30] Activating Water
  (Utilities|FlowControl|Sequence
    (:then_0
      (Utilities|FlowControl|DoOnce false
        (:Completed
          (Audio|Components|Audio|Play (Variables|Default|GetSparkle1) 0.0)
          (Transformation|SetRelativeLocation (Variables|Default|GetSparkle) "0, 0,116.910202" false false)
          (Variables|CauldronEffects|SetPotionDistilled true)
          (CallFunction|DistillPressed))))
    (:then_1
      (Transformation|SetRelativeLocation _drip "25.563572, 0,151.197052" false false)
      (Utilities|FlowControl|Delay 1.0)
      (Transformation|SetRelativeLocation _drip "25.563572, 0,-43.406830" false false))))

(event Custom|Spiced
  (bind _staticmesh3 (Variables|Default|GetStaticMesh3))
  (bind _cube (Variables|Default|GetCube))
  ;[1 1 1 1 30] Activating Water
  (Utilities|FlowControl|DoOnce false
    (:Completed
      (Utilities|FlowControl|Sequence
        (:then_0
          (CallFunction|GrindPressed)
          (Variables|CauldronEffects|SetPotionSpiced true))
        (:then_1
          ;;[1 1 1] ed
          (bind _newtrack_0 (Timeline|Timeline_4 PlayFromStart)
            (:Update
              (Transformation|SetRelativeScale3D _staticmesh3 (Math|Vector|Lerp(Vector) "0, 0, 0" "0.622482,0.622482,0.622482" _newtrack_0))
              (Transformation|SetRelativeRotation _staticmesh3 (Math|Rotator|Lerp(Rotator) "0, 0, 0" "0,360.000000, 0" _newtrack_0) false false)
              (Transformation|SetRelativeScale3D _cube (Math|Vector|Lerp(Vector) "0.040000,0.040000,0.002000" "0.040000,0.040000,0.015000" _newtrack_0))
              (Transformation|SetRelativeLocation _cube (Math|Vector|Lerp(Vector) "-9.645981,-18.672058,96.175545" "-9.645981,-18.672058,74.307602" _newtrack_0) false false)
              (Variables|CauldronEffects|SetPotionSpiced true))))))))

(event Custom|GrindButtonActivate
  ;[0.05521 0.05521 0.05521] ButtonActivation
  ;;[1 1 1] Puzzle completion activation effect
  ;;;[0.7044 1 0.569] Grind
  (Utilities|FlowControl|DoOnce false
    (:Completed
      (Variables|Puzzles|SetSpicePuzzleDone true)
      (Rendering|SetVisibility (Variables|Default|GetLeafBillboard) true false)
      (Rendering|Material|SetMaterial (Variables|Default|GetLeafBack) 0 "/Game/Materials/M_BrushRing.M_BrushRing"))))

(event Custom|DistillButtonActivate
  ;[0.05521 0.05521 0.05521] ButtonActivation
  ;;[0.849 0.6979 1] Distill
  ;;;[1 1 1] Puzzle completion activation effect
  (Utilities|FlowControl|DoOnce false
    (:Completed
      (Variables|Puzzles|SetMazePuzzleDone true)
      (Rendering|SetVisibility (Variables|Default|GetSparkleBillboard) true false)
      (Rendering|Material|SetMaterial (Variables|Default|GetSparkleBack) 0 "/Game/Materials/M_BrushRing.M_BrushRing"))))

(event Custom|GrindPressed
  ;[0.05521 0.05521 0.05521] ButtonActivation
  ;;[0.7044 1 0.569] Grind
  (Utilities|FlowControl|DoOnce false
    (:Completed
      (bind _newtrack_0 (Timeline|GrindBillboardShrink Play)
        (:Update
          (Transformation|SetRelativeScale3D (Variables|Default|GetLeafBillboard) (Math|Conversions|ToVector(Float) (Math|Float|Lerp 6.0 0.0 _newtrack_0))))
        (:Finished
          (Rendering|SetVisibility (Variables|Default|GetLeafBillboard) false false)
          (Variables|Default|SetHerbPressed? true)
          (if (and (and (Variables|Default|GetHerbPressed?) (Variables|Default|GetMagicPressed?)) (Variables|Default|GetFirePressed?))
            (Variables|/Game/Blueprints/Paintbrush/Paintrbsuh.Paintrbsuh_C|SetButtonsPressed? (Variables|References|GetBrushRefVar) true)))))))

(event Custom|DistillPressed
  ;[0.05521 0.05521 0.05521] ButtonActivation
  ;;[0.849 0.6979 1] Distill
  (Utilities|FlowControl|DoOnce false
    (:Completed
      (bind _newtrack_0 (Timeline|DistillBillboardShrink Play)
        (:Update
          (Transformation|SetRelativeScale3D (Variables|Default|GetSparkleBillboard) (Math|Conversions|ToVector(Float) (Math|Float|Lerp 6.0 0.0 _newtrack_0))))
        (:Finished
          (Rendering|SetVisibility (Variables|Default|GetSparkleBillboard) false false)
          (Variables|Default|SetMagicPressed? true)
          (if (and (and (Variables|Default|GetHerbPressed?) (Variables|Default|GetMagicPressed?)) (Variables|Default|GetFirePressed?))
            (Variables|/Game/Blueprints/Paintbrush/Paintrbsuh.Paintrbsuh_C|SetButtonsPressed? (Variables|References|GetBrushRefVar) true)))))))

(event EventBeginPlay
  (bind _location0 (Variables|Default|GetLocation0))
  (bind _location0_2 (Variables|Default|GetLocation0))
  ;[1 1 1] Begin play - pooling and setup
  (Utilities|FlowControl|Sequence
    (:then_0
      (Audio|Components|Audio|StopDelayed (Variables|Default|GetAC_CauldronBubbles) 0.0)
      (Transformation|SetRelativeLocation (Variables|Default|GetFollowCube) (Math|Vector|MakeVector _location0 _location0 (Variables|Default|GetWaterLevel)) false false)
      (bind _returnvalue (Actor|GetActorOfClass "/Game/Blueprints/Paintbrush/Paintrbsuh.Paintrbsuh_C"))
      (Variables|References|SetBrushRefVar _returnvalue)
      (bind _returnvalue_2 (Actor|GetActorOfClass "/Game/Blueprints/VR_Character/BP_UpdatedVRPawn.BP_UpdatedVRPawn_C"))
      (Variables|References|SetPawnRef _returnvalue_2)
      (Utilities|FlowControl|Delay 1.0))
    (:then_1
      (Transformation|SetRelativeLocation (Variables|Default|GetFollowCube) (Math|Vector|MakeVector _location0_2 _location0_2 (- (Variables|Default|GetWaterLevel) 5.0)) false false))))

(fn ConstructionScript)