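; Grabbable handle that turns the motion of a follow cube into a single-axis move or rotate value, with optional limits.
; While grabbed, a timeline updates MoveVal from the cube's location, or RotVal from its rotation or look-at angle around PivotPoint.
; Dropping disables hitbox physics; the snap-to-origin branch is empty and its lerp timeline is unconnected.
; The construction script applies the configurable hitbox mesh and transform.
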(event Custom|Grabbed
  (bind _followcube (Variables|Default|GetFollowCube))
  (bind _pivot_point (Variables|Default|GetPivot%20Point))
  (bind _pivot_point_2 (Variables|Default|GetPivot%20Point))
  (bind _followcube_2 (Variables|Default|GetFollowCube))
  (bind _followcube_3 (Variables|Default|GetFollowCube))
  (bind _followcube_4 (Variables|Default|GetFollowCube))
  (bind _xyz_direction (Variables|Inputs|GetXYZ%20Direction))
  (bind _followcube_5 (Variables|Default|GetFollowCube))
  (bind _relativelocation (Variables|/Script/Engine.SceneComponent|GetRelativeLocation _followcube))
  (bind _relativelocation_2 (Variables|/Script/Engine.SceneComponent|GetRelativeLocation _pivot_point))
  (bind _relativelocation_3 (Variables|/Script/Engine.SceneComponent|GetRelativeLocation _followcube_3))
  (bind _relativerotation (Variables|/Script/Engine.SceneComponent|GetRelativeRotation _followcube_2))
  (bind _relativelocation_4 (Variables|/Script/Engine.SceneComponent|GetRelativeLocation _pivot_point_2))
  (bind _relativerotation_2 (Variables|/Script/Engine.SceneComponent|GetRelativeRotation _followcube_4))
  (bind _relativerotation_3 (Variables|/Script/Engine.SceneComponent|GetRelativeRotation _followcube_5))
  (bind (_x _y _z) (Math|Vector|BreakVector _relativelocation_2))
  (bind (_x_2 _y_2 _z_2) (Math|Vector|BreakVector _relativelocation_4))
  (bind _returnvalue (Math|Vector|MakeVector (.x _relativelocation) (.y _relativelocation) _z))
  (bind _returnvalue_2 (Math|Vector|MakeVector _x (.y _relativelocation) (.z _relativelocation)))
  (bind _returnvalue_3 (Math|Vector|MakeVector (.x _relativelocation) _y (.z _relativelocation)))
  (bind _returnvalue_4 (Math|Rotator|FindLookatRotation _relativelocation_2 _returnvalue_3))
  (bind _returnvalue_5 (Math|Rotator|FindLookatRotation _relativelocation_2 _returnvalue))
  (bind _returnvalue_6 (Math|Rotator|FindLookatRotation _relativelocation_2 _returnvalue_2))
  (bind _returnvalue_7 (> (.yaw _returnvalue_6) -8e+01))
  (bind _returnvalue_8 (> (.yaw _returnvalue_4) 1.7e+02))
  (bind _returnvalue_9 (+ (.pitch _returnvalue_4) 9e+01))
  (bind _returnvalue_10 (+ (.pitch _returnvalue_6) 9e+01))
  (bind _returnvalue_11 (Math|Float|SelectFloat -1.0 1.0 _returnvalue_7))
  (bind _returnvalue_12 (Math|Float|SelectFloat -1.0 1.0 _returnvalue_8))
  (bind _returnvalue_13 (* _returnvalue_12 _returnvalue_9))
  (bind _returnvalue_14 (* _returnvalue_11 _returnvalue_10))
  (Utilities|FlowControl|Sequence
    (:then_1
      (switch Utilities|FlowControl|Switch|SwitchonFollowHandleEnum (Variables|Inputs|GetInteract%20Type)
        (:NewEnumerator0
          (Timeline|Timeline_1 PlayFromStart
            (:Update
              (Variables|Output|SetMove%20Val (Utilities|Select :Index _xyz_direction :NewEnumerator0 (Math|Vector|MakeVector (Math|Float|SelectFloat (Math|Float|Clamp(Float) (.x _relativelocation_3) (- _x_2 (Variables|Inputs|GetMinimum%20Limit)) (+ _x_2 (Variables|Inputs|GetMaximum%20Limit))) (.x _relativelocation_3) (Variables|Switches|GetLimit%20Value)) _y_2 _z_2) :NewEnumerator1 (Math|Vector|MakeVector _x_2 (Math|Float|SelectFloat (Math|Float|Clamp(Float) (.y _relativelocation_3) (- _y_2 (Variables|Inputs|GetMinimum%20Limit)) (+ _y_2 (Variables|Inputs|GetMaximum%20Limit))) (.y _relativelocation_3) (Variables|Switches|GetLimit%20Value)) _z_2) :NewEnumerator2 (Math|Vector|MakeVector _x_2 _y_2 (Math|Float|SelectFloat (Math|Float|Clamp(Float) (.z _relativelocation_3) (- _z_2 (Variables|Inputs|GetMinimum%20Limit)) (+ _z_2 (Variables|Inputs|GetMaximum%20Limit))) (.z _relativelocation_3) (Variables|Switches|GetLimit%20Value))))))))
        (:NewEnumerator1
          (Timeline|Timeline_0 PlayFromStart
            (:Update
              (Variables|Output|SetRotVal (Utilities|Select :Index _xyz_direction :NewEnumerator0 (select (Variables|Switches|GetRotation%20relative%20to%20hitbox) (Math|Rotator|MakeRotator (Math|Float|SelectFloat (Math|Float|Clamp(Float) (.roll _relativerotation_2) (Variables|Inputs|GetMinimum%20Limit) (Variables|Inputs|GetMaximum%20Limit)) (.roll _relativerotation_2) (Variables|Switches|GetLimit%20Value)) 0.0 0.0) (Math|Rotator|MakeRotator (Math|Float|SelectFloat (Math|Float|Clamp(Float) _returnvalue_14 (Variables|Inputs|GetMinimum%20Limit) (Variables|Inputs|GetMaximum%20Limit)) _returnvalue_14 (Variables|Switches|GetLimit%20Value)) 0.0 0.0)) :NewEnumerator1 (select (Variables|Switches|GetRotation%20relative%20to%20hitbox) (Math|Rotator|MakeRotator 0.0 (Math|Float|SelectFloat (Math|Float|Clamp(Float) (.pitch _relativerotation_3) (Variables|Inputs|GetMinimum%20Limit) (Variables|Inputs|GetMaximum%20Limit)) (.pitch _relativerotation_3) (Variables|Switches|GetLimit%20Value)) 0.0) (Math|Rotator|MakeRotator 0.0 (Math|Float|SelectFloat (Math|Float|Clamp(Float) _returnvalue_13 (Variables|Inputs|GetMinimum%20Limit) (Variables|Inputs|GetMaximum%20Limit)) _returnvalue_13 (Variables|Switches|GetLimit%20Value)) 0.0)) :NewEnumerator2 (select (Variables|Switches|GetRotation%20relative%20to%20hitbox) (Math|Rotator|MakeRotator 0.0 0.0 (Math|Float|SelectFloat (Math|Float|Clamp(Float) (.yaw _relativerotation) (Variables|Inputs|GetMinimum%20Limit) (Variables|Inputs|GetMaximum%20Limit)) (.yaw _relativerotation) (Variables|Switches|GetLimit%20Value))) (Math|Rotator|MakeRotator 0.0 0.0 (Math|Float|SelectFloat (Math|Float|Clamp(Float) (.yaw _returnvalue_5) (Variables|Inputs|GetMinimum%20Limit) (Variables|Inputs|GetMaximum%20Limit)) (.yaw _returnvalue_5) (Variables|Switches|GetLimit%20Value)))))))))))))

(event Custom|Dropped
  (Physics|SetSimulatePhysics (Variables|Default|GetGrabbableObject) false)
  (Utilities|FlowControl|Sequence
    (:then_1
      (if (Variables|Switches|GetSnap%20to%20original%20transform)
        _))))

(fn ConstructionScript
  (bind _grabbableobject (Variables|Default|GetGrabbableObject))
  (Components|StaticMesh|SetStaticMesh _grabbableobject (Variables|Inputs|GetHitbox%20Static%20Mesh))
  (Transformation|SetRelativeTransform _grabbableobject (Variables|Inputs|GetHitBox%20Relative%20Transform) false false))