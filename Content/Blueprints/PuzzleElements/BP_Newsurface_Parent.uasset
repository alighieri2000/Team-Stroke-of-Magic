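; Parent Blueprint for paintable puzzle surfaces, with optional growth and conduit features and empty events for children to override.
; BeginPlay finds the paintbrush, then spawns and attaches white, red and optional green paint actors.
; Brush bounds overlaps start and stop painting and sound by paint type.
; When powered, yellow paint loads at the first conduit box, and reaching the second completes the line, unloads the brush and fires Finished.
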(event OnComponentBeginOverlap(BrushBounds1)
  (params (OverlappedComponent :type Primitive%20Component%20Object%20Reference) (OtherActor :type Actor%20Object%20Reference) (OtherComp :type Primitive%20Component%20Object%20Reference) (OtherBodyIndex :type Integer) (bFromSweep :type Boolean) (SweepResult :type Hit%20Result%20Structure%20%28by%20ref%29))
  (bind _whitepaint (Variables|Default|GetWhitePaint))
  (bind _brushrefvar (Variables|Default|GetBrushRefVar))
  (bind _maingreen (Variables|Default|GetMainGreen))
  (bind _enum_paints (Variables|/Game/Blueprints/Paintbrush/Paintrbsuh.Paintrbsuh_C|GetEnum%20Paints _brushrefvar))
  (if (== (Variables|/Game/Blueprints/Paintbrush/Paintrbsuh.Paintrbsuh_C|GetCollisionSphere (Variables|Default|GetBrushRefVar)) OtherComp)
    (Utilities|FlowControl|Sequence
      (:then_0
        (Utilities|FlowControl|DoOnce false
          (:Completed
            (Variables|Default|SetIs%20Within%20Paint%20Bounds true)
            (switch Utilities|FlowControl|Switch|SwitchonEnum_Paints _enum_paints
              (:NewEnumerator3
                (CallFunction|PaintingSoundActive "/Game/Audio-Revised/Assets/Object-AMBX/CoreMechanics/cue/Brush_Blank.Brush_Blank")
                (Default|Entered _whitepaint "NewEnumerator3" :!label _label))
              (:NewEnumerator0
                (CallFunction|PaintingSoundActive "/Game/Audio-Revised/Assets/Object-AMBX/CoreMechanics/cue/Brush_Blank.Brush_Blank")
                (goto _label))
              (:NewEnumerator4
                (CallFunction|PaintingSoundActive "/Game/Audio-Revised/Assets/Object-AMBX/CoreMechanics/cue/Brush_Green.Brush_Green")
                (Default|Entered _maingreen "NewEnumerator3"))))))
      (:then_1
        (Utilities|FlowControl|DoOnce false) ; enters at Reset
      ))))

(event OnComponentEndOverlap(BrushBounds1)
  (params (OverlappedComponent :type Primitive%20Component%20Object%20Reference) (OtherActor :type Actor%20Object%20Reference) (OtherComp :type Primitive%20Component%20Object%20Reference) (OtherBodyIndex :type Integer))
  (bind _whitepaint (Variables|Default|GetWhitePaint))
  (bind _brushrefvar (Variables|Default|GetBrushRefVar))
  (bind _maingreen (Variables|Default|GetMainGreen))
  (bind _enum_paints (Variables|/Game/Blueprints/Paintbrush/Paintrbsuh.Paintrbsuh_C|GetEnum%20Paints _brushrefvar))
  (if (== (Variables|/Game/Blueprints/Paintbrush/Paintrbsuh.Paintrbsuh_C|GetCollisionSphere (Variables|Default|GetBrushRefVar)) OtherComp)
    (if (not (Variables|Default|GetSupressBrushBoundsExit))
      (Utilities|FlowControl|Sequence
        (:then_0
          (Utilities|FlowControl|DoOnce false
            (:Completed
              (Variables|Default|SetIs%20Within%20Paint%20Bounds false)
              (Variables|Default|SetPointOneCrossed false)
              (switch Utilities|FlowControl|Switch|SwitchonEnum_Paints _enum_paints
                (:NewEnumerator3
                  (Default|Exited _whitepaint :!label _label)
                  (CallFunction|PaintingSoundDeactive))
                (:NewEnumerator0
                  (Utilities|FlowControl|Sequence
                    (:then_0
                      (goto _label))
                    (:then_1
                      (Default|Exited (Variables|Default|GetRedPaint))
                      (CallFunction|PaintingSoundDeactive))))
                (:NewEnumerator4
                  (Default|Exited _maingreen)
                  (CallFunction|PaintingSoundDeactive))))))
        (:then_1
          (Utilities|FlowControl|DoOnce false) ; enters at Reset
        )))))

(event OnComponentBeginOverlap(Box1)
  (params (OverlappedComponent :type Primitive%20Component%20Object%20Reference) (OtherActor :type Actor%20Object%20Reference) (OtherComp :type Primitive%20Component%20Object%20Reference) (OtherBodyIndex :type Integer) (bFromSweep :type Boolean) (SweepResult :type Hit%20Result%20Structure%20%28by%20ref%29))
  (bind _redpaint (Variables|Default|GetRedPaint))
  (bind _brushrefvar (Variables|Default|GetBrushRefVar))
  ;[1 1 1] First connection point entered
  (if (Variables|Default|GetIncludeConduits)
    (if (== OtherComp (Variables|/Game/Blueprints/Paintbrush/Paintrbsuh.Paintrbsuh_C|GetCollisionSphere _brushrefvar))
      (if (Variables|Default|GetPowered)
        (if (Utilities|Enum|Equal(Enum) (Variables|/Game/Blueprints/Paintbrush/Paintrbsuh.Paintrbsuh_C|GetEnum%20Paints _brushrefvar) "NewEnumerator0")
          (if (Variables|Default|GetIs%20Within%20Paint%20Bounds)
            (Default|Load _brushrefvar "NewEnumerator0")
            (Variables|Default|SetPointOneCrossed true)
            (Variables|/Game/Blueprints/Palette/BP_RedPaint.BP_RedPaint_C|SetConduitPoint1Crossed _redpaint true)
            (CallFunction|PaintingSoundActive "/Game/Audio-Revised/Assets/Object-AMBX/CoreMechanics/cue/Brush_Yellow.Brush_Yellow")
            (Default|Entered _redpaint "NewEnumerator0")
            (Default|Exited (Variables|Default|GetWhitePaint))))))))

(event OnComponentBeginOverlap(Box2)
  (params (OverlappedComponent :type Primitive%20Component%20Object%20Reference) (OtherActor :type Actor%20Object%20Reference) (OtherComp :type Primitive%20Component%20Object%20Reference) (OtherBodyIndex :type Integer) (bFromSweep :type Boolean) (SweepResult :type Hit%20Result%20Structure%20%28by%20ref%29))
  (bind _redpaint (Variables|Default|GetRedPaint))
  ;[1 1 1] Second Connection point entered
  (if (== OtherComp (Variables|/Game/Blueprints/Paintbrush/Paintrbsuh.Paintrbsuh_C|GetCollisionSphere (Variables|Default|GetBrushRefVar)))
    (if (Variables|Default|GetPointOneCrossed)
      (if (Variables|Default|GetIs%20Within%20Paint%20Bounds)
        (Utilities|FlowControl|Sequence
          (:then_0
            (bind _newtrack_0 (Timeline|Timeline_6 PlayFromStart)
              (:Update
                (Transformation|SetRelativeRotation (Variables|Default|GetMagicSpin2) (Math|Rotator|MakeRotator 0.0 0.0 _newtrack_0) false false))))
          (:then_1
            (Default|Paint1Cleared (Variables|Default|GetBrushRefVar)))
          (:then_2
            (Rendering|Material|SetMaterial (Variables|Default|GetEndPoint) 0 "/Game/Materials/RedPaint.RedPaint"))
          (:then_3
            (CallFunction|Finished)
            (Variables|/Game/Blueprints/Palette/BP_RedPaint.BP_RedPaint_C|SetLineCompleted _redpaint true)
            (Default|Finished _redpaint)
            (Default|UnLoad (Variables|Default|GetBrushRefVar))
            (Audio|SpawnSoundAttached "/Game/Audio-Revised/Assets/Object-AMBX/CoreMechanics/cue/conduitIdleSpin_Cue.conduitIdleSpin_Cue" (Variables|Default|GetMagicSpin2) "None" "0, 0, 0" "0, 0, 0" "KeepRelativeOffset" false 1.0 1.0 0.0 0 0))
          (:then_4))))))

(event Custom|Finished
  ;[1 1 1] Events callable by children
)

(event Custom|PoweredUp
  (bind _magicspin (Variables|Default|GetMagicSpin))
  ;[1 1 1] Called in every child, unless that child wants to have a custom way of powering up the initial conduit
  (Utilities|FlowControl|Sequence
    (:then_0
      (Rendering|Material|SetMaterial (Variables|Default|GetBeginPoint) 0 "/Game/Materials/RedPaint.RedPaint")
      (Variables|Default|SetPowered true)
      (bind _newtrack_0 (Timeline|Timeline_5 PlayFromStart)
        (:Update
          (Transformation|SetRelativeRotation _magicspin (Math|Rotator|MakeRotator 0.0 0.0 _newtrack_0) false false))
        (:Finished
          (bind _newtrack_0_2 (Timeline|Timeline_4 PlayFromStart)
            (:Update
              (Transformation|SetRelativeRotation _magicspin (Math|Rotator|MakeRotator 0.0 0.0 _newtrack_0_2) false false))))))
    (:then_1
      (Utilities|FlowControl|DoOnce false
        (:Completed
          (bind _returnvalue (Audio|SpawnSoundAttached "/Game/Audio-Revised/Assets/Object-AMBX/CoreMechanics/cue/conduitIdleSpin_Cue.conduitIdleSpin_Cue" (Variables|Default|GetMagicSpin) "None" "0, 0, 0" "0, 0, 0" "KeepRelativeOffset" false 1.0 1.0 0.0 0 0)))))))

(event Custom|Painting
  ;[1 1 1] Events callable by children
)

(event Custom|ResetLine
  ;[1 1 1] Second Connection point entered
  ;;[1 1 1] Resets the line if needed
  (Rendering|Material|SetMaterial (Variables|Default|GetEndPoint) 0 "/Game/Materials/WhitePaint.WhitePaint")
  (Default|ResetLine (Variables|Default|GetRedPaint))
  (bind _newtrack_0 (Timeline|Timeline_6 Stop)
    (:Update
      (Transformation|SetRelativeRotation (Variables|Default|GetMagicSpin2) (Math|Rotator|MakeRotator 0.0 0.0 _newtrack_0) false false))))

(event Custom|ExitedParent
  (bind _whitepaint (Variables|Default|GetWhitePaint))
  (bind _brushrefvar (Variables|Default|GetBrushRefVar))
  (bind _maingreen (Variables|Default|GetMainGreen))
  (bind _enum_paints (Variables|/Game/Blueprints/Paintbrush/Paintrbsuh.Paintrbsuh_C|GetEnum%20Paints _brushrefvar))
  (CallFunction|PaintingSoundDeactive)
  (Utilities|FlowControl|Sequence
    (:then_0
      (Utilities|FlowControl|DoOnce false) ; enters at Reset
    )
    (:then_1
      (Variables|Default|SetIs%20Within%20Paint%20Bounds false)
      (Variables|Default|SetPointOneCrossed false)
      (switch Utilities|FlowControl|Switch|SwitchonEnum_Paints _enum_paints
        (:NewEnumerator3
          (Default|Exited _whitepaint :!label _label)
          (CallFunction|PaintingSoundDeactive))
        (:NewEnumerator0
          (Utilities|FlowControl|Sequence
            (:then_0
              (goto _label))
            (:then_1
              (Default|Exited (Variables|Default|GetRedPaint))
              (CallFunction|PaintingSoundDeactive))))
        (:NewEnumerator4
          (Default|Exited _maingreen)
          (CallFunction|PaintingSoundDeactive))))))

(event Custom|Parent%20Begin
  (bind _whitepaint (Variables|Default|GetWhitePaint))
  (bind _brushrefvar (Variables|Default|GetBrushRefVar))
  (bind _maingreen (Variables|Default|GetMainGreen))
  (bind _enum_paints (Variables|/Game/Blueprints/Paintbrush/Paintrbsuh.Paintrbsuh_C|GetEnum%20Paints _brushrefvar))
  (Utilities|FlowControl|Sequence
    (:then_0
      (Variables|Default|SetIs%20Within%20Paint%20Bounds true)
      (switch Utilities|FlowControl|Switch|SwitchonEnum_Paints _enum_paints
        (:NewEnumerator3
          (CallFunction|PaintingSoundActive "/Game/Audio-Revised/Assets/Object-AMBX/CoreMechanics/cue/Brush_Blank.Brush_Blank")
          (Default|Entered _whitepaint "NewEnumerator3" :!label _label))
        (:NewEnumerator0
          (CallFunction|PaintingSoundActive "/Game/Audio-Revised/Assets/Object-AMBX/CoreMechanics/cue/Brush_Blank.Brush_Blank")
          (goto _label))
        (:NewEnumerator4
          (CallFunction|PaintingSoundActive "/Game/Audio-Revised/Assets/Object-AMBX/CoreMechanics/cue/Brush_Green.Brush_Green")
          (Default|Entered _maingreen "NewEnumerator3"))))
    (:then_1
      (Utilities|FlowControl|DoOnce false) ; enters at Reset
    )))

(event Custom|GrowFinished
  ;[1 1 1] Events callable by children
)

(event Custom|PaintingSoundActive
  (params (SoundCue :type Sound%20Base%20Object%20Reference))
  ;[1 1 1] Paint sound active deactivate
  (Audio|Components|Audio|SetSound (Variables|Default|GetBrush_Blank) SoundCue)
  (Audio|Components|Audio|Play (Variables|Default|GetBrush_Blank) 0.0))

(event Custom|PaintingSoundDeactive
  ;[1 1 1] Paint sound active deactivate
  (Audio|Components|Audio|Stop (Variables|Default|GetBrush_Blank)))

(event EventBeginPlay
  (bind _numberofpaintpoints (Variables|Default|GetNumberOfPaintPoints))
  (bind _paintlocation (Variables|Default|GetPaintLocation))
  (bind _relativelocation (Variables|/Script/Engine.SceneComponent|GetRelativeLocation _paintlocation))
  (bind _returnvalue (Math|Transform|MakeTransform _relativelocation))
  ;[1 1 1] Sets reference to paintbrush, Spawns a child bp called "paint" that holds all paint particles and ensures correct painting effect, even with customized children
  (bind _returnvalue_2 (Actor|GetActorOfClass "/Game/Blueprints/Paintbrush/Paintrbsuh.Paintrbsuh_C"))
  (Variables|Default|SetBrushRefVar _returnvalue_2)
  (Utilities|FlowControl|Sequence
    (:then_0
      (if (Variables|Default|GetIncludeGrowth)
        (bind _returnvalue_3 (Game|SpawnActorfromClass "/Game/Blueprints/Palette/BP_MainGreenPaint.BP_MainGreenPaint_C" _returnvalue "Undefined" 0 300 _relativelocation false "0.000000,0.000000,0.000000" 0))
        (bind _output_get (Variables|Default|SetMainGreen _returnvalue_3))
        (Transformation|AttachComponentToComponent _output_get _paintlocation "None" "KeepRelative" "KeepRelative" "KeepRelative" true)
        (bind _returnvalue_4 (Game|SpawnActorfromClass "/Game/Blueprints/Palette/BP_GreenPaint2.BP_GreenPaint2_C" _returnvalue "Undefined" 0 _numberofpaintpoints _relativelocation 0))
        (bind _output_get_2 (Variables|Default|SetSubGreenPaint _returnvalue_4))
        (Transformation|AttachComponentToComponent _output_get_2 _paintlocation "None" "KeepRelative" "KeepRelative" "KeepRelative" true)))
    (:then_1
      (if (Variables|Default|GetIncludeConduits)
        (Rendering|SetVisibility (Variables|Default|GetMagicHolder) true false)))
    (:then_2
      (bind _returnvalue_5 (Game|SpawnActorfromClass "/Game/Blueprints/Palette/BP_Paint.BP_Paint_C" _returnvalue "Undefined" 0 50 _relativelocation 0))
      (bind _output_get_3 (Variables|Default|SetWhitePaint _returnvalue_5))
      (Transformation|AttachComponentToComponent _output_get_3 _paintlocation "None" "KeepRelative" "KeepRelative" "KeepRelative" true)
      (bind _returnvalue_6 (Game|SpawnActorfromClass "/Game/Blueprints/Palette/BP_RedPaint.BP_RedPaint_C" _returnvalue "Undefined" 0 _numberofpaintpoints _relativelocation (Variables|/Script/Engine.SceneComponent|GetRelativeLocation (Variables|Default|GetBeginPoint)) 0))
      (bind _output_get_4 (Variables|Default|SetRedPaint _returnvalue_6))
      (Transformation|AttachComponentToComponent _output_get_4 _paintlocation "None" "KeepRelative" "KeepRelative" "KeepRelative" true))))

(fn ConstructionScript)