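; Paintable dot actor for the Classroom Backdoor, Library Gate, Library Tree and Library Apple puzzles, with its owning puzzle actor chosen by enum and found on BeginPlay.
; When the paintbrush's collision sphere overlaps it in one specific paint mode, it becomes primed, swaps visible meshes and plays sink and paint-grow timelines.
; Reset reverses this, and both changes call UpdatePrimedList on the owning puzzle.
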(event OnComponentBeginOverlap(BrushCheckCollision)
  (params (OverlappedComponent :type Primitive%20Component%20Object%20Reference) (OtherActor :type Actor%20Object%20Reference) (OtherComp :type Primitive%20Component%20Object%20Reference) (OtherBodyIndex :type Integer) (bFromSweep :type Boolean) (SweepResult :type Hit%20Result%20Structure%20%28by%20ref%29))
  (bind _brush_ref (Variables|Default|GetBrush%20Ref))
  (if (== (Variables|/Game/Blueprints/Paintbrush/Paintrbsuh.Paintrbsuh_C|GetCollisionSphere _brush_ref) OtherComp)
    (if (Utilities|Enum|Equal(Enum) (Variables|/Game/Blueprints/Paintbrush/Paintrbsuh.Paintrbsuh_C|GetEnum%20Paints _brush_ref) "NewEnumerator4")
      (if (not (Variables|Default|GetPrimed?))
        (Variables|Default|SetPrimed? true)
        (Rendering|SetVisibility (Variables|Default|GetDarl) true false)
        (Rendering|SetVisibility (Variables|Default|GetStaticMesh) false false)
        (Utilities|FlowControl|Sequence
          (:then_0
            (bind _newtrack_0 (Timeline|Timeline_0 PlayFromStart)
              (:Update
                (Transformation|SetRelativeLocation (Variables|Default|GetFlatTransform) (Math|Vector|Lerp(Vector) "0, 0, 0" "0, 0,-2.000000" _newtrack_0) false false))))
          (:then_1
            (switch Utilities|FlowControl|Switch|SwitchonRoomEnum (Variables|Default|Getenum)
              (:NewEnumerator5
                (Default|UpdatePrimedList (Variables|Default|GetComduitRef)))
              (:NewEnumerator6
                (Default|UpdatePrimedList (Variables|Default|GetGateRef)))
              (:NewEnumerator7
                (Default|UpdatePrimedList (Variables|Default|GetTreeRing)))
              (:NewEnumerator9
                (Default|UpdatePrimedList (Variables|Default|GetAppleTables%20Ref)))))
          (:then_2
            (bind _newtrack_0_2 (Timeline|Timeline_1 Play)
              (:Update
                (Transformation|SetRelativeScale3D (Variables|Default|GetPaintTransform) (Math|Vector|Lerp(Vector) "0.010000,0.010000,0.010000" "1.000000,1.000000,1.000000" _newtrack_0_2))))))))))

(event Custom|Reset
  (if (Variables|Default|GetPrimed?)
    (Variables|Default|SetPrimed? false)
    (Rendering|SetVisibility (Variables|Default|GetDarl) false false)
    (Rendering|SetVisibility (Variables|Default|GetStaticMesh) true false)
    (Utilities|FlowControl|Sequence
      (:then_0
        (bind _newtrack_0 (Timeline|Timeline_0 ReverseFromEnd)
          (:Update
            (Transformation|SetRelativeLocation (Variables|Default|GetFlatTransform) (Math|Vector|Lerp(Vector) "0, 0, 0" "0, 0,-2.000000" _newtrack_0) false false))))
      (:then_1
        (switch Utilities|FlowControl|Switch|SwitchonRoomEnum (Variables|Default|Getenum)
          (:NewEnumerator5
            (Default|UpdatePrimedList (Variables|Default|GetComduitRef)))
          (:NewEnumerator6
            (Default|UpdatePrimedList (Variables|Default|GetGateRef)))
          (:NewEnumerator7
            (Default|UpdatePrimedList (Variables|Default|GetTreeRing)))
          (:NewEnumerator9
            (Default|UpdatePrimedList (Variables|Default|GetAppleTables%20Ref)))))
      (:then_2
        (bind _newtrack_0_2 (Timeline|Timeline_1 Reverse)
          (:Update
            (Transformation|SetRelativeScale3D (Variables|Default|GetPaintTransform) (Math|Vector|Lerp(Vector) "0.010000,0.010000,0.010000" "1.000000,1.000000,1.000000" _newtrack_0_2))))))))

(event EventBeginPlay
  (bind _returnvalue (Actor|GetActorOfClass "/Game/Blueprints/Paintbrush/Paintrbsuh.Paintrbsuh_C"))
  (Variables|Default|SetBrush%20Ref _returnvalue)
  (switch Utilities|FlowControl|Switch|SwitchonRoomEnum (Variables|Default|Getenum)
    (:NewEnumerator5
      (bind _returnvalue_2 (Actor|GetActorOfClass "/Game/Blueprints/PuzzleElements/BP_Conduit_Backdoor.BP_Conduit_Backdoor_C"))
      (Variables|Default|SetComduitRef _returnvalue_2))
    (:NewEnumerator6
      (bind _returnvalue_3 (Actor|GetActorOfClass "/Game/Blueprints/PuzzleElements/BP_SurfaceGate.BP_SurfaceGate_C"))
      (Variables|Default|SetGateRef _returnvalue_3))
    (:NewEnumerator7
      (bind _returnvalue_4 (Actor|GetActorOfClass "/Game/Blueprints/PuzzleElements/BP_TreeDrawRing.BP_TreeDrawRing_C"))
      (Variables|Default|SetTreeRing _returnvalue_4))
    (:NewEnumerator9
      (bind _returnvalue_5 (Actor|GetActorOfClass "/Game/Blueprints/PuzzleElements/BP_LibraryTables.BP_LibraryTables_C"))
      (Variables|Default|SetAppleTables%20Ref _returnvalue_5))))

(event Collision|EventActorBeginOverlap
  (params (OtherActor :type Actor%20Object%20Reference)))

(event EventTick
  (params (DeltaSeconds :type Float%20%28single-precision%29)))

(fn ConstructionScript)