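; Trigger volume that plays audio hints when the VR pawn enters while a chosen puzzle is still unsolved.
; A HintSystem enum selects immediate, do-once, delayed, or gated delayed puzzle timing.
; CheckIncompletion maps the Puzzle enum to state flags on the paintbrush, paint palette and boiler pipes, found at BeginPlay.
; If the check passes, the paintbrush plays the HintAudio dialogue; otherwise the gate closes until an overlap ends.
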(event OnComponentBeginOverlap(Box)
  (params (OverlappedComponent :type Primitive%20Component%20Object%20Reference) (OtherActor :type Actor%20Object%20Reference) (OtherComp :type Primitive%20Component%20Object%20Reference) (OtherBodyIndex :type Integer) (bFromSweep :type Boolean) (SweepResult :type Hit%20Result%20Structure%20%28by%20ref%29))
  (Utilities|Casting|CastToBP_UpdatedVRPawn OtherActor)
  (switch Utilities|FlowControl|Switch|SwitchonHintSystems (Variables|Default|GetHintSystem)
    (:NewEnumerator0
      ;[1 1 1] After 20 seconds,
      (Utilities|FlowControl|Delay (Variables|Default|GetDelayTime))
      ;[1 1 1] Use puzzle enum to specify which puzzle to check for the puzzle state
      (Utilities|FlowControl|Gate true
        (:Exit
          _)))
    (:NewEnumerator2
      (Utilities|FlowControl|Delay (Variables|Default|GetDelayTime)))
    (:NewEnumerator1
      _)
    (:NewEnumerator3
      (Utilities|FlowControl|DoOnce false
        (:Completed
          _))))
  (Utilities|PuzzleIncompletionBranch (Variables|Default|GetPuzzle)
    (:true
      (CallFunction|PlayHintSound))
    (:false
      (CallFunction|DontPlaySound))))

(event OnComponentEndOverlap(Box)
  (params (OverlappedComponent :type Primitive%20Component%20Object%20Reference) (OtherActor :type Actor%20Object%20Reference) (OtherComp :type Primitive%20Component%20Object%20Reference) (OtherBodyIndex :type Integer))
  ;[1 1 1] Use puzzle enum to specify which puzzle to check for the puzzle state
  (Utilities|FlowControl|Gate true) ; enters at Open
)

(event Custom|DontPlaySound
  ;[1 1 1] Use puzzle enum to specify which puzzle to check for the puzzle state
  (Utilities|FlowControl|Gate true) ; enters at Close
)

(event EventBeginPlay
  (Utilities|FlowControl|Sequence
    (:then_0
      (bind _returnvalue (Actor|GetActorOfClass "/Game/Blueprints/Paintbrush/Paintrbsuh.Paintrbsuh_C"))
      (Variables|Default|SetPaintbrushBP _returnvalue)
      (bind _returnvalue_2 (Actor|GetActorOfClass "/Game/Blueprints/PuzzleElements/BoilerPipes.BoilerPipes_C"))
      (Variables|Default|SetBoilerPipesRef _returnvalue_2)
      (bind _returnvalue_3 (Actor|GetActorOfClass "/Game/Blueprints/Palette/BP_Swatch.BP_Swatch_C"))
      (Variables|Default|SetPaintPaletteRef _returnvalue_3))))

(fn ConstructionScript)

(fn CheckIncompletion
  (params (Puzzle :type RoomEnum%20Enum :default "NewEnumerator0"))
  (bind _paintbrushbp (Variables|Default|GetPaintbrushBP))
  (bind _paintbrushbp_2 (Variables|Default|GetPaintbrushBP))
  (bind _paintpaletteref (Variables|Default|GetPaintPaletteRef))
  (bind _boilerpipesref (Variables|Default|GetBoilerPipesRef))
  (switch Utilities|FlowControl|Switch|SwitchonRoomEnum Puzzle
    (:NewEnumerator0
      ;[1 1 1] DipTheRedPaint!
      (Variables|Default|SetPuzzleComplete? (and (not (Variables|/Game/Blueprints/Palette/BP_Swatch.BP_Swatch_C|GetPaint1on _paintpaletteref)) (Variables|/Game/Blueprints/Palette/BP_Swatch.BP_Swatch_C|GetHasPaint1 _paintpaletteref))))
    (:NewEnumerator19
      (Variables|Default|SetPuzzleComplete? (not (Variables|/Game/Blueprints/Palette/BP_Swatch.BP_Swatch_C|GetHasPaint1 (Variables|Default|GetPaintPaletteRef)))))
    (:NewEnumerator2
      ;[1 1 1] BoilerWater
      (Variables|Default|SetPuzzleComplete? (and (not (Variables|/Game/Blueprints/Paintbrush/Paintrbsuh.Paintrbsuh_C|GetBoilPz_WaterInBoiler? (Variables|Default|GetPaintbrushBP))) (Variables|/Game/Blueprints/Paintbrush/Paintrbsuh.Paintrbsuh_C|GetBoilPz_Conduit? (Variables|Default|GetPaintbrushBP)))))
    (:NewEnumerator11
      ;[1 1 1] BoilerConduit
      (Variables|Default|SetPuzzleComplete? (and (or (Variables|/Game/Blueprints/PuzzleElements/BoilerPipes.BoilerPipes_C|GetRight _boilerpipesref) (Variables|/Game/Blueprints/PuzzleElements/BoilerPipes.BoilerPipes_C|GetDown _boilerpipesref)) (not (Variables|/Game/Blueprints/Paintbrush/Paintrbsuh.Paintrbsuh_C|GetBoilPz_Conduit? (Variables|Default|GetPaintbrushBP))))))
    (:NewEnumerator10
      ;[1 1 1] BoilerGear
      (Variables|Default|SetPuzzleComplete? (not (Variables|/Game/Blueprints/Paintbrush/Paintrbsuh.Paintrbsuh_C|GetBoilPz_Gear? (Variables|Default|GetPaintbrushBP)))))
    (:NewEnumerator13
      ;[1 1 1] GrindConduit
      (Variables|Default|SetPuzzleComplete? (not (Variables|/Game/Blueprints/Paintbrush/Paintrbsuh.Paintrbsuh_C|GetGrindPz_Conduit? (Variables|Default|GetPaintbrushBP)))))
    (:NewEnumerator12
      ;[1 1 1] GrindPipe
      (Variables|Default|SetPuzzleComplete? (not (Variables|/Game/Blueprints/Paintbrush/Paintrbsuh.Paintrbsuh_C|GetGrindPz_Pipe? (Variables|Default|GetPaintbrushBP)))))
    (:NewEnumerator14
      ;[1 1 1] GrindWaterWheel
      (Variables|Default|SetPuzzleComplete? (not (Variables|/Game/Blueprints/Paintbrush/Paintrbsuh.Paintrbsuh_C|GetGrindPz_Waterwheel? (Variables|Default|GetPaintbrushBP)))))
    (:NewEnumerator15
      ;[1 1 1] ChemConduitPiece
      (Variables|Default|SetPuzzleComplete? (not (Variables|/Game/Blueprints/Paintbrush/Paintrbsuh.Paintrbsuh_C|GetChemPz_ConPiece? (Variables|Default|GetPaintbrushBP)))))
    (:NewEnumerator5
      ;[1 1 1] No green paint? Get it!
      (Variables|Default|SetPuzzleComplete? (not (Variables|/Game/Blueprints/Palette/BP_Swatch.BP_Swatch_C|GetHasPaint2 (Variables|Default|GetPaintPaletteRef)))))
    (:NewEnumerator16
      ;[1 1 1] ButtonPress
      (Variables|Default|SetPuzzleComplete? (Math|Boolean|ANDBoolean (Variables|/Game/Blueprints/Paintbrush/Paintrbsuh.Paintrbsuh_C|GetCauld_HerbPressable? _paintbrushbp_2) (Variables|/Game/Blueprints/Paintbrush/Paintrbsuh.Paintrbsuh_C|GetCauld_MagicPressble? _paintbrushbp_2) (Variables|/Game/Blueprints/Paintbrush/Paintrbsuh.Paintrbsuh_C|GetCauld_FirePressable? _paintbrushbp_2) (not (Variables|/Game/Blueprints/Paintbrush/Paintrbsuh.Paintrbsuh_C|GetButtonsPressed? _paintbrushbp_2)))))
    (:NewEnumerator17
      ;[1 1 1] GreenPaintDip
      (Variables|Default|SetPuzzleComplete? (and (Variables|/Game/Blueprints/Paintbrush/Paintrbsuh.Paintrbsuh_C|GetButtonsPressed? _paintbrushbp) (not (Variables|/Game/Blueprints/Paintbrush/Paintrbsuh.Paintrbsuh_C|GetPaint2Imbued _paintbrushbp)))))
    (:NewEnumerator18
      (Variables|Default|SetPuzzleComplete? true))
    (:NewEnumerator20
      ;[1 1 1] FrogInsideTube
      (Variables|Default|SetPuzzleComplete? (not (Variables|/Game/Blueprints/Paintbrush/Paintrbsuh.Paintrbsuh_C|GetFrogInsideTube? (Variables|Default|GetPaintbrushBP)))))
    (:NewEnumerator21
      (Variables|Default|SetPuzzleComplete? (not (Variables|/Game/Blueprints/Paintbrush/Paintrbsuh.Paintrbsuh_C|GetDirectoadAppleFed? (Variables|Default|GetPaintbrushBP)))))
    (:NewEnumerator22
      (Variables|Default|SetPuzzleComplete? (not (Variables|/Game/Blueprints/Paintbrush/Paintrbsuh.Paintrbsuh_C|GetDirectoadJewelFed? (Variables|Default|GetPaintbrushBP)))))
    (:NewEnumerator23
      (Variables|Default|SetPuzzleComplete? (not (Variables|/Game/Blueprints/Paintbrush/Paintrbsuh.Paintrbsuh_C|GetDirectoadBookFed? (Variables|Default|GetPaintbrushBP)))))
    (:NewEnumerator24
      (Variables|Default|SetPuzzleComplete? (not (Variables|/Game/Blueprints/Paintbrush/Paintrbsuh.Paintrbsuh_C|GetLibraryCouldronComplete? (Variables|Default|GetPaintbrushBP)))))
    (:NewEnumerator25
      (Variables|Default|SetPuzzleComplete? (not (Variables|/Game/Blueprints/Paintbrush/Paintrbsuh.Paintrbsuh_C|GetPurplePaintUnlocked? (Variables|Default|GetPaintbrushBP)))))
    (:NewEnumerator26
      (Variables|Default|SetPuzzleComplete? (not (Variables|/Game/Blueprints/Paintbrush/Paintrbsuh.Paintrbsuh_C|GetFruitGrown? (Variables|Default|GetPaintbrushBP)))))
    (:NewEnumerator27
      (Variables|Default|SetPuzzleComplete? (not (Variables|/Game/Blueprints/Paintbrush/Paintrbsuh.Paintrbsuh_C|GetLunchboxUnlocked? (Variables|Default|GetPaintbrushBP)))))
    (:NewEnumerator28
      (Variables|Default|SetPuzzleComplete? (not (Variables|/Game/Blueprints/Paintbrush/Paintrbsuh.Paintrbsuh_C|GetRestrictedGateUnlocked? (Variables|Default|GetPaintbrushBP)))))
    (:NewEnumerator29
      (Variables|Default|SetPuzzleComplete? (not (Variables|/Game/Blueprints/Paintbrush/Paintrbsuh.Paintrbsuh_C|GetshelvesPushedInPlace? (Variables|Default|GetPaintbrushBP)))))
    (:NewEnumerator30
      (Variables|Default|SetPuzzleComplete? (not (Variables|/Game/Blueprints/Paintbrush/Paintrbsuh.Paintrbsuh_C|GetRestrictedAreaButtonPushed? (Variables|Default|GetPaintbrushBP)))))
    (:NewEnumerator31
      (Variables|Default|SetPuzzleComplete? (not (Variables|/Game/Blueprints/Paintbrush/Paintrbsuh.Paintrbsuh_C|GetRestrictedAreaGemObtained? (Variables|Default|GetPaintbrushBP)))))
    (:NewEnumerator32
      (Variables|Default|SetPuzzleComplete? (and (not (Variables|/Game/Blueprints/Paintbrush/Paintrbsuh.Paintrbsuh_C|GetRestrictedAreaPlanetsAlligned? (Variables|Default|GetPaintbrushBP))) (Variables|/Game/Blueprints/Paintbrush/Paintrbsuh.Paintrbsuh_C|GetRestrictedAreaButtonPushed? (Variables|Default|GetPaintbrushBP))))))
  (return (Variables|Default|GetPuzzleComplete?)))

(fn PlayHintSound
  ;[1 1 1] Play hint sound
  (for _array_element (Variables|Default|GetHintAudio)
    (Default|PlayDialogueSound (Variables|Default|GetPaintbrushBP) (Variables|Default|GetOverwrite%20Sound?) _array_element)))