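; Purple paint projectile that animates a cluster of orb components to look like pulsing, dripping paint; its graph holds only this cosmetic animation.
; On BeginPlay, one timeline pulses the scale of five core orbs.
; SpawnIn loops after a random delay, using a FlipFlop between two timelines that each lower and rescale a random one of four satellite orbs.
; SpawnOut is an empty stub.
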(event Custom|SpawnOut)

(event Custom|SpawnIn
  (bind _purpleorb_2 (Variables|Default|GetPurpleOrb_2))
  (bind _purpleorb_3 (Variables|Default|GetPurpleOrb_3))
  (bind _particlemax (Variables|Default|GetParticleMax))
  (bind _particlemin (Variables|Default|GetParticleMin))
  (bind _purpleorb_4 (Variables|Default|GetPurpleOrb_4))
  (bind _purpleorb_5 (Variables|Default|GetPurpleOrb_5))
  (bind _purpleorb_2_2 (Variables|Default|GetPurpleOrb_2))
  (bind _purpleorb_3_2 (Variables|Default|GetPurpleOrb_3))
  (bind _purpleorb_4_2 (Variables|Default|GetPurpleOrb_4))
  (bind _purpleorb_5_2 (Variables|Default|GetPurpleOrb_5))
  (Utilities|FlowControl|Delay (Math|Random|RandomFloatinRange 0.0 0.4))
  (Utilities|FlowControl|FlipFlop
    (:A
      (bind _output_get (Variables|Default|SetRandPoint (Math|Random|RandomIntegerinRange 0 3)))
      (bind _newtrack_0 (Timeline|Timeline_1 PlayFromStart)
        (:Update
          (switch int _output_get
            (:0
              (Transformation|SetRelativeLocation _purpleorb_5_2 (Math|Vector|Lerp(Vector) "3.500000,0.000000,-1.000000" "0, 0,-22.000000" _newtrack_0) false false)
              (Transformation|SetRelativeScale3D _purpleorb_5_2 (Math|Vector|Lerp(Vector) _particlemax _particlemin _newtrack_0)))
            (:1
              (Transformation|SetRelativeLocation _purpleorb_4_2 (Math|Vector|Lerp(Vector) "-3.500000,0.000000,-1.000000" "-3.500000, 0,-22.000000" _newtrack_0) false false)
              (Transformation|SetRelativeScale3D _purpleorb_4_2 (Math|Vector|Lerp(Vector) _particlemax _particlemin _newtrack_0)))
            (:2
              (Transformation|SetRelativeLocation _purpleorb_3_2 (Math|Vector|Lerp(Vector) "0,-3.500000,-1.000000" "0,-3.500000,-22.000000" _newtrack_0) false false)
              (Transformation|SetRelativeScale3D _purpleorb_3_2 (Math|Vector|Lerp(Vector) _particlemax _particlemin _newtrack_0)))
            (:3
              (Transformation|SetRelativeLocation _purpleorb_2_2 (Math|Vector|Lerp(Vector) "0,3.500000,-1.000000" "0,3.500000,-22.000000" _newtrack_0) false false)
              (Transformation|SetRelativeScale3D _purpleorb_2_2 (Math|Vector|Lerp(Vector) _particlemax _particlemin _newtrack_0)))))
        (:Finished
          (CallFunction|Spawnin :!label _label))))
    (:B
      (bind _output_get_2 (Variables|Default|SetRandPoint (Math|Random|RandomIntegerinRange 0 3)))
      (bind _newtrack_0_2 (Timeline|Timeline_2 PlayFromStart)
        (:Update
          (switch int _output_get_2
            (:0
              (Transformation|SetRelativeLocation _purpleorb_5 (Math|Vector|Lerp(Vector) "3.500000,0.000000,-1.000000" "3.500000, 0,-22.000000" _newtrack_0_2) false false)
              (Transformation|SetRelativeScale3D _purpleorb_5 (Math|Vector|Lerp(Vector) _particlemax _particlemin _newtrack_0_2)))
            (:1
              (Transformation|SetRelativeLocation _purpleorb_4 (Math|Vector|Lerp(Vector) "-3.500000,0.000000,-1.000000" "-3.500000, 0,-22.000000" _newtrack_0_2) false false)
              (Transformation|SetRelativeScale3D _purpleorb_4 (Math|Vector|Lerp(Vector) _particlemax _particlemin _newtrack_0_2)))
            (:2
              (Transformation|SetRelativeLocation _purpleorb_3 (Math|Vector|Lerp(Vector) "0,-3.500000,-1.000000" "0,-3.500000,-22.000000" _newtrack_0_2) false false)
              (Transformation|SetRelativeScale3D _purpleorb_3 (Math|Vector|Lerp(Vector) _particlemax _particlemin _newtrack_0_2)))
            (:3
              (Transformation|SetRelativeLocation _purpleorb_2 (Math|Vector|Lerp(Vector) "0,3.500000,-1.000000" "0,3.500000,-22.000000" _newtrack_0_2) false false)
              (Transformation|SetRelativeScale3D _purpleorb_2 (Math|Vector|Lerp(Vector) _particlemax _particlemin _newtrack_0_2)))))
        (:Finished
          (goto _label))))))

(event EventBeginPlay
  (CallFunction|Spawnin)
  (bind _newtrack_0 (Timeline|Timeline_3 PlayFromStart)
    (:Update
      (Transformation|SetRelativeScale3D (Variables|Default|GetPurpleOrb_1) (Math|Vector|Lerp(Vector) "1.000000,1.000000,1.000000" "1.200000,1.200000,1.200000" _newtrack_0))
      (Transformation|SetRelativeScale3D (Variables|Default|GetPurpleOrb_7) (Math|Vector|Lerp(Vector) "0.450000,0.450000,0.450000" "0.500000,0.500000,0.500000" _newtrack_0))
      (Transformation|SetRelativeScale3D (Variables|Default|GetPurpleOrb_6) (Math|Vector|Lerp(Vector) "0.350000,0.350000,0.350000" "0.540000,0.540000,0.540000" _newtrack_0))
      (Transformation|SetRelativeScale3D (Variables|Default|GetPurpleOrb_9) (Math|Vector|Lerp(Vector) "0.400000,0.400000,0.400000" "0.500000,0.500000,0.500000" _newtrack_0))
      (Transformation|SetRelativeScale3D (Variables|Default|GetPurpleOrb_8) (Math|Vector|Lerp(Vector) "0.200000,0.200000,0.200000" "0.350000,0.350000,0.350000" _newtrack_0)))))

(fn ConstructionScript)