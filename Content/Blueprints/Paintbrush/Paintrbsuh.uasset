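; Talking VR paintbrush that gains paints from a cauldron and narrates the intro and classroom puzzles.
; Dipping runs shake and glow timelines, then imbues the color, updates BP_Swatch and shows conduit or plant particles pooled by relocation.
; Load and UnLoad switch animated tip meshes and return paint to the swatch.
; Dialogue uses an interruptible sound queue with a blinking talk glow, driven by intro, grab and puzzle-completion events.
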(event OnDropped(GrabComponent)
  (bind _ring (Variables|Default|GetRing))
  ;[1 1 1] On grabbed. Shows rune ring and sets correct position
  (Variables|Default|SetGrabbed false)
  (Utilities|FlowControl|Sequence
    (:then_0
      (bind _newtrack_0 (Timeline|Timeline_2 Reverse)
        (:Update
          (Transformation|SetRelativeRotation _ring (Math|Rotator|Lerp(Rotator) "0,660.000000, 0" "0,90.000000, 0" _newtrack_0) false false)
          (Transformation|SetRelativeScale3D _ring (Math|Vector|Lerp(Vector) "0, 0, 0" "0.900000,0.900000,-0.500000" _newtrack_0)))))
    (:then_1
      (Timeline|Timeline_5 Stop))))

(event OnGrabbed(GrabComponent)
  ;[1 1 1] On grabbed. Shows rune ring and sets correct position
  (Variables|Default|SetGrabbed true)
  (Variables|DiaIntro|SetFirstGrab true)
  (Variables|Default|SetRelative%20Rotation (Variables|/Script/Engine.SceneComponent|GetRelativeRotation (Variables|Default|GetPaintbrushBase)))
  (Utilities|FlowControl|Sequence
    (:then_0
      (Default|BrushGrab (Variables|References|GetVRRef) (Variables|Default|GetGrabComponent))
      (if (Variables|Default|GetPaint1Imbued)
        (if (Variables|Default|GetPaint1_OnBrush)
          _)))
    (:then_1
      (Utilities|FlowControl|DoOnce false
        (:Completed
          (CallFunction|TransportationSeq))))))

(event OnAudioFinished(A_Dialogue1)
  ;[0 0 0] DIALOGUE SYSTEM
  ;;[1 1 1] Dialogue cue play (replace old one)
)

(event OnAudioFinished(A_Dialogue)
  ;[1 0.3901 0.07513] Dialogue system
  ;;[0 0 0] On audio ends
  ;;;[1 1 1] Check the sound index against the sound queue length
  (if (< (Variables|DiaLogic|GetsoundQueueIndex) (- (Utilities|Array|Length (Variables|DiaLogic|GetSoundQueue)) 1))
    ;;;[1 1 1] If there are sounds in the sound queue, play sound from queue
    (Audio|Components|Audio|SetSound (Variables|Default|GetA_Dialogue) (Utilities|Array|Get(acopy) (Variables|DiaLogic|GetSoundQueue) (Variables|DiaLogic|GetsoundQueueIndex)))
    (Utilities|FlowControl|Delay 0.5)
    (Audio|Components|Audio|Play (Variables|Default|GetA_Dialogue) 0.0)
    (Math|Integer|IncrementInt (Variables|DiaLogic|GetsoundQueueIndex))
    (else
      (CallFunction|PaintbrushNotTalkingState)
      (Utilities|Array|Clear (Variables|DiaLogic|GetSoundQueue))
      (Variables|DiaLogic|SetsoundQueueIndex 0))))

(event Custom|PlayDialogueCue
  (params (DialogueLineSound :type Sound%20Base%20Object%20Reference) (OverrideSound :type Boolean))
  ;[0 0 0] DIALOGUE SYSTEM
  ;;[1 1 1] Dialogue cue play (replace old one)
)

(event Custom|Paint1_Cleared
  ;[1 1 1] Brush Prime Events - Paintability for Conduit Power
)

(event Custom|CompleteGrinder
  ;[1 1 1] PuzzlesCompleteDialogue
  (Utilities|FlowControl|DoOnce false
    (:Completed
      (CallFunction|PlayDialogueSound true "/Game/Audio-Revised/Assets/Dialogue/Dia_wav/Dia_M1_Grind_6.Dia_M1_Grind_6")
      (Variables|PuzzleStatusClass|SetGrindPz_Complete? true)
      (Variables|PuzzleStatusClass|SetGrindPz_Pipe? true)
      (Variables|PuzzleStatusClass|SetGrindPz_Conduit? true)
      (Variables|PuzzleStatusClass|SetGrindPz_Waterwheel? true)
      (CallFunction|ClassroomCompletion))))

(event Custom|Exited
  (bind _swatch_ref (Variables|References|GetSwatch_Ref))
  (bind _swatch_ref_2 (Variables|References|GetSwatch_Ref))
  ;[1 1 1] Beginplay, sets reference to VR BP
  (switch Utilities|FlowControl|Switch|SwitchonEnum_Paints (Variables|Default|GetEnum%20Paints)
    (:NewEnumerator3
      (Variables|/Game/Blueprints/Palette/BP_Swatch.BP_Swatch_C|SetPaint1on _swatch_ref_2 false :!label _label)
      (Default|Glob1Grow _swatch_ref))
    (:NewEnumerator0
      (goto _label))
    (:NewEnumerator4
      (Variables|/Game/Blueprints/Palette/BP_Swatch.BP_Swatch_C|SetPaint2on _swatch_ref_2 false)
      (Default|Glob2Grow _swatch_ref))
    (:NewEnumerator5
      (Variables|/Game/Blueprints/Palette/BP_Swatch.BP_Swatch_C|SetPaint3on _swatch_ref false)
      (Default|Glob3Grow _swatch_ref))))

(event Custom|Entered
  ;[1 1 1] Beginplay, sets reference to VR BP
)

(event Custom|Paint1_Dipped
  ;[1 1 1] Brush Prime Events - Paintability for Conduit Power
)

(event Custom|IntroSequence
  ;[0 0 0] DIALOGUE SYSTEM
  (Utilities|FlowControl|Delay 3.0)
  (CallFunction|PlayDialogueCue "/Game/Audio-Revised/Assets/Dialogue/Dia_wav/Dia_M1_Intro_1p_1.Dia_M1_Intro_1p_1" false)
  (Utilities|FlowControl|Delay 7.0)
  (CallFunction|PlayDialogueCue "/Game/Audio-Revised/Assets/Dialogue/Dia_wav/Dia_M1_Intro_1p_3.Dia_M1_Intro_1p_3" false)
  (Utilities|FlowControl|Delay 7.0)
  (CallFunction|PlayDialogueCue "/Game/Audio-Revised/Assets/Dialogue/Dia_wav/Dia_M1_Intro_1p_2.Dia_M1_Intro_1p_2" false)
  (Utilities|FlowControl|Delay 7.0)
  (CallFunction|PlayDialogueCue "/Game/Audio-Revised/Assets/Dialogue/Dia_wav/Dia_M1_Intro_1p_4.Dia_M1_Intro_1p_4" false)
  (Utilities|FlowControl|Delay 7.0)
  (CallFunction|PlayDialogueCue "/Game/Audio-Revised/Assets/Dialogue/Dia_wav/Dia_M1_Intro_1p_5.Dia_M1_Intro_1p_5" false)
  (Utilities|FlowControl|Delay 7.0)
  (if (not (Variables|DiaIntro|GetFirstGrab))
    (CallFunction|PlayDialogueCue "/Game/Audio-Revised/Assets/Dialogue/Dia_wav/Dia_M1_Intro_PU_1.Dia_M1_Intro_PU_1" false)
    (Utilities|FlowControl|Delay 7.0)
    (CallFunction|PlayDialogueCue "/Game/Audio-Revised/Assets/Dialogue/Dia_wav/Dia_M1_Intro_PU_4.Dia_M1_Intro_PU_4" false)
    (Utilities|FlowControl|Delay 7.0)))

(event Custom|PlayHint
  (params (HintDialogue :type Sound%20Base%20Object%20Reference))
  ;[0 0 0] DIALOGUE SYSTEM
  ;;[1 1 1] Play hint (on delay)
)

(event Custom|ClassroomCompletion
  ;[1 1 1] ClassroomComplete
  (if (Math|Boolean|ANDBoolean (Variables|PuzzleStatusClass|GetBoilPz_Complete?) (Variables|PuzzleStatusClass|GetGrindPz_Complete?) (Variables|PuzzleStatusClass|GetChemPz_Complete?))
    (Variables|PuzzleStatusClass|SetClassPz_Complete? true)
    (CallFunction|PlayDialogueSound false "/Game/Audio-Revised/Assets/Dialogue/Dia_wav/Dia_M1_Caul_1.Dia_M1_Caul_1")))

(event Custom|HintValid?
  (params (HintDialogue :type Sound%20Base%20Object%20Reference))
  ;[0 0 0] DIALOGUE SYSTEM
)

(event Custom|DeacPlantImbueParticle
  ;[1 1 1] Plant Imbuement Particle Pooling System
  (Transformation|SetWorldLocation (Variables|Default|GetPlantImbue) (Variables|Default|GetPoolLocation) false false))

(event Custom|ActiPlantImbueParticle
  ;[1 1 1] Plant Imbuement Particle Pooling System
  (Transformation|SetRelativeLocation (Variables|Default|GetPlantImbue) (Variables|Default|GetParticleSpawnLo) false false)
  (Utilities|FlowControl|Delay 6.0)
  (bind _fadeout (Timeline|Timeline_7 Play)
    (:Update
      (Transformation|SetRelativeScale3D (Variables|Default|GetPlantImbue) (Math|Vector|Lerp(Vector) "62.940594,62.940594,50.156384" "0, 0, 0" _fadeout)))
    (:Finished
      (CallFunction|DeacPlantImbueParticle))))

(event Custom|CompleteBoiler
  ;[1 1 1] PuzzlesCompleteDialogue
  (Utilities|FlowControl|DoOnce false
    (:Completed
      (CallFunction|PlayDialogueSound true "/Game/Audio-Revised/Assets/Dialogue/Dia_wav/Dia_M1_Boil_5.Dia_M1_Boil_5")
      (Variables|PuzzleStatusClass|SetBoilPz_Complete? true)
      (Variables|PuzzleStatusClass|SetBoilPz_Conduit? true)
      (Variables|PuzzleStatusClass|SetBoilPz_WaterInBoiler? true)
      (Variables|PuzzleStatusClass|SetBoilPz_Gear? true)
      (CallFunction|ClassroomCompletion))))

(event Custom|DeacConduitImbueParticle
  ;[1 1 1] ConduitImbuement Particle Pooling System
  (Transformation|SetWorldLocation (Variables|Default|GetConduitImbue) (Variables|Default|GetPoolLocation) false false))

(event Custom|ActiConduitImbueParticle
  ;[1 1 1] ConduitImbuement Particle Pooling System
  (Transformation|SetRelativeLocation (Variables|Default|GetConduitImbue) (Variables|Default|GetParticleSpawnLo) false false)
  (Utilities|FlowControl|Delay 4.0)
  (bind _fadeout (Timeline|Timeline_6 Play)
    (:Update
      (Transformation|SetRelativeScale3D (Variables|Default|GetConduitImbue) (Math|Vector|Lerp(Vector) "62.940594,62.940594,50.156384" "0, 0, 0" _fadeout)))
    (:Finished
      (CallFunction|DeacConduitImbueParticle))))

(event Custom|PaintbrushNotTalkingState
  ;[1 1 1] Paintbrush talking visual cue
  (Utilities|FlowControl|Sequence
    (:then_0
      (bind _blinkingalpha (Timeline|Blinking Stop)
        (:Update
          (Transformation|SetRelativeScale3D (Variables|Default|GetGlow) (Math|Vector|Lerp(Vector) "8.000000,8.000000,8.000000" "18.000000,18.000000,18.000000" _blinkingalpha)))
        (:Finished
          ;;[1 1 1] RandomizeTalkSpeed
          (Components|Timeline|SetTimelineLength (Variables|Default|GetBlinking) (+ (Math|Float|SafeDivide (Math|Random|RandomFloat) 2.0) 0.5)))))
    (:then_1
      (Rendering|SetVisibility (Variables|Default|GetGlow) false false))))

(event Custom|PlayDialogueSequence
  (params (NewParam :type Array%20of%20Sound%20Base%20Object%20References) (delaytime :type Integer) (Index :type Integer))
  ;[1 1 1] Comment
)

(event Custom|PaintbrushTalkingState
  ;[1 1 1] Paintbrush talking visual cue
  (Rendering|SetVisibility (Variables|Default|GetGlow) true false)
  (bind _blinkingalpha (Timeline|Blinking Play)
    (:Update
      (Transformation|SetRelativeScale3D (Variables|Default|GetGlow) (Math|Vector|Lerp(Vector) "8.000000,8.000000,8.000000" "18.000000,18.000000,18.000000" _blinkingalpha)))
    (:Finished
      ;;[1 1 1] RandomizeTalkSpeed
      (Components|Timeline|SetTimelineLength (Variables|Default|GetBlinking) (+ (Math|Float|SafeDivide (Math|Random|RandomFloat) 2.0) 0.5)))))

(event Custom|PlayDialogueSound
  (params (OverwriteSound? :type Boolean) (Sound :type Sound%20Base%20Object%20Reference))
  ;[1 0.3901 0.07513] Dialogue system
  (CallFunction|PaintbrushTalkingState)
  (Variables|DiaLogic|SetOverwrite%20Sound? OverwriteSound?)
  ;;[1 1 1] Check if sound is playing
  (if (Audio|Components|Audio|IsPlaying (Variables|Default|GetA_Dialogue))
    ;;[0 0 0] If sound is playing,...
    ;;;[1 1 1] Check if sound needs to be overwritten
    (if (Variables|DiaLogic|GetOverwrite%20Sound?)
      ;;;[1 1 1] Overwrite sound
      (Audio|Components|Audio|SetSound (Variables|Default|GetA_Dialogue) Sound)
      (Audio|Components|Audio|Play (Variables|Default|GetA_Dialogue) 0.0)
      (else
        ;;;[1 1 1] If not, add to queue
        (Utilities|Array|Add (Variables|DiaLogic|GetSoundQueue) Sound)))
    (else
      ;;[0 0 0] If not, play sound
      (Audio|Components|Audio|SetSound (Variables|Default|GetA_Dialogue) Sound)
      (Audio|Components|Audio|Play (Variables|Default|GetA_Dialogue) 0.0))))

(event Custom|IntroSeq
  ;[1 1 1] Opening Seq
  (bind _returnvalue (CallFunction|HasPaintBoolean))
  (if _returnvalue
    (CallFunction|ClearDialogueQueue)
    (else
      (for _array_element (Variables|Default|GetIntro01)
        (bind _returnvalue_2 (CallFunction|HasPaintBoolean))
        (if _returnvalue_2
          (CallFunction|ClearDialogueQueue)
          (else
            (CallFunction|PlayDialogueSound false _array_element))))
      (Utilities|FlowControl|Delay 2e+01)
      (CallFunction|PickMeUpSeq))))

(event Custom|TransportationSeq
  ;[1 1 1] TransportationSeq
  (bind _returnvalue (CallFunction|HasPaintBoolean))
  (if _returnvalue
    (CallFunction|ClearDialogueQueue)
    (elif (not (Variables|Default|GetTeleported?))
      (CallFunction|PlayDialogueSound true "/Game/Audio-Revised/Assets/Dialogue/Dia_wav/Dia_M1_Intro_1p_7.Dia_M1_Intro_1p_7"))))

(event Custom|PickMeUpSeq
  ;[1 1 1] PickMeUpSeq
  (bind _returnvalue (CallFunction|HasPaintBoolean))
  (if _returnvalue
    (CallFunction|ClearDialogueQueue)
    (elif (not (Variables|DiaIntro|GetFirstGrab))
      (for _array_element (Variables|Default|GetPickUp)
        (if (not (Variables|DiaIntro|GetFirstGrab))
          (Utilities|FlowControl|Delay 5.0)
          (CallFunction|PlayDialogueSound false _array_element)
          (Development|PrintString (Utilities|GetDisplayName _array_element) true true "(R=0.000000,G=0.660000,B=1.000000,A=1.000000)" 5.0))))))

(event Custom|UnLoad
  (bind _swatch_ref (Variables|References|GetSwatch_Ref))
  (bind _sm_painttip_yellow (Variables|Default|GetSM_PaintTip_Yellow))
  (bind _swatch_ref_2 (Variables|References|GetSwatch_Ref))
  ;[1 1 1] Brush Prime Events - Paintability for Conduit Power
  (Utilities|FlowControl|Sequence
    (:then_0
      (Timeline|Timeline_1 ReverseFromEnd
        (:Update
          (Transformation|SetRelativeScale3D (Utilities|Select :Index (stale Custom|Load Selection) :NewEnumerator3 _sm_painttip_yellow :NewEnumerator0 _sm_painttip_yellow :NewEnumerator4 (Variables|Default|GetSM_PaintTip_Green) :NewEnumerator5 (Variables|Default|GetSM_PaintTip_Purple)) (Math|Vector|Lerp(Vector) "0, 0, 0" "1.000000,1.000000,1.000000" 0.0))
          (Transformation|SetRelativeRotation (Utilities|Select :Index (stale Custom|Load Selection) :NewEnumerator3 _sm_painttip_yellow :NewEnumerator0 _sm_painttip_yellow :NewEnumerator4 (Variables|Default|GetSM_PaintTip_Green) :NewEnumerator5 (Variables|Default|GetSM_PaintTip_Purple)) (Math|Rotator|MakeRotator 0.0 0.0 (Math|Float|Lerp 0.0 3.6e+02 0.0)) false false))
        (:Finished
          (Rendering|SetVisibility _sm_painttip_yellow false false))))
    (:then_1
      ;[1 1 1] Beginplay, sets reference to VR BP
      (switch Utilities|FlowControl|Switch|SwitchonEnum_Paints (Variables|Default|GetEnum%20Paints)
        (:NewEnumerator3
          (Variables|/Game/Blueprints/Palette/BP_Swatch.BP_Swatch_C|SetPaint1on _swatch_ref_2 false :!label _label)
          (Default|Glob1Grow _swatch_ref))
        (:NewEnumerator0
          (goto _label))
        (:NewEnumerator4
          (Variables|/Game/Blueprints/Palette/BP_Swatch.BP_Swatch_C|SetPaint2on _swatch_ref_2 false)
          (Default|Glob2Grow _swatch_ref))
        (:NewEnumerator5
          (Variables|/Game/Blueprints/Palette/BP_Swatch.BP_Swatch_C|SetPaint3on _swatch_ref false)
          (Default|Glob3Grow _swatch_ref))))))

(event Custom|ClearDialogueQueue
  (Utilities|Array|Clear (Variables|DiaLogic|GetSoundQueue))
  (Variables|DiaLogic|SetsoundQueueIndex 0))

(event Custom|Paint%20long%20shot
  (Variables|Default|SetTriggerHeld true)
  (switch Utilities|FlowControl|Switch|SwitchonEnum_Paints (Variables|Default|GetEnum%20Paints)))

(event Custom|PaintShot%20Release
  (Variables|Default|SetTriggerHeld false))

(event Custom|Zip
  (params (NewLocation :type Vector))
  ;[1 1 1] Teleport to hands
  (if (not (Variables|Default|GetGrabbed))
    (Transformation|SetWorldLocation (Variables|Default|GetBaseOffset) NewLocation false false)))

(event Custom|Loading
  (params (Selection :type Enum_Paints%20Enum :default "NewEnumerator3"))
  (bind _relative_rotation (Variables|Default|GetRelative%20Rotation))
  (bind _swatch_ref (Variables|References|GetSwatch_Ref))
  (bind _glow_sphere (Variables|Default|GetGlow_Sphere))
  (bind _swatch_ref_2 (Variables|References|GetSwatch_Ref))
  (bind _swatch_ref_3 (Variables|References|GetSwatch_Ref))
  ;[1 1 1] Loading shakiness + Glow ramping when paintbrush dipped into cauldron
  (switch Utilities|FlowControl|Switch|SwitchonEnum_Paints Selection
    (:NewEnumerator0
      (if (not (Variables|Default|GetPaint1Imbued))
        (Utilities|FlowControl|Sequence :!label _label
          (:then_0
            (Audio|Components|Audio|Play (Variables|Default|GetcauldronImbue_Cue) 0.0))
          (:then_1
            (bind _newtrack_0 (Timeline|Timeline_4 PlayFromStart)
              (:Update
                (Transformation|SetRelativeRotation (Variables|Default|GetPaintbrushBase) (Math|Rotator|MakeRotator (Math|Random|RandomFloatinRange (- (.roll _relative_rotation) (Math|Float|Lerp 0.0 1.0 _newtrack_0)) (+ (.roll _relative_rotation) (Math|Float|Lerp 0.0 1.0 _newtrack_0))) (Math|Random|RandomFloatinRange (- (.pitch _relative_rotation) (Math|Float|Lerp 0.0 1.0 _newtrack_0)) (+ (.pitch _relative_rotation) (Math|Float|Lerp 0.0 1.0 _newtrack_0))) (Math|Random|RandomFloatinRange (- (.yaw _relative_rotation) (Math|Float|Lerp 0.0 1.0 _newtrack_0)) (+ (.yaw _relative_rotation) (Math|Float|Lerp 0.0 1.0 _newtrack_0)))) false false))
              (:Finished
                (switch Utilities|FlowControl|Switch|SwitchonEnum_Paints Selection
                  (:NewEnumerator0
                    (Variables|Default|SetPaint1Imbued true)
                    (Audio|Components|Audio|Play (Variables|Default|GetA_Imbue) 0.0)
                    (CallFunction|ImbuedEvent)
                    (Transformation|SetRelativeRotation (Variables|Default|GetPaintbrushBase) (Variables|Default|GetRelative%20Rotation) false false)
                    (Variables|/Game/Blueprints/Palette/BP_Swatch.BP_Swatch_C|SetHasPaint1 _swatch_ref_2 true)
                    (Default|Glob1Grow _swatch_ref_2)
                    (CallFunction|ActiConduitImbueParticle))
                  (:NewEnumerator4
                    (Variables|Default|SetPaint2Imbued true)
                    (Audio|Components|Audio|Play (Variables|Default|GetA_Imbue) 0.0)
                    (CallFunction|ImbuedEvent)
                    (Transformation|SetRelativeRotation (Variables|Default|GetPaintbrushBase) (Variables|Default|GetRelative%20Rotation) false false)
                    (Variables|/Game/Blueprints/Palette/BP_Swatch.BP_Swatch_C|SetHasPaint2 _swatch_ref_3 true)
                    (Default|Glob2Grow _swatch_ref_3)
                    (CallFunction|ActiPlantImbueParticle))
                  (:NewEnumerator5
                    (Variables|Default|SetPaint2Imbued true)
                    (Audio|Components|Audio|Play (Variables|Default|GetA_Imbue) 0.0)
                    (CallFunction|ImbuedEvent)
                    (Transformation|SetRelativeRotation (Variables|Default|GetPaintbrushBase) (Variables|Default|GetRelative%20Rotation) false false)
                    (Variables|/Game/Blueprints/Palette/BP_Swatch.BP_Swatch_C|SetHasPaint3 _swatch_ref true)
                    (Default|Glob3Grow _swatch_ref))))))
          (:then_2
            (Rendering|SetVisibility _glow_sphere true false)
            (bind _newtrack_0_2 (Timeline|Timeline_0 PlayFromStart)
              (:Update
                (Transformation|SetRelativeScale3D _glow_sphere (Math|Vector|Lerp(Vector) "0, 0, 0" "0.177408,0.177408,0.177408" _newtrack_0_2)))
              (:Finished
                (Rendering|SetVisibility _glow_sphere false false)))))))
    (:NewEnumerator4
      (if (not (Variables|Default|GetPaint2Imbued))
        (goto _label)))
    (:NewEnumerator5
      (if (not (Variables|Default|GetPaint3Imbued))
        (goto _label)))))

(event Custom|StopLoading
  (bind _relative_rotation (Variables|Default|GetRelative%20Rotation))
  (bind _swatch_ref (Variables|References|GetSwatch_Ref))
  (bind _glow_sphere (Variables|Default|GetGlow_Sphere))
  (bind _swatch_ref_2 (Variables|References|GetSwatch_Ref))
  (bind _swatch_ref_3 (Variables|References|GetSwatch_Ref))
  ;[1 1 1] Loading shakiness + Glow ramping when paintbrush dipped into cauldron
  (switch Utilities|FlowControl|Switch|SwitchonEnum_Paints (stale Custom|Loading Selection)
    (:NewEnumerator0
      (if (not (Variables|Default|GetPaint1Imbued))
        (Utilities|FlowControl|Sequence :!label _label
          (:then_0
            (Audio|Components|Audio|Stop (Variables|Default|GetcauldronImbue_Cue)))
          (:then_1
            (bind _newtrack_0 (Timeline|Timeline_4 Stop)
              (:Update
                (Transformation|SetRelativeRotation (Variables|Default|GetPaintbrushBase) (Math|Rotator|MakeRotator (Math|Random|RandomFloatinRange (- (.roll _relative_rotation) (Math|Float|Lerp 0.0 1.0 _newtrack_0)) (+ (.roll _relative_rotation) (Math|Float|Lerp 0.0 1.0 _newtrack_0))) (Math|Random|RandomFloatinRange (- (.pitch _relative_rotation) (Math|Float|Lerp 0.0 1.0 _newtrack_0)) (+ (.pitch _relative_rotation) (Math|Float|Lerp 0.0 1.0 _newtrack_0))) (Math|Random|RandomFloatinRange (- (.yaw _relative_rotation) (Math|Float|Lerp 0.0 1.0 _newtrack_0)) (+ (.yaw _relative_rotation) (Math|Float|Lerp 0.0 1.0 _newtrack_0)))) false false))
              (:Finished
                (switch Utilities|FlowControl|Switch|SwitchonEnum_Paints (stale Custom|Loading Selection)
                  (:NewEnumerator0
                    (Variables|Default|SetPaint1Imbued true)
                    (Audio|Components|Audio|Play (Variables|Default|GetA_Imbue) 0.0)
                    (CallFunction|ImbuedEvent)
                    (Transformation|SetRelativeRotation (Variables|Default|GetPaintbrushBase) (Variables|Default|GetRelative%20Rotation) false false)
                    (Variables|/Game/Blueprints/Palette/BP_Swatch.BP_Swatch_C|SetHasPaint1 _swatch_ref_2 true)
                    (Default|Glob1Grow _swatch_ref_2)
                    (CallFunction|ActiConduitImbueParticle))
                  (:NewEnumerator4
                    (Variables|Default|SetPaint2Imbued true)
                    (Audio|Components|Audio|Play (Variables|Default|GetA_Imbue) 0.0)
                    (CallFunction|ImbuedEvent)
                    (Transformation|SetRelativeRotation (Variables|Default|GetPaintbrushBase) (Variables|Default|GetRelative%20Rotation) false false)
                    (Variables|/Game/Blueprints/Palette/BP_Swatch.BP_Swatch_C|SetHasPaint2 _swatch_ref_3 true)
                    (Default|Glob2Grow _swatch_ref_3)
                    (CallFunction|ActiPlantImbueParticle))
                  (:NewEnumerator5
                    (Variables|Default|SetPaint2Imbued true)
                    (Audio|Components|Audio|Play (Variables|Default|GetA_Imbue) 0.0)
                    (CallFunction|ImbuedEvent)
                    (Transformation|SetRelativeRotation (Variables|Default|GetPaintbrushBase) (Variables|Default|GetRelative%20Rotation) false false)
                    (Variables|/Game/Blueprints/Palette/BP_Swatch.BP_Swatch_C|SetHasPaint3 _swatch_ref true)
                    (Default|Glob3Grow _swatch_ref))))))
          (:then_2
            (bind _newtrack_0_2 (Timeline|Timeline_0 Stop)
              (:Update
                (Transformation|SetRelativeScale3D _glow_sphere (Math|Vector|Lerp(Vector) "0, 0, 0" "0.177408,0.177408,0.177408" _newtrack_0_2)))
              (:Finished
                (Rendering|SetVisibility _glow_sphere false false))))
          (:then_3
            (bind _newtrack_0_3 (Timeline|Timeline_3 Play)
              (:Update
                (Transformation|SetRelativeScale3D _glow_sphere (Math|Vector|Lerp(Vector) (Variables|/Script/Engine.SceneComponent|GetRelativeScale3D _glow_sphere) "0, 0, 0" _newtrack_0_3))))))))
    (:NewEnumerator4
      (if (not (Variables|Default|GetPaint2Imbued))
        (goto _label)))
    (:NewEnumerator5
      (if (not (Variables|Default|GetPaint3Imbued))
        (goto _label)))))

(event Custom|ImbuedEvent
  ;[1 1 1] On grabbed. Shows rune ring and sets correct position
  (CallFunction|ClearDialogueQueue)
  (if (Variables|Default|GetPaint1_OnBrush)
    _))

(event Custom|CompleteChemset
  ;[1 1 1] PuzzlesCompleteDialogue
  (Utilities|FlowControl|DoOnce false
    (:Completed
      (CallFunction|PlayDialogueSound true "/Game/Audio-Revised/Assets/Dialogue/Dia_wav/Dia_M1_Maze_4.Dia_M1_Maze_4")
      (Variables|PuzzleStatusClass|SetChemPz_Complete? true)
      (Variables|PuzzleStatusClass|SetChemPz_ConPiece? true)
      (CallFunction|ClassroomCompletion))))

(event Custom|Load
  (params (Selection :type Enum_Paints%20Enum :default "NewEnumerator0"))
  (bind _sm_painttip_yellow (Variables|Default|GetSM_PaintTip_Yellow))
  (bind _sm_painttip_green (Variables|Default|GetSM_PaintTip_Green))
  (bind _sm_painttip_purple (Variables|Default|GetSM_PaintTip_Purple))
  (bind _returnvalue (Utilities|Select :Index Selection :NewEnumerator3 _sm_painttip_yellow :NewEnumerator0 _sm_painttip_yellow :NewEnumerator4 _sm_painttip_green :NewEnumerator5 _sm_painttip_purple))
  ;[1 1 1] Brush Prime Events - Paintability for Conduit Power
  (Variables|Default|SetEnum%20Paints Selection)
  (Rendering|SetVisibility _sm_painttip_yellow false false)
  (Rendering|SetVisibility _returnvalue true false)
  (bind _newtrack_0 (Timeline|PaintLoad PlayFromStart)
    (:Update
      (Transformation|SetRelativeScale3D _returnvalue (Math|Vector|Lerp(Vector) "0.010000,0.010000,0.010000" "1.000000,1.000000,1.000000" _newtrack_0))
      (Transformation|SetRelativeRotation _returnvalue (Math|Rotator|MakeRotator 0.0 0.0 (Math|Float|Lerp 0.0 3.6e+02 _newtrack_0)) false false))))

(event EventBeginPlay
  (bind _ring (Variables|Default|GetRing))
  (bind _sm_painttip_yellow (Variables|Default|GetSM_PaintTip_Yellow))
  ;[1 1 1] Beginplay, sets reference to VR BP
  (Utilities|FlowControl|Sequence
    (:then_0
      (Variables|Default|SetPaint1Imbued false)
      (Variables|Default|SetRelative%20Rotation (Variables|/Script/Engine.SceneComponent|GetRelativeRotation (Variables|Default|GetPaintbrushBase)))
      (Transformation|SetWorldScale3D (Variables|Default|GetGlow_Sphere) "0, 0, 0")
      (bind _returnvalue (Actor|GetActorOfClass "/Game/Blueprints/VR_Character/BP_UpdatedVRPawn.BP_UpdatedVRPawn_C"))
      (Variables|References|SetVRRef _returnvalue)
      (bind _returnvalue_2 (Actor|GetActorOfClass "/Game/Blueprints/Palette/BP_Swatch.BP_Swatch_C"))
      (Variables|References|SetSwatch_Ref _returnvalue_2)
      (Rendering|SetVisibility _ring false false)
      (Transformation|SetRelativeScale3D _ring "0, 0, 0"))
    (:then_1
      (Variables|Default|SetParticleSpawnLo "-0.001855,0.002970,-675.078735"))
    (:then_2
      ;[1 1 1] Brush Prime Events - Paintability for Conduit Power
      (Variables|Default|SetEnum%20Paints (stale Custom|Load Selection))
      (Rendering|SetVisibility _sm_painttip_yellow false false)
      (Rendering|SetVisibility (Utilities|Select :Index (stale Custom|Load Selection) :NewEnumerator3 _sm_painttip_yellow :NewEnumerator0 _sm_painttip_yellow :NewEnumerator4 (Variables|Default|GetSM_PaintTip_Green) :NewEnumerator5 (Variables|Default|GetSM_PaintTip_Purple)) true false)
      (bind _newtrack_0 (Timeline|PaintLoad PlayFromStart)
        (:Update
          (Transformation|SetRelativeScale3D (Utilities|Select :Index (stale Custom|Load Selection) :NewEnumerator3 _sm_painttip_yellow :NewEnumerator0 _sm_painttip_yellow :NewEnumerator4 (Variables|Default|GetSM_PaintTip_Green) :NewEnumerator5 (Variables|Default|GetSM_PaintTip_Purple)) (Math|Vector|Lerp(Vector) "0.010000,0.010000,0.010000" "1.000000,1.000000,1.000000" _newtrack_0))
          (Transformation|SetRelativeRotation (Utilities|Select :Index (stale Custom|Load Selection) :NewEnumerator3 _sm_painttip_yellow :NewEnumerator0 _sm_painttip_yellow :NewEnumerator4 (Variables|Default|GetSM_PaintTip_Green) :NewEnumerator5 (Variables|Default|GetSM_PaintTip_Purple)) (Math|Rotator|MakeRotator 0.0 0.0 (Math|Float|Lerp 0.0 3.6e+02 _newtrack_0)) false false))))
    (:then_3
      (CallFunction|DeacConduitImbueParticle)
      (CallFunction|DeacPlantImbueParticle))
    (:then_4
      (Utilities|FlowControl|Delay 5.0)
      (CallFunction|IntroSeq))))

(fn ConstructionScript)

(fn ArraySequenceDialogue
  (params (NewParam :type Array%20of%20Sound%20Base%20Object%20References))
  (return 0))

(fn HasPaintBoolean
  (bind _swatch_ref (Variables|References|GetSwatch_Ref))
  (return (Math|Boolean|ORBoolean (Variables|/Game/Blueprints/Palette/BP_Swatch.BP_Swatch_C|GetHasPaint1 _swatch_ref) (Variables|/Game/Blueprints/Palette/BP_Swatch.BP_Swatch_C|GetHasPaint2 _swatch_ref) (Variables|/Game/Blueprints/Palette/BP_Swatch.BP_Swatch_C|GetHasPaint3 _swatch_ref))))

(fn ClearSoundQueue
  (Utilities|Array|Clear (Variables|DiaLogic|GetSoundQueue))
  (Variables|DiaLogic|SetsoundQueueIndex 0))

(fn OverlapPlayerFunction
  (return false))