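; Grinder conduit puzzle element that powers up on BeginPlay and runs a timeline-driven bumping motion.
; Grinder overlaps trigger impact sounds and briefly reposition a Niagara effect, then move it away after a delay.
; Finished plays chain audio and spins three meshes, calling SpiceFlow on the level's SpiceTransport and flagging the brush's GrindPzConduit each update.
; Brush contact with Box4 exits the brush and parent logic; paint-array checks are disconnected.
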(event OnComponentBeginOverlap(Box)
  (params (OverlappedComponent :type Primitive%20Component%20Object%20Reference) (OtherActor :type Actor%20Object%20Reference) (OtherComp :type Primitive%20Component%20Object%20Reference) (OtherBodyIndex :type Integer) (bFromSweep :type Boolean) (SweepResult :type Hit%20Result%20Structure%20%28by%20ref%29))
  (bind _niagara (Variables|Default|GetNiagara))
  (if (== OtherComp (Variables|Default|GetGrinder))
    (Utilities|FlowControl|DoOnce false
      (:Completed
        (Utilities|FlowControl|Sequence
          (:then_0
            (Audio|Components|Audio|Play (Variables|Default|GetA_Thud_Cue) 0.5)
            (Audio|Components|Audio|Play (Variables|Default|Getmortarimpact) 0.0))
          (:then_1
            (Transformation|SetRelativeLocation _niagara "75.883850,3.879547,-50.891640" false false)
            (Utilities|FlowControl|Delay 0.6)
            (Transformation|SetRelativeLocation _niagara "649.867615,3.879547,-50.891640" false false)))))))

(event OnComponentEndOverlap(Box)
  (params (OverlappedComponent :type Primitive%20Component%20Object%20Reference) (OtherActor :type Actor%20Object%20Reference) (OtherComp :type Primitive%20Component%20Object%20Reference) (OtherBodyIndex :type Integer))
  (bind _niagara (Variables|Default|GetNiagara))
  (if (== OtherComp (Variables|Default|GetGrinder))
    (Utilities|FlowControl|DoOnce false) ; enters at Reset
  ))

(event OnComponentBeginOverlap(Box3)
  (params (OverlappedComponent :type Primitive%20Component%20Object%20Reference) (OtherActor :type Actor%20Object%20Reference) (OtherComp :type Primitive%20Component%20Object%20Reference) (OtherBodyIndex :type Integer) (bFromSweep :type Boolean) (SweepResult :type Hit%20Result%20Structure%20%28by%20ref%29))
  (if (== OtherComp (Variables|Default|GetStaticMesh1))
    (Utilities|FlowControl|DoOnce false)))

(event OnComponentEndOverlap(Box3)
  (params (OverlappedComponent :type Primitive%20Component%20Object%20Reference) (OtherActor :type Actor%20Object%20Reference) (OtherComp :type Primitive%20Component%20Object%20Reference) (OtherBodyIndex :type Integer))
  (if (== OtherComp (Variables|Default|GetStaticMesh1))
    (Utilities|FlowControl|DoOnce false) ; enters at Reset
  ))

(event OnComponentBeginOverlap(Box4)
  (params (OverlappedComponent :type Primitive%20Component%20Object%20Reference) (OtherActor :type Actor%20Object%20Reference) (OtherComp :type Primitive%20Component%20Object%20Reference) (OtherBodyIndex :type Integer) (bFromSweep :type Boolean) (SweepResult :type Hit%20Result%20Structure%20%28by%20ref%29))
  (bind _brushrefvar (Variables|Default|GetBrushRefVar))
  (if (== OtherComp (Variables|/Game/Blueprints/Paintbrush/Paintrbsuh.Paintrbsuh_C|GetCollisionSphere _brushrefvar))
    ;[1 1 1] This code fucks up the game lol, probably the array
    (Default|Exited _brushrefvar)
    (CallFunction|ExitedParent)))

(event OnComponentBeginOverlap(Box5)
  (params (OverlappedComponent :type Primitive%20Component%20Object%20Reference) (OtherActor :type Actor%20Object%20Reference) (OtherComp :type Primitive%20Component%20Object%20Reference) (OtherBodyIndex :type Integer) (bFromSweep :type Boolean) (SweepResult :type Hit%20Result%20Structure%20%28by%20ref%29)))

(event Custom|GrinderStop
  (bind _boxxx (Variables|Default|GetBoxxx))
  (bind _relativelocation (Variables|/Script/Engine.SceneComponent|GetRelativeLocation _boxxx))
  (bind _newtrack_0 (Timeline|GrinderBump Stop)
    (:Update
      (Transformation|SetRelativeLocation _boxxx (Math|Vector|MakeVector (* _newtrack_0 -1.0) (.y _relativelocation) (.z _relativelocation)) false false))))

(event Custom|GrinderStart
  (bind _boxxx (Variables|Default|GetBoxxx))
  (bind _relativelocation (Variables|/Script/Engine.SceneComponent|GetRelativeLocation _boxxx))
  (bind _newtrack_0 (Timeline|GrinderBump Play)
    (:Update
      (Transformation|SetRelativeLocation _boxxx (Math|Vector|MakeVector (* _newtrack_0 -1.0) (.y _relativelocation) (.z _relativelocation)) false false))))

(event EventBeginPlay
  (|CallParentFunction)
  (CallFunction|PoweredUp)
  (CallFunction|GrinderStart)
  (bind _returnvalue (Actor|GetActorOfClass "/Game/Blueprints/PuzzleElements/Bp_SpiceTransport.Bp_SpiceTransport_C"))
  (Variables|Default|SetSpiceRef _returnvalue))

(event EventFinished
  (Audio|Components|Audio|Play (Variables|Default|GetchainMoving_Cue) 0.0)
  (bind _newtrack_0 (Timeline|Timeline_2 Play)
    (:Update
      (Transformation|SetRelativeRotation (Variables|Default|GetStaticMesh23) (Math|Rotator|Lerp(Rotator) "0, 0,-90.000000" "0,360.000000,-90.000000" _newtrack_0) false false)
      (Transformation|SetRelativeRotation (Variables|Default|GetStaticMesh22) (Math|Rotator|Lerp(Rotator) "0,360.000000,-90.000000" "0,0.000000,-90.000000" _newtrack_0) false false)
      (Default|SpiceFlow (Variables|Default|GetSpiceRef))
      (Variables|/Game/Blueprints/Paintbrush/Paintrbsuh.Paintrbsuh_C|SetGrindPz_Conduit? (Variables|Default|GetBrushRefVar) true))))

(fn ConstructionScript
  (|CallParentFunction))