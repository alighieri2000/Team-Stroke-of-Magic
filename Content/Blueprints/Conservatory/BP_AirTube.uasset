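; BP_AirTube is an air tube in the Conservatory that can capture the Janitoad frog once the tube is open.
; Grabbing it through its GrabComponent, or any hit on StaticMesh3, sets it open, and nothing here closes it again.
; When the frog overlaps the Box while it is open, the tube kills the frog, flags FrogInsideTube on the Paintrbsuh actor and reveals its skeletal mesh.
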(event OnComponentBeginOverlap(Box)
  (params (OverlappedComponent :type Primitive%20Component%20Object%20Reference) (OtherActor :type Actor%20Object%20Reference) (OtherComp :type Primitive%20Component%20Object%20Reference) (OtherBodyIndex :type Integer) (bFromSweep :type Boolean) (SweepResult :type Hit%20Result%20Structure%20%28by%20ref%29))
  (bind _frogref (Variables|Default|GetFrogRef))
  (if (== OtherActor _frogref)
    (if (Variables|Default|GetSetTubeOpen)
      (Default|Kill _frogref)
      (Variables|/Game/Blueprints/Paintbrush/Paintrbsuh.Paintrbsuh_C|SetFrogInsideTube? (Variables|Default|GetPaintrbsuh) true)
      (Rendering|SetVisibility (Variables|Default|GetSkeletalMesh) true false))))

(event OnGrabbed(GrabComponent)
  (Variables|Default|SetSetTubeOpen true))

(event OnComponentHit(StaticMesh3)
  (params (HitComponent :type Primitive%20Component%20Object%20Reference) (OtherActor :type Actor%20Object%20Reference) (OtherComp :type Primitive%20Component%20Object%20Reference) (NormalImpulse :type Vector :default "0, 0, 0") (Hit :type Hit%20Result%20Structure%20%28by%20ref%29))
  (Variables|Default|SetSetTubeOpen true))

(event EventBeginPlay
  (bind _returnvalue (Actor|GetActorOfClass "/Game/Blueprints/Janitoad/Janitoad_Character.Janitoad_Character_C"))
  (Variables|Default|SetFrogRef _returnvalue)
  (bind _returnvalue_2 (Actor|GetActorOfClass "/Game/Blueprints/Paintbrush/Paintrbsuh.Paintrbsuh_C"))
  (Variables|Default|SetPaintrbsuh _returnvalue_2))

(fn ConstructionScript)