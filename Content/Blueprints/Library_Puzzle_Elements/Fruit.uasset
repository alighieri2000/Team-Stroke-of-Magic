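; Fruit puzzle element that starts ungrabbable, then grows into a scaled-up, physics-simulated, grabbable object.
; A spline-finished event plays the CustomTick timeline, which polls a Test flag each update.
; Once the flag is set, it applies the grown state a single time and stops the timeline.
; Triggering is test scaffolding: BeginPlay calls spline-finished directly, key 9 sets the flag, and BeginGrow is empty.
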(event Custom|Spline_Finished
  ;[1 0 0] For Testing purposes ONLY, remove after OBJ REF is implemented
  (Timeline|Custom%20Tick Play
    (:Tick
      (CallFunction|TickEvent))))

(event Custom|Tick%20Event
  ;[1 0 0] For Testing purposes ONLY, remove after OBJ REF is implemented
  (if (Variables|Default|GetTest)
    (Utilities|FlowControl|DoOnce false
      (:Completed
        (Development|PrintString "Grown")
        (Transformation|SetActorScale3D "5.000000,5.000000,5.000000")
        (Components|Activation|Activate (Variables|Default|GetGrabComponent) false)
        (Physics|SetSimulatePhysics (Variables|Default|GetStaticMesh) true)
        (CallFunction|StopTick)))))

(event Custom|Stop%20Tick
  ;[1 0 0] For Testing purposes ONLY, remove after OBJ REF is implemented
  (Timeline|Custom%20Tick Stop
    (:Tick
      (CallFunction|TickEvent))))

(event Custom|Begin%20Grow)

(event EventBeginPlay
  ;[1 0 0] For Testing purposes ONLY, remove after OBJ REF is implemented
  (Components|Activation|Deactivate (Variables|Default|GetGrabComponent))
  (CallFunction|SplineFinished))

(event Input|KeyboardEvents|9
  (params (Key :type Key%20Structure :default "None"))
  ;[1 0 0] For Testing purposes ONLY, remove after OBJ REF is implemented
  (:Pressed
    (Variables|Default|SetTest true)))

(fn ConstructionScript)