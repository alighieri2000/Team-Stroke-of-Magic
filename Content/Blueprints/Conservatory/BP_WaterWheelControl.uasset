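; BP_WaterWheelControl is a grippable two-position switch that turns the conservatory's water wheel on and off.
; It finds the WaterWheel actor on BeginPlay, then watches for its Box overlapping the OnBox and OffBox triggers.
; A change of state updates IsOn, moves InitialTransform to that end's position, calls SetOn or SetOff on the wheel, and breaks the grip.
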(event OnComponentBeginOverlap(OffBox)
  (params (OverlappedComponent :type Primitive%20Component%20Object%20Reference) (OtherActor :type Actor%20Object%20Reference) (OtherComp :type Primitive%20Component%20Object%20Reference) (OtherBodyIndex :type Integer) (bFromSweep :type Boolean) (SweepResult :type Hit%20Result%20Structure%20%28by%20ref%29))
  (if (== OtherComp (Variables|Default|GetBox))
    (if (Variables|Default|GetIsOn)
      (Variables|Default|SetIsOn false)
      (Transformation|SetRelativeLocation (Variables|Default|GetInitialTransform) "0,-60.000000, 0" false false)
      (Default|SetOff (Variables|Default|GetWaterWheelRef))
      (CallFunction|BreakGrip))))

(event OnComponentBeginOverlap(OnBox)
  (params (OverlappedComponent :type Primitive%20Component%20Object%20Reference) (OtherActor :type Actor%20Object%20Reference) (OtherComp :type Primitive%20Component%20Object%20Reference) (OtherBodyIndex :type Integer) (bFromSweep :type Boolean) (SweepResult :type Hit%20Result%20Structure%20%28by%20ref%29))
  (if (== OtherComp (Variables|Default|GetBox))
    (if (not (Variables|Default|GetIsOn))
      (Variables|Default|SetIsOn true)
      (Transformation|SetRelativeLocation (Variables|Default|GetInitialTransform) "0,0.000000, 0" false false)
      (Default|Seton (Variables|Default|GetWaterWheelRef))
      (CallFunction|BreakGrip))))

(event EventBeginPlay
  (|CallParentFunction)
  (bind _returnvalue (Actor|GetActorOfClass "/Game/Blueprints/PuzzleElements/WaterWheel.WaterWheel_C"))
  (Variables|Default|SetWaterWheelRef _returnvalue))

(event Collision|EventActorBeginOverlap
  (params (OtherActor :type Actor%20Object%20Reference)))

(event EventTick
  (params (DeltaSeconds :type Float%20%28single-precision%29)))

(fn ConstructionScript
  (|CallParentFunction))