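; Puzzle conduit for the boiler: a gear train that needs a loose BP_SoloGear inserted to drive the boiler's shovels.
; Overlapping that gear with the socket reveals the fitted gear, removes the loose one, flags the paintbrush, and pulses Niagara with sound.
; The Finished event spins the gears by timeline, only two until GearOn is set, when the full train turns and a cube slides once, then triggers BP_Boiler's ShovelsPlay.
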(event OnComponentBeginOverlap(Box_0)
  (params (OverlappedComponent :type Primitive%20Component%20Object%20Reference) (OtherActor :type Actor%20Object%20Reference) (OtherComp :type Primitive%20Component%20Object%20Reference) (OtherBodyIndex :type Integer) (bFromSweep :type Boolean) (SweepResult :type Hit%20Result%20Structure%20%28by%20ref%29))
  (bind _brushrefvar (Variables|Default|GetBrushRefVar))
  (if (== (Variables|/Game/Blueprints/Paintbrush/Paintrbsuh.Paintrbsuh_C|GetCollisionSphere _brushrefvar) OtherComp)
    (Default|Exited _brushrefvar)
    (Default|Exited (Variables|Default|GetWhitePaint))))

(event OnComponentBeginOverlap(Box3)
  (params (OverlappedComponent :type Primitive%20Component%20Object%20Reference) (OtherActor :type Actor%20Object%20Reference) (OtherComp :type Primitive%20Component%20Object%20Reference) (OtherBodyIndex :type Integer) (bFromSweep :type Boolean) (SweepResult :type Hit%20Result%20Structure%20%28by%20ref%29))
  (bind _gearref (Variables|Default|GetGearRef))
  (if (== OtherActor _gearref)
    (Rendering|SetVisibility (Variables|Default|GetGear3) true false)
    (Variables|Default|SetGearOn true)
    (Variables|/Game/Blueprints/Paintbrush/Paintrbsuh.Paintrbsuh_C|SetBoilPz_Gear? (Variables|Default|GetPaintBrush%20Ref) true)
    (Default|KillMe _gearref)
    (Audio|Components|Audio|Play (Variables|Default|GetA_GearConnect) 0.0)
    (Niagara|SetNiagaraVariable(Float) (Variables|Default|GetNiagara) "Size" 1.0)
    (Utilities|FlowControl|Delay 1.0)
    (Niagara|SetNiagaraVariable(Float) (Variables|Default|GetNiagara) "Size" 0.0)))

(event EventBeginPlay
  (|CallParentFunction)
  (CallFunction|PoweredUp)
  (bind _returnvalue (Actor|GetActorOfClass "/Game/Blueprints/PuzzleElements/BP_SoloGear.BP_SoloGear_C"))
  (Variables|Default|SetGearRef _returnvalue)
  (bind _returnvalue_2 (Actor|GetActorOfClass "/Game/Blueprints/BP/BP_Boiler.BP_Boiler_C"))
  (Variables|Default|SetBoilRef _returnvalue_2)
  (bind _returnvalue_3 (Actor|GetActorOfClass "/Game/Blueprints/Paintbrush/Paintrbsuh.Paintrbsuh_C"))
  (Variables|Default|SetPaintBrush%20Ref _returnvalue_3))

(event Collision|EventActorBeginOverlap
  (params (OtherActor :type Actor%20Object%20Reference)))

(event EventTick
  (params (DeltaSeconds :type Float%20%28single-precision%29)))

(event EventFinished
  (Audio|Components|Audio|Play (Variables|Default|GetA_GearsGrinding) 0.0)
  (bind _newtrack_0 (Timeline|SpinningGears PlayFromStart)
    (:Update
      (Transformation|SetRelativeRotation (Variables|Default|GetGear2) (Math|Rotator|Lerp(Rotator) "0, 0,90.000000" "0,360.000000,90.000000" _newtrack_0) false false)
      (Transformation|SetRelativeRotation (Variables|Default|GetGear1) (Math|Rotator|Lerp(Rotator) "0,360.000000,90.000000" "0,0.000000,90.000000" _newtrack_0) false false)
      (if (Variables|Default|GetGearOn)
        (Utilities|FlowControl|DoOnce false
          (:Completed
            (bind _newtrack_0_2 (Timeline|Timeline_2 PlayFromStart)
              (:Update
                (Transformation|SetRelativeLocation (Variables|Default|GetCube_0) (Math|Vector|Lerp(Vector) "152.939423,302.149170,13.162140" "320.074280,302.149170,13.162140" _newtrack_0_2) false false))
              (:Finished
                (Default|ShovelsPlay (Variables|Default|GetBoilRef))))))))))

(fn ConstructionScript
  (|CallParentFunction))