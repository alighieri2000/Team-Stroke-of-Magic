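; Green paint actor that draws a trail of pooled static mesh points behind the paintbrush while it stays within paint bounds.
; Construction script builds hidden points; entering makes FollowCube track the brush and starts a Timeline-timed loop placing points in ring-buffer order.
; SetPaintTrail-minus5 finds the nine previous wrapped indices, and SizeTrail tapers them, smallest at the newest.
; Exiting stops tracking and painting; FrogOverlapPaint hides individual points.
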(event Custom|Frog%20Overlap%20Paint
  (params (Dimension%201 :type Integer))
  (Rendering|SetVisibility (Utilities|Array|Get(acopy) (Variables|References|GetPaintObjects) Dimension%201) false false))

(event Custom|Painting
  (bind _followcube (Variables|Default|GetFollowCube))
  (bind _iswithinpaintbounds (Variables|SurfaceParentCommunication|GetisWithinPaintBounds))
  (bind _relativelocation (Variables|/Script/Engine.SceneComponent|GetRelativeLocation _followcube))
  ;[1 1 1] Paint trail loop: Spawns a particle on a timer
  (if _iswithinpaintbounds
    (Utilities|FlowControl|Sequence
      (:then_0
        (Timeline|Timeline_0 PlayFromStart
          (:Finished
            (Utilities|FlowControl|Sequence
              (:then_0
                (Transformation|SetRelativeLocation (Utilities|Array|Get(acopy) (Variables|References|GetPaintObjects) (Variables|Default|GetInkSeq)) (Math|Vector|MakeVector (.x _relativelocation) (.y _relativelocation) (+ (.z (Variables|Default|GetSpawnLoc)) 5.0)) false false)
                (Utilities|SetPaintTrail-minus5)
                (Utilities|SizeTrail)
                (if _iswithinpaintbounds
                  (Rendering|SetVisibility (Utilities|Array|Get(acopy) (Variables|References|GetPaintObjects) (Variables|Default|GetInkSeq)) true false)
                  (else
                    (Rendering|SetVisibility (Utilities|Array|Get(acopy) (Variables|References|GetPaintObjects) (Variables|Default|GetInkSeq)) false false)))
                (Variables|Default|SetInkSeq (+ (Variables|Default|GetInkSeq) 1))
                (if (== (Variables|Default|GetInkSeq) (- (Variables|Default|GetNumberOfPaintPoints) 1))
                  (Variables|Default|SetInkSeq 0))
                (CallFunction|Painting)))))))))

(event Custom|Entered
  (params (Paints%20Enum :type Enum_Paints%20Enum :default "NewEnumerator3"))
  ;[1 1 1] Starts tracking the location of the brush, triggered when first point is entered
  (if (not (Variables|SurfaceParentCommunication|GetLineCompleted))
    (Variables|SurfaceParentCommunication|SetisWithinPaintBounds true)
    (CallFunction|Painting)
    (Timeline|Timeline_1 Play
      (:Update
        (Transformation|SetWorldLocation (Variables|Default|GetFollowCube) (Transformation|GetWorldLocation (Variables|/Game/Blueprints/Paintbrush/Paintrbsuh.Paintrbsuh_C|GetCollisionSphere (Variables|References|GetBrushRefVar))) false false)))))

(event Custom|Exited
  ;[1 1 1] Failed to stay in bounds, removes trail
  (Variables|SurfaceParentCommunication|SetisWithinPaintBounds false)
  (Utilities|FlowControl|Sequence
    (:then_0
      ;[1 1 1] Starts tracking the location of the brush, triggered when first point is entered
      (Timeline|Timeline_1 Stop
        (:Update
          (Transformation|SetWorldLocation (Variables|Default|GetFollowCube) (Transformation|GetWorldLocation (Variables|/Game/Blueprints/Paintbrush/Paintrbsuh.Paintrbsuh_C|GetCollisionSphere (Variables|References|GetBrushRefVar))) false false))))
    (:then_2
      (Rendering|SetVisibility (Utilities|Array|Get(acopy) (Variables|References|GetPaintObjects) (Variables|Default|GetInkSeq)) false false))))

(event EventBeginPlay
  ;[1 1 1] BeginPlay
  (Variables|References|SetPaintObjects (Variables|References|GetPaintPointArray))
  (bind _returnvalue (Actor|GetActorOfClass "/Game/Blueprints/Paintbrush/Paintrbsuh.Paintrbsuh_C"))
  (Variables|References|SetBrushRefVar _returnvalue))

(fn ConstructionScript
  (for _index (range 0 (Variables|Default|GetNumberOfPaintPoints))
    (bind _returnvalue (AddComponent|AddStaticMeshComponent false))
    (Rendering|SetVisibility _returnvalue false false)
    (Utilities|Array|Add (Variables|References|GetPaintPointArray) _returnvalue)))