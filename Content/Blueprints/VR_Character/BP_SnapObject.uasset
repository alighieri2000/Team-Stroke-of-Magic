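; BP_SnapObject is a VR pickup object that snaps into BP_Slot actors when dropped.
; Overlapping a free slot's Box stores it as the current Slot; the end-overlap handler is empty, so leaving does not clear it.
; Drop moves the object to the slot mesh's transform and calls AttachToSlot, or detaches and clears Slot if it is in use.
; Pickup calls DetachFromSlot on any stored Slot.
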(event OnComponentBeginOverlap(Mesh)
  (params (OverlappedComponent :type Primitive%20Component%20Object%20Reference) (OtherActor :type Actor%20Object%20Reference) (OtherComp :type Primitive%20Component%20Object%20Reference) (OtherBodyIndex :type Integer) (bFromSweep :type Boolean) (SweepResult :type Hit%20Result%20Structure%20%28by%20ref%29))
  ;[0 0 0] If we are overlapping with a slot and the slot isn't in use then this becomes our slot
  (bind _asbp_slot (Utilities|Casting|CastToBP_Slot OtherActor))
  (if (== (Variables|/Game/Blueprints/VR_Character/BP_Slot.BP_Slot_C|GetBox _asbp_slot) OtherComp)
    (if (not (Variables|/Game/Blueprints/VR_Character/BP_Slot.BP_Slot_C|GetSlotInUse _asbp_slot))
      (Variables|Default|SetSlot _asbp_slot)
      (Development|PrintString "slot available" true true "(R=0.000000,G=1.000000,B=0.135811,A=1.000000)"))))

(event OnComponentEndOverlap(Mesh)
  (params (OverlappedComponent :type Primitive%20Component%20Object%20Reference) (OtherActor :type Actor%20Object%20Reference) (OtherComp :type Primitive%20Component%20Object%20Reference) (OtherBodyIndex :type Integer))
  ;[0 0 0] If we are leaving a lost collision and the slot variable is valid and the slot we are leaving is the same slot in the variable, make the slot variable null
)

(event EventPickup
  (params (Component :type Scene%20Component%20Object%20Reference) (Hand :type EControllerHand%20Enum :default "Left"))
  (bind _slot (Variables|Default|GetSlot))
  ;[0 0 0] On pick up if the cube was already on a slot then detach from slot
  (Utilities|IsValid _slot
    (:Is%20Valid
      (Default|DetachfromSlot _slot))))

(event EventDrop
  (params (Component :type Scene%20Component%20Object%20Reference))
  ;[0 0 0] On drop if the slot variable is valid attach to slot and snap to right location and rotation
  (Utilities|IsValid (Variables|Default|GetSlot)
    (:Is%20Valid
      (if (not (Variables|/Game/Blueprints/VR_Character/BP_Slot.BP_Slot_C|GetSlotInUse (Variables|Default|GetSlot)))
        (Development|PrintString "DroppingDetach" true true "(R=1.000000,G=0.733248,B=0.000000,A=1.000000)")
        (Transformation|SetActorLocationAndRotation (Transformation|GetWorldLocation (Variables|/Game/Blueprints/VR_Character/BP_Slot.BP_Slot_C|GetStaticMesh (Variables|Default|GetSlot))) (Transformation|GetWorldRotation (Variables|/Game/Blueprints/VR_Character/BP_Slot.BP_Slot_C|GetStaticMesh (Variables|Default|GetSlot))))
        (Default|AttachtoSlot (Variables|Default|GetSlot))
        (else
          (Default|DetachfromSlot (Variables|Default|GetSlot))
          (Variables|Default|SetSlot 0))))))

(fn ConstructionScript)