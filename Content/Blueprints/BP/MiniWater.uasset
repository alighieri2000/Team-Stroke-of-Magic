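; MiniWater is a water actor that clears the paintbrush's first paint when the brush touches it.
; On BeginPlay it finds and caches the Paintrbsuh actor in the level.
; When that brush's collision sphere begins overlapping the StaticMesh12 component, it calls Paint1Cleared on the brush.
; A separate OnTTT event makes StaticMesh12 visible.
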(event OnComponentBeginOverlap(StaticMesh12)
  (params (OverlappedComponent :type Primitive%20Component%20Object%20Reference) (OtherActor :type Actor%20Object%20Reference) (OtherComp :type Primitive%20Component%20Object%20Reference) (OtherBodyIndex :type Integer) (bFromSweep :type Boolean) (SweepResult :type Hit%20Result%20Structure%20%28by%20ref%29))
  (bind _newvar_0 (Variables|Default|GetNewVar_0))
  (if (== (Variables|/Game/Blueprints/Paintbrush/Paintrbsuh.Paintrbsuh_C|GetCollisionSphere _newvar_0) OtherComp)
    (Default|Paint1Cleared _newvar_0)))

(event Custom|OnTTT
  (Rendering|SetVisibility (Variables|Default|GetStaticMesh12) true false))

(event EventBeginPlay
  (bind _returnvalue (Actor|GetActorOfClass "/Game/Blueprints/Paintbrush/Paintrbsuh.Paintrbsuh_C"))
  (Variables|Default|SetNewVar_0 _returnvalue))

(event Collision|EventActorBeginOverlap
  (params (OtherActor :type Actor%20Object%20Reference)))

(event EventTick
  (params (DeltaSeconds :type Float%20%28single-precision%29)))

(fn ConstructionScript)