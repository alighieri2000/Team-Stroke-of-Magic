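; BP_HallwayActor is a puzzle hallway trigger that hides or shows all BP_MoveShelf1 shelves based on the VR pawn's direction of travel.
; The In and Out volumes set flags through DoOnce gates, which the Center volume resets.
; Hitting In after Out calls HideShelves, and Out after In calls ShowShelves, clearing the earlier flag as each shelf is processed.
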(event OnComponentBeginOverlap(Center)
  (params (OverlappedComponent :type Primitive%20Component%20Object%20Reference) (OtherActor :type Actor%20Object%20Reference) (OtherComp :type Primitive%20Component%20Object%20Reference) (OtherBodyIndex :type Integer) (bFromSweep :type Boolean) (SweepResult :type Hit%20Result%20Structure%20%28by%20ref%29))
  (if (== OtherActor (Variables|Default|GetPawnRef))
    (Utilities|FlowControl|Sequence
      (:then_0
        (Utilities|FlowControl|DoOnce false) ; enters at Reset
      )
      (:then_1
        (Utilities|FlowControl|DoOnce false) ; enters at Reset
      ))))

(event OnComponentBeginOverlap(In)
  (params (OverlappedComponent :type Primitive%20Component%20Object%20Reference) (OtherActor :type Actor%20Object%20Reference) (OtherComp :type Primitive%20Component%20Object%20Reference) (OtherBodyIndex :type Integer) (bFromSweep :type Boolean) (SweepResult :type Hit%20Result%20Structure%20%28by%20ref%29))
  (if (== OtherActor (Variables|Default|GetPawnRef))
    (Utilities|FlowControl|DoOnce false
      (:Completed
        (Variables|Default|SetHit_In true)
        (if (Variables|Default|GetHit_Out)
          (for _array_element (Variables|Default|GetShelves)
            (Default|HideShelves _array_element)
            (Variables|Default|SetHit_Out false)))))))

(event OnComponentBeginOverlap(Out)
  (params (OverlappedComponent :type Primitive%20Component%20Object%20Reference) (OtherActor :type Actor%20Object%20Reference) (OtherComp :type Primitive%20Component%20Object%20Reference) (OtherBodyIndex :type Integer) (bFromSweep :type Boolean) (SweepResult :type Hit%20Result%20Structure%20%28by%20ref%29))
  (if (== OtherActor (Variables|Default|GetPawnRef))
    (Utilities|FlowControl|DoOnce false
      (:Completed
        (Variables|Default|SetHit_Out true)
        (if (Variables|Default|GetHit_In)
          (for _array_element (Variables|Default|GetShelves)
            (Default|ShowShelves _array_element)
            (Variables|Default|SetHit_In false)))))))

(event EventBeginPlay
  (bind _returnvalue (Actor|GetActorOfClass "/Game/Blueprints/VR_Character/BP_UpdatedVRPawn.BP_UpdatedVRPawn_C"))
  (Variables|Default|SetPawnRef _returnvalue)
  (bind _outactors (Actor|GetAllActorsOfClass "/Game/Blueprints/Conservatory/BP_MoveShelf1.BP_MoveShelf1_C"))
  (Variables|Default|SetShelves _outactors))

(event Collision|EventActorBeginOverlap
  (params (OtherActor :type Actor%20Object%20Reference)))

(event EventTick
  (params (DeltaSeconds :type Float%20%28single-precision%29)))

(fn ConstructionScript)