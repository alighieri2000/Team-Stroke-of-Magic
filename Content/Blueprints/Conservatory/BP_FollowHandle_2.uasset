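; BP_FollowHandle_2 is a grabbable handle actor, apparently an unfinished prototype for rotate-style interaction.
; While grabbed, a timeline moves FollowCube to GrabbableObject's world location each update; dropping stops it.
; In Rotate mode a second timeline only zeroes RotVal before an empty switch.
; Pivot look-at rotation math, constrained by RotDirection, is left unconnected, and the construction script's InteractType switch does nothing.
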(event OnGrabbed(GrabComponent)
  (Utilities|FlowControl|Sequence
    (:then_0
      (Timeline|Start%20following%20grab%20component PlayFromStart
        (:Update
          (Transformation|SetWorldLocation (Variables|Default|GetFollowCube) (Transformation|GetWorldLocation (Variables|Default|GetGrabbableObject)) false false))))
    (:then_1
      (switch Utilities|FlowControl|Switch|SwitchonFollowHandleEnum (Variables|Default|GetInteract%20Type)
        (:NewEnumerator1
          (Timeline|Timeline_0 PlayFromStart
            (:Update
              (Variables|Default|SetRot%20Val 0.0)
              (switch Utilities|FlowControl|Switch|SwitchonRotValEnum "NewEnumerator0"))))))))

(event OnDropped(GrabComponent)
  (Utilities|FlowControl|Sequence
    (:then_0
      (Timeline|Start%20following%20grab%20component Stop
        (:Update
          (Transformation|SetWorldLocation (Variables|Default|GetFollowCube) (Transformation|GetWorldLocation (Variables|Default|GetGrabbableObject)) false false))))
    (:then_1
      (if true
        _))))

(event EventBeginPlay)

(event Collision|EventActorBeginOverlap
  (params (OtherActor :type Actor%20Object%20Reference)))

(event EventTick
  (params (DeltaSeconds :type Float%20%28single-precision%29)))

(fn ConstructionScript
  (switch Utilities|FlowControl|Switch|SwitchonFollowHandleEnum (Variables|Default|GetInteract%20Type)))