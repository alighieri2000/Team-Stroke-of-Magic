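; BP_BigToad is a conservatory toad that wants a book, jewel or apple, chosen by ToadEnum.
; When the VR pawn comes near an unfed toad, timelines raise staggered thought-bubble billboards showing the item; grabbing hides them.
; Overlap with the wanted item marks it fed, shows that item's mesh, kills the original and sets a flag on the paintbrush actor.
; The eat-jump, particle and shrink sequence is present but never runs.
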(event OnComponentBeginOverlap(Box)
  (params (OverlappedComponent :type Primitive%20Component%20Object%20Reference) (OtherActor :type Actor%20Object%20Reference) (OtherComp :type Primitive%20Component%20Object%20Reference) (OtherBodyIndex :type Integer) (bFromSweep :type Boolean) (SweepResult :type Hit%20Result%20Structure%20%28by%20ref%29))
  (bind _paintbrushref (Variables|Default|GetPaintBrushRef))
  (bind _bookref (Variables|Default|GetBookRef))
  (bind _toadenum (Variables|Default|GetToadEnum))
  (bind _jewel_ref (Variables|Default|GetJewel%20Ref))
  (bind _appleref (Variables|Default|GetAppleRef))
  (if (== OtherActor (Utilities|Select :Index _toadenum :NewEnumerator0 _bookref :NewEnumerator1 _jewel_ref :NewEnumerator2 _appleref))
    (Variables|Default|SetAte true)
    (CallFunction|BacktoOriginal)
    (Rendering|SetVisibility (Utilities|Select :Index _toadenum :NewEnumerator0 (Variables|Default|GetFancyBook) :NewEnumerator1 (Variables|Default|GetJemm) :NewEnumerator2 (Variables|Default|Getapple)) true false)
    (switch Utilities|FlowControl|Switch|SwitchonFrogRequestEnum (Variables|Default|GetToadEnum)
      (:NewEnumerator0
        (Default|Kill _bookref)
        (Variables|/Game/Blueprints/Paintbrush/Paintrbsuh.Paintrbsuh_C|SetDirectoadBookFed? _paintbrushref true))
      (:NewEnumerator1
        (Default|Kill _jewel_ref)
        (Variables|/Game/Blueprints/Paintbrush/Paintrbsuh.Paintrbsuh_C|SetDirectoadJewelFed? _paintbrushref true))
      (:NewEnumerator2
        (Default|Kill _appleref)
        (Variables|/Game/Blueprints/Paintbrush/Paintrbsuh.Paintrbsuh_C|SetDirectoadAppleFed? _paintbrushref true)))))

(event OnComponentBeginOverlap(Box1)
  (params (OverlappedComponent :type Primitive%20Component%20Object%20Reference) (OtherActor :type Actor%20Object%20Reference) (OtherComp :type Primitive%20Component%20Object%20Reference) (OtherBodyIndex :type Integer) (bFromSweep :type Boolean) (SweepResult :type Hit%20Result%20Structure%20%28by%20ref%29))
  (if (== OtherActor (Variables|Default|GetPawnref))
    (if (not (Variables|Default|GetAte))
      (Utilities|FlowControl|DoOnce false :!label _label
        (:Completed
          (CallFunction|ThoughtBubble true)
          (Variables|Default|SetMouthOpen true)
          (Timeline|Timeline_9 PlayFromStart
            (:Finished
              (CallFunction|ThoughtBubble false)
              (Variables|Default|SetMouthOpen false)
              (goto _label Reset))))))))

(event Custom|ThoughtBubble
  (params (Condition :type Boolean))
  (bind _materialbillboard0 (Variables|Default|GetMaterialBillboard0))
  (bind _materialbillboard1 (Variables|Default|GetMaterialBillboard1))
  (bind _materialbillboard2 (Variables|Default|GetMaterialBillboard2))
  (bind _materialbillboard3 (Variables|Default|GetMaterialBillboard3))
  (Rendering|ToggleVisibility (Variables|Default|GetMaterialBillboard0) false)
  (Utilities|FlowControl|Sequence
    (:then_0
      (if Condition
        (Rendering|SetVisibility _materialbillboard0 true false)
        (bind _newtrack_0 (Timeline|Timeline_2 PlayFromStart)
          (:Update
            (Transformation|SetRelativeLocation _materialbillboard0 (Math|Vector|Lerp(Vector) "0, 0, 0" "0.000000,0.000000,5.000000" _newtrack_0) false false))
          (:Finished
            (if (not Condition)
              (Rendering|SetVisibility _materialbillboard0 false false))))
        (else
          (Timeline|Timeline_2 ReverseFromEnd))))
    (:then_1
      (Utilities|FlowControl|Delay 0.1)
      (if Condition
        (Rendering|SetVisibility _materialbillboard1 true false)
        (bind _newtrack_0_2 (Timeline|Timeline_5 PlayFromStart)
          (:Update
            (Transformation|SetRelativeLocation _materialbillboard1 (Math|Vector|Lerp(Vector) "0, 0, 0" "0, 0,5.000000" _newtrack_0_2) false false))
          (:Finished
            (if (not Condition)
              (Rendering|SetVisibility _materialbillboard1 false false))))
        (else
          (Timeline|Timeline_5 ReverseFromEnd))))
    (:then_2
      (Utilities|FlowControl|Delay 0.2)
      (if Condition
        (Rendering|SetVisibility _materialbillboard2 true false)
        (bind _newtrack_0_3 (Timeline|Timeline_7 PlayFromStart)
          (:Update
            (Transformation|SetRelativeLocation _materialbillboard2 (Math|Vector|Lerp(Vector) "0, 0, 0" "0, 0,5.000000" _newtrack_0_3) false false))
          (:Finished
            (if (not Condition)
              (Rendering|SetVisibility _materialbillboard2 false false))))
        (else
          (Timeline|Timeline_7 ReverseFromEnd))))
    (:then_3
      (Utilities|FlowControl|Delay 0.3)
      (if Condition
        (Rendering|SetVisibility _materialbillboard3 true false)
        (bind _newtrack_0_4 (Timeline|Timeline_6 PlayFromStart)
          (:Update
            (Transformation|SetRelativeLocation _materialbillboard3 (Math|Vector|Lerp(Vector) "0, 0, 0" "0, 0,5.000000" _newtrack_0_4) false false))
          (:Finished
            (if (not Condition)
              (Rendering|SetVisibility _materialbillboard3 false false))))
        (else
          (Timeline|Timeline_6 ReverseFromEnd))))
    (:then_4
      (if (Variables|Default|GetGrabbed)
        (Variables|Default|SetGrabbed false)
        (elif Condition
          (bind _newtrack_0_5 (Timeline|Timeline_8 PlayFromStart)
            (:Update
              (Variables|Default|SetOut%20Rotation (Math|Rotator|MakeRotator (Math|Float|Lerp 9e+01 7e+01 _newtrack_0_5) 0.0 0.0))))
          (else
            (Timeline|Timeline_8 ReverseFromEnd)))))))

(event Custom|CustomEvent_0)

(event EventBeginPlay
  (|CallParentFunction)
  (Class|NiagaraComponent|SetPaused (Variables|Default|GetNiagara) true)
  (bind _returnvalue (Actor|GetActorOfClass "/Game/Blueprints/BP/Apple.Apple_C"))
  (Variables|Default|SetAppleRef _returnvalue)
  (bind _returnvalue_2 (Actor|GetActorOfClass "/Game/Blueprints/VR_Character/BP_UpdatedVRPawn.BP_UpdatedVRPawn_C"))
  (Variables|Default|SetPawnref _returnvalue_2)
  (bind _returnvalue_3 (Actor|GetActorOfClass "/Game/Blueprints/BP/BP_Jewel.BP_Jewel_C"))
  (Variables|Default|SetJewel%20Ref _returnvalue_3)
  (bind _returnvalue_4 (Actor|GetActorOfClass "/Game/Blueprints/BP/BP_FancyBook.BP_FancyBook_C"))
  (Variables|Default|SetBookRef _returnvalue_4)
  (bind _returnvalue_5 (Actor|GetActorOfClass "/Game/Blueprints/Paintbrush/Paintrbsuh.Paintrbsuh_C"))
  (Variables|Default|SetPaintBrushRef _returnvalue_5))

(event EventBacktoOriginal
  (if (Variables|Default|GetAte)
    (Utilities|FlowControl|DoOnce false)))

(event EventOnGrabbed
  (if (Variables|Default|GetMouthOpen)
    (Utilities|FlowControl|Sequence
      (:then_0
        (Timeline|Timeline_9 Stop
          (:Finished
            _)))
      (:then_1
        (Variables|Default|SetGrabbed true)
        (Variables|Default|SetMouthOpen false)))
    (CallFunction|ThoughtBubble false)
    (Variables|Default|SetMouthOpen false)
    (Utilities|FlowControl|DoOnce false) ; enters at Reset
  ))

(event EventOnDropped
  (Timeline|Timeline_3 Stop))

(fn ConstructionScript
  (|CallParentFunction))