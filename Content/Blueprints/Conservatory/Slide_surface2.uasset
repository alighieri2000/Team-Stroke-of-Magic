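; Second sliding surface in the Conservatory, a grabbable child Blueprint that forms part of the conduit shelves connection.
; UnlockLeft sets its maximum travel limit; dropping it near that end locks grabbing, snaps it into place and calls 2Connected on BP_Conduit_Shelves.
; Its box overlap breaks the grip on contact with Slide_surface1, and a roller sound plays while held.
; A BP_MoveShelf1 lookup is left unconnected.
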(event OnComponentBeginOverlap(Box)
  (params (OverlappedComponent :type Primitive%20Component%20Object%20Reference) (OtherActor :type Actor%20Object%20Reference) (OtherComp :type Primitive%20Component%20Object%20Reference) (OtherBodyIndex :type Integer) (bFromSweep :type Boolean) (SweepResult :type Hit%20Result%20Structure%20%28by%20ref%29))
  (if (== (Variables|Default|GetSlideRef) OtherActor)
    (CallFunction|BreakGrip)))

(event OnComponentEndOverlap(Box)
  (params (OverlappedComponent :type Primitive%20Component%20Object%20Reference) (OtherActor :type Actor%20Object%20Reference) (OtherComp :type Primitive%20Component%20Object%20Reference) (OtherBodyIndex :type Integer)))

(event OnGrabbed(GrabComponent)
  (Audio|Components|Audio|Play (Variables|Default|GetRollers_Small_Cue) 0.0))

(event OnDropped(GrabComponent)
  (Audio|Components|Audio|Stop (Variables|Default|GetRollers_Small_Cue)))

(event Custom|UnlockLeft
  (Variables|Default|SetMaximum%20Limit 388.0))

(event Custom|Finished)

(event EventBeginPlay
  (|CallParentFunction)
  (bind _returnvalue (Actor|GetActorOfClass "/Game/Blueprints/Conservatory/Slide_surface1.Slide_surface1_C"))
  (Variables|Default|SetSlideRef _returnvalue)
  (bind _returnvalue_2 (Actor|GetActorOfClass "/Game/Blueprints/PuzzleElements/BP_Conduit_Shelves.BP_Conduit_Shelves_C"))
  (Variables|Default|SetCondRef _returnvalue_2))

(event EventOnDropped
  (if (> (.x (Variables|Default|GetOut%20Vector)) 385.0)
    (Variables|Default|SetGrabLocked true)
    (Transformation|SetRelativeLocation (Variables|Default|GetRecieveTransform) (Math|Vector|MakeVector 388.0 0.0 0.0) false false)
    (Default|2Connected (Variables|Default|GetCondRef))))

(fn ConstructionScript
  (|CallParentFunction))