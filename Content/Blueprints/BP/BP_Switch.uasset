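; BP_Switch is a physics-driven switch with a valve mesh and two end trigger boxes, tracking its side in an LR flag.
; While ValveMesh overlaps either box, that box's timeline pushes Cube1 along the Scene-to-box direction each update.
; A timeline started at BeginPlay copies Cube1's yaw, clamped to a half turn, onto ValveMesh1.
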(event OnComponentBeginOverlap(ColBox2)
  (params (OverlappedComponent :type Primitive%20Component%20Object%20Reference) (OtherActor :type Actor%20Object%20Reference) (OtherComp :type Primitive%20Component%20Object%20Reference) (OtherBodyIndex :type Integer) (bFromSweep :type Boolean) (SweepResult :type Hit%20Result%20Structure%20%28by%20ref%29))
  (if (== OtherComp (Variables|Default|GetValveMesh))
    (Variables|Default|SetL/R true)
    (Utilities|FlowControl|Sequence
      (:then_0
        (Timeline|Timeline_0 Play
          (:Update
            (Physics|AddForce (Variables|Default|GetCube1) (* (- (Variables|/Script/Engine.SceneComponent|GetRelativeLocation (Variables|Default|GetColBox2)) (Variables|/Script/Engine.SceneComponent|GetRelativeLocation (Variables|Default|GetScene))) 2e+02) "None" false)))))))

(event OnComponentBeginOverlap(ColBox1)
  (params (OverlappedComponent :type Primitive%20Component%20Object%20Reference) (OtherActor :type Actor%20Object%20Reference) (OtherComp :type Primitive%20Component%20Object%20Reference) (OtherBodyIndex :type Integer) (bFromSweep :type Boolean) (SweepResult :type Hit%20Result%20Structure%20%28by%20ref%29))
  (if (== OtherComp (Variables|Default|GetValveMesh))
    (Variables|Default|SetL/R false)
    (Timeline|Timeline_1 Play
      (:Update
        (Physics|AddForce (Variables|Default|GetCube1) (* (- (Variables|/Script/Engine.SceneComponent|GetRelativeLocation (Variables|Default|GetColBox1)) (Variables|/Script/Engine.SceneComponent|GetRelativeLocation (Variables|Default|GetScene))) 2e+02) "None" false)))))

(event OnComponentEndOverlap(ColBox2)
  (params (OverlappedComponent :type Primitive%20Component%20Object%20Reference) (OtherActor :type Actor%20Object%20Reference) (OtherComp :type Primitive%20Component%20Object%20Reference) (OtherBodyIndex :type Integer))
  (if (== OtherComp (Variables|Default|GetValveMesh))
    (Timeline|Timeline_0 Stop
      (:Update
        (Physics|AddForce (Variables|Default|GetCube1) (* (- (Variables|/Script/Engine.SceneComponent|GetRelativeLocation (Variables|Default|GetColBox2)) (Variables|/Script/Engine.SceneComponent|GetRelativeLocation (Variables|Default|GetScene))) 2e+02) "None" false)))))

(event OnComponentEndOverlap(ColBox1)
  (params (OverlappedComponent :type Primitive%20Component%20Object%20Reference) (OtherActor :type Actor%20Object%20Reference) (OtherComp :type Primitive%20Component%20Object%20Reference) (OtherBodyIndex :type Integer))
  (if (== OtherComp (Variables|Default|GetValveMesh))
    (Timeline|Timeline_1 Stop
      (:Update
        (Physics|AddForce (Variables|Default|GetCube1) (* (- (Variables|/Script/Engine.SceneComponent|GetRelativeLocation (Variables|Default|GetColBox1)) (Variables|/Script/Engine.SceneComponent|GetRelativeLocation (Variables|Default|GetScene))) 2e+02) "None" false)))))

(event EventBeginPlay
  (Variables|Default|SetCube_0 0)
  (Timeline|Timeline_2 Play
    (:Update
      (Transformation|SetRelativeRotation (Variables|Default|GetValveMesh1) (Math|Rotator|MakeRotator 0.0 0.0 (Math|Float|Clamp(Float) (.yaw (Variables|/Script/Engine.SceneComponent|GetRelativeRotation (Variables|Default|GetCube1))) 0.0 1.8e+02)) false false))))

(fn ConstructionScript)