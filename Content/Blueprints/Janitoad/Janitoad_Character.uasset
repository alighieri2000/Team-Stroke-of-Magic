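; Janitoad character that cleans up green paint particles and resets Dot actors it touches.
; On play it gathers Dots and picks a green paint actor within 600 units of its mesh.
; It targets that paint's oldest particle, calling Yeet on it when Sphere3 overlaps it, then refreshes the target.
; A timeline helps re-trigger overlap checks, and Sphere4 overlaps reset gathered Dots.
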(event OnComponentBeginOverlap(Sphere3)
  (params (OverlappedComponent :type Primitive%20Component%20Object%20Reference) (OtherActor :type Actor%20Object%20Reference) (OtherComp :type Primitive%20Component%20Object%20Reference) (OtherBodyIndex :type Integer) (bFromSweep :type Boolean) (SweepResult :type Hit%20Result%20Structure%20%28by%20ref%29))
  (bind _green_paint_ref (Variables|Default|GetGreen%20Paint%20Ref))
  (bind _oldestparticle (Variables|/Game/Blueprints/Palette/BP_MainGreenPaint.BP_MainGreenPaint_C|GetOldestParticle _green_paint_ref))
  (Utilities|IsValid _green_paint_ref
    (:Is%20Valid
      (if (== _oldestparticle OtherComp)
        (Default|Yeet _green_paint_ref (Utilities|Array|FindItem (Variables|/Game/Blueprints/Palette/BP_MainGreenPaint.BP_MainGreenPaint_C|GetPaintObjects _green_paint_ref) _oldestparticle))
        (CallFunction|CollisionRefresh)))))

(event OnComponentBeginOverlap(Sphere4)
  (params (OverlappedComponent :type Primitive%20Component%20Object%20Reference) (OtherActor :type Actor%20Object%20Reference) (OtherComp :type Primitive%20Component%20Object%20Reference) (OtherBodyIndex :type Integer) (bFromSweep :type Boolean) (SweepResult :type Hit%20Result%20Structure%20%28by%20ref%29))
  (for _array_element (Variables|Default|GetDots%20Actors)
    (if (== _array_element OtherActor)
      (Default|Reset _array_element))))

(event Custom|Update%20Paint%20Location
  (bind _green_paint_ref (Variables|Default|GetGreen%20Paint%20Ref))
  (bind _oldestparticle (Variables|/Game/Blueprints/Palette/BP_MainGreenPaint.BP_MainGreenPaint_C|GetOldestParticle _green_paint_ref))
  (Utilities|IsValid _oldestparticle
    (:Is%20Valid
      (bind _output_get (Variables|Default|SetChase%20Point (Transformation|GetWorldLocation _oldestparticle))))
    (:Is%20Not%20Valid
      _))
  (if (Math|Vector|Equal(Vector) (Transformation|GetWorldLocation (Variables|Default|GetSphere1)) _output_get 0.0001)
    (Variables|Default|SetNewVar_0 false)
    (CallFunction|StopSearch)))

(event Custom|Kill
  (Actor|DestroyActor))

(event Custom|Collision%20Refresh
  (bind _green_paint_ref (Variables|Default|GetGreen%20Paint%20Ref))
  (bind _oldestparticle (Variables|/Game/Blueprints/Palette/BP_MainGreenPaint.BP_MainGreenPaint_C|GetOldestParticle _green_paint_ref))
  (CallFunction|UpdatePaintLocation)
  (for _array_element (Class|PrimitiveComponent|GetOverlappingComponents (Variables|Default|GetSphere3))
    (if (== _array_element _oldestparticle)
      (Utilities|IsValid _oldestparticle
        (:Is%20Valid
          (Default|Yeet _green_paint_ref (Utilities|Array|FindItem (Variables|/Game/Blueprints/Palette/BP_MainGreenPaint.BP_MainGreenPaint_C|GetPaintObjects (Variables|Default|GetGreen%20Paint%20Ref)) _oldestparticle))
          (Timeline|Timeline_0 PlayFromStart
            (:Finished
              (CallFunction|CollisionRefresh))))
        (:Is%20Not%20Valid
          (Timeline|Timeline_0 PlayFromStart))))))

(event Custom|StopSearch
  (Timeline|Timeline_0 Stop
    (:Finished
      (CallFunction|CollisionRefresh))))

(event EventBeginPlay
  (if (Variables|Default|GetDots)
    (bind _outactors (Actor|GetAllActorsOfClass "/Game/Blueprints/Spline_BP/Dot.Dot_C"))
    (Variables|Default|SetDots%20Actors _outactors))
  (bind _outactors_2 (Actor|GetAllActorsOfClass "/Game/Blueprints/Palette/BP_MainGreenPaint.BP_MainGreenPaint_C"))
  (bind _output_get (Variables|Default|SetGreen%20Paint%20Actors _outactors_2))
  (for _array_element _output_get
    (if (< (Math|Vector|VectorLength (- (Transformation|GetWorldLocation (Variables|Character|GetMesh)) (Transformation|GetActorLocation _array_element))) 6e+02)
      (Utilities|FlowControl|DoOnce false
        (:Completed
          (Utilities|IsValid _array_element
            (:Is%20Valid
              (Variables|Default|SetGreen%20Paint%20Ref _array_element)))))))
  (CallFunction|CollisionRefresh))

(fn ConstructionScript)