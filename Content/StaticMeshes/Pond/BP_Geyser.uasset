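; BP_Geyser is a pond prop that animates a rising, wobbling bubble mesh (SMCrystal) with a bubble sound.
; On BeginPlay it plays BubblesCue and starts two timelines, with play rates derived from their durations and randomized start times.
; BubbleLocation lerps the mesh's relative Z up to HowFarZ.
; BubbleWaver applies squash and stretch around BubbleScale, moving X/Y opposite to Z.
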(event EventBeginPlay
  (bind _bubblelocation (Variables|Default|GetBubbleLocation))
  (bind _duration (Variables|Default|GetDuration))
  (bind _bubblewaver (Variables|Default|GetBubbleWaver))
  (bind _waverduration (Variables|Default|GetWaverDuration))
  (Audio|Components|Audio|Play (Variables|Default|GetBubbles_Cue) 0.0)
  (Utilities|FlowControl|Sequence
    (:then_0
      (Components|Timeline|SetPlayRate _bubblelocation (Math|Float|SafeDivide 1.0 _duration))
      (Components|Timeline|SetNewTime _bubblelocation (Math|Float|Lerp 0.0 _duration (Math|Random|RandomFloat)))
      (bind _newtrack_0 (Timeline|BubbleLocation Play)
        (:Update
          (Transformation|SetRelativeTransform (Variables|Default|GetSM_Crystal) (Math|Transform|MakeTransform (Math|Vector|MakeVector 0.0 0.0 (Math|Float|Lerp 0.0 (Variables|Default|GethowFarZ) _newtrack_0)) "0, 0, 0" "1,1,1") false false))))
    (:then_1
      (Components|Timeline|SetPlayRate _bubblewaver (Math|Float|SafeDivide 1.0 _waverduration))
      (Components|Timeline|SetNewTime _bubblewaver (Math|Float|Lerp 0.0 _waverduration (Math|Random|RandomFloat)))
      (bind _newtrack_0_2 (Timeline|BubbleWaver Play)
        (:Update
          (Transformation|SetRelativeScale3D (Variables|Default|GetSM_Crystal) (Math|Vector|MakeVector (* (+ 1.0 _newtrack_0_2) (Variables|Default|GetBubbleScale)) (* (+ 1.0 _newtrack_0_2) (Variables|Default|GetBubbleScale)) (* (- 1.0 _newtrack_0_2) (Variables|Default|GetBubbleScale)))))))))

(fn ConstructionScript)