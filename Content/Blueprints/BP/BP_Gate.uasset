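; BP_Gate is a mechanical gate that animates with chains, gears and grinding sounds when its LowerGate event is called.
; LowerGate starts two offset grinding sounds and a timeline that lerps the gate's relative Z and rotates two gear meshes.
; A second timeline runs alongside to slide two chain meshes, and is stopped when the gate timeline finishes.
; The delayed stops for the grinding audio are unconnected, and BeginPlay does nothing.
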(event Custom|LowerGate
  (Utilities|FlowControl|Sequence
    (:then_0
      (Audio|Components|Audio|Play (Variables|Default|GetAC_Gear_Grinding) 0.0)
      (Audio|Components|Audio|Play (Variables|Default|GetAC_Gear_Grinding1) 0.1))
    (:then_1
      (bind _lower (Timeline|Timeline_0 Play)
        (:Update
          (Transformation|SetRelativeLocation (Variables|Default|GetGate) (Math|Vector|MakeVector 0.0 0.0 (Math|Float|Lerp 0.0 (Variables|Default|Get250) _lower)) false false)
          (Transformation|SetRelativeRotation (Variables|Default|Getsm_ChainGear) (Math|Rotator|Lerp(Rotator) "0, 0, 0" "-260.000000, 0, 0" _lower) false false))
        (:Finished
          (Utilities|FlowControl|Sequence
            (:then_0
              (bind _newtrack_0 (Timeline|Timeline_1 Stop)
                (:Update
                  (Transformation|SetRelativeLocation (Variables|Default|Getsm_Chain) (Math|Vector|Lerp(Vector) "-34.758598,607.517151,141.269836" "-34.758598,607.517151,96.831032" _newtrack_0) false false)
                  (Transformation|SetRelativeLocation (Variables|Default|Getsm_Chain4) (Math|Vector|Lerp(Vector) "33.910690,607.517151,141.269836" "33.910690,607.517151,96.831032" (* _newtrack_0 -1.0)) false false))))))))
    (:then_2
      (Timeline|Timeline_1 Play))))

(event EventBeginPlay
  (Utilities|FlowControl|Sequence))

(event Collision|EventActorBeginOverlap
  (params (OtherActor :type Actor%20Object%20Reference)))

(event EventTick
  (params (DeltaSeconds :type Float%20%28single-precision%29)))

(fn ConstructionScript)