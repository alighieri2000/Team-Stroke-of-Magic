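; BP_BubbleGeyser is an animated bubble effect that moves and wobbles a Sphere component.
; On BeginPlay it starts two timelines: BubbleUp lerps the sphere's relative Z from zero toward NewLocationZ.
; BubbleWaver applies squash and stretch, offsetting X and Y scale opposite to Z, multiplied by BubbleScale.
; It has no active overlap, tick or construction logic.
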(event EventBeginPlay
  (Utilities|FlowControl|Sequence
    (:then_0
      (bind _newtrack_0 (Timeline|Bubble%20up Play)
        (:Update
          (Transformation|SetRelativeLocation (Variables|Default|GetSphere) (Math|Vector|MakeVector 0.0 0.0 (Math|Float|Lerp 0.0 (Variables|Default|GetNew%20Location%20Z) _newtrack_0)) false false))))
    (:then_1
      (bind _newtrack_0_2 (Timeline|BubbleWaver Play)
        (:Update
          (Transformation|SetRelativeScale3D (Variables|Default|GetSphere) (Math|Vector|MakeVector (* (+ 1.0 _newtrack_0_2) (Variables|Default|GetBubbleScale)) (* (+ 1.0 _newtrack_0_2) (Variables|Default|GetBubbleScale)) (* (- 1.0 _newtrack_0_2) (Variables|Default|GetBubbleScale)))))))))

(event Collision|EventActorBeginOverlap
  (params (OtherActor :type Actor%20Object%20Reference)))

(event EventTick
  (params (DeltaSeconds :type Float%20%28single-precision%29)))

(fn ConstructionScript)