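; Conduit puzzle element that unlocks the classroom backdoor once all of its dots are primed.
; On BeginPlay it caches the classroom door and every Dot actor in the level.
; UpdatePrimedList checks only dots tagged Classroom Backdoor by enum; when all are primed, it notifies the door and unlocks it.
; Overlaps between BrushBounds2 and the brush's collision sphere call the parent's begin and exit handling.
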(event OnComponentBeginOverlap(BrushBounds2)
  (params (OverlappedComponent :type Primitive%20Component%20Object%20Reference) (OtherActor :type Actor%20Object%20Reference) (OtherComp :type Primitive%20Component%20Object%20Reference) (OtherBodyIndex :type Integer) (bFromSweep :type Boolean) (SweepResult :type Hit%20Result%20Structure%20%28by%20ref%29))
  (if (== OtherComp (Variables|/Game/Blueprints/Paintbrush/Paintrbsuh.Paintrbsuh_C|GetCollisionSphere (Variables|Default|GetBrushRefVar)))
    (CallFunction|ParentBegin)))

(event OnComponentEndOverlap(BrushBounds2)
  (params (OverlappedComponent :type Primitive%20Component%20Object%20Reference) (OtherActor :type Actor%20Object%20Reference) (OtherComp :type Primitive%20Component%20Object%20Reference) (OtherBodyIndex :type Integer))
  (if (== OtherComp (Variables|/Game/Blueprints/Paintbrush/Paintrbsuh.Paintrbsuh_C|GetCollisionSphere (Variables|Default|GetBrushRefVar)))
    (CallFunction|ExitedParent)))

(event Custom|UpdatePrimedList
  (Variables|Default|SetAll%20Primed_0 true)
  (for _array_element (stale EventBeginPlay _output_get)
    (switch Utilities|FlowControl|Switch|SwitchonRoomEnum (Variables|/Game/Blueprints/Spline_BP/Dot.Dot_C|Getenum _array_element)
      (:NewEnumerator5
        (if (not (Variables|/Game/Blueprints/Spline_BP/Dot.Dot_C|GetPrimed? _array_element))
          (Variables|Default|SetAll%20Primed_0 false)))))
  (if (Variables|Default|GetAll%20Primed_0)
    (CallFunction|Finished)
    (Default|UnlockBackdoor (Variables|Default|GetClassroom_Door_Ref))))

(event EventBeginPlay
  (|CallParentFunction)
  (bind _returnvalue (Actor|GetActorOfClass "/Game/Blueprints/PuzzleElements/SM_Classroom_Door_Unlock.SM_Classroom_Door_Unlock_C"))
  (Variables|Default|SetClassroom_Door_Ref _returnvalue)
  (bind _outactors (Actor|GetAllActorsOfClass "/Game/Blueprints/Spline_BP/Dot.Dot_C"))
  (bind _output_get (Variables|Default|SetOut%20Actors _outactors)))

(event EventFinished
  (Default|ConduitBackdoorFinished (Variables|Default|GetClassroom_Door_Ref)))

(fn ConstructionScript
  (|CallParentFunction))