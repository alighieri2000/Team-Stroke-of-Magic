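; BP_SlidePuzzle is a star-piece slide puzzle in the Conservatory that reveals the library key when solved.
; It caches four child-actor pieces, and three trigger boxes each snap and lock their matching piece (01, 03 or 04).
; Once those three are locked, a timeline shifts the Scene component while triggering a completion sound, unpausing particles and calling PoofIn on the key.
; A second timeline pauses the particles when finished.
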(event OnComponentBeginOverlap(Box)
  (params (OverlappedComponent :type Primitive%20Component%20Object%20Reference) (OtherActor :type Actor%20Object%20Reference) (OtherComp :type Primitive%20Component%20Object%20Reference) (OtherBodyIndex :type Integer) (bFromSweep :type Boolean) (SweepResult :type Hit%20Result%20Structure%20%28by%20ref%29))
  (bind _as_bp_slide_puzzle_01 (Variables|Default|GetAs%20BP%20Slide%20Puzzle%2001))
  (bind _ps (Variables|Default|GetPS))
  (if (== OtherActor _as_bp_slide_puzzle_01)
    (Transformation|SetWorldLocation (Variables|/Game/Blueprints/Conservatory/BP_InteractableParent.BP_InteractableParent_C|GetInitialTransform (Variables|Default|GetAs%20BP%20Slide%20Puzzle%2001)) (Transformation|GetWorldLocation (Variables|Default|GetBox)) false false)
    (bind _output_get (Variables|/Game/Blueprints/Conservatory/BP_InteractableParent.BP_InteractableParent_C|SetGrabLocked _as_bp_slide_puzzle_01 true))
    (if (Math|Boolean|ANDBoolean _output_get (stale OnComponentBeginOverlap(Box1) _output_get) (stale OnComponentBeginOverlap(Box2) _output_get))
      (bind _newtrack_0 (Timeline|Timeline_1 PlayFromStart)
        (:Update
          (Transformation|SetRelativeLocation (Variables|Default|GetScene) (Math|Vector|Lerp(Vector) "0, 0, 0" "-3.000000, 0, 0" _newtrack_0) false false)
          (Audio|Components|Audio|Play (Variables|Default|GetcompletionStars_Cue) 0.0)
          (Class|NiagaraComponent|SetPaused _ps false)
          (Default|Poofin (Variables|Default|GetKeyReff))
          (Timeline|Timeline_0 PlayFromStart
            (:Finished
              (Class|NiagaraComponent|SetPaused _ps true))))))))

(event OnComponentBeginOverlap(Box1)
  (params (OverlappedComponent :type Primitive%20Component%20Object%20Reference) (OtherActor :type Actor%20Object%20Reference) (OtherComp :type Primitive%20Component%20Object%20Reference) (OtherBodyIndex :type Integer) (bFromSweep :type Boolean) (SweepResult :type Hit%20Result%20Structure%20%28by%20ref%29))
  (bind _as_bp_slide_puzzle_03 (Variables|Default|GetAs%20BP%20Slide%20Puzzle%2003))
  (bind _ps (Variables|Default|GetPS))
  (if (== OtherActor _as_bp_slide_puzzle_03)
    (Transformation|SetWorldLocation (Variables|/Game/Blueprints/Conservatory/BP_InteractableParent.BP_InteractableParent_C|GetInitialTransform _as_bp_slide_puzzle_03) (Transformation|GetWorldLocation (Variables|Default|GetBox1)) false false)
    (bind _output_get (Variables|/Game/Blueprints/Conservatory/BP_InteractableParent.BP_InteractableParent_C|SetGrabLocked _as_bp_slide_puzzle_03 true))
    (if (Math|Boolean|ANDBoolean (stale OnComponentBeginOverlap(Box) _output_get) _output_get (stale OnComponentBeginOverlap(Box2) _output_get))
      (bind _newtrack_0 (Timeline|Timeline_1 PlayFromStart)
        (:Update
          (Transformation|SetRelativeLocation (Variables|Default|GetScene) (Math|Vector|Lerp(Vector) "0, 0, 0" "-3.000000, 0, 0" _newtrack_0) false false)
          (Audio|Components|Audio|Play (Variables|Default|GetcompletionStars_Cue) 0.0)
          (Class|NiagaraComponent|SetPaused _ps false)
          (Default|Poofin (Variables|Default|GetKeyReff))
          (Timeline|Timeline_0 PlayFromStart
            (:Finished
              (Class|NiagaraComponent|SetPaused _ps true))))))))

(event OnComponentBeginOverlap(Box2)
  (params (OverlappedComponent :type Primitive%20Component%20Object%20Reference) (OtherActor :type Actor%20Object%20Reference) (OtherComp :type Primitive%20Component%20Object%20Reference) (OtherBodyIndex :type Integer) (bFromSweep :type Boolean) (SweepResult :type Hit%20Result%20Structure%20%28by%20ref%29))
  (bind _ps (Variables|Default|GetPS))
  (bind _as_bp_slide_puzzle_04 (Variables|Default|GetAs%20BP%20Slide%20Puzzle%2004))
  (if (== OtherActor _as_bp_slide_puzzle_04)
    (Transformation|SetWorldLocation (Variables|/Game/Blueprints/Conservatory/BP_InteractableParent.BP_InteractableParent_C|GetInitialTransform _as_bp_slide_puzzle_04) (Transformation|GetWorldLocation (Variables|Default|GetBox2)) false false)
    (bind _output_get (Variables|/Game/Blueprints/Conservatory/BP_InteractableParent.BP_InteractableParent_C|SetGrabLocked _as_bp_slide_puzzle_04 true))
    (if (Math|Boolean|ANDBoolean (stale OnComponentBeginOverlap(Box) _output_get) (stale OnComponentBeginOverlap(Box1) _output_get) _output_get)
      (bind _newtrack_0 (Timeline|Timeline_1 PlayFromStart)
        (:Update
          (Transformation|SetRelativeLocation (Variables|Default|GetScene) (Math|Vector|Lerp(Vector) "0, 0, 0" "-3.000000, 0, 0" _newtrack_0) false false)
          (Audio|Components|Audio|Play (Variables|Default|GetcompletionStars_Cue) 0.0)
          (Class|NiagaraComponent|SetPaused _ps false)
          (Default|Poofin (Variables|Default|GetKeyReff))
          (Timeline|Timeline_0 PlayFromStart
            (:Finished
              (Class|NiagaraComponent|SetPaused _ps true))))))))

(event EventBeginPlay
  (Class|NiagaraComponent|SetPaused (Variables|Default|GetPS) true)
  (bind _asbp_slide_puzzle_01 (Utilities|Casting|CastToBP_SlidePuzzle01 (Variables|/Script/Engine.ChildActorComponent|GetChildActor (Variables|Default|GetStarPiece1))))
  (Variables|Default|SetAs%20BP%20Slide%20Puzzle%2001 _asbp_slide_puzzle_01)
  (bind _asbp_slide_puzzle_02 (Utilities|Casting|CastToBP_SlidePuzzle02 (Variables|/Script/Engine.ChildActorComponent|GetChildActor (Variables|Default|GetStarPiece2))))
  (Variables|Default|SetAs%20BP%20Slide%20Puzzle%2002 _asbp_slide_puzzle_02)
  (bind _asbp_slide_puzzle_03 (Utilities|Casting|CastToBP_SlidePuzzle03 (Variables|/Script/Engine.ChildActorComponent|GetChildActor (Variables|Default|GetStarPiece4))))
  (Variables|Default|SetAs%20BP%20Slide%20Puzzle%2003 _asbp_slide_puzzle_03)
  (bind _asbp_slide_puzzle_04 (Utilities|Casting|CastToBP_SlidePuzzle04 (Variables|/Script/Engine.ChildActorComponent|GetChildActor (Variables|Default|GetStarPiece3))))
  (Variables|Default|SetAs%20BP%20Slide%20Puzzle%2004 _asbp_slide_puzzle_04)
  (bind _returnvalue (Actor|GetActorOfClass "/Game/Blueprints/Library_Puzzle_Elements/BP_LibraryKey.BP_LibraryKey_C"))
  (Variables|Default|SetKeyReff _returnvalue))

(event Collision|EventActorBeginOverlap
  (params (OtherActor :type Actor%20Object%20Reference)))

(event EventTick
  (params (DeltaSeconds :type Float%20%28single-precision%29)))

(fn ConstructionScript)