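; BP_Swatch is a grabbable VR paint palette with up to three paint globs, gated by HasPaint flags, for loading the paintbrush.
; Brush overlap on a rune loads that paint, plays splash and dip sounds, shrinks its glob and regrows the previously taken one.
; Timelines lerp glob transforms, reversing to shrink; only Rune1 guards against reloading its active paint.
; Grabs are forwarded to the VR pawn's MatrixGrab.
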(event OnComponentBeginOverlap(Rune1)
  (params (OverlappedComponent :type Primitive%20Component%20Object%20Reference) (OtherActor :type Actor%20Object%20Reference) (OtherComp :type Primitive%20Component%20Object%20Reference) (OtherBodyIndex :type Integer) (bFromSweep :type Boolean) (SweepResult :type Hit%20Result%20Structure%20%28by%20ref%29))
  (bind _brushreff (Variables|Default|GetBrushREFF))
  (if (Variables|Default|GetHasPaint1)
    (if (not (Variables|Default|GetPaint1on))
      (if (== (Variables|/Game/Blueprints/Paintbrush/Paintrbsuh.Paintrbsuh_C|GetCollisionSphere _brushreff) OtherComp)
        (Default|Load _brushreff "NewEnumerator0")
        (Variables|Default|SetPaint1on true)
        (Audio|Components|Audio|Play (Variables|Default|GetcauldronMagicSplash_Cue) 0.0)
        (CallFunction|Glob1Shrink)
        (if (Variables|Default|GetPaint2on)
          (CallFunction|Glob2Grow)
          (Variables|Default|SetPaint2on false))
        (if (Variables|Default|GetPaint3on)
          (CallFunction|Glob3Grow)
          (Variables|Default|SetPaint3on false))))))

(event OnComponentBeginOverlap(Rune2)
  (params (OverlappedComponent :type Primitive%20Component%20Object%20Reference) (OtherActor :type Actor%20Object%20Reference) (OtherComp :type Primitive%20Component%20Object%20Reference) (OtherBodyIndex :type Integer) (bFromSweep :type Boolean) (SweepResult :type Hit%20Result%20Structure%20%28by%20ref%29))
  (bind _brushreff (Variables|Default|GetBrushREFF))
  (if (== (Variables|/Game/Blueprints/Paintbrush/Paintrbsuh.Paintrbsuh_C|GetCollisionSphere _brushreff) OtherComp)
    (if (Variables|Default|GetHasPaint2)
      (Default|Load _brushreff "NewEnumerator4")
      (Variables|Default|SetPaint2on true)
      (Audio|Components|Audio|Play (Variables|Default|GetcauldronMagicSplash_Cue) 0.0)
      (CallFunction|Glob2Shrink)
      (if (Variables|Default|GetPaint1on)
        (CallFunction|Glob1Grow)
        (Variables|Default|SetPaint1on false))
      (if (Variables|Default|GetPaint3on)
        (CallFunction|Glob3Grow)
        (Variables|Default|SetPaint3on false)))))

(event OnComponentBeginOverlap(Rune3)
  (params (OverlappedComponent :type Primitive%20Component%20Object%20Reference) (OtherActor :type Actor%20Object%20Reference) (OtherComp :type Primitive%20Component%20Object%20Reference) (OtherBodyIndex :type Integer) (bFromSweep :type Boolean) (SweepResult :type Hit%20Result%20Structure%20%28by%20ref%29))
  (bind _brushreff (Variables|Default|GetBrushREFF))
  (if (== (Variables|/Game/Blueprints/Paintbrush/Paintrbsuh.Paintrbsuh_C|GetCollisionSphere _brushreff) OtherComp)
    (if (Variables|Default|GetHasPaint3)
      (Default|Load _brushreff "NewEnumerator5")
      (Variables|Default|SetPaint3on true)
      (Audio|Components|Audio|Play (Variables|Default|GetcauldronMagicSplash_Cue) 0.0)
      (CallFunction|Glob3Shrink)
      (if (Variables|Default|GetPaint1on)
        (CallFunction|Glob1Grow)
        (Variables|Default|SetPaint1on false))
      (if (Variables|Default|GetPaint2on)
        (CallFunction|Glob2Grow)
        (Variables|Default|SetPaint2on false)))))

(event OnGrabbed(GrabComponent)
  (Default|MatrixGrab (Variables|Default|GetVRRef) (Variables|Default|GetGrabComponent)))

(event Custom|Glob1Shrink
  (CallFunction|SetComponentSound (Variables|Default|GetBrush_Dip1) "/Game/Audio-Revised/Assets/Object-AMBX/CoreMechanics/cue/Brush_Dip.Brush_Dip")
  (bind _newtrack_0 (Timeline|GlobScaleUp ReverseFromEnd)
    (:Update
      (Transformation|SetRelativeTransform (Variables|Default|GetPaintGlob1) (Math|Transform|Lerp(Transform) (Variables|Default|GetGlob1_Start) (Variables|Default|GetGlob2_Start) _newtrack_0) false false))))

(event Custom|Glob2Shrink
  (CallFunction|SetComponentSound (Variables|Default|GetBrush_Dip2) "/Game/Audio-Revised/Assets/Object-AMBX/CoreMechanics/cue/Brush_Dip.Brush_Dip")
  (bind _newtrack_0 (Timeline|Timeline_0 ReverseFromEnd)
    (:Update
      (Transformation|SetRelativeTransform (Variables|Default|GetPaintGlob2) (Math|Transform|Lerp(Transform) (Variables|Default|GetGlob1_Start) (Variables|Default|GetGlob2_Start) _newtrack_0) false false))))

(event Custom|Glob2Grow
  (Rendering|SetVisibility (Variables|Default|GetPaintGlob2) true false)
  (bind _newtrack_0 (Timeline|Timeline_0 PlayFromStart)
    (:Update
      (Transformation|SetRelativeTransform (Variables|Default|GetPaintGlob2) (Math|Transform|Lerp(Transform) (Variables|Default|GetGlob1_Start) (Variables|Default|GetGlob2_Start) _newtrack_0) false false))))

(event Custom|Glob3Shrink
  (CallFunction|SetComponentSound (Variables|Default|GetBrush_Dip3) "/Game/Audio-Revised/Assets/Object-AMBX/CoreMechanics/wav/Brush_Dip.Brush_Dip")
  (bind _newtrack_0 (Timeline|Timeline_1 ReverseFromEnd)
    (:Update
      (Transformation|SetRelativeTransform (Variables|Default|GetPaintGlob3) (Math|Transform|Lerp(Transform) (Variables|Default|GetGlob1_Start) (Variables|Default|GetGlob2_Start) _newtrack_0) false false))))

(event Custom|SetComponentSound
  (params (AudioRef :type Audio%20Component%20Object%20Reference) (AudioPlay :type Sound%20Base%20Object%20Reference))
  (Audio|Components|Audio|SetSound AudioRef AudioPlay)
  (Audio|Components|Audio|Play AudioRef 0.0))

(event Custom|Zop
  (params (NewLocation :type Vector))
  (Transformation|SetWorldLocation (Variables|Default|GetCube) NewLocation false false))

(event Custom|Glob3Grow
  (Rendering|SetVisibility (Variables|Default|GetPaintGlob3) true false)
  (bind _newtrack_0 (Timeline|Timeline_1 PlayFromStart)
    (:Update
      (Transformation|SetRelativeTransform (Variables|Default|GetPaintGlob3) (Math|Transform|Lerp(Transform) (Variables|Default|GetGlob1_Start) (Variables|Default|GetGlob2_Start) _newtrack_0) false false))))

(event Custom|Glob1Grow
  (Rendering|SetVisibility (Variables|Default|GetPaintGlob1) true false)
  (bind _newtrack_0 (Timeline|GlobScaleUp PlayFromStart)
    (:Update
      (Transformation|SetRelativeTransform (Variables|Default|GetPaintGlob1) (Math|Transform|Lerp(Transform) (Variables|Default|GetGlob1_Start) (Variables|Default|GetGlob2_Start) _newtrack_0) false false))))

(event EventBeginPlay
  (bind _returnvalue (Actor|GetActorOfClass "/Game/Blueprints/Paintbrush/Paintrbsuh.Paintrbsuh_C"))
  (Variables|Default|SetBrushREFF _returnvalue)
  (bind _returnvalue_2 (Actor|GetActorOfClass "/Game/Blueprints/VR_Character/BP_UpdatedVRPawn.BP_UpdatedVRPawn_C"))
  (Variables|Default|SetVRRef _returnvalue_2)
  (if (Variables|Default|GetHasPaint1)
    (CallFunction|Glob1Grow))
  (if (Variables|Default|GetHasPaint2)
    (CallFunction|Glob2Grow))
  (if (Variables|Default|GetHasPaint3)
    (CallFunction|Glob3Grow)))

(fn ConstructionScript)

(fn OverlapPlayerFunction
  (return false))