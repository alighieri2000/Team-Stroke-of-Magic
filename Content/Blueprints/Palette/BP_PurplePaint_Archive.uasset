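; Paint particle actor that animates a paint mesh in and out, with the static mesh picked from the Paint value in the construction script.
; SpawnIn runs timelines that grow the mesh to the given ParticleSize and shift its relative location, calling SpawnOut when the movement finishes.
; SpawnOut stops the grow timeline and shrinks the mesh.
; Leave drops the root to Z -300 through a DoOnce that each SpawnIn resets.
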(event Custom|Spawn%20In
  (params (ParticleSize :type Vector))
  (bind _particlemesh (Variables|Default|GetParticleMesh))
  (Variables|Default|SetB ParticleSize)
  (Utilities|FlowControl|Sequence
    (:then_0
      (bind _newtrack_0 (Timeline|Timeline_0 PlayFromStart)
        (:Update
          (Transformation|SetRelativeScale3D _particlemesh (Math|Vector|Lerp(Vector) "0.001000,0.001000,0.001000" (Variables|Default|GetB) _newtrack_0)))))
    (:then_1
      (bind _newtrack_0_2 (Timeline|Timeline_1 PlayFromStart)
        (:Update
          (Transformation|SetRelativeLocation _particlemesh (Math|Vector|Lerp(Vector) "0, 0,1.000000" "0, 0, 0" _newtrack_0_2) false false))
        (:Finished
          (CallFunction|SpawnOut))))
    (:then_2
      (bind _newtrack_0_3 (Timeline|Timeline_2 Stop)
        (:Update
          (Transformation|SetRelativeScale3D _particlemesh (Math|Vector|Lerp(Vector) (Variables|Default|GetB) "0.001000,0.001000,0.001000" _newtrack_0_3)))))
    (:then_3
      (Utilities|FlowControl|DoOnce false) ; enters at Reset
    )))

(event Custom|Spawn%20Out
  (bind _particlemesh (Variables|Default|GetParticleMesh))
  (bind _b (Variables|Default|GetB))
  (Utilities|FlowControl|Sequence
    (:then_0
      (bind _newtrack_0 (Timeline|Timeline_2 PlayFromStart)
        (:Update
          (Transformation|SetRelativeScale3D _particlemesh (Math|Vector|Lerp(Vector) _b "0.001000,0.001000,0.001000" _newtrack_0)))))
    (:then_1
      (bind _newtrack_0_2 (Timeline|Timeline_0 Stop)
        (:Update
          (Transformation|SetRelativeScale3D _particlemesh (Math|Vector|Lerp(Vector) "0.001000,0.001000,0.001000" _b _newtrack_0_2)))))))

(event Custom|Leave
  (Utilities|FlowControl|DoOnce false
    (:Completed
      (Transformation|SetRelativeLocation (Variables|Default|GetDefaultSceneRoot) "0, 0,-300.000000" false false))))

(event EventBeginPlay)

(fn ConstructionScript
  (Components|StaticMesh|SetStaticMesh (Variables|Default|GetParticleMesh) (Utilities|Select :Index (Variables|Default|GetPaint) :NewEnumerator3 "/Game/StaticMeshes/Interactables/SM_WhitePaintParticle.SM_WhitePaintParticle" :NewEnumerator0 "/Game/StaticMeshes/Interactables/SM_RedPaintDull.SM_RedPaintDull" :NewEnumerator4 "/Game/StaticMeshes/Interactables/SM_GreenPaintDull.SM_GreenPaintDull" :NewEnumerator5 0 :NewEnumerator1 "/Game/StaticMeshes/Interactables/SM_GreenPaint.SM_GreenPaint")))