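; Final paint puzzle door that opens once its green, purple and yellow slots are all filled with the paintbrush.
; Three overlap boxes check the brush's collision sphere and current paint, then set a flag, play a sound and grow the matching blob mesh via a timeline transform lerp.
; With all three flags set, a DoOnce-guarded timeline swings both doors open with a sound, then unlocks the BP_LevelTransfer actor.
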(event OnComponentBeginOverlap(Box1)
  (params (OverlappedComponent :type Primitive%20Component%20Object%20Reference) (OtherActor :type Actor%20Object%20Reference) (OtherComp :type Primitive%20Component%20Object%20Reference) (OtherBodyIndex :type Integer) (bFromSweep :type Boolean) (SweepResult :type Hit%20Result%20Structure%20%28by%20ref%29))
  (bind _brushref (Variables|Default|GetBrushRef))
  (bind _enum_paints (Variables|/Game/Blueprints/Paintbrush/Paintrbsuh.Paintrbsuh_C|GetEnum%20Paints _brushref))
  (if (== (Variables|/Game/Blueprints/Paintbrush/Paintrbsuh.Paintrbsuh_C|GetCollisionSphere _brushref) OtherComp)
    (if (Utilities|Enum|Equal(Enum) _enum_paints "NewEnumerator5")
      (CallFunction|GrowPaints _enum_paints)
      (bind _output_get (Variables|Default|SetPurpOn true))
      (Audio|Components|Audio|Play (Variables|Default|GetGreensound) 0.0)
      (if (Math|Boolean|ANDBoolean (stale OnComponentBeginOverlap(Box) _output_get) _output_get (stale OnComponentBeginOverlap(Box2) _output_get))
        (CallFunction|AllFinished)))))

(event OnComponentBeginOverlap(Box)
  (params (OverlappedComponent :type Primitive%20Component%20Object%20Reference) (OtherActor :type Actor%20Object%20Reference) (OtherComp :type Primitive%20Component%20Object%20Reference) (OtherBodyIndex :type Integer) (bFromSweep :type Boolean) (SweepResult :type Hit%20Result%20Structure%20%28by%20ref%29))
  (bind _brushref (Variables|Default|GetBrushRef))
  (bind _enum_paints (Variables|/Game/Blueprints/Paintbrush/Paintrbsuh.Paintrbsuh_C|GetEnum%20Paints _brushref))
  (if (== (Variables|/Game/Blueprints/Paintbrush/Paintrbsuh.Paintrbsuh_C|GetCollisionSphere _brushref) OtherComp)
    (switch Utilities|FlowControl|Switch|SwitchonEnum_Paints _enum_paints
      (:NewEnumerator1
        _)
      (:NewEnumerator4
        _))
    (CallFunction|GrowPaints _enum_paints)
    (bind _output_get (Variables|Default|SetGreenOn true))
    (Audio|Components|Audio|Play (Variables|Default|GetGreensound) 0.0)
    (if (Math|Boolean|ANDBoolean _output_get (stale OnComponentBeginOverlap(Box1) _output_get) (stale OnComponentBeginOverlap(Box2) _output_get))
      (CallFunction|AllFinished))))

(event OnComponentBeginOverlap(Box2)
  (params (OverlappedComponent :type Primitive%20Component%20Object%20Reference) (OtherActor :type Actor%20Object%20Reference) (OtherComp :type Primitive%20Component%20Object%20Reference) (OtherBodyIndex :type Integer) (bFromSweep :type Boolean) (SweepResult :type Hit%20Result%20Structure%20%28by%20ref%29))
  (bind _brushref (Variables|Default|GetBrushRef))
  (bind _enum_paints (Variables|/Game/Blueprints/Paintbrush/Paintrbsuh.Paintrbsuh_C|GetEnum%20Paints _brushref))
  (if (== (Variables|/Game/Blueprints/Paintbrush/Paintrbsuh.Paintrbsuh_C|GetCollisionSphere _brushref) OtherComp)
    (switch Utilities|FlowControl|Switch|SwitchonEnum_Paints _enum_paints
      (:NewEnumerator3
        _)
      (:NewEnumerator0
        _))
    (CallFunction|GrowPaints _enum_paints)
    (bind _output_get (Variables|Default|SetYellowOn true))
    (Audio|Components|Audio|Play (Variables|Default|Getyellowsound) 0.0)
    (if (Math|Boolean|ANDBoolean (stale OnComponentBeginOverlap(Box) _output_get) (stale OnComponentBeginOverlap(Box1) _output_get) _output_get)
      (CallFunction|AllFinished))))

(event Custom|GrowPaints
  (params (Selection :type Enum_Paints%20Enum :default "NewEnumerator3"))
  (bind _staticmesh1 (Variables|Default|GetStaticMesh1))
  (bind _staticmesh (Variables|Default|GetStaticMesh))
  (bind _newtrack_0 (Timeline|Timeline_0 PlayFromStart)
    (:Update
      (Transformation|SetRelativeTransform (Utilities|Select :Index Selection :NewEnumerator3 _staticmesh :NewEnumerator0 _staticmesh :NewEnumerator1 _staticmesh1 :NewEnumerator4 _staticmesh1 :NewEnumerator5 (Variables|Default|GetStaticMesh2)) (Math|Transform|Lerp(Transform) (Variables|Default|GetBlobStart) (Variables|Default|GetBlobEnd) _newtrack_0) false false))))

(event Custom|AllFinished
  (Utilities|FlowControl|DoOnce false
    (:Completed
      (Utilities|FlowControl|Delay 0.2)
      (Audio|Components|Audio|Play (Variables|Default|GetDoorOpening_Cue) 0.0)
      (bind _newtrack_0 (Timeline|Timeline_1 PlayFromStart)
        (:Update
          (Transformation|SetRelativeRotation (Variables|Default|GetDoor) (Math|Rotator|MakeRotator 0.0 0.0 (Math|Float|Lerp 0.0 7e+01 _newtrack_0)) false false)
          (Transformation|SetRelativeRotation (Variables|Default|GetDoor1) (Math|Rotator|MakeRotator 0.0 0.0 (Math|Float|Lerp 0.0 -7e+01 _newtrack_0)) false false))
        (:Finished
          (Default|UnlockDoor (Variables|Default|GetTransferRef)))))))

(event EventBeginPlay
  (bind _returnvalue (Actor|GetActorOfClass "/Game/Blueprints/Paintbrush/Paintrbsuh.Paintrbsuh_C"))
  (Variables|Default|SetBrushRef _returnvalue)
  (bind _returnvalue_2 (Actor|GetActorOfClass "/Game/Blueprints/BP/BP_LevelTransfer.BP_LevelTransfer_C"))
  (Variables|Default|SetTransferRef _returnvalue_2)
  (Transformation|SetRelativeTransform (Variables|Default|GetStaticMesh2) (Variables|Default|GetBlobStart) false false))

(event Collision|EventActorBeginOverlap
  (params (OtherActor :type Actor%20Object%20Reference)))

(event EventTick
  (params (DeltaSeconds :type Float%20%28single-precision%29)))

(fn ConstructionScript)