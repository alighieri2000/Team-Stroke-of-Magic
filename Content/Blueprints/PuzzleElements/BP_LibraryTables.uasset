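; BP_LibraryTables is a library puzzle element that unlocks the lunchbox and grows the apple once all Library Apple dots are primed.
; It caches the Apple and Dot actors on BeginPlay, and UpdatePrimedList checks the dots' primed state.
; Completion plays a cue and chains two timelines that animate meshes, triggering the unlock and growth between them.
; Brush sphere overlaps with BrushBounds2 call parent enter and exit logic.
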(event OnComponentBeginOverlap(BrushBounds2)
  (params (OverlappedComponent :type Primitive%20Component%20Object%20Reference) (OtherActor :type Actor%20Object%20Reference) (OtherComp :type Primitive%20Component%20Object%20Reference) (OtherBodyIndex :type Integer) (bFromSweep :type Boolean) (SweepResult :type Hit%20Result%20Structure%20%28by%20ref%29))
  (if (== OtherComp (Variables|/Game/Blueprints/Paintbrush/Paintrbsuh.Paintrbsuh_C|GetCollisionSphere (Variables|Default|GetBrushRefVar)))
    (CallFunction|ParentBegin)))

(event OnComponentEndOverlap(BrushBounds2)
  (params (OverlappedComponent :type Primitive%20Component%20Object%20Reference) (OtherActor :type Actor%20Object%20Reference) (OtherComp :type Primitive%20Component%20Object%20Reference) (OtherBodyIndex :type Integer))
  (if (== OtherComp (Variables|/Game/Blueprints/Paintbrush/Paintrbsuh.Paintrbsuh_C|GetCollisionSphere (Variables|Default|GetBrushRefVar)))
    (CallFunction|ExitedParent)))

(event Custom|UpdatePrimedList
  (Variables|Default|SetAllPrimed_0 true)
  (for _array_element (stale EventBeginPlay _output_get)
    (switch Utilities|FlowControl|Switch|SwitchonRoomEnum (Variables|/Game/Blueprints/Spline_BP/Dot.Dot_C|Getenum _array_element)
      (:NewEnumerator9
        (if (not (Variables|/Game/Blueprints/Spline_BP/Dot.Dot_C|GetPrimed? _array_element))
          (Variables|Default|SetAllPrimed_0 false)))))
  (if (Variables|Default|GetAllPrimed_0)
    (CallFunction|Finished)))

(event EventBeginPlay
  (|CallParentFunction)
  (bind _returnvalue (Actor|GetActorOfClass "/Game/Blueprints/BP/Apple.Apple_C"))
  (Variables|Default|SetAppleRef _returnvalue)
  (bind _outactors (Actor|GetAllActorsOfClass "/Game/Blueprints/Spline_BP/Dot.Dot_C"))
  (bind _output_get (Variables|Default|SetDot%20Actors _outactors)))

(event Collision|EventActorBeginOverlap
  (params (OtherActor :type Actor%20Object%20Reference)))

(event EventTick
  (params (DeltaSeconds :type Float%20%28single-precision%29)))

(event EventFinished
  (Audio|Components|Audio|Play (Variables|Default|GetLunchBoxOpening_Cue) 0.0)
  (bind _newtrack_0 (Timeline|Timeline_0 PlayFromStart)
    (:Update
      (Transformation|SetRelativeTransform (Variables|Default|GetStaticMesh11) (Math|Transform|Lerp(Transform) (Math|Transform|MakeTransform "3.761438,-7.632965,-0.614803" "0, 0, 0" "0.001000,0.001000,0.001000") (Math|Transform|MakeTransform "3.761438,-7.632965,-0.614803" "0,-115.000000, 0" "0.100000,0.100000,0.100000") _newtrack_0) false false))
    (:Finished
      (Variables|/Game/Blueprints/Paintbrush/Paintrbsuh.Paintrbsuh_C|SetLunchboxUnlocked? (Variables|Default|GetBrushRefVar) true)
      (Default|Grow (Variables|Default|GetAppleRef))
      (bind _newtrack_0_2 (Timeline|Timeline_1 PlayFromStart)
        (:Update
          (Transformation|SetRelativeRotation (Variables|Default|GetStaticMesh8) (Math|Rotator|Lerp(Rotator) "0, 0, 0" "180.000000, 0, 0" _newtrack_0_2) false false))))))

(fn ConstructionScript
  (|CallParentFunction))