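; Puzzle gate that opens once every Library Gate Dot in the level is primed.
; UpdatePrimedList runs or stops spline light trails for each numbered Dot, though trails 2–5 all read the first timeline's alpha.
; On completion it plays a cue, animates the Flow and Scene pieces with timelines, and disables Flow collision.
; Four brush bounds forward brush sphere overlaps to the parent class.
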(event OnComponentEndOverlap(BrushBounds2)
  (params (OverlappedComponent :type Primitive%20Component%20Object%20Reference) (OtherActor :type Actor%20Object%20Reference) (OtherComp :type Primitive%20Component%20Object%20Reference) (OtherBodyIndex :type Integer))
  (if (== (Variables|/Game/Blueprints/Paintbrush/Paintrbsuh.Paintrbsuh_C|GetCollisionSphere (Variables|Default|GetBrushRefVar)) OtherComp)
    (CallFunction|ExitedParent)))

(event OnComponentEndOverlap(BrushBounds4)
  (params (OverlappedComponent :type Primitive%20Component%20Object%20Reference) (OtherActor :type Actor%20Object%20Reference) (OtherComp :type Primitive%20Component%20Object%20Reference) (OtherBodyIndex :type Integer))
  (if (== (Variables|/Game/Blueprints/Paintbrush/Paintrbsuh.Paintrbsuh_C|GetCollisionSphere (Variables|Default|GetBrushRefVar)) OtherComp)
    (CallFunction|ExitedParent)))

(event OnComponentBeginOverlap(BrushBounds2)
  (params (OverlappedComponent :type Primitive%20Component%20Object%20Reference) (OtherActor :type Actor%20Object%20Reference) (OtherComp :type Primitive%20Component%20Object%20Reference) (OtherBodyIndex :type Integer) (bFromSweep :type Boolean) (SweepResult :type Hit%20Result%20Structure%20%28by%20ref%29))
  (if (== OtherComp (Variables|/Game/Blueprints/Paintbrush/Paintrbsuh.Paintrbsuh_C|GetCollisionSphere (Variables|Default|GetBrushRefVar)))
    (CallFunction|ParentBegin)))

(event OnComponentBeginOverlap(BrushBounds3)
  (params (OverlappedComponent :type Primitive%20Component%20Object%20Reference) (OtherActor :type Actor%20Object%20Reference) (OtherComp :type Primitive%20Component%20Object%20Reference) (OtherBodyIndex :type Integer) (bFromSweep :type Boolean) (SweepResult :type Hit%20Result%20Structure%20%28by%20ref%29))
  (if (== OtherComp (Variables|/Game/Blueprints/Paintbrush/Paintrbsuh.Paintrbsuh_C|GetCollisionSphere (Variables|Default|GetBrushRefVar)))
    (CallFunction|ParentBegin)))

(event OnComponentBeginOverlap(BrushBounds4)
  (params (OverlappedComponent :type Primitive%20Component%20Object%20Reference) (OtherActor :type Actor%20Object%20Reference) (OtherComp :type Primitive%20Component%20Object%20Reference) (OtherBodyIndex :type Integer) (bFromSweep :type Boolean) (SweepResult :type Hit%20Result%20Structure%20%28by%20ref%29))
  (if (== OtherComp (Variables|/Game/Blueprints/Paintbrush/Paintrbsuh.Paintrbsuh_C|GetCollisionSphere (Variables|Default|GetBrushRefVar)))
    (CallFunction|ParentBegin)))

(event OnComponentEndOverlap(BrushBounds3)
  (params (OverlappedComponent :type Primitive%20Component%20Object%20Reference) (OtherActor :type Actor%20Object%20Reference) (OtherComp :type Primitive%20Component%20Object%20Reference) (OtherBodyIndex :type Integer))
  (if (== (Variables|/Game/Blueprints/Paintbrush/Paintrbsuh.Paintrbsuh_C|GetCollisionSphere (Variables|Default|GetBrushRefVar)) OtherComp)
    (CallFunction|ExitedParent)))

(event OnComponentBeginOverlap(BrushBounds1)
  (params (OverlappedComponent :type Primitive%20Component%20Object%20Reference) (OtherActor :type Actor%20Object%20Reference) (OtherComp :type Primitive%20Component%20Object%20Reference) (OtherBodyIndex :type Integer) (bFromSweep :type Boolean) (SweepResult :type Hit%20Result%20Structure%20%28by%20ref%29))
  (if (== (Variables|/Game/Blueprints/Paintbrush/Paintrbsuh.Paintrbsuh_C|GetCollisionSphere (Variables|Default|GetBrushRefVar)) OtherComp)
    (CallFunction|ParentBegin)))

(event OnComponentEndOverlap(BrushBounds1)
  (params (OverlappedComponent :type Primitive%20Component%20Object%20Reference) (OtherActor :type Actor%20Object%20Reference) (OtherComp :type Primitive%20Component%20Object%20Reference) (OtherBodyIndex :type Integer))
  (if (== (Variables|/Game/Blueprints/Paintbrush/Paintrbsuh.Paintrbsuh_C|GetCollisionSphere (Variables|Default|GetBrushRefVar)) OtherComp)
    (CallFunction|ExitedParent)))

(event Custom|UpdatePrimedList
  (Variables|Default|SetAllPrimed_0 true)
  (for _array_element (stale EventBeginPlay _output_get)
    (switch Utilities|FlowControl|Switch|SwitchonRoomEnum (Variables|/Game/Blueprints/Spline_BP/Dot.Dot_C|Getenum _array_element)
      (:NewEnumerator6
        (if (Variables|/Game/Blueprints/Spline_BP/Dot.Dot_C|GetPrimed? _array_element)
          _
          (else
            (Variables|Default|SetAllPrimed_0 false)))
        (switch int (Variables|/Game/Blueprints/Spline_BP/Dot.Dot_C|GetDotNumber _array_element)
          (:1
            (CallFunction|D01 (Variables|/Game/Blueprints/Spline_BP/Dot.Dot_C|GetPrimed? _array_element)))
          (:2
            (CallFunction|D02 (Variables|/Game/Blueprints/Spline_BP/Dot.Dot_C|GetPrimed? _array_element))
            (Development|PrintString "Hello"))
          (:3
            (CallFunction|D03 (Variables|/Game/Blueprints/Spline_BP/Dot.Dot_C|GetPrimed? _array_element)))
          (:4
            (CallFunction|D04 (Variables|/Game/Blueprints/Spline_BP/Dot.Dot_C|GetPrimed? _array_element)))
          (:5
            (CallFunction|D05 (Variables|/Game/Blueprints/Spline_BP/Dot.Dot_C|GetPrimed? _array_element)))))))
  (if (Variables|Default|GetAllPrimed_0)
    (CallFunction|Finished)
    (CallFunction|PuzzleComplete)))

(event Custom|PuzzleComplete
  (Utilities|FlowControl|Sequence
    (:then_0
      (Audio|Components|Audio|Play (Variables|Default|GetplantPuzzleCompletion_Cue) 0.0)
      (bind _newtrack_1 (Timeline|Grow Play)
        (:Update
          (Transformation|SetRelativeRotation (Variables|Default|GetFlow062) (Math|Rotator|Lerp(Rotator) "0, 0,90.000000" "0, 0,-10.000000" _newtrack_1) false false)
          (Transformation|SetRelativeRotation (Variables|Default|GetFlow016) (Math|Rotator|Lerp(Rotator) "0, 0,60.000000" "0, 0,-10.000000" _newtrack_1) false false)
          (Transformation|SetRelativeLocation (Variables|Default|GetScene7) (Math|Vector|Lerp(Vector) "0, 0, 0" "0, 0,-20.000000" _newtrack_1) false false)
          (Transformation|SetRelativeLocation (Variables|Default|GetStaticMesh3) (Math|Vector|Lerp(Vector) "0, 0, 0" "0, 0,-40.000000" _newtrack_1) false false))))
    (:then_1
      (bind _newtrack_1_2 (Timeline|Timeline_2 PlayFromStart)
        (:Update
          (Transformation|SetRelativeLocation (Variables|Default|GetScene9) (Math|Vector|Lerp(Vector) "0,-125.895401,-15.596748" "0,-125.895401,-100.000000" _newtrack_1_2) false false))))
    (:then_2
      (Collision|SetCollisionEnabled (Variables|Default|GetFlow016) "NoCollision"))))

(event Custom|D03
  (params (Condition :type Boolean))
  (bind _spline3 (Variables|Default|GetSpline3))
  (if Condition
    (Timeline|Timeline_7 Play
      (:Update
        (Transformation|SetWorldLocation (Variables|Default|GetPart3) (Spline|GetLocationatDistanceAlongSpline _spline3 (Math|Float|Lerp 0.0 (Spline|GetSplineLength _spline3) (stale Custom|D01 _newtrack_0)) "World") false false)))
    (else
      (Timeline|Timeline_7 Stop))))

(event Custom|d05
  (params (Condition :type Boolean))
  (bind _spline5 (Variables|Default|GetSpline5))
  (if Condition
    (Timeline|Timeline_9 Play
      (:Update
        (Transformation|SetWorldLocation (Variables|Default|GetPart5) (Spline|GetLocationatDistanceAlongSpline _spline5 (Math|Float|Lerp 0.0 (Spline|GetSplineLength _spline5) (stale Custom|D01 _newtrack_0)) "World") false false)))
    (else
      (Timeline|Timeline_9 Stop))))

(event Custom|D04
  (params (Condition :type Boolean))
  (bind _spline4 (Variables|Default|GetSpline4))
  (if Condition
    (Timeline|Timeline_8 Play
      (:Update
        (Transformation|SetWorldLocation (Variables|Default|GetPart4) (Spline|GetLocationatDistanceAlongSpline _spline4 (Math|Float|Lerp 0.0 (Spline|GetSplineLength _spline4) (stale Custom|D01 _newtrack_0)) "World") false false)))
    (else
      (Timeline|Timeline_8 Stop))))

(event Custom|D01
  (params (Condition :type Boolean))
  (bind _spline1 (Variables|Default|GetSpline1))
  (if Condition
    (bind _newtrack_0 (Timeline|Light%20Trail Play)
      (:Update
        (Transformation|SetWorldLocation (Variables|Default|GetPart1) (Spline|GetLocationatDistanceAlongSpline _spline1 (Math|Float|Lerp 0.0 (Spline|GetSplineLength _spline1) _newtrack_0) "World") false false)))
    (else
      (Timeline|Light%20Trail Stop))))

(event Custom|D02
  (params (Condition :type Boolean))
  (bind _spline2 (Variables|Default|GetSpline2))
  (if Condition
    (Timeline|Timeline_3 Play
      (:Update
        (Transformation|SetWorldLocation (Variables|Default|GetPart2) (Spline|GetLocationatDistanceAlongSpline _spline2 (Math|Float|Lerp 0.0 (Spline|GetSplineLength _spline2) (stale Custom|D01 _newtrack_0)) "World") false false)))
    (else
      (Timeline|Timeline_3 Stop))))

(event EventBeginPlay
  (|CallParentFunction)
  (bind _outactors (Actor|GetAllActorsOfClass "/Game/Blueprints/Spline_BP/Dot.Dot_C"))
  (bind _output_get (Variables|Default|SetDot%20Actors _outactors)))

(event EventFinished
  (Utilities|FlowControl|Sequence
    (:then_0
      (Audio|Components|Audio|Play (Variables|Default|GetplantPuzzleCompletion_Cue) 0.0)
      (bind _newtrack_1 (Timeline|Grow Play)
        (:Update
          (Transformation|SetRelativeRotation (Variables|Default|GetFlow062) (Math|Rotator|Lerp(Rotator) "0, 0,90.000000" "0, 0,-10.000000" _newtrack_1) false false)
          (Transformation|SetRelativeRotation (Variables|Default|GetFlow016) (Math|Rotator|Lerp(Rotator) "0, 0,60.000000" "0, 0,-10.000000" _newtrack_1) false false)
          (Transformation|SetRelativeLocation (Variables|Default|GetScene7) (Math|Vector|Lerp(Vector) "0, 0, 0" "0, 0,-20.000000" _newtrack_1) false false)
          (Transformation|SetRelativeLocation (Variables|Default|GetStaticMesh3) (Math|Vector|Lerp(Vector) "0, 0, 0" "0, 0,-40.000000" _newtrack_1) false false))))
    (:then_1
      (bind _newtrack_1_2 (Timeline|Timeline_2 PlayFromStart)
        (:Update
          (Transformation|SetRelativeLocation (Variables|Default|GetScene9) (Math|Vector|Lerp(Vector) "0,-125.895401,-15.596748" "0,-125.895401,-100.000000" _newtrack_1_2) false false))))
    (:then_2
      (Collision|SetCollisionEnabled (Variables|Default|GetFlow016) "NoCollision"))))

(fn ConstructionScript
  (|CallParentFunction))